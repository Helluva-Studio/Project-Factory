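; Dialogue audio Blueprint that wraps an Audio component and exposes events to control its playback.
; On BeginPlay it assigns its sound cue variable to the component.
; Events then swap the sound, play from a start time, stop immediately or after a delay, and fade in or out, each forwarding directly to the component.
; SetSoundAndPlay combines the sound swap and playback in one call.
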(event `self.ReceiveBeginPlay`
  (`AudioComponent.SetSound` (`self.Audio`) (`self.SouncCue`)))

(event `SetAudio`
  (params (NewSound :type "SoundBase Object Reference"))
  (`AudioComponent.SetSound` (`self.Audio`) NewSound))

(event `Play`
  (params (StartTime :type "Float (single-precision)"))
  (`AudioComponent.Play` (`self.Audio`) StartTime))

(event `SetSoundAndPlay`
  (params (NewSound :type "SoundBase Object Reference") (StartTime :type "Float (single-precision)"))
  (`AudioComponent.SetSound` (`self.Audio`) NewSound)
  (`self.Play` StartTime))

(event `Stop`
  (`AudioComponent.Stop` (`self.Audio`)))

(event `StopDelay`
  (params (DelayTime :type "Float (single-precision)"))
  (`AudioComponent.StopDelayed` (`self.Audio`) DelayTime))

(event `FadeIn`
  (params (FadeInDuration :type "Float (single-precision)"))
  (`AudioComponent.FadeIn` (`self.Audio`) FadeInDuration 1.0 0.0 "Linear"))

(event `FadeOut`
  (params (FadeOutDuration :type "Float (single-precision)"))
  (`AudioComponent.FadeOut` (`self.Audio`) FadeOutDuration 0.0 "Linear"))

(fn `UserConstructionScript`)