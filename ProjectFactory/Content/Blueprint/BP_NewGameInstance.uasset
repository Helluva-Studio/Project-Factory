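; Game instance that holds run state and persists turret unlocks, loading or creating the UnlockedTurretsSlot save on Init.
; Save snapshots Roberto's transform, stats, resources, shop power-ups and turret levels, then triggers the game mode's WriteToGameInstance.
; It builds a type-to-class turret map from a data table and moves the chosen turret out of it.
; Pickups save new unlocks to disk, while separate functions store and partially reset death-screen statistics.
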(event `self.ReceiveInit`
  (bind _returnvalue (`GameplayStatics.DoesSaveGameExist` "UnlockedTurretsSlot"))
  (if _returnvalue
    (bind _returnvalue_2 (`GameplayStatics.LoadGameFromSlot` "UnlockedTurretsSlot"))
    (bind _asbp_unlocked_turrets_data (cast `/Game/Blueprint/Save/BP_UnlockedTurretsData` _returnvalue_2))
    (set `self.UnlockedTurretsData` _asbp_unlocked_turrets_data)
    (else
      (bind _returnvalue_3 (`GameplayStatics.CreateSaveGameObject` "/Game/Blueprint/Save/BP_UnlockedTurretsData.BP_UnlockedTurretsData_C"))
      (set `self.UnlockedTurretsData` _returnvalue_3))))

(fn `InitializeTurretBlueprints`
  (for _index (range 1 (+ (`self.NumberOfTurrets`) 1))
    (bind _returnvalue (`|GetDataTableRow` "/Game/Blueprint/Turrets/TurretGetter/Turrets.Turrets" (`KismetStringLibrary.Conv_StringToName` (`KismetStringLibrary.Conv_IntToString` _index)))
      (:`then`
        (`BlueprintMapLibrary.Map_Add` (`self.TurretTypeMap`) (break `/Game/Blueprint/Turrets/TurretGetter/S_Turrets` _returnvalue) (`.Turret_8_A6EC76C84679FDD6ABD9D4842CDC8B0A` (break `/Game/Blueprint/Turrets/TurretGetter/S_Turrets` _returnvalue)))))))

(fn `ResetSavedValuesForDeathScreen`
  (set `self.Lever to Pull` 0)
  (set `self.Enemies Killed` 0)
  (set `self.Enemies Killed` 0)
  (set `self.Current Day` 0)
  (set `self.Seconds` 0)
  (set `self.Seconds` 0)
  (set `self.LeversPulled` 0))

(fn `Save`
  (bind _asbp_roberto (cast `/Game/Blueprint/Robot/Blueprints/BP_Roberto` (`GameplayStatics.GetPlayerPawn` 0)))
  (set `self.S Player Data` (make `/Game/DataStructures/S_PlayerData` (`Actor.GetTransform` _asbp_roberto) (`/Game/Blueprint/Robot/Blueprints/BPC_Shop.PowerUpItems` (`/Game/Blueprint/Robot/Blueprints/BP_Roberto.BPC_Shop` _asbp_roberto)) (`/Game/Blueprint/Robot/Blueprints/BPC_TurretSelectionSystem.TurretLevel` (`/Game/Blueprint/Robot/Blueprints/BP_Roberto.BPC_TurretSelectionSystem` _asbp_roberto)) (`/Game/Blueprint/Robot/Blueprints/BP_Roberto.Health` _asbp_roberto) (`/Game/Blueprint/Robot/Blueprints/BP_Roberto.MaxHealth` _asbp_roberto) (`/Game/Blueprint/Robot/Blueprints/BP_Roberto.Energy` _asbp_roberto) (`/Game/Blueprint/Robot/Blueprints/BP_Roberto.MaxEnergy` _asbp_roberto) (`/Game/Blueprint/Robot/Blueprints/BP_Roberto.Gear` _asbp_roberto) (`/Game/Blueprint/Robot/Blueprints/BP_Roberto.Steel` _asbp_roberto) (`/Game/Blueprint/Robot/Blueprints/BP_Roberto.Circuit` _asbp_roberto) (`/Game/Blueprint/Robot/Blueprints/BP_Roberto.Essence` _asbp_roberto) (`/Game/Blueprint/Robot/Blueprints/BP_Roberto.JunkDamage` _asbp_roberto)))
  (bind _asbp_new_game_mode (cast `/Game/GameMode/BP_NewGameMode` (`GameplayStatics.GetGameMode`)))
  (`/Game/GameMode/BP_NewGameMode.WriteToGameInstance` _asbp_new_game_mode))

(fn `SaveForDeathScreen`
  (params (LeverToPull :type Integer) (ExploredRooms :type Integer) (EnemiesKilled :type Integer) (CurrentDay :type Integer) (Minutes :type Integer) (Seconds :type Integer))
  (set `self.Lever to Pull` LeverToPull)
  (set `self.Explored Rooms` ExploredRooms)
  (set `self.Enemies Killed` EnemiesKilled)
  (set `self.Current Day` CurrentDay)
  (set `self.Minutes` Minutes)
  (set `self.Seconds` Seconds))

(fn `SetChosenTurret`
  (params (ChosenTurret :type "/Game/Blueprint/Turrets/BP_Turret_Base Class Reference"))
  (bind _turrettypemap (`self.TurretTypeMap`))
  (bind _values (`BlueprintMapLibrary.Map_Values` (`self.TurretTypeMap`)))
  (for (_array_element _array_index) _values
    (if (== _array_element ChosenTurret)
      (bind _keys (`BlueprintMapLibrary.Map_Keys` _turrettypemap))
      (bind _output (`|GetArrayItem` _keys _array_index))
      (`BlueprintMapLibrary.Map_Remove` _turrettypemap _output)
      (set `self.ChosenTurretClass` ChosenTurret)
      (set `self.ChosenTurretType` _output))))

(fn `TurretPickedUp`
  (params (TurretUnlocked :type "/Game/Blueprint/Turrets/BP_Turret_Base Class Reference"))
  (bind _unlockedturrets (`/Game/Blueprint/Save/BP_UnlockedTurretsData.UnlockedTurrets` (`self.UnlockedTurretsData`)))
  (bind (_value _returnvalue) (`BlueprintMapLibrary.Map_Find` _unlockedturrets TurretUnlocked))
  (if _returnvalue
    (if (not _value)
      (`BlueprintMapLibrary.Map_Add` _unlockedturrets TurretUnlocked true)
      (`GameplayStatics.SaveGameToSlot` (`self.UnlockedTurretsData`) "UnlockedTurretsSlot")
      (`KismetSystemLibrary.PrintString` "SAVING COMPLETE")
      (else
        (`KismetSystemLibrary.PrintString` "TURRET ALREADY UNLOCKED")))
    (else
      (`KismetSystemLibrary.PrintString` "TURRET NOT FOUND"))))