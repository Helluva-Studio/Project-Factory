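; Damage system component that handles Burn and Poison damage over time on its owning actor through a damage interface message.
; A new request hits immediately if that type's timer handle is invalid, then records causer and damage in per-type parallel arrays.
; Looping timer events, set up behind an array-length check, are meant to reapply each stored damage.
; Stopping removes the causer's array entries without clearing the timer.
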(event `/Game/Blueprint/Interfaces/BPI_Damageable.TakeDamageOverTime`
  (params (Time :type "Float (double-precision)") (Damage :type "Float (double-precision)") (DamageCauser :type "Actor Object Reference") (DamageType :type "/Game/Blueprint/Interfaces/E_DamageType Enum" :default "NewEnumerator0"))
  (set `self.DamageTick` Time)
  (set `self.DamageValue` Damage)
  (set `self.Damage Causer` DamageCauser)
  (switch `/Game/Blueprint/Interfaces/E_DamageType` DamageType
    (:`NewEnumerator1`
      (if (not (`KismetSystemLibrary.K2_IsValidTimerHandle` (`self.BurnTimer`)))
        (message `/Game/Blueprint/Interfaces/BPI_TakeDamage.TakeDamageByInterface` (`self.GetOwner`) (`self.DamageValue`)))
      (`self.DamageByBurn` (`self.DamageTick`) (`self.Damage Causer`) (`self.DamageValue`)))
    (:`NewEnumerator2`
      (if (not (`KismetSystemLibrary.K2_IsValidTimerHandle` (`self.PoisonTimer`)))
        (message `/Game/Blueprint/Interfaces/BPI_TakeDamage.TakeDamageByInterface` (`self.GetOwner`) (`self.DamageValue`)))
      (`self.DamageByPoison` (`self.DamageTick`) (`self.Damage Causer`) (`self.DamageValue`)))))

(event `/Game/Blueprint/Interfaces/BPI_Damageable.StopDamageOverTime`
  (params (DamageType :type "/Game/Blueprint/Interfaces/E_DamageType Enum" :default "NewEnumerator0") (DamageCauser :type "Actor Object Reference"))
  (switch `/Game/Blueprint/Interfaces/E_DamageType` DamageType
    (:`NewEnumerator1`
      (`self.StopDamageByBurn` DamageCauser))
    (:`NewEnumerator2`
      (`self.StopDamageByPoison` DamageCauser))))

(event `DoDavemeByPoison`
  (for (_ _array_index) (`self.PoisonCausers`)
    (message `/Game/Blueprint/Interfaces/BPI_TakeDamage.TakeDamageByInterface` (`self.GetOwner`) (`|GetArrayItem` (`self.PoisonDamages`) _array_index))))

(event `DoDamageByBurn`
  (for (_ _array_index) (`self.BurnCausers`)
    (message `/Game/Blueprint/Interfaces/BPI_TakeDamage.TakeDamageByInterface` (`self.GetOwner`) (`|GetArrayItem` (`self.BurnDamages`) _array_index))))

(fn `DamageByBurn`
  (params (Time :type "Float (single-precision)") (Damager :type "Actor Object Reference") (Damage :type "Float (double-precision)"))
  (bind _burncausers (`self.BurnCausers`))
  (`KismetArrayLibrary.Array_AddUnique` (`self.BurnDamages`) Damage)
  (`KismetArrayLibrary.Array_AddUnique` _burncausers Damager)
  (if (< (`KismetArrayLibrary.Array_Length` _burncausers) 1)
    (bind _returnvalue (`KismetSystemLibrary.K2_SetTimerDelegate` (`|CreateDelegate` :!event `DoDamageByBurn`) Time true))
    (set `self.BurnTimer` _returnvalue)))

(fn `DamageByPoison`
  (params (Time :type "Float (single-precision)") (Damager :type "Actor Object Reference") (Damage :type "Float (double-precision)"))
  (bind _poisoncausers (`self.PoisonCausers`))
  (`KismetArrayLibrary.Array_AddUnique` (`self.PoisonDamages`) Damage)
  (`KismetArrayLibrary.Array_AddUnique` _poisoncausers Damager)
  (if (< (`KismetArrayLibrary.Array_Length` _poisoncausers) 1)
    (bind _returnvalue (`KismetSystemLibrary.K2_SetTimerDelegate` (`|CreateDelegate` :!event `DoDamageByBurn`) Time true))
    (set `self.PoisonTimer` _returnvalue)))

(fn `StopDamageByBurn`
  (params (CauserToRemove :type "Actor Object Reference (by ref)"))
  (bind _returnvalue (`KismetArrayLibrary.Array_Find` (`self.BurnCausers`) CauserToRemove))
  (`KismetArrayLibrary.Array_Remove` (`self.BurnCausers`) _returnvalue)
  (`KismetArrayLibrary.Array_Remove` (`self.BurnDamages`) _returnvalue))

(fn `StopDamageByPoison`
  (params (CauserToRemove :type "Actor Object Reference (by ref)"))
  (bind _returnvalue (`KismetArrayLibrary.Array_Find` (`self.PoisonCausers`) CauserToRemove))
  (`KismetArrayLibrary.Array_Remove` (`self.PoisonCausers`) _returnvalue)
  (`KismetArrayLibrary.Array_Remove` (`self.PoisonDamages`) _returnvalue))