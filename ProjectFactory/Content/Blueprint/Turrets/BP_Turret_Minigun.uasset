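; Minigun turret that aims at and shoots BP_BaseEnemy pawns detected by its PawnSensing component.
; While IsFiring is true, each sighting rotates the Handler toward the enemy, waits FireRate, then spawns a BP_Bullet at the Arrow and initializes it with Damage.
; When not firing, a sighting resets the Handler's world rotation to zero.
; The sensing event alone drives aiming and firing, without Tick or a timer.
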(event `self.PawnSensing.OnSeePawn`
  (params (Pawn :type "Pawn Object Reference"))
  (bind _asbp_base_enemy (cast `/Game/Blueprint/Enemies/BP_BaseEnemy` Pawn))
  (if (`self.IsFiring`)
    (bind (_returnvalue_roll _returnvalue_pitch _returnvalue_yaw) (`KismetMathLibrary.BreakRotator` (`KismetMathLibrary.FindLookAtRotation` (`SceneComponent.K2_GetComponentLocation` (`self.Handler`)) (`self.K2_GetActorLocation` _asbp_base_enemy))))
    (`SceneComponent.K2_SetWorldRotation` (`self.Handler`) (`KismetMathLibrary.MakeRotator` _returnvalue_roll _returnvalue_pitch _returnvalue_yaw) false false)
    (`KismetSystemLibrary.Delay` (`self.FireRate`))
    (bind _returnvalue (`|SpawnActorFromClass` "/Game/Blueprint/Turrets/Ammunation/BP_Bullet.BP_Bullet_C" (`SceneComponent.K2_GetComponentToWorld` (`self.Arrow`)) "AdjustIfPossibleButAlwaysSpawn" "MultiplyWithRoot" null null))
    (`/Engine/EditorBlueprintResources/StandardMacros.IsValid` _returnvalue
      (:`Is Valid`
        (`/Game/Blueprint/Turrets/Ammunation/BP_Bullet.Initialize` _returnvalue (`self.Damage`))))
    (else
      (`SceneComponent.K2_SetWorldRotation` (`self.Handler`) (`KismetMathLibrary.MakeRotator` 0.0) false false))))

(fn `UserConstructionScript`
  (`parent.UserConstructionScript`))