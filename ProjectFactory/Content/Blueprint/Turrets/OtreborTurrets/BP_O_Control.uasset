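; Otrebor crowd-control turret that holds a CC ammo actor at its center, with a slow, stun or gravity variant.
; SpawnAmmo picks the ammo class from TypeOfCc, spawns it at zero scale on the Center component and attaches it there.
; Cooldown overrides destroy the ammo when cooldown starts and respawn it when cooldown ends if none exists, and Death also destroys it.
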(event `self.SpawnAmmo`
  (switch `/Game/Blueprint/Turrets/TurretFeature/Aoe/E_CcType` (`self.TypeOfCc`)
    (:`NewEnumerator2`
      (set `self.CcAmmoToSpawn` "/Game/Blueprint/Turrets/TurretFeature/Aoe/BP_OtreborCcSlow.BP_OtreborCcSlow_C"))
    (:`NewEnumerator1`
      (set `self.CcAmmoToSpawn` "/Game/Blueprint/Turrets/TurretFeature/Aoe/BP_CcStun.BP_CcStun_C"))
    (:`NewEnumerator4`
      (set `self.CcAmmoToSpawn` "/Game/Blueprint/Turrets/TurretFeature/Aoe/BP_CcGravity.BP_CcGravity_C")))
  (bind _returnvalue (`|SpawnActorFromClass` (`self.CcAmmoToSpawn`) (`KismetMathLibrary.MakeTransform` (`SceneComponent.K2_GetComponentLocation` (`self.Center`)) (struct) (0.0 0.0 0.0)) "AdjustIfPossibleButAlwaysSpawn" "MultiplyWithRoot" null null))
  (bind _output_get (set `self.CcAmmo` _returnvalue))
  (`/Engine/EditorBlueprintResources/StandardMacros.IsValid` _output_get
    (:`Is Valid`
      (`self.K2_AttachToComponent` _output_get (`self.Center`) "None" "KeepWorld" "KeepRelative" "KeepWorld" true))))

(fn `Death`
  (bind _ccammo (`self.CcAmmo`))
  (`/Engine/EditorBlueprintResources/StandardMacros.IsValid` _ccammo
    (:`Is Valid`
      (`self.K2_DestroyActor` _ccammo))))

(fn `DestroyAmmo_0`
  (`self.K2_DestroyActor` (`self.CcAmmo`)))

(fn `OnCDEnded`
  (`parent.OnCDEnded`)
  (`/Engine/EditorBlueprintResources/StandardMacros.IsValid` (`self.CcAmmo`)
    (:`Is Not Valid`
      (`self.SpawnAmmo`))))

(fn `OnCDStarted`
  (bind _ccammo (`self.CcAmmo`))
  (`parent.OnCDStarted`)
  (`/Engine/EditorBlueprintResources/StandardMacros.IsValid` _ccammo
    (:`Is Valid`
      (`self.K2_DestroyActor` _ccammo))))

(fn `UserConstructionScript`
  (`parent.UserConstructionScript`))