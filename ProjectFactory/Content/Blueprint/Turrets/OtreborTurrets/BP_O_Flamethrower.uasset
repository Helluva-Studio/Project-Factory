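; Flamethrower turret, a child turret Blueprint that loads per-level health, timing, cone angle and damage stats from DT_O_Flamethrower.
; SpawnAmmo passes the cone, hit and DoT stats to the damage ammo.
; Tick toggles flame particles with cooldown and wobbles the ammo mesh, which is hidden at level 1.
; From level 3, BeginPlay starts a looping timer for lerped yaw steps; cooldown start clears it and cooldown end sets a new one.
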(event `self.ReceiveBeginPlay`
  (`parent.ReceiveBeginPlay`)
  (`SceneComponent.K2_AttachToComponent` (`self.NS_CdEffect`) (`self.P_Flamethrower`) "None" "KeepRelative" "KeepRelative" "KeepRelative" true)
  (`SceneComponent.K2_SetRelativeLocation` (`self.NS_CdEffect`) (-10.7 0.0 0.0) false false)
  (if (>= (`self.CurrentLevel`) 3)
    (bind _asmaterial_instance_dynamic (cast `MaterialInstanceDynamic` (`PrimitiveComponent.GetMaterial` (`self.Ammo`) 1)))
    (`MaterialInstanceDynamic.SetScalarParameterValue` _asmaterial_instance_dynamic "TransitionValue" 1.0)
    (bind _returnvalue (`KismetSystemLibrary.K2_SetTimerDelegate` (delegate `RotateTurret`) (`self.RotateTime`) true))
    (set `self.RotateTimer` _returnvalue)))

(event `RotateTurret`
  (bind (_relativerotation_roll _relativerotation_pitch _relativerotation_yaw) (`KismetMathLibrary.BreakRotator` (`SceneComponent.RelativeRotation` (`self.HandlerLR`))))
  (if (not (`self.IsInCooldown`))
    (set `self.RotationLerp` 0.0)
    (bind _output_get (set `self.InitialZRotation` _relativerotation_yaw))
    (set `self.NextZRotation` (+ _output_get (`self.DeltaRotation`)))
    (set `self.CanChangeMode` false)))

(event `self.ReceiveTick`
  (params (DeltaSeconds :type "Float (single-precision)"))
  (`parent.ReceiveTick` DeltaSeconds)
  (`|ExecutionSequence`
    (:`then_0`
      (`self.DisableEnableFlame`))
    (:`then_1`
      (if (not (`self.IsInCooldown`))
        (`self.AmmoFeedback`))
      (if (not (`self.CanChangeMode`))
        (set `self.RotationLerp` (`KismetMathLibrary.FClamp` (+ (`self.RotationLerp`) (* (`GameplayStatics.GetWorldDeltaSeconds`) (`self.RotationSpeed`)))))
        (`SceneComponent.K2_SetRelativeRotation` (`self.HandlerLR`) (`KismetMathLibrary.MakeRotator` 0.0 0.0 (`KismetMathLibrary.Lerp` (`self.InitialZRotation`) (`self.NextZRotation`) (`self.RotationLerp`))) false false)
        (if (>= (`self.RotationLerp`) 1.0)
          (set `self.RotationLerp` 0.0)
          (set `self.CanChangeMode` true))))))

(event `DisableEnableFlame`
  (`/Engine/EditorBlueprintResources/StandardMacros.IsValid` self
    (:`Is Valid`
      (if (and true (not (`self.IsInCooldown`)) (`self.IsActorTickEnabled`))
        (`ActorComponent.Activate` (`self.P_Flamethrower`) false)
        (else
          (`KismetSystemLibrary.Delay` 1.0)
          (`ActorComponent.Deactivate` (`self.P_Flamethrower`)))))))

(event `self.SpawnAmmo`
  (`parent.SpawnAmmo`)
  (`/Engine/EditorBlueprintResources/StandardMacros.IsValid` (`self.DamageAmmo`)
    (:`Is Valid`
      (message `/Game/Blueprint/Turrets/Interfaces/BPI_TurretDamageAmmo.InitializeFlameAmmo` (`self.DamageAmmo`) (`self.CanHitPlayer`) (`self.D_TypeOfDamage`) (`self.D_TypeOfAoe`) (`self.MaxAngleOfEffect(Cone)`) (`self.DamageTick`) (`self.MaxDamageOnHit`) (`self.MaxDotInsideAoe`) (`self.MaxDotOutsideAoe`) (`self.MaxDotDuration`) (`self.DamageReductionByDistance`))
      (set `self.CanChangeMode` true))))

(event `AmmoFeedback`
  (bind _ammo (`self.Ammo`))
  (`/Engine/EditorBlueprintResources/StandardMacros.IsValid` self
    (:`Is Valid`
      (`/Engine/EditorBlueprintResources/StandardMacros.FlipFlop`
        (:`A`
          (`SceneComponent.K2_SetRelativeRotation` _ammo (struct :`Pitch` 1.0 :`Yaw` -90.0) false false))
        (:`B`
          (`SceneComponent.K2_SetRelativeRotation` _ammo (struct :`Pitch` -1.0 :`Yaw` -90.0) false false))))))

(fn `InitializeTurret`
  (`parent.InitializeTurret`)
  (bind _returnvalue (`|GetDataTableRow` "/Game/Blueprint/Turrets/TurretFeature/Leveling/TurretSpecificDataTable/DT_O_Flamethrower.DT_O_Flamethrower" (`KismetStringLibrary.Conv_StringToName` (`KismetStringLibrary.Conv_IntToString` (`self.CurrentLevel`))))
    (:`then`
      (bind (_maxhealth _maxactivitytime _maxcdtime _baseaoetype _baseangle _anglepercentagemodifier _basedamagetype _damagetick _damageonhit _damageovertimeinsideaoe _damageovertimeoutsideaoe _dotduration _basedamagereductionondistance _rotatetime) (break `/Game/Blueprint/Turrets/TurretFeature/Leveling/TurretStructs/S_O_Flamethrower` _returnvalue))
      (bind _output_get (set `self.MaxHealth` _maxhealth))
      (set `self.CurrentHealth` _output_get)
      (set `self.MaxActivityTime(NoFarm)` _maxactivitytime)
      (set `self.MaxCdTime` _maxcdtime)
      (set `self.D_TypeOfAoe` _baseaoetype)
      (bind _output_get_2 (set `self.D_BaseAngleOfEffect(Cone)` _baseangle))
      (set `self.MaxAngleOfEffect(Cone)` (+ _output_get_2 (* _output_get_2 (/ _anglepercentagemodifier 100.0))))
      (set `self.D_TypeOfDamage` _basedamagetype)
      (set `self.DamageTick` _damagetick)
      (set `self.MaxDamageOnHit` _damageonhit)
      (set `self.MaxDotInsideAoe` _damageovertimeinsideaoe)
      (set `self.MaxDotOutSideAoe` _damageovertimeoutsideaoe)
      (set `self.MaxDotDuration` _dotduration)
      (set `self.DamageReductionByDistance` _basedamagereductionondistance)
      (set `self.RotateTime` _rotatetime))))

(fn `OnCDEnded`
  (`parent.OnCDEnded`)
  (bind _returnvalue (`KismetSystemLibrary.K2_SetTimerDelegate` (`|CreateDelegate` :!event `RotateTurret`) (`self.RotateTime`) true))
  (set `self.RotateTimer` _returnvalue))

(fn `OnCDStarted`
  (`parent.OnCDStarted`)
  (`KismetSystemLibrary.K2_ClearAndInvalidateTimerHandle` (`self.RotateTimer`)))

(fn `UpdateGraphicByLevel`
  (params (Level :type Integer))
  (`/Engine/EditorBlueprintResources/StandardMacros.IsValid` self
    (:`Is Valid`
      (switch `int` Level
        (:`1`
          (`SceneComponent.SetVisibility` (`self.Ammo`) false true))
        (:`2`
          (`SceneComponent.SetVisibility` (`self.Ammo`) true true))
        (:`3`
          (`SceneComponent.SetVisibility` (`self.Ammo`) true true))))))

(fn `UserConstructionScript`
  (`parent.UserConstructionScript`))