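; Slow turret Blueprint that spawns crowd-control ammo to apply a slow effect over an area, with ice-themed visuals.
; Initialization reads health, timing, radius and slow stats from DT_O_Slow by current level, feeding the computed radius to Niagara.
; Spawning passes those effect settings to the ammo, while spawn and cooldown events toggle Niagara or fade audio.
; Level changes reveal additional ice components.
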(event `self.SpawnAmmo`
  (`parent.SpawnAmmo`)
  (`/Engine/EditorBlueprintResources/StandardMacros.IsValid` (`self.CcAmmo`)
    (:`Is Valid`
      (message `/Game/Blueprint/Turrets/Interfaces/BPI_TurretCcAmmo.InitializeSlowAmmo` (`self.CcAmmo`) (`self.CanHitPlayer`) (`self.TypeOfCc`) (`self.TypeOfAoe`) (`self.MaxDistance(Cone)/MaxRadius(Sphere)`) (`self.SlowEffect`))
      (`KismetSystemLibrary.Delay` 1.0)
      (`ActorComponent.Activate` (`self.Niagara`) false)
      (`AudioComponent.FadeIn` (`self.Audio`) 3.0 1.0 0.0 "Linear"))))

(event `self.DeactivateNiagara`
  (`parent.DeactivateNiagara`)
  (`ActorComponent.Deactivate` (`self.Niagara`)))

(fn `InitializeTurret`
  (`parent.InitializeTurret`)
  (bind _returnvalue (`|GetDataTableRow` "/Game/Blueprint/Turrets/TurretFeature/Leveling/TurretSpecificDataTable/DT_O_Slow.DT_O_Slow" (`KismetStringLibrary.Conv_StringToName` (`KismetStringLibrary.Conv_IntToString` (`self.CurrentLevel`))))
    (:`then`
      (bind (_maxhealth _maxactivitytime _maxcdtime _baseaoetype _baseradius _radiuspercentagemodifier _basecctype _sloweffectpercentage) (break `/Game/Blueprint/Turrets/TurretFeature/Leveling/TurretStructs/S_C_Slow` _returnvalue))
      (bind _output_get (set `self.MaxHealth` _maxhealth))
      (set `self.CurrentHealth` _output_get)
      (set `self.MaxActivityTime(NoFarm)` _maxactivitytime)
      (set `self.MaxCdTime` _maxcdtime)
      (set `self.TypeOfAoe` _baseaoetype)
      (bind _output_get_2 (set `self.BaseDistance(Cone)/BaseRadius(Sphere)` _baseradius))
      (set `self.MaxDistance(Cone)/MaxRadius(Sphere)` (+ _output_get_2 (* _output_get_2 (/ _radiuspercentagemodifier 100.0))))
      (set `self.TypeOfCc` _basecctype)
      (set `self.SlowEffect` _sloweffectpercentage)
      (`FXSystemComponent.SetFloatParameter` (`self.Niagara`) "SphereRadius" (`self.MaxDistance(Cone)/MaxRadius(Sphere)`)))))

(fn `OnCDEnded`
  (`parent.OnCDEnded`)
  (`ActorComponent.Activate` (`self.Niagara`) false)
  (`AudioComponent.FadeOut` (`self.Audio`) 1.0 0.0 "Linear"))

(fn `OnCDStarted`
  (`parent.OnCDStarted`)
  (`ActorComponent.Deactivate` (`self.Niagara`)))

(fn `UpdateGraphicByLevel`
  (params (Level :type Integer))
  (`/Engine/EditorBlueprintResources/StandardMacros.IsValid` self
    (:`Is Valid`
      (switch `int` Level
        (:`1`
          (`SceneComponent.SetVisibility` (`self.Ice2`) false false)
          (`SceneComponent.SetVisibility` (`self.Ice3`) false false))
        (:`2`
          (`SceneComponent.SetVisibility` (`self.Ice2`) true false)
          (`SceneComponent.SetVisibility` (`self.Ice3`) false false))
        (:`3`
          (`SceneComponent.SetVisibility` (`self.Ice2`) true false)
          (`SceneComponent.SetVisibility` (`self.Ice3`) true false))))))

(fn `UserConstructionScript`
  (`parent.UserConstructionScript`))