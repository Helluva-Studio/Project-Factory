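; Otrebor turret aiming Blueprint that patrols, spots BP_Roberto through PawnSensing and rotates to track it.
; Tick alternates between random-point patrol and aiming, lerping separate yaw and pitch handlers until an accuracy threshold allows Shoot, which here only clears CanShoot.
; Distance checks and line traces reset the turret when the target is out of range or blocked.
; Cooldown start also resets it and disables sight until cooldown ends.
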(event `CheckTarget`
  (`/Engine/EditorBlueprintResources/StandardMacros.IsValid` (`self.Target`)
    (:`Is Valid`
      (`|ExecutionSequence`
        (:`then_0`
          ;[0 0 0] CheckTargetDistance
          (`/Engine/EditorBlueprintResources/StandardMacros.IsValid` (`self.Target`)
            (:`Is Valid`
              (if (> (`KismetMathLibrary.Vector_Distance` (`SceneComponent.K2_GetComponentLocation` (`self.HandlerUD`)) (`self.K2_GetActorLocation` (`self.Target`))) (`self.Max Target Distance`))
                (`self.ResetTurret`)))
            (:`Is Not Valid`
              (`self.ResetTurret`))))
        (:`then_2`
          ;[0 0 0] CheckObstacles
          (`/Engine/EditorBlueprintResources/StandardMacros.IsValid` (`self.Target`)
            (:`Is Valid`
              (bind _returnvalue (`GameplayStatics.GetActorOfClass` "/Game/Blueprint/Enemies/BP_Otrebor.BP_Otrebor_C"))
              (bind _outhit (`KismetSystemLibrary.LineTraceSingleForObjects` (`SceneComponent.K2_GetComponentLocation` (`self.HandlerUD`)) (`SceneComponent.K2_GetComponentLocation` (`Actor.RootComponent` (`self.Target`))) (`|MakeArray` "ObjectTypeQuery2" "ObjectTypeQuery1" "ObjectTypeQuery3" :!type "EObjectTypeQuery Enum") true (`|MakeArray` _returnvalue :!type "Actor Object Reference")))
              (bind (_bblockinghit _binitialoverlap _time _distance _location _impactpoint _normal _impactnormal _physmat _hitactor) (`GameplayStatics.BreakHitResult` _outhit))
              (if (!= (`self.Target`) _hitactor)
                (if (not (`KismetSystemLibrary.DoesImplementInterface` _hitactor "/Game/Blueprint/Enemies/Interfaces/BPI_Otrebor.BPI_Otrebor_C"))
                  (`self.ResetTurret`))))
            (:`Is Not Valid`
              (`self.ResetTurret`))))))))

(event `self.PawnSensing.OnSeePawn`
  (params (Pawn :type "Pawn Object Reference"))
  ;[1 1 1] FlyingMonster
  (bind _asbp_roberto (cast `/Game/Blueprint/Robot/Blueprints/BP_Roberto` Pawn))
  (set `self.Target` _asbp_roberto))

(event `self.ReceiveTick`
  (params (DeltaSeconds :type "Float (single-precision)"))
  (bind (_relativerotation_roll _relativerotation_pitch _relativerotation_yaw) (`KismetMathLibrary.BreakRotator` (`SceneComponent.RelativeRotation` (`self.HandlerLR`))))
  (bind (_relativerotation_roll_2 _relativerotation_pitch_2) (`KismetMathLibrary.BreakRotator` (`SceneComponent.RelativeRotation` (`self.HandlerUD`))))
  (bind (_relativerotation_roll_3 _relativerotation_pitch_3) (`KismetMathLibrary.BreakRotator` (`SceneComponent.RelativeRotation` (`self.HandlerUD`))))
  (bind (_relativerotation_roll_4 _relativerotation_pitch_4 _relativerotation_yaw_2) (`KismetMathLibrary.BreakRotator` (`SceneComponent.RelativeRotation` (`self.HandlerLR`))))
  (`parent.ReceiveTick` DeltaSeconds)
  (`|ExecutionSequence`
    (:`then_0`
      (`/Engine/EditorBlueprintResources/StandardMacros.IsValid` (`self.Target`)
        (:`Is Valid`
          (set `self.IsInFunction(NoFarm)` true)
          (`self.CheckTarget`))
        (:`Is Not Valid`
          (set `self.IsInFunction(NoFarm)` false))))
    (:`then_1`
      (if (not (`self.IsInCooldown`))
        (`/Engine/EditorBlueprintResources/StandardMacros.IsValid` (`self.Target`)
          (:`Is Valid`
            (if (`self.TargetAimed`)
              (if (`self.AimTaken`)
                (if (`self.CanShoot`)
                  (`self.Shoot`)
                  (else
                    (`self.TakeAim`)))
                (else
                  (`self.TakeAim`)))
              (else
                (set `self.TargetAimed` true)
                (set `self.AimRotationLerp` 0.0)
                (set `self.InitialDirection` _relativerotation_yaw)
                (set `self.InitialAltitude` _relativerotation_pitch_2))))
          (:`Is Not Valid`
            (if (`self.NotInPatrol`)
              (set `self.NotInPatrol` false)
              (set `self.PatrolRotationLerp` 0.0)
              (set `self.InitialDirection` _relativerotation_yaw_2)
              (set `self.InitialAltitude` _relativerotation_pitch_3)
              (set `self.NextPatrolLocation` (`self.GetNextPatrolPosition` (`SceneComponent.K2_GetComponentLocation` (`self.HandlerUD`)) (`self.Max Lower Angle`) (`self.Max Upper Angle`)))
              (else
                (`self.Patrol`)))))))))

(event `ResetTurret`
  (set `self.NotInPatrol` true)
  (set `self.PatrolRotationLerp` 0.0)
  (set `self.TargetAimed` false)
  (set `self.AimTaken` false)
  (set `self.CanShoot` true)
  (set `self.AimRotationLerp` 0.0)
  (set `self.Target` null))

(event `Shoot`
  (set `self.CanShoot` false))

(event `Patrol`
  (bind (_returnvalue_roll _returnvalue_pitch) (`KismetMathLibrary.BreakRotator` (`KismetMathLibrary.FindLookAtRotation` (`SceneComponent.K2_GetComponentLocation` (`self.HandlerUD`)) (`self.NextPatrolLocation`))))
  (bind (_returnvalue_roll_2 _returnvalue_pitch_2 _returnvalue_yaw) (`KismetMathLibrary.BreakRotator` (`KismetMathLibrary.FindLookAtRotation` (`SceneComponent.K2_GetComponentLocation` (`self.HandlerLR`)) (`self.NextPatrolLocation`))))
  ;[0.4333 1 0.6597] Patrol
  (set `self.PatrolRotationLerp` (`KismetMathLibrary.FClamp` (+ (`self.PatrolRotationLerp`) (* (`GameplayStatics.GetWorldDeltaSeconds`) (`self.PatrolRotationSpeed`)))))
  (`/Engine/EditorBlueprintResources/StandardMacros.IsValid` self
    (:`Is Valid`
      (`SceneComponent.K2_SetRelativeRotation` (`self.HandlerLR`) (`KismetMathLibrary.MakeRotator` 0.0 0.0 (`KismetMathLibrary.Lerp` (`self.InitialDirection`) (* _returnvalue_yaw -1.0) (`self.PatrolRotationLerp`))) false false)
      (`/Engine/EditorBlueprintResources/StandardMacros.IsValid` self
        (:`Is Valid`
          (`SceneComponent.K2_SetRelativeRotation` (`self.HandlerUD`) (`KismetMathLibrary.MakeRotator` 0.0 (`KismetMathLibrary.Lerp` (`self.InitialAltitude`) _returnvalue_pitch (`self.PatrolRotationLerp`))) false false)
          (if (>= (`self.PatrolRotationLerp`) 1.0)
            (`KismetSystemLibrary.Delay` (`self.TimeBetweenNextPatrol`))
            (set `self.NotInPatrol` true)))))))

(event `TakeAim`
  (bind (_returnvalue_roll _returnvalue_pitch) (`KismetMathLibrary.BreakRotator` (`KismetMathLibrary.FindLookAtRotation` (`SceneComponent.K2_GetComponentLocation` (`self.HandlerUD`)) (`self.K2_GetActorLocation` (`self.Target`)))))
  (bind (_returnvalue_roll_2 _returnvalue_pitch_2 _returnvalue_yaw) (`KismetMathLibrary.BreakRotator` (`KismetMathLibrary.FindLookAtRotation` (`SceneComponent.K2_GetComponentLocation` (`self.HandlerLR`)) (`self.K2_GetActorLocation` (`self.Target`)))))
  ;[1 0.5673 0.4162] Aim
  (if (`self.CanRotate`)
    (set `self.AimRotationLerp` (`KismetMathLibrary.FClamp` (+ (`self.AimRotationLerp`) (* (`GameplayStatics.GetWorldDeltaSeconds`) (`self.Aim Rotation Speed`)))))
    (`/Engine/EditorBlueprintResources/StandardMacros.IsValid` self
      (:`Is Valid`
        (`SceneComponent.K2_SetRelativeRotation` (`self.HandlerLR`) (`KismetMathLibrary.MakeRotator` 0.0 0.0 (`KismetMathLibrary.Lerp` (`self.InitialDirection`) _returnvalue_yaw (`self.AimRotationLerp`))) false false)
        (`/Engine/EditorBlueprintResources/StandardMacros.IsValid` self
          (:`Is Valid`
            (`SceneComponent.K2_SetRelativeRotation` (`self.HandlerUD`) (`KismetMathLibrary.MakeRotator` 0.0 (`KismetMathLibrary.Lerp` (`self.InitialAltitude`) _returnvalue_pitch (`self.AimRotationLerp`))) false false)
            (if (>= (`self.AimRotationLerp`) (/ (`self.AccuracyPercentage`) 100.0))
              (set `self.AimTaken` true))))))))

(event `/Game/Blueprint/InteractionArea/BPI_Focusable.ToggleFocus`
  (params (Focus :type Boolean)))

(fn `GetNextPatrolPosition`
  (params (CenterPosition :type "Vector Structure") (MaxLowerAngle :type "Float (double-precision)") (MaxUpperAngle :type "Float (double-precision)"))
  (returns (TargetPosition :type "Vector Structure"))
  (locals (Angle :type "Float (double-precision)") (RandomX :type "Float (double-precision)") (RandomY :type "Float (double-precision)"))
  (bind (_returnvalue_x _returnvalue_y) (`KismetMathLibrary.BreakVector` (`KismetMathLibrary.RandomUnitVector`)))
  (set `local.Angle` (`KismetMathLibrary.RandomFloatInRange` (* MaxLowerAngle -1.0) MaxUpperAngle))
  (set `local.RandomX` _returnvalue_x)
  (set `local.RandomY` _returnvalue_y)
  (return (+ CenterPosition (* (`KismetMathLibrary.Normal` (`KismetMathLibrary.MakeVector` (`local.RandomX`) (`local.RandomY`) (`KismetMathLibrary.SelectFloat` (* (`KismetMathLibrary.Sqrt` (+ (`KismetMathLibrary.MultiplyMultiply_FloatFloat` (`local.RandomX`) 2.0) (`KismetMathLibrary.MultiplyMultiply_FloatFloat` (`local.RandomY`) 2.0))) (`KismetMathLibrary.DegTan` (`local.Angle`))) (* (`KismetMathLibrary.Sqrt` (+ (`KismetMathLibrary.MultiplyMultiply_FloatFloat` (`local.RandomX`) 2.0) (`KismetMathLibrary.MultiplyMultiply_FloatFloat` (`local.RandomY`) 2.0))) (`KismetMathLibrary.DegTan` (`local.Angle`))) (`KismetMathLibrary.RandomBool`)))) 100.0))))

(fn `InitializeTurretSight`
  (params (MaxTargetDistance :type "Float (double-precision)") (PawnSensing :type "PawnSensingComponent Object Reference"))
  (set `PawnSensingComponent.SightRadius` MaxTargetDistance PawnSensing)
  (set `PawnSensingComponent.HearingThreshold` MaxTargetDistance PawnSensing)
  (set `PawnSensingComponent.LOSHearingThreshold` MaxTargetDistance PawnSensing))

(fn `OnCDEnded`
  (`parent.OnCDEnded`)
  (set `PawnSensingComponent.bSeePawns` true (`self.PawnSensing`)))

(fn `OnCDStarted`
  (`parent.OnCDStarted`)
  (`self.ResetTurret`)
  (set `PawnSensingComponent.bSeePawns` false (`self.PawnSensing`)))

(fn `UserConstructionScript`
  (`parent.UserConstructionScript`))