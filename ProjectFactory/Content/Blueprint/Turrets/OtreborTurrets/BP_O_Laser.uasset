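; Otrebor laser turret, a child turret that fires a charged beam, with stats read per level from DT_O_Plasmageddon.
; Shoot spawns a beam attached to Center and plays a charge timeline, locking rotation past the accuracy threshold and stopping if the target is lost before full charge.
; At full charge it counts ammo toward cooldown, then detaches the beam and applies damage once.
; Gun mesh, muzzle position and cooldown effect placement vary by level.
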(event `self.ReceiveBeginPlay`
  (`parent.ReceiveBeginPlay`)
  (`SceneComponent.K2_SetRelativeLocation` (`self.NS_CdEffect`) (`KismetMathLibrary.MakeVector` 0.0 (select `int` (`self.CurrentLevel`) :`0` 0.0 :`1` 15.0 :`2` 20.0 :`3` 25.0) 69.0) false false))

(event `self.ReceiveTick`
  (params (DeltaSeconds :type "Float (single-precision)"))
  (`parent.ReceiveTick` DeltaSeconds))

(event `self.Shoot`
  (bind _ammoshooted (`self.AmmoShooted`))
  (bind _ammo (`self.Ammo`))
  (`parent.Shoot`)
  (bind _returnvalue (`|SpawnActorFromClass` "/Game/Blueprint/Turrets/Ammunation/BP_OtreborLaserBeam.BP_OtreborLaserBeam_C" (`SceneComponent.K2_GetComponentToWorld` (`self.Center`)) "Undefined" "MultiplyWithRoot" null (`self.BulletDamage`) (`self.BaseBeamRadius`) (`self.Beam Radius Percentage Modifier`) null))
  (bind _output_get (set `self.Ammo` _returnvalue))
  (`self.K2_AttachToComponent` _output_get (`self.Center`) "None" "KeepWorld" "KeepWorld" "KeepWorld" true)
  (bind (_direction _cahrgebullet) (`Timeline|ShootBeam` :!via `PlayFromStart` :!label _label)
    (:`Update`
      (if (>= _cahrgebullet (/ (`self.AccuracyPercentage`) 100.0))
        (set `self.CanRotate` false)
        (if (>= _cahrgebullet 1.0)
          (`/Engine/EditorBlueprintResources/StandardMacros.DoOnce` false :!label _label_2
            (:`Completed`
              (`/Engine/EditorBlueprintResources/StandardMacros.IncrementInt` _ammoshooted
                (:`  `
                  (if (>= _ammoshooted (`self.MaxAmmo`))
                    (set `self.AmmoShooted` 0)
                    (set `self.IsInCooldown` true))
                  (set `self.CanDeleteBeam` false)
                  (`/Engine/EditorBlueprintResources/StandardMacros.IsValid` (`self.Ammo`)
                    (:`Is Valid`
                      (`self.K2_DetachFromActor` (`self.Ammo`) "KeepWorld" "KeepWorld" "KeepWorld")
                      (`/Game/Blueprint/Turrets/Ammunation/BP_OtreborLaserBeam.GetBeamDistance` _ammo)
                      (`/Game/Blueprint/Turrets/Ammunation/BP_OtreborLaserBeam.DoDamage` _ammo)
                      (`self.ResetTurret`)))))))
          (else
            (set `self.CanDeleteBeam` true :!label _label_3)
            (`/Engine/EditorBlueprintResources/StandardMacros.IsValid` (`self.Target`)
              (:`Is Not Valid`
                (goto _label :!via `Stop`)))))
        (else
          (goto _label_3))))
    (:`Finished`
      (`|ExecutionSequence`
        (:`then_0`
          (goto _label_2 :!via `Reset`))
        (:`then_1`
          (`self.ResetTurret`))))))

(event `self.ResetTurret`
  (`parent.ResetTurret`)
  (set `self.CanRotate` true)
  (if (`self.CanDeleteBeam`)
    (set `self.CanDeleteBeam` false)
    (`/Engine/EditorBlueprintResources/StandardMacros.IsValid` (`self.Ammo`)
      (:`Is Valid`
        (`self.K2_DestroyActor` (`self.Ammo`))))))

(fn `InitializeTurret`
  (`parent.InitializeTurret`)
  (bind _returnvalue (`|GetDataTableRow` "/Game/Blueprint/Turrets/TurretFeature/Leveling/TurretSpecificDataTable/DT_O_Plasmageddon.DT_O_Plasmageddon" (`KismetStringLibrary.Conv_StringToName` (`KismetStringLibrary.Conv_IntToString` (`self.CurrentLevel`))))
    (:`then`
      (bind (_maxhealth _maxactivitytime _maxcdtime _beamdamage _aimrotationspeed _basetargetdistance _distancepercentagemodifier _basebeamradius _beamradiuspercentagemodifier _accuracypercentage _maxammo) (break `/Game/Blueprint/Turrets/TurretFeature/Leveling/TurretStructs/S_A_Laser` _returnvalue))
      (bind _output_get (set `self.MaxHealth` _maxhealth))
      (set `self.CurrentHealth` _output_get)
      (set `self.MaxActivityTime(NoFarm)` _maxactivitytime)
      (set `self.MaxCdTime` _maxcdtime)
      (set `self.BulletDamage` _beamdamage)
      (set `self.Aim Rotation Speed` _aimrotationspeed)
      (bind _output_get_2 (set `self.Max Target Distance` (+ _basetargetdistance (* _basetargetdistance (/ _distancepercentagemodifier 100.0)))))
      (set `self.Base Target Distance` _output_get_2)
      (set `self.BaseBeamRadius` (* (* _basebeamradius _beamradiuspercentagemodifier) 0.5))
      (set `self.Beam Radius Percentage Modifier` _beamradiuspercentagemodifier)
      (set `self.AccuracyPercentage` _accuracypercentage)
      (set `self.MaxAmmo` _maxammo)
      (`self.InitializeTurretSight` (`self.Max Target Distance`) (`self.PawnSensing`)))))

(fn `OnCDStarted`
  (`parent.OnCDStarted`)
  (set `self.ActivityTime(NoFarm)` 0.0))

(fn `UpdateGraphicByLevel`
  (params (Level :type Integer))
  (`/Engine/EditorBlueprintResources/StandardMacros.IsValid` self
    (:`Is Valid`
      (switch `int` Level
        (:`1`
          (`StaticMeshComponent.SetStaticMesh` (`self.Gun`) "/Game/Models/Turret/Meshes/Laser/Otrebor/SM_O_L_Gun1.SM_O_L_Gun1")
          (`SceneComponent.K2_SetRelativeLocation` (`self.Center`) (45.0 0.0 60.0) false false))
        (:`2`
          (`StaticMeshComponent.SetStaticMesh` (`self.Gun`) "/Game/Models/Turret/Meshes/Laser/Otrebor/SM_O_L_Gun2.SM_O_L_Gun2")
          (`SceneComponent.K2_SetRelativeLocation` (`self.Center`) (55.0 0.0 60.0) false false))
        (:`3`
          (`StaticMeshComponent.SetStaticMesh` (`self.Gun`) "/Game/Models/Turret/Meshes/Laser/Otrebor/SM_O_L_Gun3.SM_O_L_Gun3")
          (`SceneComponent.K2_SetRelativeLocation` (`self.Center`) (75.0 0.0 60.0) false false))))))

(fn `UserConstructionScript`
  (`parent.UserConstructionScript`))