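; Bombard turret, a child turret that fires volleys of area-damage missiles at its target.
; Shoot spawns BP_Missile from random arrow components in a delayed loop sized by ammo, then re-enables firing after a cooldown, or resets when the target is invalid.
; InitializeTurret loads per-level stats from DT_A_TurretBombard and configures sight range.
; UpdateGraphicByLevel swaps the barrel mesh and rescales the side cannons for each level.
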(event `self.ReceiveBeginPlay`
  (`parent.ReceiveBeginPlay`))

(event `self.ReceiveTick`
  (params (DeltaSeconds :type "Float (single-precision)"))
  (`parent.ReceiveTick` DeltaSeconds))

(event `self.Shoot`
  (bind (_returnvalue_location _returnvalue_rotation) (`KismetMathLibrary.BreakTransform` (`SceneComponent.K2_GetComponentToWorld` (`KismetArrayLibrary.Array_Random` (`self.K2_GetComponentsByClass` "/Script/Engine.ArrowComponent")))))
  ;[1 0.1732 0.1235] Shoot
  (`parent.Shoot`)
  (`/Game/Blueprint/BP_MacroLibrary_Actor.ForLoopWithDelay` 0 (`self.MaxAmmo`) 0.1
    (:`Loop Body`
      (`/Engine/EditorBlueprintResources/StandardMacros.IsValid` (`self.Target`)
        (:`Is Valid`
          (if (> (`self.CurrentHealth`) 0.0)
            (`|SpawnActorFromClass` "/Game/Blueprint/Turrets/Ammunation/BP_Missile.BP_Missile_C" (`KismetMathLibrary.MakeTransform` _returnvalue_location _returnvalue_rotation) "AlwaysSpawn" "MultiplyWithRoot" null (`self.BulletDamage`) (`self.Aoe Damage`) (`self.Aoe Radius`) (`self.Target`) null)))
        (:`Is Not Valid`
          (`self.ResetTurret`))))
    (:`Completed`
      (`/Engine/EditorBlueprintResources/StandardMacros.IsValid` (`self.Target`)
        (:`Is Valid`
          (`KismetSystemLibrary.Delay` (`self.DelayBetweenShoot`))
          (set `self.CanShoot` true)
          (set `self.AimTaken` false))
        (:`Is Not Valid`
          (`self.ResetTurret`))))))

(fn `InitializeTurret`
  (bind _returnvalue (`|GetDataTableRow` "/Game/Blueprint/Turrets/TurretFeature/Leveling/TurretSpecificDataTable/DT_A_TurretBombard.DT_A_TurretBombard" (`KismetStringLibrary.Conv_StringToName` (`KismetStringLibrary.Conv_IntToString` (`self.CurrentLevel`))))
    (:`then`
      (bind (_maxhealth _maxactivitytime _maxcdtime _totalammo _singlebulletdamage _aoedamage _aoeradius _delaybetweenshoot _baseaimrotationspeed _basetargetdistance _distancepercentagemodifier _baseaccuracypercentage) (break `/Game/Blueprint/Turrets/TurretFeature/Leveling/TurretStructs/S_A_TurretBombardStats` _returnvalue))
      (bind _output_get (set `self.MaxHealth` _maxhealth))
      (set `self.CurrentHealth` _output_get)
      (set `self.MaxActivityTime(NoFarm)` _maxactivitytime)
      (set `self.MaxCdTime` _maxcdtime)
      (set `self.MaxAmmo` _totalammo)
      (set `self.BulletDamage` _singlebulletdamage)
      (set `self.Aoe Damage` _aoedamage)
      (set `self.Aoe Radius` _aoeradius)
      (set `self.DelayBetweenShoot` _delaybetweenshoot)
      (set `self.Aim Rotation Speed` _baseaimrotationspeed)
      (bind _output_get_2 (set `self.Max Target Distance` (+ _basetargetdistance (* _basetargetdistance (/ _distancepercentagemodifier 100.0)))))
      (set `self.Base Target Distance` _output_get_2)
      (set `self.AccuracyPercentage` _baseaccuracypercentage)
      (`self.InitializeTurretSight` (`self.Max Target Distance`) (`self.PawnSensing`)))))

(fn `UpdateGraphicByLevel`
  (params (Level :type Integer))
  (`/Engine/EditorBlueprintResources/StandardMacros.IsValid` self
    (:`Is Valid`
      (switch `int` Level
        (:`1`
          (`StaticMeshComponent.SetStaticMesh` (`self.Barrel1`) "/Game/Models/Turret/Meshes/Bombard/SM_BO_Barrel1.SM_BO_Barrel1")
          (`SceneComponent.SetRelativeScale3D` (`self.LeftCannon`) (0.0 0.0 1.0))
          (`SceneComponent.SetRelativeScale3D` (`self.RightCannon`) (0.0 0.0 1.0)))
        (:`2`
          (`StaticMeshComponent.SetStaticMesh` (`self.Barrel1`) "/Game/Models/Turret/Meshes/Bombard/SM_BO_Barrel2.SM_BO_Barrel2")
          (`SceneComponent.SetRelativeScale3D` (`self.LeftCannon`) (1.0 0.0 1.0))
          (`SceneComponent.SetRelativeScale3D` (`self.RightCannon`) (1.0 0.0 1.0)))
        (:`3`
          (`StaticMeshComponent.SetStaticMesh` (`self.Barrel1`) "/Game/Models/Turret/Meshes/Bombard/SM_BO_Barrel3.SM_BO_Barrel3")
          (`SceneComponent.SetRelativeScale3D` (`self.LeftCannon`) (1.0 1.0 1.0))
          (`SceneComponent.SetRelativeScale3D` (`self.RightCannon`) (1.0 1.0 1.0)))))))

(fn `UserConstructionScript`
  (`parent.UserConstructionScript`))