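; BP_HazardTurret is a turret that toggles an area-of-effect hazard with its cooldown state.
; Tick uses two DoOnce gates that re-arm each other, destroying the AoE actor once when cooldown begins and calling SpawnAoe once when it ends.
; SpawnAoe is empty here.
; The nodes that spawn a configured BP_AoeBase and attach it to Center are disconnected, so they never run.
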(event `self.ReceiveBeginPlay`
  (`parent.ReceiveBeginPlay`))

(event `self.ReceiveTick`
  (params (DeltaSeconds :type "Float (single-precision)"))
  (`parent.ReceiveTick` DeltaSeconds)
  (if (`self.IsInCooldown`)
    (`/Engine/EditorBlueprintResources/StandardMacros.DoOnce` false :!label _label
      (:`Completed`
        (`self.K2_DestroyActor` (`self.AoeActor`))
        (goto _label_2 :!via `Reset`)))
    (else
      (`/Engine/EditorBlueprintResources/StandardMacros.DoOnce` false :!label _label_2
        (:`Completed`
          (`self.SpawnAoe`)
          (goto _label :!via `Reset`))))))

(event `SpawnAoe`)

(fn `UserConstructionScript`
  (`parent.UserConstructionScript`))