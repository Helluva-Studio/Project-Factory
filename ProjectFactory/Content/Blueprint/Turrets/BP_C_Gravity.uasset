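; Gravity crowd-control turret, a child turret class that spawns gravity ammo to exert force within an area of effect.
; Stats for the current level load from DT_C_Gravity and are passed to the ammo on spawn.
; A looping timer pulses two black hole meshes via a timeline, playing sound and attraction Niagara effects each GravityTick.
; Cooldown hides the black holes, stops the timer and destroys the ammo, restoring them when it ends.
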(event `self.ReceiveBeginPlay`
  (`parent.ReceiveBeginPlay`)
  (bind _returnvalue (`KismetSystemLibrary.K2_SetTimerDelegate` (delegate `ScaleBlackHole`) (`self.GravityTick`) true))
  (set `self.AttractionTimer` _returnvalue)
  (`self.ScaleBlackHole`))

(event `ScaleBlackHole`
  (`TimelineComponent.SetPlayRate` (`self.Scaling`) (`KismetMathLibrary.SafeDivide` 1.0 (`self.GravityTick`)))
  (`GameplayStatics.PlaySoundAtLocation` "/Game/Audio/SFX/Turrets/Gravity/SC_Gravity.SC_Gravity" (`SceneComponent.K2_GetComponentLocation` (`self.LowerBH`)) (struct) 1.0 1.0 0.0 null null null null)
  (`GameplayStatics.PlaySoundAtLocation` "/Game/Audio/SFX/Turrets/Gravity/SC_Gravity.SC_Gravity" (`SceneComponent.K2_GetComponentLocation` (`self.UpperBH`)) (struct) 1.0 1.0 0.0 null null null null)
  (bind (_direction _scalebh) (`Timeline|Scaling` :!via `PlayFromStart`)
    (:`Update`
      (`SceneComponent.SetRelativeScale3D` (`self.UpperBH`) (* _scalebh (`self.InitialScale`)))
      (`SceneComponent.SetRelativeScale3D` (`self.LowerBH`) (* _scalebh (`self.InitialScale`)))
      (if (> _scalebh 1.25)
        (`/Engine/EditorBlueprintResources/StandardMacros.DoOnce` false :!label _label
          (:`Completed`
            (`NiagaraFunctionLibrary.SpawnSystemAtLocation` "/Game/Blueprint/Turrets/TurretFeature/Gravity/NS_AttractionForce.NS_AttractionForce" (`SceneComponent.K2_GetComponentLocation` (`self.LowerBH`)))
            (`NiagaraFunctionLibrary.SpawnSystemAtLocation` "/Game/Blueprint/Turrets/TurretFeature/Gravity/NS_AttractionForce.NS_AttractionForce" (`SceneComponent.K2_GetComponentLocation` (`self.UpperBH`)))))))
    (:`Finished`
      (goto _label :!via `Reset`))))

(event `self.SpawnAmmo`
  (`parent.SpawnAmmo`)
  (`/Engine/EditorBlueprintResources/StandardMacros.IsValid` (`self.CcAmmo`)
    (:`Is Valid`
      (message `/Game/Blueprint/Turrets/Interfaces/BPI_TurretCcAmmo.InitializeGravityAmmo` (`self.CcAmmo`) (`self.CanHitPlayer`) (`self.TypeOfCc`) (`self.TypeOfAoe`) (`self.MaxDistance(Cone)/MaxRadius(Sphere)`) (`self.GravityForce`) (`self.Min Gravity Force Percentage`) (`self.GravityTick`)))))

(fn `InitializeTurret`
  (`parent.InitializeTurret`)
  (bind _returnvalue (`|GetDataTableRow` "/Game/Blueprint/Turrets/TurretFeature/Leveling/TurretSpecificDataTable/DT_C_Gravity.DT_C_Gravity" (`KismetStringLibrary.Conv_StringToName` (`KismetStringLibrary.Conv_IntToString` (`self.CurrentLevel`))))
    (:`then`
      (bind (_maxhealth _maxactivitytime _maxcdtime _baseaoetype _baseradius _radiuspercentagemodifier _basecctype _basegravityforce _basemingravityforcepercentage _gravityforcepercentagemodifier _gravitytick) (break `/Game/Blueprint/Turrets/TurretFeature/Leveling/TurretStructs/S_C_Gravity` _returnvalue))
      (bind _output_get (set `self.MaxHealth` _maxhealth))
      (set `self.CurrentHealth` _output_get)
      (set `self.MaxActivityTime(NoFarm)` _maxactivitytime)
      (set `self.MaxCdTime` _maxcdtime)
      (set `self.TypeOfAoe` _baseaoetype)
      (bind _output_get_2 (set `self.MaxDistance(Cone)/MaxRadius(Sphere)` (+ _baseradius (* _baseradius (/ _radiuspercentagemodifier 100.0)))))
      (set `self.BaseDistance(Cone)/BaseRadius(Sphere)` _output_get_2)
      (set `self.Min Gravity Force Percentage` _basemingravityforcepercentage)
      (set `self.TypeOfCc` _basecctype)
      (set `self.GravityForce` (+ _basegravityforce (* _basegravityforce (/ _gravityforcepercentagemodifier 100.0))))
      (set `self.GravityTick` _gravitytick))))

(fn `OnCDEnded`
  (`SceneComponent.SetVisibility` (`self.UpperBH`) true false)
  (`SceneComponent.SetVisibility` (`self.LowerBH`) true false)
  (`ActorComponent.Deactivate` (`self.NS_CdEffect`))
  (bind _returnvalue (`KismetSystemLibrary.K2_SetTimerDelegate` (`|CreateDelegate` :!event `ScaleBlackHole`) (`self.GravityTick`) true))
  (set `self.AttractionTimer` _returnvalue)
  (`/Engine/EditorBlueprintResources/StandardMacros.IsValid` (`self.CcAmmo`)
    (:`Is Not Valid`
      (`self.SpawnAmmo`))))

(fn `OnCDStarted`
  (bind _ccammo (`self.CcAmmo`))
  (`SceneComponent.SetVisibility` (`self.UpperBH`) false false)
  (`SceneComponent.SetVisibility` (`self.LowerBH`) false false)
  (`ActorComponent.Activate` (`self.NS_CdEffect`) false)
  (`KismetSystemLibrary.K2_ClearAndInvalidateTimerHandle` (`self.AttractionTimer`))
  (`/Engine/EditorBlueprintResources/StandardMacros.IsValid` _ccammo
    (:`Is Valid`
      (`self.K2_DestroyActor` _ccammo))))

(fn `UpdateGraphicByLevel`
  (params (Level :type Integer))
  (`/Engine/EditorBlueprintResources/StandardMacros.IsValid` self
    (:`Is Valid`
      (switch `int` Level
        (:`1`
          (`SceneComponent.SetWorldScale3D` (`self.UpperBH`) (0.5 0.5 0.5))
          (`SceneComponent.SetWorldScale3D` (`self.LowerBH`) (0.5 0.5 0.5))
          (set `self.InitialScale` (`SceneComponent.RelativeScale3D` (`self.LowerBH`))))
        (:`2`
          (`SceneComponent.SetWorldScale3D` (`self.UpperBH`) (0.85 0.85 0.85))
          (`SceneComponent.SetWorldScale3D` (`self.LowerBH`) (0.85 0.85 0.85))
          (set `self.InitialScale` (`SceneComponent.RelativeScale3D` (`self.LowerBH`))))
        (:`3`
          (`SceneComponent.SetWorldScale3D` (`self.UpperBH`) (1.2 1.2 1.2))
          (`SceneComponent.SetWorldScale3D` (`self.LowerBH`) (1.2 1.2 1.2))
          (set `self.InitialScale` (`SceneComponent.RelativeScale3D` (`self.LowerBH`))))))))

(fn `UserConstructionScript`
  (`parent.UserConstructionScript`))