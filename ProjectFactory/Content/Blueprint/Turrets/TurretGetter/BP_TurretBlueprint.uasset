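; Turret blueprint pickup that dissolves into view on BeginPlay and unlocks a turret type when a robot collects it.
; The first overlap by a BPI_Robot actor passes the turret to that robot, records it in the game instance, plays a sound and shows the unlock on the player HUD.
; One timeline drives a dynamic material's Fade parameter both ways, destroying the actor after the reverse dissolve.
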(event `self.ReceiveBeginPlay`
  (bind _returnvalue (`PrimitiveComponent.CreateDynamicMaterialInstance` (`self.StaticMesh`) 0 null "None"))
  (`PrimitiveComponent.SetMaterial` (`self.StaticMesh`) 0 _returnvalue)
  (`MaterialInstanceDynamic.SetScalarParameterValue` _returnvalue "Fade" 0.0)
  (`self.Dissolve` true))

(event `Dissolve`
  (params (ShouldAppear :type Boolean))
  (if ShouldAppear
    (bind (_direction _appearlerp) (`Timeline|DissolveEffect` :!via `PlayFromStart` :!label _label)
      (:`Update`
        (bind _asmaterial_instance_dynamic (cast `MaterialInstanceDynamic` (`PrimitiveComponent.GetMaterial` (`self.StaticMesh`) 0)))
        (`MaterialInstanceDynamic.SetScalarParameterValue` _asmaterial_instance_dynamic "Fade" _appearlerp))
      (:`Finished`
        (if (not ShouldAppear)
          (`self.K2_DestroyActor`))))
    (else
      (goto _label :!via `ReverseFromEnd`))))

(event `self.ReceiveActorBeginOverlap`
  (params (OtherActor :type "Actor Object Reference"))
  (if (`KismetSystemLibrary.DoesImplementInterface` OtherActor "/Game/Blueprint/Robot/Interfaces/BPI_Robot.BPI_Robot_C")
    (`/Engine/EditorBlueprintResources/StandardMacros.DoOnce` false
      (:`Completed`
        (message `/Game/Blueprint/Robot/Interfaces/BPI_Robot.GetNewTurret` OtherActor (`self.Type`) (`self.Turret`))
        (`GameplayStatics.PlaySoundAtLocation` "/Game/Audio/SFX/Environment/SC_BlueprintPickup.SC_BlueprintPickup" (`self.K2_GetActorLocation`) (struct) 1.0 1.0 0.0 null null null null)
        (bind _asbp_new_game_instance (cast `/Game/Blueprint/BP_NewGameInstance` (`GameplayStatics.GetGameInstance`)))
        (`/Game/Blueprint/BP_NewGameInstance.TurretPickedUp` _asbp_new_game_instance (`self.Turret`))
        (bind _foundwidgets (`WidgetBlueprintLibrary.GetAllWidgetsOfClass` "/Game/HUD/PlayerHUD/WB_PlayerHUD.WB_PlayerHUD_C"))
        (`/Game/HUD/PlayerHUD/WB_PlayerHUD.TurretUnlockedEvent` (`|GetArrayItem` _foundwidgets) (`KismetTextLibrary.Conv_StringToText` (`|GetEnumeratorNameAsString` (`self.Type`))))
        (`self.Dissolve` false)))))

(fn `UserConstructionScript`)