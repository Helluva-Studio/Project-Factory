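; Bombard turret, a child of a base turret, that fires bursts of bullets at its target and gains visible parts as it levels up.
; Each tick it sizes a Niagara laser by line trace and spins the barrels at patrol or shooting speed, except during cooldown.
; Shoot spawns BP_Bullet through a delayed loop, then reloads, or resets if the target is lost.
; LevelUp reveals the Ammo and Aim components progressively.
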(event `self.ReceiveBeginPlay`
  (`parent.ReceiveBeginPlay`))

(event `self.ReceiveTick`
  (params (DeltaSeconds :type "Float (single-precision)"))
  (`parent.ReceiveTick` DeltaSeconds)
  (`|ExecutionSequence`
    (:`then_0`
      (`self.Laser`))
    (:`then_1`
      (`self.RotateBarrel`))))

(event `Laser`
  (bind _niagara (`self.Niagara`))
  (bind _returnvalue (`SceneComponent.K2_GetComponentLocation` _niagara))
  (`/Engine/EditorBlueprintResources/StandardMacros.IsValid` self
    (:`Is Valid`
      ;[1 1 1] Graphic Feedback
      (if (not (`self.IsInCooldown`))
        (`FXSystemComponent.SetVectorParameter` _niagara "Beam End" (`KismetMathLibrary.MakeVector` (`self.Max Target Distance`)))
        (bind (_outhit _returnvalue_2) (`KismetSystemLibrary.LineTraceSingleForObjects` _returnvalue (+ _returnvalue (* (`SceneComponent.GetForwardVector` _niagara) (`self.Max Target Distance`))) (`|MakeArray` "ObjectTypeQuery3" "ObjectTypeQuery2" "ObjectTypeQuery1" :!type "EObjectTypeQuery Enum")))
        (if _returnvalue_2
          (`FXSystemComponent.SetVectorParameter` (`self.Niagara`) "Beam End" (`KismetMathLibrary.MakeVector` (+ (`.Distance` (`GameplayStatics.BreakHitResult` _outhit)) 50.0))))
        (else
          (`FXSystemComponent.SetVectorParameter` (`self.Niagara`) "Beam End" (0.0 0.0 0.0)))))))

(event `RotateBarrel`
  ;[1 1 1] Graphic Feedback
  (`/Engine/EditorBlueprintResources/StandardMacros.IsValid` self
    (:`Is Valid`
      (if (not (`self.IsInCooldown`))
        (`SceneComponent.K2_AddLocalRotation` (`self.Barrels`) (`KismetMathLibrary.MakeRotator` 0.0 (`KismetMathLibrary.SelectFloat` (`self.ShootingBarrelRotation`) (`self.PatrolBarrelRotation`) (`KismetSystemLibrary.IsValid` (`self.Target`)))) false false)))))

(event `self.Shoot`
  ;[1 0.1732 0.1235] Shoot
  (`parent.Shoot`)
  (`/Game/Blueprint/BP_MacroLibrary_Actor.For Loop With Delay` 1 (`self.MaxAmmo`) (`self.DelayBetweenShoot`)
    (:`Loop Body`
      (`/Engine/EditorBlueprintResources/StandardMacros.IsValid` (`self.Target`)
        (:`Is Valid`
          (`|SpawnActorFromClass` "/Game/Blueprint/Turrets/Ammunation/BP_Bullet.BP_Bullet_C" (`SceneComponent.K2_GetComponentToWorld` (`self.BulletLocation`)) "AlwaysSpawn" "MultiplyWithRoot" null (`self.BulletDamage`) null))
        (:`Is Not Valid`
          (`self.ResetTurret`))))
    (:`Completed`
      (`/Engine/EditorBlueprintResources/StandardMacros.IsValid` (`self.Target`)
        (:`Is Valid`
          (`KismetSystemLibrary.Delay` (`self.ReloadAmmoTime`))
          (set `self.CanShoot` true)
          (set `self.AimTaken` false))
        (:`Is Not Valid`
          (`self.ResetTurret`))))))

(event `self.LevelUp`
  (params (Level :type Integer))
  (`parent.LevelUp` Level)
  (`/Engine/EditorBlueprintResources/StandardMacros.IsValid` self
    (:`Is Valid`
      (switch `int` Level
        (:`1`
          (`SceneComponent.SetHiddenInGame` (`self.Ammo`) true true)
          (`SceneComponent.SetHiddenInGame` (`self.Aim`) true true))
        (:`2`
          (`SceneComponent.SetHiddenInGame` (`self.Aim`) true true)
          (`SceneComponent.SetHiddenInGame` (`self.Ammo`) false true))
        (:`3`
          (`SceneComponent.SetHiddenInGame` (`self.Ammo`) false true)
          (`SceneComponent.SetHiddenInGame` (`self.Aim`) false true))))))

(fn `UserConstructionScript`
  (`parent.UserConstructionScript`))