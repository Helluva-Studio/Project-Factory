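; Poison turret, child of a parent turret Blueprint, that spawns a damage-over-time AoE and animates bobbing, spinning flowers while off cooldown.
; InitializeTurret loads per-level stats from DT_H_TurretPoison, spawns the AoE and passes stats to its ammo.
; Interact flip-flops a timeline that scales damage and DoT against radius and tick, live-updating the ammo; tick lerps from its current value, so compounds.
; UpdateGraphicByLevel shows one neck mesh per level.
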(event `self.ReceiveBeginPlay`
  (`parent.ReceiveBeginPlay`))

(event `self.ReceiveTick`
  (params (DeltaSeconds :type "Float (single-precision)"))
  (`parent.ReceiveTick` DeltaSeconds)
  (if (not (`self.IsInCooldown`))
    (`self.FlowerFeedback`)))

(event `self.SpawnDamageAoe`
  (`parent.SpawnDamageAoe`)
  (`/Engine/EditorBlueprintResources/StandardMacros.IsValid` (`self.DamageAmmo`)
    (:`Is Valid`
      (message `/Game/Blueprint/Turrets/Interfaces/BPI_TurretDamageAmmo.InitializePoisonAmmo` (`self.DamageAmmo`) (`self.CanHitPlayer`) (`self.D_TypeOfDamage`) (`self.D_TypeOfAoe`) (`self.MaxDistance(Cone)/MaxRadius(Sphere)`) (`self.DamageTick`) (`self.MaxDamageOnHit`) (`self.MaxDotInsideAoe`) (`self.MaxDotOutsideAoe`) (`self.MaxDotDuration`)))))

(event `FlowerFeedback`
  (bind _returnvalue (/ (`KismetMathLibrary.DegSin` (* (`self.GetGameTimeSinceCreation`) 200.0)) 20.0))
  (`/Engine/EditorBlueprintResources/StandardMacros.IsValid` self
    (:`Is Valid`
      (`SceneComponent.K2_AddWorldOffset` (`self.FlowerB`) (`KismetMathLibrary.MakeVector` 0.0 0.0 _returnvalue) false false)
      (`SceneComponent.K2_AddWorldOffset` (`self.FlowerA`) (`KismetMathLibrary.MakeVector` 0.0 0.0 _returnvalue) false false)
      (`SceneComponent.K2_AddWorldOffset` (`self.FlowerC`) (`KismetMathLibrary.MakeVector` 0.0 0.0 _returnvalue) false false)
      (`SceneComponent.K2_AddWorldOffset` (`self.FlowerA2`) (`KismetMathLibrary.MakeVector` 0.0 0.0 (* _returnvalue -1.0)) false false)
      (`SceneComponent.K2_AddWorldOffset` (`self.FlowerB2`) (`KismetMathLibrary.MakeVector` 0.0 0.0 (* _returnvalue -1.0)) false false)
      (`SceneComponent.K2_AddWorldOffset` (`self.FlowerA1`) (`KismetMathLibrary.MakeVector` 0.0 0.0 _returnvalue) false false)
      (`SceneComponent.K2_AddLocalRotation` (`self.FlowerA1`) (struct :`Yaw` 0.3) false false)
      (`SceneComponent.K2_AddLocalRotation` (`self.FlowerA2`) (struct :`Yaw` 0.3) false false)
      (`SceneComponent.K2_AddLocalRotation` (`self.FlowerA`) (struct :`Yaw` 0.3) false false)
      (`SceneComponent.K2_AddLocalRotation` (`self.FlowerC`) (struct :`Yaw` 0.3) false false)
      (`SceneComponent.K2_AddLocalRotation` (`self.FlowerB`) (struct :`Yaw` -0.3) false false)
      (`SceneComponent.K2_AddLocalRotation` (`self.FlowerB2`) (struct :`Yaw` -0.3) false false))))

(event `/Game/Blueprint/Turrets/Interfaces/BI_Interactable.Interact`
  (bind _basedotoutsideaoe (`self.BaseDotOutsideAoe`))
  (bind _damageammo (`self.DamageAmmo`))
  (bind _basedotduration (`self.BaseDotDuration`))
  (bind _basedamageonhit (`self.BaseDamageOnHit`))
  (bind _damagetick (`self.DamageTick`))
  (bind _d_basedistance_cone__baseradius_sphere_ (`self.D_BaseDistance(Cone)/BaseRadius(Sphere)`))
  (bind _basedotinsideaoe (`self.BaseDotInsideAoe`))
  (if (and (`self.CanChangeMode`) (not (`self.IsInCooldown`)))
    (set `self.CanChangeMode` false)
    (`TimelineComponent.SetPlayRate` (`self.ChangeValue`) (`KismetMathLibrary.SafeDivide` 1.0 (`self.TimeToChangeMode`)))
    (`/Engine/EditorBlueprintResources/StandardMacros.FlipFlop`
      (:`A`
        (bind (_direction _value) (`Timeline|ChangeValue` :!via `PlayFromStart` :!label _label)
          (:`Update`
            (set `self.ChangeModeLerpValue` _value)
            (`|ExecutionSequence`
              (:`then_0`
                (set `self.MaxDamageOnHit` (`KismetMathLibrary.Lerp` _basedamageonhit (* _basedamageonhit (`self.ChangeModeModifierPercentage`)) (`self.ChangeModeLerpValue`))))
              (:`then_1`
                (set `self.MaxDotInsideAoe` (`KismetMathLibrary.Lerp` _basedotinsideaoe (* _basedotinsideaoe (`self.ChangeModeModifierPercentage`)) (`self.ChangeModeLerpValue`))))
              (:`then_2`
                (set `self.MaxDotOutsideAoe` (`KismetMathLibrary.Lerp` _basedotoutsideaoe (* _basedotoutsideaoe (`self.ChangeModeModifierPercentage`)) (`self.ChangeModeLerpValue`))))
              (:`then_3`
                (set `self.MaxDotDuration` (`KismetMathLibrary.Lerp` _basedotduration (* _basedotduration (`self.ChangeModeModifierPercentage`)) (`self.ChangeModeLerpValue`))))
              (:`then_4`
                (set `self.DamageTick` (`KismetMathLibrary.Lerp` _damagetick (* _damagetick (- 2.0 (`self.ChangeModeModifierPercentage`))) (`self.ChangeModeLerpValue`))))
              (:`then_5`
                (set `self.MaxDistance(Cone)/MaxRadius(Sphere)` (`KismetMathLibrary.Lerp` _d_basedistance_cone__baseradius_sphere_ (* _d_basedistance_cone__baseradius_sphere_ (- 2.0 (`self.ChangeModeModifierPercentage`))) (`self.ChangeModeLerpValue`))))
              (:`then_6`
                (`/Engine/EditorBlueprintResources/StandardMacros.IsValid` _damageammo
                  (:`Is Valid`
                    (`SceneComponent.SetWorldScale3D` (`Actor.RootComponent` _damageammo) (`KismetMathLibrary.Conv_DoubleToVector` (/ (`self.MaxDistance(Cone)/MaxRadius(Sphere)`) 100.0)))
                    (message `/Game/Blueprint/Turrets/Interfaces/BPI_TurretDamageAmmo.InitializePoisonAmmo` (`self.DamageAmmo`) (`self.CanHitPlayer`) (`self.D_TypeOfDamage`) (`self.D_TypeOfAoe`) (`self.MaxDistance(Cone)/MaxRadius(Sphere)`) (`self.DamageTick`) (`self.MaxDamageOnHit`) (`self.MaxDotInsideAoe`) (`self.MaxDotOutsideAoe`) (`self.MaxDotDuration`)))))))
          (:`Finished`
            (set `self.CanChangeMode` true))))
      (:`B`
        (goto _label :!via `ReverseFromEnd`)))))

(fn `CanInteract`
  (returns (CanInteract :type Boolean))
  (return (and (`self.CanChangeMode`) (not (`self.IsInCooldown`)))))

(fn `GetCost`
  (returns (GetCost :type "Float (double-precision)"))
  (return 0.0))

(fn `GetInteractImage`
  (returns (Image :type "Texture Object Reference"))
  (return null))

(fn `GetInteractMessage`
  (returns (InteractMessage :type Text) (Image :type "Texture Object Reference"))
  (return "" null))

(fn `InitializeTurret`
  (`parent.InitializeTurret`)
  (bind _returnvalue (`|GetDataTableRow` "/Game/Blueprint/Turrets/TurretFeature/Leveling/TurretSpecificDataTable/DT_H_TurretPoison.DT_H_TurretPoison" (`KismetStringLibrary.Conv_StringToName` (`KismetStringLibrary.Conv_IntToString` (`self.CurrentLevel`))))
    (:`then`
      (bind (_maxhealth _maxactivitytime _maxcdtime _baseaoetype _baseradius _radiuspercentagemodifier _basedamagetype _damagetick _damageonhit _damageovertimeinsideaoe _damageovertimeoutsideaoe _dotduration _changemodemodifierpercentage) (break `/Game/Blueprint/Turrets/TurretFeature/Leveling/TurretStructs/S_H_TurretPoisonStats` _returnvalue))
      (bind _output_get (set `self.MaxHealth` _maxhealth))
      (set `self.CurrentHealth` _output_get)
      (set `self.MaxActivityTime(NoFarm)` _maxactivitytime)
      (set `self.MaxCdTime` _maxcdtime)
      (set `self.D_TypeOfAoe` _baseaoetype)
      (bind _output_get_2 (set `self.MaxDistance(Cone)/MaxRadius(Sphere)` (+ _baseradius (* _baseradius (/ _radiuspercentagemodifier 100.0)))))
      (set `self.D_BaseDistance(Cone)/BaseRadius(Sphere)` _output_get_2)
      (set `self.D_TypeOfDamage` _basedamagetype)
      (bind _output_get_3 (set `self.DamageTick` _damagetick))
      (set `self.BaseDamageTick` _output_get_3)
      (bind _output_get_4 (set `self.MaxDamageOnHit` _damageonhit))
      (set `self.BaseDamageOnHit` _output_get_4)
      (bind _output_get_5 (set `self.MaxDotInsideAoe` _damageovertimeinsideaoe))
      (set `self.BaseDotInsideAoe` _output_get_5)
      (bind _output_get_6 (set `self.MaxDotOutSideAoe` _damageovertimeoutsideaoe))
      (set `self.BaseDotOutsideAoe` _output_get_6)
      (bind _output_get_7 (set `self.MaxDotDuration` _dotduration))
      (set `self.BaseDotDuration` _output_get_7)
      (set `self.ChangeModeModifierPercentage` (+ 1.0 (/ _changemodemodifierpercentage 100.0)))
      (`self.SetActorTickEnabled` true)
      (`self.SpawnDamageAoe`))))

(fn `UpdateGraphicByLevel`
  (params (Level :type Integer))
  (`/Engine/EditorBlueprintResources/StandardMacros.IsValid` self
    (:`Is Valid`
      (switch `int` Level
        (:`1`
          (`SceneComponent.SetVisibility` (`self.Neck`) false true)
          (`SceneComponent.SetVisibility` (`self.Neck2`) false true)
          (`SceneComponent.SetVisibility` (`self.Neck1`) true true))
        (:`2`
          (`SceneComponent.SetVisibility` (`self.Neck`) false true)
          (`SceneComponent.SetVisibility` (`self.Neck2`) true true)
          (`SceneComponent.SetVisibility` (`self.Neck1`) false true))
        (:`3`
          (`SceneComponent.SetVisibility` (`self.Neck`) true true)
          (`SceneComponent.SetVisibility` (`self.Neck2`) false true)
          (`SceneComponent.SetVisibility` (`self.Neck1`) false true))))))

(fn `UserConstructionScript`
  (`parent.UserConstructionScript`))

(fn `WhichInteraction`
  (returns (TypeInteraction :type "/Game/Blueprint/Enum/EInteractable Enum"))
  (return "NewEnumerator0"))