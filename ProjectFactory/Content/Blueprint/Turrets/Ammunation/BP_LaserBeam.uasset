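; Laser beam turret ammunition that damages enemies along a Niagara beam.
; A forward line trace ends the beam at BI_Room actors or maximum range, setting the length for a player-ignoring sphere trace.
; DoDamage accumulates unique BPI_Enemy hits in an uncleared list and damages every entry on each call.
; The turret's destroy event removes only young beams; effect completion re-enables BP_A_Aim rotation and destroys the actor.
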(event `OnSystemFinished_Event`
  (params (PSystem :type "NiagaraComponent Object Reference"))
  (bind _asbp_a_aim (cast `/Game/Blueprint/Turrets/BP_A_Aim` (`self.Instigator`)))
  (set `/Game/Blueprint/Turrets/BP_A_Aim.CanRotate` true _asbp_a_aim)
  (`self.K2_DestroyActor`))

(event `self.ReceiveBeginPlay`
  (`AudioComponent.FadeIn` (`self.SpawnSound`) 0.5 1.0 0.0 "Linear")
  (`FXSystemComponent.SetFloatParameter` (`self.Niagara`) "ScaleMultiplier" (* (`self.BeamRadiusModifier`) 0.5))
  (bind _asbp_turret_base (cast `/Game/Blueprint/Turrets/BP_Turret_Base` (`self.Instigator`)))
  (add `/Game/Blueprint/Turrets/BP_Turret_Base.DestroyAmmo` _asbp_turret_base (delegate `DestroyAmmo`))
  (add `NiagaraComponent.OnSystemFinished` (`self.Niagara`) (delegate `OnSystemFinished_Event`)))

(event `DestroyAmmo`
  (if (< (`self.GetGameTimeSinceCreation`) 3.4)
    (`self.K2_DestroyActor`)))

(event `GetBeamDistance`
  (bind _returnvalue (`self.K2_GetActorLocation`))
  (bind _niagara (`self.Niagara`))
  (bind _outhit (`KismetSystemLibrary.LineTraceSingle` :`Start` _returnvalue :`End` (+ _returnvalue (* (`self.GetActorForwardVector`) (`self.MaxBeamDistance`))) :`TraceChannel` "TraceTypeQuery1" :`TraceColor` (struct :`R` 0.051397 :`G` 0.06834 :`B` 1.0 :`A` 1.0)))
  (bind (_bblockinghit _binitialoverlap _time _distance _location _impactpoint _normal _impactnormal _physmat _hitactor) (`GameplayStatics.BreakHitResult` _outhit))
  (if (`KismetSystemLibrary.DoesImplementInterface` _hitactor "/Game/Blueprint/Envirorment/Rooms/BI_Room.BI_Room_C")
    (`FXSystemComponent.SetVectorParameter` _niagara "BeamEnd" (`KismetMathLibrary.MakeVector` _distance))
    (set `self.BeamEndDistance` _distance)
    (else
      (`FXSystemComponent.SetVectorParameter` _niagara "BeamEnd" (`KismetMathLibrary.MakeVector` (`self.MaxBeamDistance`)))
      (set `self.BeamEndDistance` (`self.MaxBeamDistance`)))))

(event `DoDamage`
  (bind _returnvalue (`self.K2_GetActorLocation`))
  (`AudioComponent.FadeIn` (`self.DamageAudio`) 0.5 1.0 0.0 "Linear")
  (bind _outhits (`KismetSystemLibrary.SphereTraceMultiForObjects` _returnvalue (+ _returnvalue (* (`self.GetActorForwardVector`) (`self.BeamEndDistance`))) (`self.BaseBeamRadius`) (`|MakeArray` "ObjectTypeQuery3" :!type "EObjectTypeQuery Enum") false (`|MakeArray` (`GameplayStatics.GetPlayerPawn` 0) :!type "Actor Object Reference")))
  (for _array_element _outhits
    (bind (_bblockinghit _binitialoverlap _time _distance _location _impactpoint _normal _impactnormal _physmat _hitactor) (`GameplayStatics.BreakHitResult` _array_element))
    (if (`KismetSystemLibrary.DoesImplementInterface` _hitactor "/Game/Blueprint/Enemies/Interfaces/BPI_Enemy.BPI_Enemy_C")
      (`KismetArrayLibrary.Array_AddUnique` (`self.HittedActor`) _hitactor)))
  (for _array_element_2 (`self.HittedActor`)
    (`GameplayStatics.ApplyDamage` _array_element_2 (`self.BulletDamage`) null (`self.Instigator`))))

(fn `UserConstructionScript`)