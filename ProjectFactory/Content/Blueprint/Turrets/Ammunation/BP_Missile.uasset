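; Homing missile projectile that chases a target, damages an enemy it strikes and explodes for area damage.
; A timeline scaled to its lifetime drives homing acceleration and detonates it on finish; Tick stops homing when a BP_BaseEnemy target dies.
; Overlaps also detonate it, except with the player and resource spawnables.
; The explosion damages nearby enemies except the assigned target, plays effects and releases the attached trail actor.
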(event `self.ReceiveBeginPlay`
  (`GameplayStatics.PlaySoundAtLocation` "/Game/Audio/SFX/Turrets/Bombard/SC_MissileLaunch.SC_MissileLaunch" (`self.K2_GetActorLocation`) (struct) 1.0 1.0 0.0 null null null null)
  (bind _returnvalue (`|SpawnActorFromClass` "/Game/Blueprint/Turrets/Ammunation/BP_MissileTrail.BP_MissileTrail_C" (`KismetMathLibrary.MakeTransform` (-15.0 0.0 0.0)) "Undefined" "MultiplyWithRoot" null null))
  (bind _output_get (set `self.MissileTrail` _returnvalue))
  (`self.K2_AttachToActor` _output_get self "None" "KeepRelative" "KeepRelative" "KeepRelative" true)
  (`TimelineComponent.SetPlayRate` (`self.HomingVelocity`) (`KismetMathLibrary.SafeDivide` 1.0 (`self.LifeTime`)))
  (bind (_direction _newtrack_0) (`Timeline|HomingVelocity` :!via `PlayFromStart`)
    (:`Update`
      (set `ProjectileMovementComponent.HomingAccelerationMagnitude` (* _newtrack_0 100000.0) (`self.ProjectileMovement`)))
    (:`Finished`
      (`self.Explosion`))))

(event `self.Sphere.OnComponentBeginOverlap`
  (params (OverlappedComponent :type "PrimitiveComponent Object Reference") (OtherActor :type "Actor Object Reference") (OtherComp :type "PrimitiveComponent Object Reference") (OtherBodyIndex :type Integer) (bFromSweep :type Boolean) (SweepResult :type "HitResult Structure (by ref)"))
  (if (`KismetSystemLibrary.DoesImplementInterface` OtherActor "/Game/Blueprint/Enemies/Interfaces/BPI_Enemy.BPI_Enemy_C")
    (`GameplayStatics.ApplyDamage` OtherActor (`self.Damage`) null (`self.Instigator`))
    (`self.Explosion`)
    (elif (and (!= OtherActor (`GameplayStatics.GetPlayerPawn` 0)) (not (`KismetSystemLibrary.DoesImplementInterface` OtherActor "/Game/Blueprint/Resources/BPI_ResourceSpawnable.BPI_ResourceSpawnable_C")))
      (`self.Explosion`))))

(event `self.ReceiveTick`
  (params (DeltaSeconds :type "Float (single-precision)"))
  (bind _asbp_base_enemy (cast `/Game/Blueprint/Enemies/BP_BaseEnemy` (`self.Target`)))
  (`/Engine/EditorBlueprintResources/StandardMacros.IsValid` _asbp_base_enemy
    (:`Is Valid`
      (if (<= (`/Game/Blueprint/Enemies/BP_BaseEnemy.CurrentHealth` _asbp_base_enemy) 0.0)
        (set `ProjectileMovementComponent.bIsHomingProjectile` false (`self.ProjectileMovement`) :!label _label)))
    (:`Is Not Valid`
      (goto _label))))

(event `Explosion`
  (bind _missiletrail (`self.MissileTrail`))
  (bind _returnvalue (`SceneComponent.K2_GetComponentLocation` (`self.Bullet`)))
  (bind _outhits (`KismetSystemLibrary.SphereTraceMultiForObjects` _returnvalue _returnvalue (`self.AoeRadius`) (`|MakeArray` "ObjectTypeQuery3" :!type "EObjectTypeQuery Enum")))
  (for _array_element _outhits
    (bind (_bblockinghit _binitialoverlap _time _distance _location _impactpoint _normal _impactnormal _physmat _hitactor) (`GameplayStatics.BreakHitResult` _array_element))
    (if (`KismetSystemLibrary.DoesImplementInterface` _hitactor "/Game/Blueprint/Enemies/Interfaces/BPI_Enemy.BPI_Enemy_C")
      (`KismetArrayLibrary.Array_AddUnique` (`self.HittedActor`) _hitactor)))
  (for _array_element_2 (`self.HittedActor`)
    (if (!= (`self.Target`) _array_element_2)
      (`GameplayStatics.ApplyDamage` _array_element_2 (`self.AoeDamage`) null (`self.Instigator`))))
  (`GameplayStatics.SpawnEmitterAtLocation` "/Game/StarterContent/Particles/P_Explosion.P_Explosion" (`self.K2_GetActorLocation`) (struct) (`KismetMathLibrary.Conv_DoubleToVector` (/ (`self.AoeRadius`) 150.0)))
  (`self.K2_DetachFromActor` _missiletrail "KeepWorld" "KeepWorld" "KeepWorld")
  (`/Game/Blueprint/Turrets/Ammunation/BP_MissileTrail.Destruction` _missiletrail)
  (`GameplayStatics.PlaySoundAtLocation` "/Game/Audio/SFX/Turrets/Bombard/SC_MissileExplosion.SC_MissileExplosion" (`self.K2_GetActorLocation`) (struct) 1.0 1.0 0.0 null null null null)
  (`self.K2_DestroyActor`))

(fn `Initialize`
  (params (Damage :type "Float (double-precision)")))

(fn `UserConstructionScript`
  (set `ProjectileMovementComponent.HomingTargetComponent` (`Actor.RootComponent` (`self.Target`)) (`self.ProjectileMovement`)))