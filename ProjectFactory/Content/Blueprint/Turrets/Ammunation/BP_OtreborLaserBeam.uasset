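; Laser beam ammunition for the Otrebor turret, drawn with a Niagara effect scaled by a radius modifier.
; A visibility trace sets the beam length, stopping only at room actors, and a sphere trace along it damages the first robot found.
; The turret's destroy-ammo event removes the beam only early in its life.
; Otherwise, the effect finishing re-enables rotation on a BP_O_Aim instigator and destroys the beam.
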(event `OnSystemFinished_Event`
  (params (PSystem :type "NiagaraComponent Object Reference"))
  (bind _asbp_o_aim (cast `/Game/Blueprint/Turrets/OtreborTurrets/BP_O_Aim` (`self.Instigator`)))
  (`/Engine/EditorBlueprintResources/StandardMacros.IsValid` _asbp_o_aim
    (:`Is Valid`
      (set `/Game/Blueprint/Turrets/OtreborTurrets/BP_O_Aim.CanRotate` true _asbp_o_aim))
    (:`Is Not Valid`
      _))
  (`self.K2_DestroyActor`))

(event `self.ReceiveBeginPlay`
  (`AudioComponent.FadeIn` (`self.SpawnSound`) 0.5 1.0 0.0 "Linear")
  (`FXSystemComponent.SetFloatParameter` (`self.Niagara`) "ScaleMultiplier" (* (`self.BeamRadiusModifier`) 0.5))
  (bind _asbp_turret_base (cast `/Game/Blueprint/Turrets/BP_Turret_Base` (`self.Instigator`)))
  (add `/Game/Blueprint/Turrets/BP_Turret_Base.DestroyAmmo` _asbp_turret_base (delegate `DestroyAmmo`))
  (add `NiagaraComponent.OnSystemFinished` (`self.Niagara`) (delegate `OnSystemFinished_Event`)))

(event `DestroyAmmo`
  (if (< (`self.GetGameTimeSinceCreation`) 3.4)
    (`self.K2_DestroyActor`)))

(event `GetBeamDistance`
  (bind _returnvalue (`self.K2_GetActorLocation`))
  (bind _niagara (`self.Niagara`))
  (bind _outhit (`KismetSystemLibrary.LineTraceSingle` :`Start` _returnvalue :`End` (+ _returnvalue (* (`self.GetActorForwardVector`) (`self.MaxBeamDistance`))) :`TraceChannel` "TraceTypeQuery1" :`TraceColor` (struct :`R` 0.051397 :`G` 0.06834 :`B` 1.0 :`A` 1.0)))
  (bind (_bblockinghit _binitialoverlap _time _distance _location _impactpoint _normal _impactnormal _physmat _hitactor) (`GameplayStatics.BreakHitResult` _outhit))
  (if (`KismetSystemLibrary.DoesImplementInterface` _hitactor "/Game/Blueprint/Envirorment/Rooms/BI_Room.BI_Room_C")
    (`FXSystemComponent.SetVectorParameter` _niagara "BeamEnd" (`KismetMathLibrary.MakeVector` _distance))
    (set `self.BeamEndDistance` _distance)
    (else
      (`FXSystemComponent.SetVectorParameter` _niagara "BeamEnd" (`KismetMathLibrary.MakeVector` (`self.MaxBeamDistance`)))
      (set `self.BeamEndDistance` (`self.MaxBeamDistance`)))))

(event `DoDamage`
  (bind _returnvalue (`self.K2_GetActorLocation`))
  (`AudioComponent.FadeIn` (`self.DamageAudio`) 0.5 1.0 0.0 "Linear")
  (bind _outhits (`KismetSystemLibrary.SphereTraceMultiForObjects` _returnvalue (+ _returnvalue (* (`self.GetActorForwardVector`) (`self.BeamEndDistance`))) (`self.BaseBeamRadius`) (`|MakeArray` "ObjectTypeQuery3" :!type "EObjectTypeQuery Enum")))
  (for _array_element _outhits
    (bind (_bblockinghit _binitialoverlap _time _distance _location _impactpoint _normal _impactnormal _physmat _hitactor) (`GameplayStatics.BreakHitResult` _array_element))
    (if (`KismetSystemLibrary.DoesImplementInterface` _hitactor "/Game/Blueprint/Robot/Interfaces/BPI_Robot.BPI_Robot_C")
      (`GameplayStatics.ApplyDamage` _hitactor (`self.BulletDamage`) null (`self.Instigator`))
      (break))))

(fn `UserConstructionScript`)