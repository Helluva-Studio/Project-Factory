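; Farming turret that passively stores Essence, Gear or Steel over time until its tank is full.
; Tick drives charging, cooldown, health-widget bar, storage bobbing and a dynamic material showing fill and state.
; Interacting spawns pickups around the turret in a delayed loop, building a cooldown proportional to the amount released, during which charging stops.
; Also adjusts visuals per upgrade level and resumes interrupted spawning from a save.
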(event `self.ReceiveBeginPlay`
  (bind _currentlevel (`self.CurrentLevel`))
  (`parent.ReceiveBeginPlay`)
  (`SceneComponent.K2_SetRelativeLocation` (`self.NS_CdEffect`) (`KismetMathLibrary.MakeVector` 0.0 (select `int` _currentlevel :`0` 0.0 :`1` 16.5 :`2` 25.0 :`3` 25.0) (select `int` _currentlevel :`0` 0.0 :`1` 42.0 :`2` 57.0 :`3` 106.0)) false false))

(event `Charge`
  (if (`self.IsInCooldown`)
    (`MaterialInstanceDynamic.SetVectorParameterValue` (`self.GetChargeMaterial`) "BaseColor" (`self.CoolDownColor`))
    (else
      (`MaterialInstanceDynamic.SetVectorParameterValue` (`self.GetChargeMaterial`) "BaseColor" (`self.ChargeColor`))
      (if (`self.IsTankFull`)
        _
        (elif (not (`self.IsSpawningResource`))
          ;[1 1 1] Time Required To Charge 1 Resource
          (bind _output_get (set `self.ChargeValue` (+ (`GameplayStatics.GetWorldDeltaSeconds`) (`self.ChargeValue`))))
          (if (>= _output_get (`self.ChargeTimePerResource`))
            (`/Engine/EditorBlueprintResources/StandardMacros.IncrementInt` (`self.ResourceStored`)
              (:`  `
                (set `self.ChargeValue` 0.0)
                (if (`self.IsTankFull`)
                  (`MaterialInstanceDynamic.SetScalarParameterValue` (`self.GetChargeMaterial`) "TransitionValue" (`KismetMathLibrary.SafeDivide` (`KismetMathLibrary.Conv_IntToDouble` (`self.ResourceStored`)) (`KismetMathLibrary.Conv_IntToDouble` (`self.MaxResourceStored`))) :!label _label))))
            (else
              (goto _label))))))))

(event `self.ReceiveTick`
  (params (DeltaSeconds :type "Float (single-precision)"))
  (`parent.ReceiveTick` DeltaSeconds)
  (`|ExecutionSequence`
    (:`then_0`
      (`self.ManageTurretFunctioning`))
    (:`then_1`
      (`self.Charge`))
    (:`then_2`
      (`self.StorageFeedback`))))

(event `StorageFeedback`
  (`/Engine/EditorBlueprintResources/StandardMacros.IsValid` self
    (:`Is Valid`
      (if (not (`self.IsInCooldown`))
        (if (`self.IsSpawningResource`)
          (`MaterialInstanceDynamic.SetVectorParameterValue` (`self.GetChargeMaterial`) "BaseColor" (`self.CdChargeColor`))
          (else
            (`MaterialInstanceDynamic.SetVectorParameterValue` (`self.GetChargeMaterial`) "BaseColor" (`self.ChargeColor`))))
        (`SceneComponent.K2_AddWorldOffset` (`self.Storage`) (`KismetMathLibrary.MakeVector` 0.0 0.0 (/ (`KismetMathLibrary.DegSin` (* (`self.GetGameTimeSinceCreation`) 200.0)) 20.0)) false false)
        (`SceneComponent.K2_AddWorldRotation` (`self.Storage`) (struct :`Yaw` 2.0) false false)))))

(event `SpawnResource`
  (bind (_returnvalue_x _returnvalue_y) (`KismetMathLibrary.BreakVector` (`KismetMathLibrary.RandomUnitVector`)))
  (bind (_returnvalue_x_2 _returnvalue_y_2) (`KismetMathLibrary.BreakVector` (* (`KismetMathLibrary.Normal` (`KismetMathLibrary.MakeVector` _returnvalue_x _returnvalue_y)) (* (`self.SpawnDistanceFromTurret`) (`KismetMathLibrary.RandomFloatInRange` 0.85 1.0)))))
  (switch `/Game/Blueprint/Resources/E_Resources` (`self.TypeOfResource`)
    (:`NewEnumerator0`
      (set `self.ResourceToSpawn` "/Game/Blueprint/Resources/BP_Essence.BP_Essence_C"))
    (:`NewEnumerator1`
      (set `self.ResourceToSpawn` "/Game/Blueprint/Resources/BP_Gears.BP_Gears_C"))
    (:`NewEnumerator2`
      (set `self.ResourceToSpawn` "/Game/Blueprint/Resources/BP_Steel.BP_Steel_C")))
  (`|SpawnActorFromClass` (`self.ResourceToSpawn`) (`KismetMathLibrary.MakeTransform` (+ (`self.K2_GetActorLocation`) (`KismetMathLibrary.MakeVector` _returnvalue_x_2 _returnvalue_y_2 50.0))) "AlwaysSpawn" "MultiplyWithRoot" null (`self.ResourceValue`) (`|MakeArray` self :!type "Actor Object Reference") null))

(event `/Game/Blueprint/Turrets/Interfaces/BI_Interactable.Interact`
  (set `self.IsSpawningResource` true)
  (set `self.MaxCdTime` (* (`self.ResourceStored`) (`self.CdTimePerResource`)))
  (bind _index (`/Game/Blueprint/BP_MacroLibrary_Actor.ForLoopWithDelay` 1 (`self.ResourceStored`) (`self.TimeBetweenResourceSpawn`))
    (:`Loop Body`
      (`self.SpawnResource`)
      (set `self.CdTime` (* (`self.CdTimePerResource`) _index))
      (`MaterialInstanceDynamic.SetScalarParameterValue` (`self.GetChargeMaterial`) "TransitionValue" (`KismetMathLibrary.SafeDivide` (- (`self.ResourceStored`) _index) (`KismetMathLibrary.Conv_IntToDouble` (`self.MaxResourceStored`)))))
    (:`Completed`
      (set `self.IsInCooldown` true)
      (set `self.IsSpawningResource` false)
      (set `self.ResourceStored` 0))))

(event `/Game/Blueprint/InteractionArea/BPI_Focusable.ToggleFocus`
  (params (Focus :type Boolean))
  (for _array_element (`self.MeshesToOutline`)
    (`PrimitiveComponent.SetRenderCustomDepth` _array_element (and Focus (not (`self.IsInCooldown`)) (not (`self.IsSpawningResource`))))))

(fn `CanInteract`
  (returns (CanInteract :type Boolean))
  (return (and (not (`self.IsInCooldown`)) (not (`self.IsSpawningResource`)) (`self.IsActorTickEnabled`))))

(fn `GetChargeMaterial`
  (returns (`AsMaterial Instance Dynamic` :type "MaterialInstanceDynamic Object Reference"))
  (bind _asmaterial_instance_dynamic (cast `MaterialInstanceDynamic` (`PrimitiveComponent.GetMaterial` (`self.Body`) 1)))
  (return _asmaterial_instance_dynamic))

(fn `GetCost`
  (returns (GetCost :type "Float (double-precision)"))
  (return 0.0))

(fn `GetInteractImage`
  (returns (Image :type "Texture Object Reference"))
  (return "/Game/2DImage/FARM_Interact.FARM_Interact"))

(fn `GetInteractMessage`
  (returns (InteractMessage :type Text) (Image :type "Texture Object Reference"))
  (return "" null))

(fn `InitializeFromSave`
  (params (ResourceStored :type Integer) (IsSpawningResource :type Boolean) (CdTime :type "Float (double-precision)"))
  (set `self.ResourceStored` ResourceStored)
  (bind _output_get (set `self.IsSpawningResource` IsSpawningResource))
  (set `self.CdTime` CdTime)
  (if _output_get
    (`/Game/Blueprint/Turrets/Interfaces/BI_Interactable.Interact`)))

(fn `IsTankFull`
  (returns (IsFull :type Boolean))
  (return (>= (`self.ResourceStored`) (`self.MaxResourceStored`))))

(fn `ManageTurretFunctioning`
  (bind _cdtime (`self.CdTime`))
  (`/Engine/EditorBlueprintResources/StandardMacros.IsValid` self
    (:`Is Valid`
      (if (`self.IsSpawningResource`)
        (bind _aswb_turret_health_1 (cast `/Game/HUD/WB_TurretHealth1` (`WidgetComponent.GetWidget` (`self.Widget`))))
        (set `Widget.RenderOpacity` 1.0 (`/Game/HUD/WB_TurretHealth1.CdBar` _aswb_turret_health_1))
        (bind _aswb_turret_health_1_2 (cast `/Game/HUD/WB_TurretHealth1` (`WidgetComponent.GetWidget` (`self.Widget`))))
        (set `/Game/HUD/WB_TurretHealth1.WB_CdColor` (struct :`R` 1.0 :`G` 0.5 :`A` 1.0) _aswb_turret_health_1_2)
        (bind _aswb_turret_health_1_3 (cast `/Game/HUD/WB_TurretHealth1` (`WidgetComponent.GetWidget` (`self.Widget`))))
        (set `/Game/HUD/WB_TurretHealth1.WB_MaxCdTime` (`self.MaxCdTime`) _aswb_turret_health_1_3)
        (set `/Game/HUD/WB_TurretHealth1.WB_CurrentCdTime` (`self.CdTime`) _aswb_turret_health_1_3)
        (elif (`self.IsInCooldown`)
          (`ActorComponent.Activate` (`self.NS_CdEffect`) false)
          (bind _aswb_turret_health_1_4 (cast `/Game/HUD/WB_TurretHealth1` (`WidgetComponent.GetWidget` (`self.Widget`))))
          (set `/Game/HUD/WB_TurretHealth1.WB_CdColor` (struct :`R` 1.0 :`A` 1.0) _aswb_turret_health_1_4)
          (set `self.CdTime` (- (`self.CdTime`) (`GameplayStatics.GetWorldDeltaSeconds`)))
          (bind _aswb_turret_health_1_5 (cast `/Game/HUD/WB_TurretHealth1` (`WidgetComponent.GetWidget` (`self.Widget`))))
          (set `/Game/HUD/WB_TurretHealth1.WB_CurrentCdTime` _cdtime _aswb_turret_health_1_5)
          (if (<= _cdtime 0.0)
            (set `self.IsInCooldown` false))
          (else
            (`ActorComponent.Deactivate` (`self.NS_CdEffect`))
            (bind _aswb_turret_health_1_6 (cast `/Game/HUD/WB_TurretHealth1` (`WidgetComponent.GetWidget` (`self.Widget`))))
            (set `Widget.RenderOpacity` 0.0 (`/Game/HUD/WB_TurretHealth1.CdBar` _aswb_turret_health_1_6))))))))

(fn `UpdateGraphicByLevel`
  (params (Level :type Integer))
  (bind _currentlevel (`self.CurrentLevel`))
  (bind _currentlevel_2 (`self.CurrentLevel`))
  (bind _returnvalue (`KismetMathLibrary.Conv_IntToDouble` (`self.CurrentLevel`)))
  (bind _returnvalue_2 (`KismetMathLibrary.Conv_IntToDouble` _currentlevel))
  (bind _returnvalue_3 (* _currentlevel_2 1.5))
  (bind _returnvalue_4 (* _returnvalue 2.0))
  (`/Engine/EditorBlueprintResources/StandardMacros.IsValid` self
    (:`Is Valid`
      (switch `int` Level
        (:`1`
          (`SceneComponent.SetRelativeScale3D` (`self.Scene`) (`KismetMathLibrary.MakeVector` _returnvalue_4 _returnvalue_4 _returnvalue))
          (`SceneComponent.K2_SetRelativeLocation` (`self.HandlerLR`) (0.0 0.0 -25.0) false false)
          (`SceneComponent.SetVisibility` (`self.Neck`) false false))
        (:`2`
          (`SceneComponent.SetRelativeScale3D` (`self.Scene`) (`KismetMathLibrary.MakeVector` _returnvalue_3 _returnvalue_3 (* _currentlevel_2 0.75)))
          (`SceneComponent.K2_SetRelativeLocation` (`self.HandlerLR`) (0.0 0.0 -25.0) false false)
          (`SceneComponent.SetVisibility` (`self.Neck`) false false))
        (:`3`
          (`SceneComponent.SetRelativeScale3D` (`self.Scene`) (`KismetMathLibrary.MakeVector` _returnvalue_2 _returnvalue_2 (* _currentlevel 0.5)))
          (`SceneComponent.K2_SetRelativeLocation` (`self.HandlerLR`) (0.0 0.0 7.5) false false)
          (`SceneComponent.SetVisibility` (`self.Neck`) true false))))))

(fn `UserConstructionScript`
  (`parent.UserConstructionScript`))

(fn `WhichInteraction`
  (returns (TypeInteraction :type "/Game/Blueprint/Enum/EInteractable Enum"))
  (return "NewEnumerator0"))