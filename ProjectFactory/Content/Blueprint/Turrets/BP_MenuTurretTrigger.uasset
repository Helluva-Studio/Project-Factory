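; Menu variant of a turret trigger that displays a preview of a chosen turret at its own location.
; SpawnPreview destroys any existing preview, then spawns the actor class mapped to TurretToShow in PreviewActors, at a fixed level and marked buildable.
; The turret type comes from the chosen turret's class defaults, and IsUnlocked drives both the tutorial flag and the SetPreview call.
; The GetTurretSelected override is empty, with its parent calls left unconnected.
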(event `self.SpawnPreview`
  (bind _previewactors (`self.PreviewActors`))
  (bind _turrettoshow (`self.TurretToShow`))
  (bind _turretpreviewed (`self.TurretPreviewed`))
  (`/Engine/EditorBlueprintResources/StandardMacros.IsValid` _turretpreviewed
    (:`Is Valid`
      (`self.K2_DestroyActor` _turretpreviewed))
    (:`Is Not Valid`
      _))
  (bind _keys (`BlueprintMapLibrary.Map_Keys` _previewactors))
  (bind _values (`BlueprintMapLibrary.Map_Values` _previewactors))
  (bind _returnvalue (`|SpawnActorFromClass` (`|GetArrayItem` _values (`KismetArrayLibrary.Array_Find` _keys _turrettoshow)) (`KismetMathLibrary.MakeTransform` (`self.K2_GetActorLocation`)) "AlwaysSpawn" "MultiplyWithRoot" null 3 (`.TurretType` (defaults `Object` _turrettoshow)) true (`self.IsUnlocked`) null))
  (bind _output_get (set `self.TurretPreviewed` _returnvalue))
  (`/Game/Blueprint/Turrets/TurretFeature/TurretTrigger/TurretPreview/BP_TurretPreview.SetPreview` _output_get (`self.IsUnlocked`)))

(fn `GetTurretSelected`
  (returns (HaveResourceToBuild :type Boolean) (TurretSelected :type "/Game/Blueprint/Turrets/TurretFeature/TurretTrigger/TurretPreview/BP_TurretPreview Class Reference") (Level :type Integer) (`Turret Type` :type "/Game/Blueprint/Turrets/TurretGetter/E_TurretType Enum")))

(fn `UserConstructionScript`
  (`parent.UserConstructionScript`))