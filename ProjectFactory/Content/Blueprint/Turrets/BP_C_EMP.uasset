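; BP_C_EMP is an EMP turret that fires crowd-control stun ammo over an area of effect, built on a parent turret class.
; InitializeTurret loads health, timers, radius and stun settings from a per-level data table row, and SpawnAmmo passes the crowd-control values to the spawned ammo.
; While off cooldown, Tick spins three rings and bobs them on sine waves.
; UpdateGraphicByLevel reveals more rings at higher levels.
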(event `self.ReceiveTick`
  (params (DeltaSeconds :type "Float (single-precision)"))
  (`parent.ReceiveTick` DeltaSeconds)
  (if (not (`self.IsInCooldown`))
    (`self.RingRotation`)))

(event `self.SpawnAmmo`
  (`parent.SpawnAmmo`)
  (`/Engine/EditorBlueprintResources/StandardMacros.IsValid` (`self.CcAmmo`)
    (:`Is Valid`
      (message `/Game/Blueprint/Turrets/Interfaces/BPI_TurretCcAmmo.InitializeStunAmmo` (`self.CcAmmo`) (`self.CanHitPlayer`) (`self.TypeOfCc`) (`self.TypeOfAoe`) (`self.MaxDistance(Cone)/MaxRadius(Sphere)`) (`self.StunDuration`) (`self.StunTick`)))))

(event `RingRotation`
  (`/Engine/EditorBlueprintResources/StandardMacros.IsValid` self
    (:`Is Valid`
      (`SceneComponent.K2_AddWorldRotation` (`self.BigRing`) (struct :`Yaw` 1.0) false false)
      (`SceneComponent.K2_AddWorldRotation` (`self.MediumRing`) (struct :`Yaw` 1.0) false false)
      (`SceneComponent.K2_AddWorldRotation` (`self.SmallRing`) (struct :`Yaw` -1.0) false false)
      (`SceneComponent.K2_AddWorldOffset` (`self.BigRing`) (`KismetMathLibrary.MakeVector` 0.0 0.0 (/ (`KismetMathLibrary.DegSin` (* (`self.GetGameTimeSinceCreation`) 200.0)) 20.0)) false false)
      (`SceneComponent.K2_AddWorldOffset` (`self.SmallRing`) (`KismetMathLibrary.MakeVector` 0.0 0.0 (/ (`KismetMathLibrary.DegSin` (* (`self.GetGameTimeSinceCreation`) 200.0)) 30.0)) false false)
      (`SceneComponent.K2_AddWorldOffset` (`self.MediumRing`) (`KismetMathLibrary.MakeVector` 0.0 0.0 (/ (`KismetMathLibrary.DegSin` (* (`self.GetGameTimeSinceCreation`) 200.0)) 10.0)) false false))))

(fn `InitializeTurret`
  (`parent.InitializeTurret`)
  (bind _returnvalue (`|GetDataTableRow` "/Game/Blueprint/Turrets/TurretFeature/Leveling/TurretSpecificDataTable/DT_C_TurretEmp.DT_C_TurretEmp" (`KismetStringLibrary.Conv_StringToName` (`KismetStringLibrary.Conv_IntToString` (`self.CurrentLevel`))))
    (:`then`
      (bind (_maxhealth _maxactivitytime _maxcdtime _baseaoetype _baseradius _radiuspercentagemodifier _basecctype _stuntick _stunduration) (break `/Game/Blueprint/Turrets/TurretFeature/Leveling/TurretStructs/S_C_TurretEmpStats` _returnvalue))
      (bind _output_get (set `self.MaxHealth` _maxhealth))
      (set `self.CurrentHealth` _output_get)
      (set `self.MaxActivityTime(NoFarm)` _maxactivitytime)
      (set `self.MaxCdTime` _maxcdtime)
      (set `self.TypeOfAoe` _baseaoetype)
      (bind _output_get_2 (set `self.MaxDistance(Cone)/MaxRadius(Sphere)` (+ _baseradius (* _baseradius (/ _radiuspercentagemodifier 100.0)))))
      (set `self.BaseDistance(Cone)/BaseRadius(Sphere)` _output_get_2)
      (set `self.TypeOfCc` _basecctype)
      (set `self.StunTick` _stuntick)
      (set `self.StunDuration` _stunduration))))

(fn `UpdateGraphicByLevel`
  (params (Level :type Integer))
  (`/Engine/EditorBlueprintResources/StandardMacros.IsValid` self
    (:`Is Valid`
      (switch `int` Level
        (:`1`
          (`SceneComponent.SetVisibility` (`self.MediumRing`) false false)
          (`SceneComponent.SetVisibility` (`self.BigRing`) false false))
        (:`2`
          (`SceneComponent.SetVisibility` (`self.MediumRing`) true false)
          (`SceneComponent.SetVisibility` (`self.BigRing`) false false))
        (:`3`
          (`SceneComponent.SetVisibility` (`self.MediumRing`) true false)
          (`SceneComponent.SetVisibility` (`self.BigRing`) true false))))))

(fn `UserConstructionScript`
  (`parent.UserConstructionScript`))