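; BP_F_Steel is the steel farm turret, a resource-producing building derived from a parent turret Blueprint.
; InitializeTurret loads the DT_F_FarmSteel row matching CurrentLevel to set health, charge and cooldown times, storage cap, spawn rate and distance, and resource type and value.
; Interaction overrides return a fixed interaction type, zero cost and the Rotate image.
; Production logic is not in this file, which only supplies data and overrides.
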(fn `GetCost`
  (returns (GetCost :type "Float (double-precision)"))
  (return 0.0))

(fn `GetInteractImage`
  (returns (Image :type "Texture Object Reference"))
  (return "/Game/2DImage/Rotate.Rotate"))

(fn `InitializeTurret`
  (bind _returnvalue (`|GetDataTableRow` "/Game/Blueprint/Turrets/TurretFeature/Leveling/TurretSpecificDataTable/DT_F_FarmSteel.DT_F_FarmSteel" (`KismetStringLibrary.Conv_StringToName` (`KismetStringLibrary.Conv_IntToString` (`self.CurrentLevel`))))
    (:`then`
      (bind (_maxhealth _chargetimeperresource _cdtimeperresource _maxresourcestored _resourcevalue _baseresourcespawnrate _baseresourcedistancefromturret _typeofresource) (break `/Game/Blueprint/Turrets/TurretFeature/Leveling/TurretStructs/S_F_Farm` _returnvalue))
      (bind _output_get (set `self.MaxHealth` _maxhealth))
      (set `self.CurrentHealth` _output_get)
      (set `self.ChargeTimePerResource` _chargetimeperresource)
      (set `self.CdTimePerResource` _cdtimeperresource)
      (set `self.MaxResourceStored` _maxresourcestored)
      (set `self.TimeBetweenResourceSpawn` _baseresourcespawnrate)
      (set `self.SpawnDistanceFromTurret` _baseresourcedistancefromturret)
      (set `self.TypeOfResource` _typeofresource)
      (set `self.ResourceValue` _resourcevalue))))

(fn `UserConstructionScript`
  (`parent.UserConstructionScript`))

(fn `WhichInteraction`
  (returns (TypeInteraction :type "/Game/Blueprint/Enum/EInteractable Enum"))
  (return "NewEnumerator0"))