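; BP_C_Slow is a crowd-control turret child Blueprint whose ammo applies a slow effect over an area.
; InitializeTurret reads the DT_C_TurretSlow row for the current level to set health, timings, CC and AoE types, modified radius and slow strength.
; SpawnAmmo runs the parent spawn, then passes those effect settings to the spawned CcAmmo.
; UpdateGraphicByLevel reveals additional ice components at higher levels.
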(event `self.SpawnAmmo`
  (`parent.SpawnAmmo`)
  (`/Engine/EditorBlueprintResources/StandardMacros.IsValid` (`self.CcAmmo`)
    (:`Is Valid`
      (message `/Game/Blueprint/Turrets/Interfaces/BPI_TurretCcAmmo.InitializeSlowAmmo` (`self.CcAmmo`) (`self.CanHitPlayer`) (`self.TypeOfCc`) (`self.TypeOfAoe`) (`self.MaxDistance(Cone)/MaxRadius(Sphere)`) (`self.SlowEffect`)))))

(fn `InitializeTurret`
  (`parent.InitializeTurret`)
  (bind _returnvalue (`|GetDataTableRow` "/Game/Blueprint/Turrets/TurretFeature/Leveling/TurretSpecificDataTable/DT_C_TurretSlow.DT_C_TurretSlow" (`KismetStringLibrary.Conv_StringToName` (`KismetStringLibrary.Conv_IntToString` (`self.CurrentLevelh`))))
    (:`then`
      (bind (_maxhealth _maxactivitytime _maxcdtime _baseaoetype _baseradius _radiuspercentagemodifier _basecctype _sloweffectpercentage) (break `/Game/Blueprint/Turrets/TurretFeature/Leveling/TurretStructs/S_C_TurretSlowStats` _returnvalue))
      (bind _output_get (set `self.MaxHealth` _maxhealth))
      (set `self.CurrentHealth` _output_get)
      (set `self.MaxActivityTime(NoFarm)` _maxactivitytime)
      (set `self.MaxCdTime` _maxcdtime)
      (set `self.TypeOfAoe` _baseaoetype)
      (bind _output_get_2 (set `self.BaseDistance(Cone)/BaseRadius(Sphere)` _baseradius))
      (set `self.MaxDistance(Cone)/MaxRadius(Sphere)` (+ _output_get_2 (* _output_get_2 (/ _radiuspercentagemodifier 100.0))))
      (set `self.TypeOfCc` _basecctype)
      (set `self.SlowEffect` _sloweffectpercentage))))

(fn `UpdateGraphicByLevel`
  (params (Level :type Integer))
  (`/Engine/EditorBlueprintResources/StandardMacros.IsValid` self
    (:`Is Valid`
      (switch `int` Level
        (:`1`
          (`SceneComponent.SetVisibility` (`self.Ice2`) false false)
          (`SceneComponent.SetVisibility` (`self.Ice3`) false false))
        (:`2`
          (`SceneComponent.SetVisibility` (`self.Ice2`) true false)
          (`SceneComponent.SetVisibility` (`self.Ice3`) false false))
        (:`3`
          (`SceneComponent.SetVisibility` (`self.Ice2`) true false)
          (`SceneComponent.SetVisibility` (`self.Ice3`) true false))))))

(fn `UserConstructionScript`
  (`parent.UserConstructionScript`))