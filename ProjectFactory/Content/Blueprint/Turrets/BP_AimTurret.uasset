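; Auto-aiming turret base that patrols at random pitch-limited directions until it spots a BP_BaseEnemy, then turns to track it.
; PawnSensing acquires targets through line traces that ignore the player, and resets on blocked sight or excessive distance.
; Tick drives patrol and aim by lerping separate yaw and pitch handlers.
; Once the aim lerp passes the Accuracy threshold, CanShoot gates an empty Shoot event; nothing here sets that flag true.
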(event `self.ReceiveBeginPlay`
  (`parent.ReceiveBeginPlay`)
  (`self.InitializeTurretSight` 0.0))

(event `self.ReceiveTick`
  (params (DeltaSeconds :type "Float (single-precision)"))
  (bind (_relativerotation_roll _relativerotation_pitch _relativerotation_yaw) (`KismetMathLibrary.BreakRotator` (`SceneComponent.RelativeRotation` (`self.HandlerLR`))))
  (bind (_relativerotation_roll_2 _relativerotation_pitch_2 _relativerotation_yaw_2) (`KismetMathLibrary.BreakRotator` (`SceneComponent.RelativeRotation` (`self.HandlerLR`))))
  (bind (_relativerotation_roll_3 _relativerotation_pitch_3) (`KismetMathLibrary.BreakRotator` (`SceneComponent.RelativeRotation` (`self.HandlerUD`))))
  (bind (_relativerotation_roll_4 _relativerotation_pitch_4) (`KismetMathLibrary.BreakRotator` (`SceneComponent.RelativeRotation` (`self.HandlerUD`))))
  (`parent.ReceiveTick` DeltaSeconds)
  (if (`self.HasTarget`)
    (`/Engine/EditorBlueprintResources/StandardMacros.IsValid` (`self.Target`)
      (:`Is Valid`
        (if (`self.TargetAimed`)
          (if (`self.AimTaken`)
            (if (`self.CanShoot`)
              (set `self.CanShoot` false)
              (`self.Shoot`)
              (else
                (`self.TakeAim`)))
            (else
              (`self.TakeAim`)))
          (else
            (set `self.TargetAimed` true)
            (set `self.AimRotationLerp` 0.0)
            (set `self.InitialDirection` _relativerotation_yaw_2)
            (set `self.InitialAltitude` _relativerotation_pitch_4))))
      (:`Is Not Valid`
        (`self.ResetTurret`)))
    (elif (`self.NotInPatrol`)
      (set `self.NotInPatrol` false)
      (set `self.PatrolRotationLerp` 0.0)
      (set `self.InitialDirection` _relativerotation_yaw)
      (set `self.InitialAltitude` _relativerotation_pitch_3)
      (bind _output_get (set `self.NextPatrolLocation` (`self.GetNextPatrolPosition` (`SceneComponent.K2_GetComponentLocation` (`self.HandlerUD`)) (`self.Max Lower Angle`) (`self.Max Upper Angle`))))
      (else
        (`self.Patrol`)))))

(event `ResetTurret`
  (set `self.NotInPatrol` false)
  (set `self.PatrolRotationLerp` 0.0)
  (set `self.HasTarget` false)
  (set `self.TargetAimed` false)
  (set `self.AimTaken` false)
  (set `self.CanShoot` false)
  (set `self.AimRotationLerp` 0.0)
  (set `self.Target` null))

(event `Shoot`)

(event `self.PawnSensing.OnSeePawn`
  (params (Pawn :type "Pawn Object Reference"))
  ;[1 1 1] Targetting
  (`/Engine/EditorBlueprintResources/StandardMacros.IsValid` (`self.Target`)
    (:`Is Valid`
      (`|ExecutionSequence`
        (:`then_0`
          (bind _outhit (`KismetSystemLibrary.LineTraceSingleForObjects` (`SceneComponent.K2_GetComponentLocation` (`self.HandlerUD`)) (`SceneComponent.K2_GetComponentLocation` (`Actor.RootComponent` (`self.Target`))) (`|MakeArray` "ObjectTypeQuery2" "ObjectTypeQuery1" "ObjectTypeQuery3" :!type "EObjectTypeQuery Enum") false (`|MakeArray` (`GameplayStatics.GetPlayerPawn` 0) :!type "Actor Object Reference")))
          (bind (_bblockinghit _binitialoverlap _time _distance _location _impactpoint _normal _impactnormal _physmat _hitactor) (`GameplayStatics.BreakHitResult` _outhit))
          (if (!= (`self.Target`) _hitactor)
            (if (not (`KismetSystemLibrary.DoesImplementInterface` _hitactor "/Game/Blueprint/Enemies/Interfaces/BPI_Enemy.BPI_Enemy_C"))
              (`self.ResetTurret`))))
        (:`then_1`
          (`/Engine/EditorBlueprintResources/StandardMacros.IsValid` (`self.Target`)
            (:`Is Valid`
              (if (> (`KismetMathLibrary.Vector_Distance` (`SceneComponent.K2_GetComponentLocation` (`self.HandlerUD`)) (`self.K2_GetActorLocation` (`self.Target`))) (`self.Max Target Distance`))
                (`self.ResetTurret`)))
            (:`Is Not Valid`
              (`self.ResetTurret`))))))
    (:`Is Not Valid`
      (bind _asbp_base_enemy (cast `/Game/Blueprint/Enemies/BP_BaseEnemy` Pawn))
      (bind _outhit_2 (`KismetSystemLibrary.LineTraceSingleForObjects` (`SceneComponent.K2_GetComponentLocation` (`self.HandlerUD`)) (`SceneComponent.K2_GetComponentLocation` (`Actor.RootComponent` _asbp_base_enemy)) (`|MakeArray` "ObjectTypeQuery2" "ObjectTypeQuery1" "ObjectTypeQuery3" :!type "EObjectTypeQuery Enum") false (`|MakeArray` (`GameplayStatics.GetPlayerPawn` 0) :!type "Actor Object Reference")))
      (if (== _asbp_base_enemy (`.HitActor` (`GameplayStatics.BreakHitResult` _outhit_2)))
        (if (not (`self.HasTarget`))
          (set `self.Target` _asbp_base_enemy)
          (set `self.HasTarget` true))))))

(event `Patrol`
  (bind (_returnvalue_roll _returnvalue_pitch) (`KismetMathLibrary.BreakRotator` (`KismetMathLibrary.FindLookAtRotation` (`SceneComponent.K2_GetComponentLocation` (`self.HandlerUD`)) (`self.NextPatrolLocation`))))
  (bind (_returnvalue_roll_2 _returnvalue_pitch_2 _returnvalue_yaw) (`KismetMathLibrary.BreakRotator` (`KismetMathLibrary.FindLookAtRotation` (`SceneComponent.K2_GetComponentLocation` (`self.HandlerLR`)) (`self.NextPatrolLocation`))))
  ;[0.4333 1 0.6597] Patrol
  (set `self.PatrolRotationLerp` (`KismetMathLibrary.FClamp` (+ (`self.PatrolRotationLerp`) (* 0.1 (`self.PatrolRotationSpeed`)))))
  (`/Engine/EditorBlueprintResources/StandardMacros.IsValid` self
    (:`Is Valid`
      (`SceneComponent.K2_SetRelativeRotation` (`self.HandlerLR`) (`KismetMathLibrary.MakeRotator` 0.0 0.0 (`KismetMathLibrary.Lerp` (`self.InitialDirection`) (* _returnvalue_yaw -1.0) (`self.PatrolRotationLerp`))) false false)
      (`/Engine/EditorBlueprintResources/StandardMacros.IsValid` self
        (:`Is Valid`
          (`SceneComponent.K2_SetRelativeRotation` (`self.HandlerUD`) (`KismetMathLibrary.MakeRotator` 0.0 (`KismetMathLibrary.Lerp` (`self.InitialAltitude`) _returnvalue_pitch (`self.PatrolRotationLerp`))) false false)
          (if (>= (`self.PatrolRotationLerp`) 1.0)
            (`KismetSystemLibrary.Delay` (`self.TimeBetweenNextPatrol`))
            (set `self.NotInPatrol` true)))))))

(event `TakeAim`
  (bind (_returnvalue_roll _returnvalue_pitch) (`KismetMathLibrary.BreakRotator` (`KismetMathLibrary.FindLookAtRotation` (`SceneComponent.K2_GetComponentLocation` (`self.HandlerUD`)) (`self.K2_GetActorLocation` (`self.Target`)))))
  (bind (_returnvalue_roll_2 _returnvalue_pitch_2 _returnvalue_yaw) (`KismetMathLibrary.BreakRotator` (`KismetMathLibrary.FindLookAtRotation` (`SceneComponent.K2_GetComponentLocation` (`self.HandlerLR`)) (`self.K2_GetActorLocation` (`self.Target`)))))
  ;[1 0.5673 0.4162] Aim
  (set `self.AimRotationLerp` (`KismetMathLibrary.FClamp` (+ (`self.AimRotationLerp`) (* 0.1 (`self.Aim Rotation Speed`)))))
  (`/Engine/EditorBlueprintResources/StandardMacros.IsValid` self
    (:`Is Valid`
      (`SceneComponent.K2_SetRelativeRotation` (`self.HandlerLR`) (`KismetMathLibrary.RLerp` (`KismetMathLibrary.MakeRotator` 0.0 0.0 (`self.InitialDirection`)) (`KismetMathLibrary.MakeRotator` 0.0 0.0 (+ _returnvalue_yaw 180.0)) (`self.AimRotationLerp`) true) false false)
      (`/Engine/EditorBlueprintResources/StandardMacros.IsValid` self
        (:`Is Valid`
          (`SceneComponent.K2_SetRelativeRotation` (`self.HandlerUD`) (`KismetMathLibrary.MakeRotator` 0.0 (`KismetMathLibrary.Lerp` (`self.InitialAltitude`) _returnvalue_pitch (`self.AimRotationLerp`))) false false)
          (if (>= (`self.AimRotationLerp`) (/ (`self.Accuracy%`) 100.0))
            (set `self.AimTaken` true)))))))

(fn `GetNextPatrolPosition`
  (params (CenterPosition :type "Vector Structure") (MaxLowerAngle :type "Float (double-precision)") (MaxUpperAngle :type "Float (double-precision)"))
  (returns (TargetPosition :type "Vector Structure"))
  (locals (Angle :type "Float (double-precision)") (RandomX :type "Float (double-precision)") (RandomY :type "Float (double-precision)"))
  (bind (_returnvalue_x _returnvalue_y) (`KismetMathLibrary.BreakVector` (`KismetMathLibrary.RandomUnitVector`)))
  (set `local.Angle` (`KismetMathLibrary.RandomFloatInRange` (* MaxLowerAngle -1.0) MaxUpperAngle))
  (set `local.RandomX` _returnvalue_x)
  (set `local.RandomY` _returnvalue_y)
  (return (+ CenterPosition (* (`KismetMathLibrary.Normal` (`KismetMathLibrary.MakeVector` (`local.RandomX`) (`local.RandomY`) (`KismetMathLibrary.SelectFloat` (* (`KismetMathLibrary.Sqrt` (+ (`KismetMathLibrary.MultiplyMultiply_FloatFloat` (`local.RandomX`) 2.0) (`KismetMathLibrary.MultiplyMultiply_FloatFloat` (`local.RandomY`) 2.0))) (`KismetMathLibrary.DegTan` (`local.Angle`))) (* (`KismetMathLibrary.Sqrt` (+ (`KismetMathLibrary.MultiplyMultiply_FloatFloat` (`local.RandomX`) 2.0) (`KismetMathLibrary.MultiplyMultiply_FloatFloat` (`local.RandomY`) 2.0))) (`KismetMathLibrary.DegTan` (`local.Angle`))) (`KismetMathLibrary.RandomBool`)))) 100.0))))

(fn `InitializeTurretSight`
  (params (MaxTargetDistance :type "Float (double-precision)") (PawnSensing :type "PawnSensingComponent Object Reference"))
  (set `PawnSensingComponent.SightRadius` MaxTargetDistance PawnSensing)
  (set `PawnSensingComponent.HearingThreshold` MaxTargetDistance PawnSensing)
  (set `PawnSensingComponent.LOSHearingThreshold` MaxTargetDistance PawnSensing))

(fn `UserConstructionScript`
  (`parent.UserConstructionScript`))