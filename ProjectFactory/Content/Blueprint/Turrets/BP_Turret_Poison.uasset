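; BP_Turret_Poison is a poison turret Blueprint that defers BeginPlay, Tick and construction to its parent class.
; Focus toggles custom depth rendering on MeshesToOutline to drive an outline highlight.
; Its interaction functions always allow interaction, report zero cost and return the first interaction type.
; LevelUp switches on level but has no behavior wired, and no poison-specific logic appears in these graphs.
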(event `self.ReceiveBeginPlay`
  (`parent.ReceiveBeginPlay`))

(event `self.ReceiveTick`
  (params (DeltaSeconds :type "Float (single-precision)"))
  (`parent.ReceiveTick` DeltaSeconds))

(event `self.Focus`
  (params (IsFocused :type Boolean))
  (for _array_element (`self.MeshesToOutline`)
    (`PrimitiveComponent.SetRenderCustomDepth` _array_element IsFocused)))

(event `self.LevelUp`
  (params (Level :type Integer))
  (`/Engine/EditorBlueprintResources/StandardMacros.IsValid` self
    (:`Is Valid`
      (switch `int` Level))))

(fn `CanInteract`
  (returns (CanInteract :type Boolean))
  (return true))

(fn `GetCost`
  (returns (GetCost :type "Float (double-precision)"))
  (return 0.0))

(fn `UserConstructionScript`
  (`parent.UserConstructionScript`))

(fn `WhichInteraction`
  (returns (TypeInteraction :type "/Game/Blueprint/Enum/EInteractable Enum"))
  (return "NewEnumerator0"))