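; BP_H_Hazard is a hazard in the turret family that produces a flame, poison or shock AoE, chosen by its damage type.
; SpawnAmmo spawns the matching AoE actor at Center, attaches it there and stores it as DamageAmmo.
; The parent's cooldown hooks toggle the effect: cooldown start destroys it and cooldown end respawns it if absent.
; Interaction overrides return empty defaults and zero cost.
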(event `self.ReceiveBeginPlay`
  (`parent.ReceiveBeginPlay`))

(event `self.ReceiveTick`
  (params (DeltaSeconds :type "Float (single-precision)"))
  (`parent.ReceiveTick` DeltaSeconds))

(event `self.SpawnAmmo`
  (switch `/Game/Blueprint/Interfaces/E_DamageType` (`self.D_TypeOfDamage`)
    (:`NewEnumerator1`
      (set `self.DamageAmmoToSpawn` "/Game/Blueprint/Turrets/TurretFeature/Aoe/BP_AoeFlame.BP_AoeFlame_C"))
    (:`NewEnumerator2`
      (set `self.DamageAmmoToSpawn` "/Game/Blueprint/Turrets/TurretFeature/Aoe/BP_AoePoison.BP_AoePoison_C"))
    (:`NewEnumerator3`
      (set `self.DamageAmmoToSpawn` "/Game/Blueprint/Turrets/TurretFeature/Aoe/BP_AoeShock.BP_AoeShock_C")))
  (bind _returnvalue (`|SpawnActorFromClass` (`self.DamageAmmoToSpawn`) (`KismetMathLibrary.MakeTransform` (`SceneComponent.K2_GetComponentLocation` (`self.Center`))) "AlwaysSpawn" "MultiplyWithRoot" null null))
  (bind _asbp_turret_damage_base (cast `/Game/Blueprint/Turrets/TurretFeature/Aoe/BP_Turret_DamageBase` _returnvalue))
  (bind _output_get (set `self.DamageAmmo` _asbp_turret_damage_base))
  (`/Engine/EditorBlueprintResources/StandardMacros.IsValid` _output_get
    (:`Is Valid`
      (`self.K2_AttachToComponent` _output_get (`self.Center`) "None" "KeepWorld" "KeepRelative" "KeepWorld" true))))

(fn `Death`
  (`/Engine/EditorBlueprintResources/StandardMacros.IsValid` (`self.DamageAmmo`)
    (:`Is Valid`
      (`self.K2_DestroyActor`))
    (:`Is Not Valid`
      _))
  (`parent.Death`))

(fn `GetCost`
  (returns (GetCost :type "Float (double-precision)"))
  (return 0.0))

(fn `GetInteractImage`
  (returns (Image :type "Texture Object Reference"))
  (return null))

(fn `GetInteractMessage`
  (returns (InteractMessage :type Text) (Image :type "Texture Object Reference"))
  (return "" null))

(fn `OnCDEnded`
  (`parent.OnCDEnded`)
  (`/Engine/EditorBlueprintResources/StandardMacros.IsValid` (`self.DamageAmmo`)
    (:`Is Not Valid`
      (`self.SpawnAmmo`))))

(fn `OnCDStarted`
  (bind _damageammo (`self.DamageAmmo`))
  (`parent.OnCDStarted`)
  (`/Engine/EditorBlueprintResources/StandardMacros.IsValid` _damageammo
    (:`Is Valid`
      (`self.K2_DestroyActor` _damageammo))))

(fn `UserConstructionScript`
  (`parent.UserConstructionScript`))

(fn `WhichInteraction`
  (returns (TypeInteraction :type "/Game/Blueprint/Enum/EInteractable Enum"))
  (return "NewEnumerator0"))