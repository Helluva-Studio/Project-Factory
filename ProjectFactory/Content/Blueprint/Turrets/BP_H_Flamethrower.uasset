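; Flamethrower turret, a child Blueprint that loads per-level stats from a data table and passes cone, damage and damage-over-time settings to its spawned damage ammo.
; Interacting rotates it at no cost through a tick-driven yaw lerp, blocked during cooldown or an ongoing turn.
; Tick also jitters the ammo mesh and runs the Niagara flame only while on screen and off cooldown.
; Turret level sets the ammo mesh's visibility and material look.
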(event `self.ReceiveBeginPlay`
  (bind _asmaterial_instance_dynamic (cast `MaterialInstanceDynamic` (`PrimitiveComponent.GetMaterial` (`self.Ammo`) 1) :!pure true))
  (`parent.ReceiveBeginPlay`)
  (if (>= (`self.CurrentLevel`) 3)
    (`MaterialInstanceDynamic.SetScalarParameterValue` _asmaterial_instance_dynamic "TransitionValue" 1.0)
    (`MaterialInstanceDynamic.SetScalarParameterValue` _asmaterial_instance_dynamic "Brightness" 1.0)))

(event `self.ReceiveTick`
  (params (DeltaSeconds :type "Float (single-precision)"))
  (`parent.ReceiveTick` DeltaSeconds)
  (`|ExecutionSequence`
    (:`then_0`
      (`self.DisableEnableFlame`))
    (:`then_1`
      (if (not (`self.IsInCooldown`))
        (`self.AmmoFeedback`)
        (if (not (`self.CanChangeMode`))
          (set `self.RotationLerp` (`KismetMathLibrary.FClamp` (+ (`self.RotationLerp`) (* (`GameplayStatics.GetWorldDeltaSeconds`) (`self.RotationSpeed`)))))
          (`SceneComponent.K2_SetRelativeRotation` (`self.HandlerLR`) (`KismetMathLibrary.MakeRotator` 0.0 0.0 (`KismetMathLibrary.Lerp` (`self.InitialZRotation`) (`self.NextZRotation`) (`self.RotationLerp`))) false false)
          (if (>= (`self.RotationLerp`) 1.0)
            (set `self.RotationLerp` 0.0)
            (set `self.CanChangeMode` true)))))))

(event `DisableEnableFlame`
  (bind (_returnvalue_x _returnvalue_y) (`KismetMathLibrary.BreakVector2D` (`WidgetLayoutLibrary.GetViewportSize`)))
  (bind _ns_flame01 (`self.NS_Flame01`))
  (bind _ns_flame01_2 (`self.NS_Flame01`))
  (bind _screenlocation (`PlayerController.ProjectWorldLocationToScreen` (`GameplayStatics.GetPlayerController` 0) (`SceneComponent.K2_GetComponentLocation` (`self.NS_Flame01`)) false))
  (`/Engine/EditorBlueprintResources/StandardMacros.IsValid` self
    (:`Is Valid`
      (if (and (> (`KismetMathLibrary.BreakVector2D` _screenlocation) 0.0) (> (`.Y` (`KismetMathLibrary.BreakVector2D` _screenlocation)) 0.0) (< (`KismetMathLibrary.BreakVector2D` _screenlocation) _returnvalue_x) (< (`.Y` (`KismetMathLibrary.BreakVector2D` _screenlocation)) _returnvalue_y) (not (`self.IsInCooldown`)) (`self.IsActorTickEnabled`))
        (`ActorComponent.Activate` _ns_flame01_2 false)
        (`NiagaraComponent.SetVariableFloat` _ns_flame01_2 "SpawnRate" 2500.0)
        (else
          (`NiagaraComponent.SetVariableFloat` _ns_flame01 "SpawnRate" 0.0)
          (`KismetSystemLibrary.Delay` 1.0)
          (`ActorComponent.Deactivate` _ns_flame01))))))

(event `self.SpawnAmmo`
  (`parent.SpawnAmmo`)
  (`/Engine/EditorBlueprintResources/StandardMacros.IsValid` (`self.DamageAmmo`)
    (:`Is Valid`
      (message `/Game/Blueprint/Turrets/Interfaces/BPI_TurretDamageAmmo.InitializeFlameAmmo` (`self.DamageAmmo`) (`self.CanHitPlayer`) (`self.D_TypeOfDamage`) (`self.D_TypeOfAoe`) (`self.MaxAngleOfEffect(Cone)`) (`self.DamageTick`) (`self.MaxDamageOnHit`) (`self.MaxDotInsideAoe`) (`self.MaxDotOutsideAoe`) (`self.MaxDotDuration`) (`self.DamageReductionByDistance`)))))

(event `AmmoFeedback`
  (bind _ammo (`self.Ammo`))
  (`/Engine/EditorBlueprintResources/StandardMacros.IsValid` self
    (:`Is Valid`
      (`/Engine/EditorBlueprintResources/StandardMacros.FlipFlop`
        (:`A`
          (`SceneComponent.K2_SetRelativeRotation` _ammo (struct :`Pitch` 1.0 :`Yaw` -90.0) false false))
        (:`B`
          (`SceneComponent.K2_SetRelativeRotation` _ammo (struct :`Pitch` -1.0 :`Yaw` -90.0) false false))))))

(event `/Game/Blueprint/Turrets/Interfaces/BI_Interactable.Interact`
  (bind (_relativerotation_roll _relativerotation_pitch _relativerotation_yaw) (`KismetMathLibrary.BreakRotator` (`SceneComponent.RelativeRotation` (`self.HandlerLR`))))
  (set `self.RotationLerp` 0.0)
  (bind _output_get (set `self.InitialZRotation` _relativerotation_yaw))
  (set `self.NextZRotation` (+ _output_get (`self.DeltaRotation`)))
  (set `self.CanChangeMode` false))

(fn `CanInteract`
  (returns (CanInteract :type Boolean))
  (return (and (`self.CanChangeMode`) (not (`self.IsInCooldown`)))))

(fn `GetCost`
  (returns (GetCost :type "Float (double-precision)"))
  (return 0.0))

(fn `GetInteractImage`
  (returns (Image :type "Texture Object Reference"))
  (return "/Game/2DImage/ruota.ruota"))

(fn `GetInteractMessage`
  (returns (InteractMessage :type Text) (Image :type "Texture Object Reference"))
  (return "Rotate 45°" null))

(fn `InitializeTurret`
  (`parent.InitializeTurret`)
  (bind _returnvalue (`|GetDataTableRow` "/Game/Blueprint/Turrets/TurretFeature/Leveling/TurretSpecificDataTable/DT_H_TurretFlameThrower.DT_H_TurretFlameThrower" (`KismetStringLibrary.Conv_StringToName` (`KismetStringLibrary.Conv_IntToString` (`self.CurrentLevel`))))
    (:`then`
      (bind (_maxhealth _maxactivitytime _maxcdtime _baseaoetype _baseangle _anglepercentagemodifier _basedamagetype _damagetick _damageonhit _damageovertimeinsideaoe _damageovertimeoutsideaoe _dotduration _basedamagereductionondistance) (break `/Game/Blueprint/Turrets/TurretFeature/Leveling/TurretStructs/S_H_TurretFlamethrowerStats` _returnvalue))
      (bind _output_get (set `self.MaxHealth` _maxhealth))
      (set `self.CurrentHealth` _output_get)
      (set `self.MaxActivityTime(NoFarm)` _maxactivitytime)
      (set `self.MaxCdTime` _maxcdtime)
      (set `self.D_TypeOfAoe` _baseaoetype)
      (bind _output_get_2 (set `self.D_BaseAngleOfEffect(Cone)` _baseangle))
      (set `self.MaxAngleOfEffect(Cone)` (+ _output_get_2 (* _output_get_2 (/ _anglepercentagemodifier 100.0))))
      (set `self.D_TypeOfDamage` _basedamagetype)
      (set `self.DamageTick` _damagetick)
      (set `self.MaxDamageOnHit` _damageonhit)
      (set `self.MaxDotInsideAoe` _damageovertimeinsideaoe)
      (set `self.MaxDotOutSideAoe` _damageovertimeoutsideaoe)
      (set `self.MaxDotDuration` _dotduration)
      (set `self.DamageReductionByDistance` _basedamagereductionondistance))))

(fn `OnCDStarted`
  (`parent.OnCDStarted`)
  (set `self.IsInitialized` false))

(fn `UpdateGraphicByLevel`
  (params (Level :type Integer))
  (bind _asmaterial_instance_dynamic (cast `MaterialInstanceDynamic` (`PrimitiveComponent.GetMaterial` (`self.Ammo`) 1) :!pure true))
  (`/Engine/EditorBlueprintResources/StandardMacros.IsValid` self
    (:`Is Valid`
      (switch `int` Level
        (:`1`
          (`SceneComponent.SetVisibility` (`self.Ammo`) false true)
          (`MaterialInstanceDynamic.SetScalarParameterValue` _asmaterial_instance_dynamic "TransitionValue" 0.0 :!label _label))
        (:`2`
          (`SceneComponent.SetVisibility` (`self.Ammo`) true true)
          (goto _label))
        (:`3`
          (`SceneComponent.SetVisibility` (`self.Ammo`) true true)
          (`MaterialInstanceDynamic.SetScalarParameterValue` _asmaterial_instance_dynamic "TransitionValue" 1.0)
          (`MaterialInstanceDynamic.SetScalarParameterValue` _asmaterial_instance_dynamic "Brightness" 1.0))))))

(fn `UserConstructionScript`
  (`parent.UserConstructionScript`)
  (`NiagaraComponent.SetVariableFloat` (`self.NS_Flame01`) "SpawnRate" 0.0))

(fn `WhichInteraction`
  (returns (TypeInteraction :type "/Game/Blueprint/Enum/EInteractable Enum"))
  (return "NewEnumerator0"))