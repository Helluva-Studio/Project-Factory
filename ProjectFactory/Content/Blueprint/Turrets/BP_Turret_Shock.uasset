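; Shock turret Blueprint, a child turret that adds its own beam effect, level indicators and interaction responses on top of parent setup.
; The construction script points the Shock effect's BeamEnd parameter at the Center component's world location.
; Turret level toggles the visibility of Light2 and Light3, and focus toggles custom depth on meshes for outlining.
; It always reports as interactable at zero cost, but Interact only checks cooldown and performs no action.
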(event `self.ReceiveBeginPlay`
  (`parent.ReceiveBeginPlay`))

(event `self.ReceiveTick`
  (params (DeltaSeconds :type "Float (single-precision)"))
  (`parent.ReceiveTick` DeltaSeconds))

(event `self.Focus`
  (params (IsFocused :type Boolean))
  (for _array_element (`self.MeshesToOutline`)
    (`PrimitiveComponent.SetRenderCustomDepth` _array_element IsFocused)))

(event `self.Interact`
  (if (not (`self.IsInCooldown`))
    _))

(fn `CanInteract`
  (returns (CanInteract :type Boolean))
  (return true))

(fn `GetCost`
  (returns (GetCost :type "Float (double-precision)"))
  (return 0.0))

(fn `InitializeTurret`
  (`parent.InitializeTurret`))

(fn `UpdateGraphicByLevel`
  (params (Level :type Integer))
  (`/Engine/EditorBlueprintResources/StandardMacros.IsValid` self
    (:`Is Valid`
      (switch `int` Level
        (:`1`
          (`SceneComponent.SetVisibility` (`self.Light2`) false false)
          (`SceneComponent.SetVisibility` (`self.Light3`) false false))
        (:`2`
          (`SceneComponent.SetVisibility` (`self.Light2`) true false)
          (`SceneComponent.SetVisibility` (`self.Light3`) false false))
        (:`3`
          (`SceneComponent.SetVisibility` (`self.Light2`) true false)
          (`SceneComponent.SetVisibility` (`self.Light3`) true false))))))

(fn `UserConstructionScript`
  (`parent.UserConstructionScript`)
  (`FXSystemComponent.SetVectorParameter` (`self.Shock`) "BeamEnd" (`SceneComponent.K2_GetComponentLocation` (`self.Center`))))

(fn `WhichInteraction`
  (returns (TypeInteraction :type "/Game/Blueprint/Enum/EInteractable Enum"))
  (return "NewEnumerator0"))