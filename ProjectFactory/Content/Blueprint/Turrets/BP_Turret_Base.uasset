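; Base turret actor that loads health and timing stats from DT_TurretByLevel by type and level.
; Tick turns the health widget toward the camera, drains health over time and runs an activity/cooldown cycle shown on the widget bar.
; Damage or decay triggers Death, which spawns a BP_TurretTrigger carrying RemainingActivation before destroying the turret.
; Cooldown and level-graphic hooks are empty stubs, InitializeLevel is unwired, and focus outlines meshes via custom depth.
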(event `self.ReceiveBeginPlay`
  (`self.InitializeTurret`))

(event `self.ReceiveTick`
  (params (DeltaSeconds :type "Float (single-precision)"))
  (`|ExecutionSequence`
    (:`then_1`
      (`self.RotateHealthWidget`))
    (:`then_2`
      (`self.ManageDepleteHealth`))
    (:`then_3`
      (`self.ManageTurretFunctioning`))))

(event `RotateHealthWidget`
  (bind _widget (`self.Widget`)
    (:`then`
      (if (`SceneComponent.IsVisible` _widget)
        (`SceneComponent.K2_SetWorldRotation` (`self.Widget`) (`KismetMathLibrary.FindLookAtRotation` (`SceneComponent.K2_GetComponentLocation` _widget) (`SceneComponent.K2_GetComponentLocation` (`PlayerCameraManager.TransformComponent` (`GameplayStatics.GetPlayerCameraManager` 0)))) false false)
        (bind _aswb_turret_health_1 (cast `/Game/HUD/WB_TurretHealth1` (`WidgetComponent.GetWidget` (`self.Widget`))))
        (set `/Game/HUD/WB_TurretHealth1.WB_MaxHealth` (`self.MaxHealth`) _aswb_turret_health_1)
        (set `/Game/HUD/WB_TurretHealth1.WB_CurrentHealth` (`self.CurrentHealth`) _aswb_turret_health_1)))
    (:`else`)))

(event `/Game/Blueprint/Turrets/Interfaces/BI_Healable.Heal`
  (bind _returnvalue (+ (`self.CurrentHealth`) (`self.HealthRepairAmount`)))
  (if (> _returnvalue (`self.MaxHealth`))
    (set `self.CurrentHealth` (`self.MaxHealth`))
    (else
      (set `self.CurrentHealth` _returnvalue))))

(event `GainExp`
  (if (< (`self.CurrentLevel`) (`self.MaxLevel`))
    (if (>= (`self.GetGameTimeSinceCreation`) (`self.TimeRequiredForLevel`))
      (bind _result (`/Engine/EditorBlueprintResources/StandardMacros.IncrementInt` (`self.CurrentLevel`))
        (:`  `
          (set `self.TimeRequiredForLevel` (* (`self.TimeRequiredForLevel`) _result))
          (`self.UpdateGraphicByLevel` _result))))))

(event `self.ReceiveAnyDamage`
  (params (Damage :type "Float (single-precision)") (DamageType :type "DamageType Object Reference") (InstigatedBy :type "Controller Object Reference") (DamageCauser :type "Actor Object Reference"))
  (`self.Take Damage` Damage))

(event `/Game/Blueprint/Turrets/Interfaces/BPI_LevelUppable.InitializeLevel`
  (params (LevelSelected :type Integer) (RemaingActivation :type Integer)))

(event `/Game/Blueprint/Interfaces/BPI_TakeDamage.TakeDamageByInterface`
  (params (Damage :type "Float (double-precision)"))
  (`self.Take Damage` Damage))

(event `/Game/Blueprint/InteractionArea/BPI_Focusable.ToggleFocus`
  (params (Focus :type Boolean))
  (for _array_element (`self.MeshToOutline`)
    (`PrimitiveComponent.SetRenderCustomDepth` _array_element Focus)))

(fn `Death`
  (`|SpawnActorFromClass` "/Game/Blueprint/Turrets/BP_TurretTrigger.BP_TurretTrigger_C" (`KismetMathLibrary.MakeTransform` (`self.K2_GetActorLocation`)) "Undefined" "MultiplyWithRoot" null (`self.RemainingActivation`) true null)
  (`self.K2_DestroyActor`))

(fn `InitializeTurret`
  (bind _returnvalue (`|GetDataTableRow` "/Game/Blueprint/Turrets/TurretFeature/Leveling/DT_TurretByLevel.DT_TurretByLevel" (`KismetStringLibrary.Conv_StringToName` (`KismetStringLibrary.Conv_IntToString` (+ (* (`KismetMathLibrary.Conv_ByteToInt` (`self.TurretType`)) (`self.MaxLevel`)) (`self.CurrentLevel`)))))
    (:`then`
      (bind _output_get (set `self.InitializationRow` _returnvalue))
      (bind (_turrettype _level _maxhealth _constructioncost _repaircost _maxactivitytimenofarm _maxcdtimenofarm) (break `/Game/Blueprint/Turrets/TurretFeature/Leveling/S_TurretChangebleValue` _output_get))
      (bind _output_get_2 (set `self.MaxHealth` _maxhealth))
      (set `self.CurrentHealth` _output_get_2)
      (set `self.MaxActivityTime(NoFarm)` _maxactivitytimenofarm)
      (set `self.MaxCdTime` _maxcdtimenofarm))
    (:`RowNotFound`
      (`KismetSystemLibrary.PrintString` "BP_BaseTurret_InitializeTurret Not Succeded!"))))

(fn `ManageDepleteHealth`
  (bind _returnvalue (- (`self.CurrentHealth`) (* (`GameplayStatics.GetWorldDeltaSeconds`) (`self.HealthLostOverTime`))))
  (if (> _returnvalue 0.0)
    (set `self.CurrentHealth` _returnvalue)
    (else
      (`self.Death`))))

(fn `ManageTurretFunctioning`
  (bind _maxcdtime (`self.MaxCdTime`))
  (bind _activitytime_nofarm_ (`self.ActivityTime(NoFarm)`))
  (`/Engine/EditorBlueprintResources/StandardMacros.IsValid` self
    (:`Is Valid`
      (if (`self.IsInCooldown`)
        (`self.OnCDStarted`)
        (bind _aswb_turret_health_1 (cast `/Game/HUD/WB_TurretHealth1` (`WidgetComponent.GetWidget` (`self.Widget`))))
        (set `Widget.RenderOpacity` 1.0 (`/Game/HUD/WB_TurretHealth1.CdBar` _aswb_turret_health_1))
        (bind _aswb_turret_health_1_2 (cast `/Game/HUD/WB_TurretHealth1` (`WidgetComponent.GetWidget` (`self.Widget`))))
        (set `/Game/HUD/WB_TurretHealth1.WB_CdColor` (struct :`R` 1.0 :`A` 1.0) _aswb_turret_health_1_2)
        (set `self.CdTime` (`KismetMathLibrary.FClamp` (+ (`self.CdTime`) (`GameplayStatics.GetWorldDeltaSeconds`)) 0.0 (`self.MaxCdTime`)))
        (if (>= (`self.CdTime`) (`self.MaxCdTime`))
          (set `self.IsInCooldown` false)
          (set `self.CdTime` 0.0)
          (else
            (set `self.IsInCooldown` true)
            (bind _aswb_turret_health_1_3 (cast `/Game/HUD/WB_TurretHealth1` (`WidgetComponent.GetWidget` (`self.Widget`))))
            (set `/Game/HUD/WB_TurretHealth1.WB_MaxCdTime` _maxcdtime _aswb_turret_health_1_3)
            (set `/Game/HUD/WB_TurretHealth1.WB_CurrentCdTime` (- _maxcdtime (`self.CdTime`)) _aswb_turret_health_1_3)))
        (else
          (`self.OnCDEnded`)
          (bind _aswb_turret_health_1_4 (cast `/Game/HUD/WB_TurretHealth1` (`WidgetComponent.GetWidget` (`self.Widget`))))
          (set `/Game/HUD/WB_TurretHealth1.WB_CdColor` (struct :`R` 1.0 :`G` 0.5 :`A` 1.0) _aswb_turret_health_1_4)
          (if (`self.IsInFunction(NoFarm)`)
            (bind _aswb_turret_health_1_5 (cast `/Game/HUD/WB_TurretHealth1` (`WidgetComponent.GetWidget` (`self.Widget`))))
            (set `Widget.RenderOpacity` 1.0 (`/Game/HUD/WB_TurretHealth1.CdBar` _aswb_turret_health_1_5))
            (set `self.ActivityTime(NoFarm)` (`KismetMathLibrary.FClamp` (+ (`self.ActivityTime(NoFarm)`) (`GameplayStatics.GetWorldDeltaSeconds`)) 0.0 (`self.MaxActivityTime(NoFarm)`)))
            (if (>= (`self.ActivityTime(NoFarm)`) (`self.MaxActivityTime(NoFarm)`))
              (set `self.IsInCooldown` true)
              (set `self.ActivityTime(NoFarm)` 0.0)
              (else
                (set `self.IsInCooldown` false)
                (bind _aswb_turret_health_1_6 (cast `/Game/HUD/WB_TurretHealth1` (`WidgetComponent.GetWidget` (`self.Widget`))))
                (set `/Game/HUD/WB_TurretHealth1.WB_MaxCdTime` (`self.MaxActivityTime(NoFarm)`) _aswb_turret_health_1_6)
                (set `/Game/HUD/WB_TurretHealth1.WB_CurrentCdTime` (`self.ActivityTime(NoFarm)`) _aswb_turret_health_1_6)))
            (else
              (set `self.ActivityTime(NoFarm)` (`KismetMathLibrary.FClamp` (- (`self.ActivityTime(NoFarm)`) (`GameplayStatics.GetWorldDeltaSeconds`)) 0.0 (`self.MaxActivityTime(NoFarm)`)))
              (bind _aswb_turret_health_1_7 (cast `/Game/HUD/WB_TurretHealth1` (`WidgetComponent.GetWidget` (`self.Widget`))))
              (set `/Game/HUD/WB_TurretHealth1.WB_MaxCdTime` (`self.MaxActivityTime(NoFarm)`) _aswb_turret_health_1_7)
              (set `/Game/HUD/WB_TurretHealth1.WB_CurrentCdTime` _activitytime_nofarm_ _aswb_turret_health_1_7)
              (if (> _activitytime_nofarm_ 0.0)
                (bind _aswb_turret_health_1_8 (cast `/Game/HUD/WB_TurretHealth1` (`WidgetComponent.GetWidget` (`self.Widget`))))
                (set `Widget.RenderOpacity` 1.0 (`/Game/HUD/WB_TurretHealth1.CdBar` _aswb_turret_health_1_8))
                (else
                  (bind _aswb_turret_health_1_9 (cast `/Game/HUD/WB_TurretHealth1` (`WidgetComponent.GetWidget` (`self.Widget`))))
                  (set `Widget.RenderOpacity` 0.0 (`/Game/HUD/WB_TurretHealth1.CdBar` _aswb_turret_health_1_9)))))))))))

(fn `MeshToOutline`
  (returns (Meshes :type "Array of StaticMeshComponent Object Reference"))
  (bind _output_get (set `self.MeshesToOutline` (`self.K2_GetComponentsByClass` "/Script/Engine.StaticMeshComponent")))
  (return _output_get))

(fn `OnCDEnded`)

(fn `OnCDStarted`)

(fn `Take Damage`
  (params (Damage :type "Float (double-precision)"))
  (if (< Damage (`self.CurrentHealth`))
    (set `self.CurrentHealth` (- (`self.CurrentHealth`) Damage))
    (else
      (set `self.CurrentHealth` 0.0)
      (`self.Death`))))

(fn `UpdateGraphicByLevel`
  (params (Level :type Integer)))

(fn `UserConstructionScript`
  (`self.UpdateGraphicByLevel` (`self.CurrentLevel`)))