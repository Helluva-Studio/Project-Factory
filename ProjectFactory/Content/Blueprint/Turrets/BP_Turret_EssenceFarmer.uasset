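; BP_Turret_EssenceFarmer is a turret Blueprint, named for essence farming, that contains no farming logic of its own.
; BeginPlay, Tick and the construction script only forward to the parent class.
; Its interaction functions are stubs: WhichInteraction returns a fixed enum value, GetCost returns zero, and CanInteract always evaluates to false, so it reports itself as non-interactable.
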(event `self.ReceiveBeginPlay`
  (`parent.ReceiveBeginPlay`))

(event `self.ReceiveTick`
  (params (DeltaSeconds :type "Float (single-precision)"))
  (`parent.ReceiveTick` DeltaSeconds))

(fn `CanInteract`
  (returns (CanInteract :type Boolean))
  (return (and false (not false))))

(fn `GetCost`
  (returns (GetCost :type "Float (double-precision)"))
  (return 0.0))

(fn `UserConstructionScript`
  (`parent.UserConstructionScript`))

(fn `WhichInteraction`
  (returns (TypeInteraction :type "/Game/Blueprint/Enum/EInteractable Enum"))
  (return "NewEnumerator0"))