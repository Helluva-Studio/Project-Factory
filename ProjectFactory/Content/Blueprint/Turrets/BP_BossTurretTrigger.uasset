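; BP_BossTurretTrigger is a turret trigger that keeps the boss BP_Otrebor informed of whether it is available.
; Its UpdateBoss event finds the boss with GetActorOfClass, then adds itself as a turret trigger when off cooldown and removes itself when in cooldown.
; The event is its only active logic, and nothing in this graph calls it or changes the cooldown state.
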(event `self.UpdateBoss`
  (if (not (`self.IsInCooldown`))
    (bind _returnvalue (`GameplayStatics.GetActorOfClass` "/Game/Blueprint/Enemies/BP_Otrebor.BP_Otrebor_C"))
    (`/Engine/EditorBlueprintResources/StandardMacros.IsValid` _returnvalue
      (:`Is Valid`
        (`/Game/Blueprint/Enemies/Interfaces/BPI_Otrebor.AddTurretTrigger` _returnvalue self)))
    (else
      (bind _returnvalue_2 (`GameplayStatics.GetActorOfClass` "/Game/Blueprint/Enemies/BP_Otrebor.BP_Otrebor_C"))
      (`/Engine/EditorBlueprintResources/StandardMacros.IsValid` _returnvalue_2
        (:`Is Valid`
          (`/Game/Blueprint/Enemies/Interfaces/BPI_Otrebor.RemoveTurretTrigger` _returnvalue_2 self))))))

(fn `UserConstructionScript`
  (`parent.UserConstructionScript`))