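; Hazard turret that emits an area effect, spawned as a separate effect actor, whenever it is not in cooldown.
; Tick uses two DoOnce gates that re-arm each other, destroying the effect on entering cooldown and spawning a new one afterward.
; SpawnAoe picks the class from EffectActors by TypeOfEffect, attaches it to Center and initializes it with the turret's settings.
; Death also destroys the active effect.
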(event `self.ReceiveBeginPlay`
  (`parent.ReceiveBeginPlay`))

(event `self.ReceiveTick`
  (params (DeltaSeconds :type "Float (single-precision)"))
  (`parent.ReceiveTick` DeltaSeconds)
  (if (`self.IsInCooldown`)
    (`/Engine/EditorBlueprintResources/StandardMacros.DoOnce` false :!label _label
      (:`Completed`
        (`/Engine/EditorBlueprintResources/StandardMacros.IsValid` (`self.EffectActorAmmo`)
          (:`Is Valid`
            (`self.K2_DestroyActor` (`self.EffectActorAmmo`))
            (goto _label_2 :!via `Reset`)))))
    (else
      (`/Engine/EditorBlueprintResources/StandardMacros.DoOnce` false :!label _label_2
        (:`Completed`
          (`self.SpawnAoe`)
          (goto _label :!via `Reset`))))))

(event `SpawnAoe`
  (bind _keys (`BlueprintMapLibrary.Map_Keys` (`self.Effect Actors`)))
  (bind _values (`BlueprintMapLibrary.Map_Values` (`self.Effect Actors`)))
  (bind _returnvalue (`|SpawnActorFromClass` (`|GetArrayItem` _values (`KismetArrayLibrary.Array_Find` _keys (`self.TypeOfEffect`))) (`KismetMathLibrary.MakeTransform` (`SceneComponent.K2_GetComponentLocation` (`self.Center`))) "AdjustIfPossibleButAlwaysSpawn" "MultiplyWithRoot" null null))
  (bind _output_get (set `self.EffectActorAmmo` _returnvalue))
  (`/Engine/EditorBlueprintResources/StandardMacros.IsValid` _output_get
    (:`Is Valid`
      (`self.K2_AttachToComponent` _output_get (`self.Center`) "None" "KeepWorld" "KeepRelative" "KeepWorld" true)
      (bind _asbp_turret_effect (cast `/Game/Blueprint/Turrets/TurretFeature/Aoe/BP_Turret_Effect` _returnvalue))
      (`/Game/Blueprint/Turrets/TurretFeature/Aoe/BP_Turret_Effect.Initialize` _asbp_turret_effect (`self.CanHitPlayer`) 0.0 0.0 0.0 (`self.TypeOfAoe`) "NewEnumerator0" (`self.MaxDistance(Cone)/MaxRadius(Sphere)`) (`self.MaxAngleOfEffect(Cone)`) (`self.TimeTick`) (`self.TypeOfEffect`) (`self.Slow Effect`) (`self.Stun Time`) (`self.Gravity Force`)))))

(fn `Death`
  (bind _effectactorammo (`self.EffectActorAmmo`))
  (`/Engine/EditorBlueprintResources/StandardMacros.IsValid` _effectactorammo
    (:`Is Valid`
      (`self.K2_DestroyActor` _effectactorammo))
    (:`Is Not Valid`
      _))
  (`parent.Death`))

(fn `UserConstructionScript`
  (`parent.UserConstructionScript`))