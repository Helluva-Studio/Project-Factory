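; Farming turret that stores resources over time until full, then releases them when the player interacts.
; Tick drives charging, the widget's cooldown bar, and material and bobbing storage feedback.
; Interact uses a delayed loop to scatter BPI_ResourceSpawnable pickups around the turret, then starts a cooldown proportional to the amount released.
; Focus outlines meshes through custom depth when the turret is ready, and LevelUp only reshapes the model.
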(event `self.ReceiveBeginPlay`
  (`parent.ReceiveBeginPlay`))

(event `Charge`
  (if (`self.IsInCooldown`)
    (`MaterialInstanceDynamic.SetVectorParameterValue` (`self.ChargeMaterial`) "Color" (`self.CoolDownColor`))
    (else
      (`MaterialInstanceDynamic.SetVectorParameterValue` (`self.ChargeMaterial`) "Color" (`self.ResourceColor`))
      (if (`self.IsTankFull`)
        _
        (elif (not (`self.IsSpawningResource`))
          ;[1 1 1] Time Required To Charge 1 Resource
          (bind _output_get (set `self.ChargeValue` (+ (`GameplayStatics.GetWorldDeltaSeconds`) (`self.ChargeValue`))))
          (if (>= _output_get (`self.ChargeTimePerResource`))
            (`/Engine/EditorBlueprintResources/StandardMacros.IncrementInt` (`self.ResourceStored`)
              (:`  `
                (set `self.ChargeValue` 0.0)
                (if (`self.IsTankFull`)
                  (`MaterialInstanceDynamic.SetScalarParameterValue` (`self.ChargeMaterial`) "TransitionValue" (/ (`self.ResourceStored`) (`KismetMathLibrary.Conv_IntToDouble` (`self.MaxResourceStored`))) :!label _label))))
            (else
              (goto _label))))))))

(event `self.ReceiveTick`
  (params (DeltaSeconds :type "Float (single-precision)"))
  (`parent.ReceiveTick` DeltaSeconds)
  (`|ExecutionSequence`
    (:`then_0`
      (`self.ManageTurretFunctioning`))
    (:`then_1`
      (`self.Charge`))
    (:`then_2`
      (`self.StorageFeedback`))))

(event `SpawnResource`
  (bind (_returnvalue_x _returnvalue_y) (`KismetMathLibrary.BreakVector` (`KismetMathLibrary.RandomUnitVector`)))
  (bind (_returnvalue_x_2 _returnvalue_y_2) (`KismetMathLibrary.BreakVector` (* (`KismetMathLibrary.Normal` (`KismetMathLibrary.MakeVector` _returnvalue_x _returnvalue_y)) (* (`self.SpawnDistanceFromTurret`) (`KismetMathLibrary.RandomFloatInRange` 0.85 1.0)))))
  (bind _returnvalue (`|SpawnActorFromClass` (`self.ResourceToSpawn`) (`KismetMathLibrary.MakeTransform` (+ (`self.K2_GetActorLocation`) (`KismetMathLibrary.MakeVector` _returnvalue_x_2 _returnvalue_y_2 60.0))) "AdjustIfPossibleButAlwaysSpawn" "MultiplyWithRoot" null null))
  (`/Engine/EditorBlueprintResources/StandardMacros.IsValid` _returnvalue
    (:`Is Valid`
      (if (`KismetSystemLibrary.DoesImplementInterface` _returnvalue "/Game/Blueprint/Resources/BPI_ResourceSpawnable.BPI_ResourceSpawnable_C")
        (message `/Game/Blueprint/Resources/BPI_ResourceSpawnable.Initialize` _returnvalue (`self.ResourceValue`))))))

(event `StorageFeedback`
  (bind _storagematerial (`self.StorageMaterial`))
  (`/Engine/EditorBlueprintResources/StandardMacros.IsValid` self
    (:`Is Valid`
      (if (`self.IsInCooldown`)
        (`MaterialInstanceDynamic.SetScalarParameterValue` (`self.StorageMaterial`) "Brightness" 0.0)
        (else
          (if (`self.IsSpawningResource`)
            (`MaterialInstanceDynamic.SetVectorParameterValue` (`self.ChargeMaterial`) "Color" (`self.CdResourceColor`))
            (else
              (`MaterialInstanceDynamic.SetVectorParameterValue` (`self.ChargeMaterial`) "Color" (`self.ResourceColor`))))
          (`SceneComponent.K2_AddWorldOffset` (`self.Storage`) (`KismetMathLibrary.MakeVector` 0.0 0.0 (/ (`KismetMathLibrary.DegSin` (* (`self.GetGameTimeSinceCreation`) 200.0)) 20.0)) false false)
          (`SceneComponent.K2_AddWorldRotation` (`self.Storage`) (struct :`Yaw` 2.0) false false)
          (if (and (`self.IsTankFull`) (not (`self.IsSpawningResource`)))
            (`MaterialInstanceDynamic.SetScalarParameterValue` _storagematerial "Brightness" 0.01)
            (else
              (`MaterialInstanceDynamic.SetScalarParameterValue` _storagematerial "Brightness" 0.0))))))))

(event `/Game/Blueprint/Turrets/Interfaces/BI_Interactable.Interact`
  (if (and (not (`self.IsInCooldown`)) (not (`self.IsSpawningResource`)))
    (set `self.IsSpawningResource` true)
    (set `self.MaxCdTime` (* (`self.ResourceStored`) (`self.CdTimePerResource`)))
    (bind _index (`/Game/Blueprint/BP_MacroLibrary_Actor.For Loop With Delay` 1 (`self.ResourceStored`) (`self.TimeBetweenSpawn`))
      (:`Loop Body`
        (`self.SpawnResource`)
        (set `self.CdTime` (* (`self.CdTimePerResource`) _index))
        (`MaterialInstanceDynamic.SetScalarParameterValue` (`self.ChargeMaterial`) "TransitionValue" (/ (- (`self.ResourceStored`) _index) (`KismetMathLibrary.Conv_IntToDouble` (`self.MaxResourceStored`)))))
      (:`Completed`
        (set `self.IsInCooldown` true)
        (set `self.IsSpawningResource` false)
        (set `self.ResourceStored` 0)))))

(event `self.Focus`
  (params (IsFocused :type Boolean))
  (for _array_element (`self.MeshesToOutline`)
    (`PrimitiveComponent.SetRenderCustomDepth` _array_element (and IsFocused (not (`self.IsInCooldown`)) (not (`self.IsSpawningResource`))))))

(event `self.LevelUp`
  (params (Level :type Integer))
  (bind _currentlevel (`self.CurrentLevel`))
  (bind _currentlevel_2 (`self.CurrentLevel`))
  (bind _neck (`self.Neck`))
  (bind _neck_2 (`self.Neck`))
  (bind _neck_3 (`self.Neck`))
  (bind _returnvalue (`KismetMathLibrary.Conv_IntToDouble` (`self.CurrentLevel`)))
  (bind _returnvalue_2 (`KismetMathLibrary.Conv_IntToDouble` _currentlevel))
  (bind _returnvalue_3 (* _currentlevel_2 1.5))
  (bind _returnvalue_4 (* _returnvalue 2.0))
  (`/Engine/EditorBlueprintResources/StandardMacros.IsValid` self
    (:`Is Valid`
      (switch `int` Level
        (:`1`
          (`SceneComponent.SetRelativeScale3D` (`self.Scene`) (`KismetMathLibrary.MakeVector` _returnvalue_4 _returnvalue_4 _returnvalue))
          (`SceneComponent.K2_SetRelativeLocation` (`self.HandlerLR`) (0.0 0.0 -25.0) false false)
          (`SceneComponent.SetHiddenInGame` _neck true false)
          (`SceneComponent.SetVisibility` _neck false false))
        (:`2`
          (`SceneComponent.SetRelativeScale3D` (`self.Scene`) (`KismetMathLibrary.MakeVector` _returnvalue_3 _returnvalue_3 (* _currentlevel_2 0.75)))
          (`SceneComponent.K2_SetRelativeLocation` (`self.HandlerLR`) (0.0 0.0 -25.0) false false)
          (`SceneComponent.SetHiddenInGame` _neck_2 true false)
          (`SceneComponent.SetVisibility` _neck_2 false false))
        (:`3`
          (`SceneComponent.SetRelativeScale3D` (`self.Scene`) (`KismetMathLibrary.MakeVector` _returnvalue_2 _returnvalue_2 (* _currentlevel 0.5)))
          (`SceneComponent.K2_SetRelativeLocation` (`self.HandlerLR`) (0.0 0.0 7.5) false false)
          (`SceneComponent.SetHiddenInGame` _neck_3 false false)
          (`SceneComponent.SetVisibility` _neck_3 true false))))))

(fn `CanInteract`
  (returns (CanInteract :type Boolean))
  (return true))

(fn `GetCost`
  (returns (GetCost :type "Float (double-precision)"))
  (return 0.0))

(fn `IsTankFull`
  (returns (IsFull :type Boolean))
  (return (>= (`self.ResourceStored`) (`self.MaxResourceStored`))))

(fn `ManageTurretFunctioning`
  (bind _cdtime (`self.CdTime`))
  (`/Engine/EditorBlueprintResources/StandardMacros.IsValid` self
    (:`Is Valid`
      (if (`self.IsSpawningResource`)
        (bind _aswb_turret_health_1 (cast `/Game/HUD/WB_TurretHealth1` (`WidgetComponent.GetWidget` (`self.Widget`))))
        (set `Widget.RenderOpacity` 1.0 (`/Game/HUD/WB_TurretHealth1.CdBar` _aswb_turret_health_1))
        (bind _aswb_turret_health_1_2 (cast `/Game/HUD/WB_TurretHealth1` (`WidgetComponent.GetWidget` (`self.Widget`))))
        (set `/Game/HUD/WB_TurretHealth1.WB_CdColor` (struct :`R` 1.0 :`G` 0.5 :`A` 1.0) _aswb_turret_health_1_2)
        (bind _aswb_turret_health_1_3 (cast `/Game/HUD/WB_TurretHealth1` (`WidgetComponent.GetWidget` (`self.Widget`))))
        (set `/Game/HUD/WB_TurretHealth1.WB_MaxCdTime` (`self.MaxCdTime`) _aswb_turret_health_1_3)
        (set `/Game/HUD/WB_TurretHealth1.WB_CurrentCdTime` (`self.CdTime`) _aswb_turret_health_1_3)
        (elif (`self.IsInCooldown`)
          (bind _aswb_turret_health_1_4 (cast `/Game/HUD/WB_TurretHealth1` (`WidgetComponent.GetWidget` (`self.Widget`))))
          (set `/Game/HUD/WB_TurretHealth1.WB_CdColor` (struct :`R` 1.0 :`A` 1.0) _aswb_turret_health_1_4)
          (set `self.CdTime` (- (`self.CdTime`) (`GameplayStatics.GetWorldDeltaSeconds`)))
          (bind _aswb_turret_health_1_5 (cast `/Game/HUD/WB_TurretHealth1` (`WidgetComponent.GetWidget` (`self.Widget`))))
          (set `/Game/HUD/WB_TurretHealth1.WB_CurrentCdTime` _cdtime _aswb_turret_health_1_5)
          (if (<= _cdtime 0.0)
            (set `self.IsInCooldown` false))
          (else
            (bind _aswb_turret_health_1_6 (cast `/Game/HUD/WB_TurretHealth1` (`WidgetComponent.GetWidget` (`self.Widget`))))
            (set `Widget.RenderOpacity` 0.0 (`/Game/HUD/WB_TurretHealth1.CdBar` _aswb_turret_health_1_6))))))))

(fn `UserConstructionScript`
  (`parent.UserConstructionScript`)
  (bind _returnvalue (`PrimitiveComponent.CreateDynamicMaterialInstance` (`self.Body`) 1 null "None"))
  (set `self.ChargeMaterial` _returnvalue)
  (bind _returnvalue_2 (`PrimitiveComponent.CreateDynamicMaterialInstance` (`self.Storage`) 0 null "None"))
  (set `self.StorageMaterial` _returnvalue_2))

(fn `WhichInteraction`
  (returns (TypeInteraction :type "/Game/Blueprint/Enum/EInteractable Enum"))
  (return "NewEnumerator0"))