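; BP_Turret_Gun is a gun turret Blueprint that alternates between firing and resting for as long as it runs.
; BeginPlay calls the parent, then starts Fire, which sets IsFiring, waits FireTime and calls Rest.
; Rest clears the flag, waits RestTime and calls Fire again, forming an endless delay-driven loop.
; This graph only toggles IsFiring and contains no shooting logic.
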(event `Fire`
  (set `self.IsFiring` true)
  (`KismetSystemLibrary.Delay` (`self.FireTime`))
  (`self.Rest`))

(event `Rest`
  (set `self.IsFiring` false)
  (`KismetSystemLibrary.Delay` (`self.RestTime`))
  (`self.Fire`))

(event `self.ReceiveBeginPlay`
  (`parent.ReceiveBeginPlay`)
  (`self.Fire`))

(fn `UserConstructionScript`
  (`parent.UserConstructionScript`))