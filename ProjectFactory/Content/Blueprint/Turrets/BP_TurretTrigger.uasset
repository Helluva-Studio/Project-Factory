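; Interactable turret build spot that previews the player's selected turret on focus and spawns the real one on purchase.
; BPC_TurretSelectionSystem picks the preview, DT_TurretsCosts determines affordability, and enemies or the player inside NoBuildCollision block building.
; Building puts the spot in cooldown and hides it, passing itself to the turret as Trigger.
; Reactivation shows it again and runs a reversed timeline driving world and minimap radial timers before re-enabling building.
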(event `self.ReceiveBeginPlay`
  (`|ExecutionSequence`
    (:`then_0`
      (`ActorComponent.K2_DestroyComponent` (`self.PreRange`))
      (`self.UpdateBoss`)
      (`SceneComponent.K2_SetWorldRotation` (`self.MinimapIcon`) (struct :`Yaw` 90.0) false false))
    (:`then_1`
      (bind (_as_normal_widget _as_minimap_widget) (`self.GetReactivationTrigger`))
      (`|ExecutionSequence`
        (:`then_0`
          (bind _radialslider (`/Game/Blueprint/Turrets/TurretFeature/TurretTrigger/WB_ReactivationTime.RadialSlider` _as_normal_widget))
          (`/Engine/EditorBlueprintResources/StandardMacros.IsValid` _radialslider
            (:`Is Valid`
              (set `Widget.RenderOpacity` 0.0 _radialslider))))
        (:`then_1`
          (bind _radialslider_2 (`/Game/Blueprint/Turrets/TurretFeature/TurretTrigger/WB_ReactivationTime.RadialSlider` _as_minimap_widget))
          (`/Engine/EditorBlueprintResources/StandardMacros.IsValid` _radialslider_2
            (:`Is Valid`
              (set `Widget.RenderOpacity` 0.0 _radialslider_2))))))
    (:`then_2`
      (set `self.IsInCooldown` false)
      (set `self.CanBuild` true))))

(event `Reactivation`
  (`self.SetActorHiddenInGame` false)
  (`SceneComponent.SetVisibility` (`self.MinimapIcon`) true true)
  (`TimelineComponent.SetPlayRate` (`self.ReactivationTimeline`) (`KismetMathLibrary.SafeDivide` 1.0 (`self.MaxReactivationTime`)))
  (bind (_as_normal_widget _as_minimap_widget) (`self.GetReactivationTrigger`))
  (set `Widget.RenderOpacity` 1.0 (`/Game/Blueprint/Turrets/TurretFeature/TurretTrigger/WB_ReactivationTime.RadialSlider` _as_normal_widget))
  (set `Widget.RenderOpacity` 1.0 (`/Game/Blueprint/Turrets/TurretFeature/TurretTrigger/WB_ReactivationTime.RadialSlider` _as_minimap_widget))
  (bind (_direction _reactivationpercentagenormalized) (`Timeline|ReactivationTimeline` :!via `ReverseFromEnd`)
    (:`Update`
      (bind (_as_normal_widget_2 _as_minimap_widget_2) (`self.GetReactivationTrigger`))
      (set `/Game/Blueprint/Turrets/TurretFeature/TurretTrigger/WB_ReactivationTime.CurrentValue` _reactivationpercentagenormalized _as_normal_widget_2)
      (set `/Game/Blueprint/Turrets/TurretFeature/TurretTrigger/WB_ReactivationTime.CurrentValue` _reactivationpercentagenormalized _as_minimap_widget_2))
    (:`Finished`
      (bind (_as_normal_widget_3 _as_minimap_widget_3) (`self.GetReactivationTrigger`))
      (set `Widget.RenderOpacity` 0.0 (`/Game/Blueprint/Turrets/TurretFeature/TurretTrigger/WB_ReactivationTime.RadialSlider` _as_normal_widget_3))
      (set `Widget.RenderOpacity` 0.0 (`/Game/Blueprint/Turrets/TurretFeature/TurretTrigger/WB_ReactivationTime.RadialSlider` _as_minimap_widget_3))
      (set `self.IsInCooldown` false)
      (set `self.CanBuild` true)
      (`self.UpdateBoss`))))

(event `/Game/Blueprint/InteractionArea/BPI_Focusable.ToggleFocus`
  (params (Focus :type Boolean))
  (bind _turretpreviewed (`self.TurretPreviewed`))
  (if (and Focus (not (`self.IsInCooldown`)))
    (`/Engine/EditorBlueprintResources/StandardMacros.DoOnce` false :!label _label
      (:`Completed`
        (add `/Game/Blueprint/Robot/Blueprints/BPC_TurretSelectionSystem.OnTurretSelectedChange` (`self.GetComponentByClass` (`GameplayStatics.GetPlayerPawn` 0) "/Game/Blueprint/Robot/Blueprints/BPC_TurretSelectionSystem.BPC_TurretSelectionSystem_C") (delegate `SpawnPreview`))
        (`self.SpawnPreview`)))
    (else
      (`/Engine/EditorBlueprintResources/StandardMacros.IsValid` _turretpreviewed :!label _label_2
        (:`Is Valid`
          (`/Game/Blueprint/Turrets/TurretFeature/TurretTrigger/TurretPreview/BP_TurretPreview.Dissolve` _turretpreviewed false true))
        (:`Is Not Valid`
          (clear `/Game/Blueprint/Robot/Blueprints/BPC_TurretSelectionSystem.OnTurretSelectedChange` (`self.GetComponentByClass` (`GameplayStatics.GetPlayerPawn` 0) "/Game/Blueprint/Robot/Blueprints/BPC_TurretSelectionSystem.BPC_TurretSelectionSystem_C"))))
      (`self.ResetPreview`))))

(event `self.Sphere.OnComponentEndOverlap`
  (params (OverlappedComponent :type "PrimitiveComponent Object Reference") (OtherActor :type "Actor Object Reference") (OtherComp :type "PrimitiveComponent Object Reference") (OtherBodyIndex :type Integer))
  (if (== OtherActor (`GameplayStatics.GetPlayerPawn` 0))
    (goto _label_2)))

(event `SpawnPreview`
  (bind (_haveresourcetobuild _turretselected _level _turret_type) (`self.GetTurretSelected`))
  (`/Engine/EditorBlueprintResources/StandardMacros.IsValid` (`self.TurretPreviewed`)
    (:`Is Valid`
      (`self.ResetPreview`)
      (`self.K2_DestroyActor` (`self.TurretPreviewed`)))
    (:`Is Not Valid`
      _))
  (`/Engine/EditorBlueprintResources/StandardMacros.DoOnce` false :!label _label_3
    (:`Completed`
      (bind _returnvalue (`|SpawnActorFromClass` _turretselected (`KismetMathLibrary.MakeTransform` (`self.K2_GetActorLocation`)) "AlwaysSpawn" "MultiplyWithRoot" null _level _turret_type (and _haveresourcetobuild (`self.CanBuild`)) null))
      (set `self.TurretPreviewed` _returnvalue))))

(event `ResetPreview`
  (`|ExecutionSequence`
    (:`then_0`
      (goto _label :!via `Reset`))
    (:`then_1`
      (goto _label_3 :!via `Reset`))
    (:`then_2`
      (goto _label_4 :!via `Reset`))))

(event `/Game/Blueprint/Turrets/Interfaces/BI_Interactable.InteractPurchaseWithTurret`
  (params (TurreetToSpawn :type "/Game/Blueprint/Turrets/BP_Turret_Base Class Reference") (Level :type Integer))
  (if (`self.CanBuild`)
    (`/Engine/EditorBlueprintResources/StandardMacros.DoOnce` false :!label _label_4
      (:`Completed`
        (`|SpawnActorFromClass` TurreetToSpawn (`KismetMathLibrary.MakeTransform` (`self.K2_GetActorLocation`)) "AlwaysSpawn" "MultiplyWithRoot" null Level self null)
        (set `self.IsInCooldown` true)
        (`SceneComponent.SetVisibility` (`self.MinimapIcon`) false true)
        (`/Engine/EditorBlueprintResources/StandardMacros.IsValid` (`self.TurretPreviewed`)
          (:`Is Valid`
            (`/Game/Blueprint/Turrets/TurretFeature/TurretTrigger/TurretPreview/BP_TurretPreview.Dissolve` (`self.TurretPreviewed`) false true)
            (clear `/Game/Blueprint/Robot/Blueprints/BPC_TurretSelectionSystem.OnTurretSelectedChange` (`self.GetComponentByClass` (`GameplayStatics.GetPlayerPawn` 0) "/Game/Blueprint/Robot/Blueprints/BPC_TurretSelectionSystem.BPC_TurretSelectionSystem_C"))
            (`self.ResetPreview`))
          (:`Is Not Valid`
            (`self.UpdateBoss`)))
        (`KismetSystemLibrary.Delay` 1.0)
        (`self.SetActorHiddenInGame` true)))))

(event `UpdateBoss`)

(event `self.NoBuildCollision.OnComponentBeginOverlap`
  (params (OverlappedComponent :type "PrimitiveComponent Object Reference") (OtherActor :type "Actor Object Reference") (OtherComp :type "PrimitiveComponent Object Reference") (OtherBodyIndex :type Integer) (bFromSweep :type Boolean) (SweepResult :type "HitResult Structure (by ref)"))
  (bind _turretpreviewed (`self.TurretPreviewed`))
  (if (and (or (`KismetSystemLibrary.DoesImplementInterface` OtherActor "/Game/Blueprint/Enemies/Interfaces/BPI_Enemy.BPI_Enemy_C") (== OtherActor (`GameplayStatics.GetPlayerPawn` 0))) (not (`self.IsInCooldown`)))
    (set `self.CanBuild` false)
    (`/Engine/EditorBlueprintResources/StandardMacros.IsValid` _turretpreviewed
      (:`Is Valid`
        (`/Game/Blueprint/Turrets/TurretFeature/TurretTrigger/TurretPreview/BP_TurretPreview.SetPreview` _turretpreviewed (and (`self.GetTurretSelected`) (`self.CanBuild`)))))))

(event `self.NoBuildCollision.OnComponentEndOverlap`
  (params (OverlappedComponent :type "PrimitiveComponent Object Reference") (OtherActor :type "Actor Object Reference") (OtherComp :type "PrimitiveComponent Object Reference") (OtherBodyIndex :type Integer))
  (bind _turretpreviewed (`self.TurretPreviewed`))
  (if (and (or (`KismetSystemLibrary.DoesImplementInterface` OtherActor "/Game/Blueprint/Enemies/Interfaces/BPI_Enemy.BPI_Enemy_C") (== OtherActor (`GameplayStatics.GetPlayerPawn` 0))) (not (`self.IsInCooldown`)))
    (set `self.CanBuild` true)
    (`/Engine/EditorBlueprintResources/StandardMacros.IsValid` _turretpreviewed
      (:`Is Valid`
        (`/Game/Blueprint/Turrets/TurretFeature/TurretTrigger/TurretPreview/BP_TurretPreview.SetPreview` _turretpreviewed (and (`self.GetTurretSelected`) (`self.CanBuild`)))))))

(fn `CanInteract`
  (returns (CanInteract :type Boolean))
  (return (and (not (`self.IsInCooldown`)) (`self.CanBuild`) (`self.GetTurretSelected`))))

(fn `GetCost`
  (returns (GetCost :type "Float (double-precision)"))
  (return 0.0))

(fn `GetInteractImage`
  (returns (Image :type "Texture Object Reference"))
  (return "/Game/2DImage/costruisci.costruisci"))

(fn `GetInteractMessage`
  (returns (InteractMessage :type Text) (Image :type "Texture Object Reference"))
  (return "" null))

(fn `GetReactivationTrigger`
  (returns (`As Normal Widget` :type "/Game/Blueprint/Turrets/TurretFeature/TurretTrigger/WB_ReactivationTime Object Reference") (`As Minimap Widget` :type "/Game/Blueprint/Turrets/TurretFeature/TurretTrigger/WB_ReactivationTime Object Reference"))
  (bind _aswb_reactivation_time (cast `/Game/Blueprint/Turrets/TurretFeature/TurretTrigger/WB_ReactivationTime` (`WidgetComponent.GetWidget` (`self.ReactivationWidget`))))
  (bind _aswb_reactivation_time_2 (cast `/Game/Blueprint/Turrets/TurretFeature/TurretTrigger/WB_ReactivationTime` (`WidgetComponent.GetWidget` (`self.MinimapReactivationWidget`))))
  (return _aswb_reactivation_time _aswb_reactivation_time_2))

(fn `GetTurretSelected`
  (returns (HaveResourceToBuild :type Boolean) (TurretSelected :type "/Game/Blueprint/Turrets/TurretFeature/TurretTrigger/TurretPreview/BP_TurretPreview Class Reference") (Level :type Integer) (`Turret Type` :type "/Game/Blueprint/Turrets/TurretGetter/E_TurretType Enum"))
  (bind _previewactors (`self.PreviewActors`))
  (bind _returnvalue (`self.GetComponentByClass` (`GameplayStatics.GetPlayerPawn` 0) "/Game/Blueprint/Robot/Blueprints/BPC_TurretSelectionSystem.BPC_TurretSelectionSystem_C"))
  (bind _turretselected (`/Game/Blueprint/Robot/Blueprints/BPC_TurretSelectionSystem.TurretSelected` _returnvalue))
  (bind (_currenthealth _maxhealth _healthlostovertime _healthrepairpercentage _currentlevel _maxlevel _maxactivitytime_nofarm_ _activitytime_nofarm_ _maxcdtime _cdtime _isinfunction_nofarm_ _isincooldown _turrettype) (defaults `Object` _turretselected))
  (bind _value (`BlueprintMapLibrary.Map_Find` (`/Game/Blueprint/Robot/Blueprints/BPC_TurretSelectionSystem.TurretLevel` _returnvalue) _turrettype))
  (bind _keys (`BlueprintMapLibrary.Map_Keys` _previewactors))
  (bind _values (`BlueprintMapLibrary.Map_Values` _previewactors))
  (bind _returnvalue_2 (`|GetDataTableRow` "/Game/Blueprint/Turrets/TurretFeature/Leveling/DT_TurretsCosts.DT_TurretsCosts" (`KismetStringLibrary.Conv_StringToName` (`KismetStringLibrary.Conv_IntToString` (+ _value (* (`KismetMathLibrary.Conv_ByteToInt` _turrettype) 3)))))
    (:`then`
      (bind _executioncompleted (`/Game/Blueprint/Robot/Blueprints/BP_Roberto.CanTakeResource` (cast `/Game/Blueprint/Robot/Blueprints/BP_Roberto` (`GameplayStatics.GetPlayerPawn` 0) :!pure true) (`.C-Gear_20_453F455A469FF81F4137AC90709ACBBF` (break `/Game/Blueprint/Turrets/TurretFeature/Leveling/S_TurretCosts` _returnvalue_2)) (`.C-Steel_22_986F2BC24314E28AC5F7BBAFC0CDB194` (break `/Game/Blueprint/Turrets/TurretFeature/Leveling/S_TurretCosts` _returnvalue_2)) (`.C-Circuit_24_810DF48F451A9E27CB15FC8E077EA828` (break `/Game/Blueprint/Turrets/TurretFeature/Leveling/S_TurretCosts` _returnvalue_2))))
      (return _executioncompleted (`|GetArrayItem` _values (`KismetArrayLibrary.Array_Find` _keys _turretselected)) _value _turrettype))))

(fn `UserConstructionScript`
  (`SceneComponent.SetWorldScale3D` (`self.PreRange`) (`KismetMathLibrary.Conv_DoubleToVector` (/ (`self.RangePreview`) 100.0))))

(fn `WhichInteraction`
  (returns (TypeInteraction :type "/Game/Blueprint/Enum/EInteractable Enum"))
  (return "NewEnumerator2"))