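; Essence-farming turret that fills an internal tank over time and releases it as BP_Essence pickups when interacted with.
; A recursive delayed Farming event adds essence until the tank is full, then stops and makes interaction available at zero cost.
; Interact spawns essence actors at random nearby offsets, each initialized with EssenceValue, then empties the tank and restarts farming.
; Widget visibility and camera-facing logic is disconnected, and the box overlap events are empty.
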(event `self.ReceiveBeginPlay`
  (`parent.ReceiveBeginPlay`)
  (`self.Farming`))

(event `self.ReceiveTick`
  (params (DeltaSeconds :type "Float (single-precision)"))
  (`parent.ReceiveTick` DeltaSeconds))

(event `Farming`
  (`KismetSystemLibrary.Delay` (`self.Time`))
  (bind _output_get (set `self.Tank` (+ (`self.Tank`) (`self.Essence/Time`))))
  (if (>= _output_get (`self.TankSize`))
    (set `self.IsTankFull` true)
    (else
      (`self.Farming`))))

(event `/Game/Blueprint/Turrets/Interfaces/BI_Interactable.Interact`
  (if (`self.IsTankFull`)
    (for _ (range (`KismetMathLibrary.FTrunc` (/ (`self.TankSize`) (`self.EssenceValue`))))
      (`self.SpawnEssence`))
    (set `self.IsTankFull` false)
    (set `self.Tank` 0.0)
    (`self.Farming`)))

(event `self.Box.OnComponentBeginOverlap`
  (params (OverlappedComponent :type "PrimitiveComponent Object Reference") (OtherActor :type "Actor Object Reference") (OtherComp :type "PrimitiveComponent Object Reference") (OtherBodyIndex :type Integer) (bFromSweep :type Boolean) (SweepResult :type "HitResult Structure (by ref)")))

(event `self.Box.OnComponentEndOverlap`
  (params (OverlappedComponent :type "PrimitiveComponent Object Reference") (OtherActor :type "Actor Object Reference") (OtherComp :type "PrimitiveComponent Object Reference") (OtherBodyIndex :type Integer)))

(fn `CanInteract`
  (returns (CanInteract :type Boolean))
  (return (`self.IsTankFull`)))

(fn `GetCost`
  (returns (GetCost :type "Float (double-precision)"))
  (return 0.0))

(fn `SpawnEssence`
  (bind _returnvalue (`|SpawnActorFromClass` "/Game/Blueprint/Essence/BP_Essence.BP_Essence_C" (`KismetMathLibrary.MakeTransform` (`KismetMathLibrary.TransformLocation` (`self.GetTransform`) (`KismetMathLibrary.MakeVector` (`KismetMathLibrary.Conv_IntToDouble` (`KismetMathLibrary.RandomIntegerInRange` -100 100)) (`KismetMathLibrary.Conv_IntToDouble` (`KismetMathLibrary.RandomIntegerInRange` -100 100)) 50.0))) "AdjustIfPossibleButAlwaysSpawn" "MultiplyWithRoot" null null))
  (`/Engine/EditorBlueprintResources/StandardMacros.IsValid` _returnvalue
    (:`Is Valid`
      (`/Game/Blueprint/Essence/BP_Essence.Initialize` _returnvalue (`self.EssenceValue`)))))

(fn `UserConstructionScript`
  (`parent.UserConstructionScript`))

(fn `WhichInteraction`
  (returns (TypeInteraction :type "/Game/Blueprint/Enum/EInteractable Enum"))
  (return "NewEnumerator0"))