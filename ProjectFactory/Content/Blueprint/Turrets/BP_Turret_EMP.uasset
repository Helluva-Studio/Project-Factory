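; EMP turret Blueprint that adds animated ring visuals, with its parent class supplying the inherited Tick behavior.
; While not in cooldown, Tick spins three rings, the small one opposite the others, and bobs them with a time-based sine offset.
; LevelUp reveals one more ring per level and repositions the medium ring at the upper two levels.
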(event `self.ReceiveTick`
  (params (DeltaSeconds :type "Float (single-precision)"))
  (`parent.ReceiveTick` DeltaSeconds)
  (if (not (`self.IsInCooldown`))
    (`self.RingRotation`)))

(event `RingRotation`
  (`/Engine/EditorBlueprintResources/StandardMacros.IsValid` self
    (:`Is Valid`
      (`SceneComponent.K2_AddWorldRotation` (`self.BigRing`) (struct :`Yaw` 1.0) false false)
      (`SceneComponent.K2_AddWorldRotation` (`self.MediumRing`) (struct :`Yaw` 1.0) false false)
      (`SceneComponent.K2_AddWorldRotation` (`self.SmallRing`) (struct :`Yaw` -1.0) false false)
      (`SceneComponent.K2_AddWorldOffset` (`self.BigRing`) (`KismetMathLibrary.MakeVector` 0.0 0.0 (/ (`KismetMathLibrary.DegSin` (* (`self.GetGameTimeSinceCreation`) 200.0)) 20.0)) false false)
      (`SceneComponent.K2_AddWorldOffset` (`self.SmallRing`) (`KismetMathLibrary.MakeVector` 0.0 0.0 (/ (`KismetMathLibrary.DegSin` (* (`self.GetGameTimeSinceCreation`) 200.0)) 30.0)) false false)
      (`SceneComponent.K2_AddWorldOffset` (`self.MediumRing`) (`KismetMathLibrary.MakeVector` 0.0 0.0 (/ (`KismetMathLibrary.DegSin` (* (`self.GetGameTimeSinceCreation`) 200.0)) 10.0)) false false))))

(event `self.LevelUp`
  (params (Level :type Integer))
  (`/Engine/EditorBlueprintResources/StandardMacros.IsValid` self
    (:`Is Valid`
      (switch `int` Level
        (:`1`
          (`SceneComponent.SetVisibility` (`self.SmallRing`) true false)
          (`SceneComponent.SetVisibility` (`self.MediumRing`) false false)
          (`SceneComponent.SetVisibility` (`self.BigRing`) false false))
        (:`2`
          (`SceneComponent.SetVisibility` (`self.SmallRing`) true false)
          (`SceneComponent.SetVisibility` (`self.MediumRing`) true false)
          (`SceneComponent.SetVisibility` (`self.BigRing`) false false)
          (`SceneComponent.K2_SetRelativeLocation` (`self.MediumRing`) (0.0 0.0 30.0) false false))
        (:`3`
          (`SceneComponent.SetVisibility` (`self.SmallRing`) true false)
          (`SceneComponent.SetVisibility` (`self.MediumRing`) true false)
          (`SceneComponent.SetVisibility` (`self.BigRing`) true false)
          (`SceneComponent.K2_SetRelativeLocation` (`self.MediumRing`) (0.0 0.0 80.0) false false))))))

(fn `UserConstructionScript`
  (`parent.UserConstructionScript`))