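; BP_CCTurret is a turret that applies a crowd-control area effect through a spawned effect ammo actor.
; Tick uses paired DoOnce gates to destroy the effect when cooldown starts and spawn one when it ends.
; SpawnAoe picks the ammo class by CcType from the EffectAmmos map, attaches it to Center and passes it the effect settings.
; Death also destroys the active effect.
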(event `self.ReceiveBeginPlay`
  (`parent.ReceiveBeginPlay`))

(event `self.ReceiveTick`
  (params (DeltaSeconds :type "Float (single-precision)"))
  (`parent.ReceiveTick` DeltaSeconds)
  (if (`self.IsInCooldown`)
    (`/Engine/EditorBlueprintResources/StandardMacros.DoOnce` false :!label _label
      (:`Completed`
        (`/Engine/EditorBlueprintResources/StandardMacros.IsValid` (`self.EffectAmmo`)
          (:`Is Valid`
            (`self.K2_DestroyActor` (`self.EffectAmmo`))
            (goto _label_2 :!via `Reset`)))))
    (else
      (`/Engine/EditorBlueprintResources/StandardMacros.DoOnce` false :!label _label_2
        (:`Completed`
          (`self.SpawnAoe`)
          (goto _label :!via `Reset`))))))

(event `SpawnAoe`
  (bind _keys (`BlueprintMapLibrary.Map_Keys` (`self.EffectAmmos`)))
  (bind _values (`BlueprintMapLibrary.Map_Values` (`self.EffectAmmos`)))
  (bind _returnvalue (`|SpawnActorFromClass` (`|GetArrayItem` _values (`KismetArrayLibrary.Array_Find` _keys (`self.CcType`))) (`KismetMathLibrary.MakeTransform` (`SceneComponent.K2_GetComponentLocation` (`self.Center`)) (struct) (0.0 0.0 0.0)) "AdjustIfPossibleButAlwaysSpawn" "MultiplyWithRoot" null null))
  (bind _output_get (set `self.EffectAmmo` _returnvalue))
  (`/Engine/EditorBlueprintResources/StandardMacros.IsValid` _output_get
    (:`Is Valid`
      (`self.K2_AttachToComponent` _output_get (`self.Center`) "None" "KeepWorld" "KeepRelative" "KeepWorld" true)
      (message `/Game/Blueprint/Turrets/Interfaces/BPI_TurretCcAmmo.InitializeCcAmmo` _returnvalue (`self.CanHitPlayer`) (`self.CcType`) (`self.TypeOfAoe`) (`self.MaxAngleOfEffect(Cone)`) (`self.MaxDistance(Cone)/MaxRadius(Sphere)`) (`self.TimeTick`) (`self.SlowEffect`) (`self.StunDuration`) (`self.GravityForce`)))))

(fn `Death`
  (bind _effectammo (`self.EffectAmmo`))
  (`/Engine/EditorBlueprintResources/StandardMacros.IsValid` _effectammo
    (:`Is Valid`
      (`self.K2_DestroyActor` _effectammo))
    (:`Is Not Valid`
      _))
  (`parent.Death`))

(fn `UserConstructionScript`
  (`parent.UserConstructionScript`))