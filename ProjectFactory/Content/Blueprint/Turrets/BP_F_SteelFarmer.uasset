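; Steel farmer turret, a resource-producing turret configured from the DT_F_TurretSteel data table.
; InitializeTurret looks up the row named after CurrentLevel, copies health, repair, charge, cooldown, storage and resource spawn stats, then enables tick and marks itself initialized.
; Construction defers to the parent, GetCost returns zero and WhichInteraction returns a fixed enum value.
; The graphs here only configure the turret and contain no spawning logic.
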(fn `GetCost`
  (returns (GetCost :type "Float (double-precision)"))
  (return 0.0))

(fn `InitializeTurret`
  (bind _returnvalue (`|GetDataTableRow` "/Game/Blueprint/Turrets/TurretFeature/Leveling/DataTable/DT_F_TurretSteel.DT_F_TurretSteel" (`KismetStringLibrary.Conv_StringToName` (`KismetStringLibrary.Conv_IntToString` (`self.CurrentLevel`))))
    (:`then`
      (bind (_baseturrettype _maxhealth _basehealthrepairpercentage _constructioncostgsc _baserepaircostgsc _chargetimeperresource _cdtimeperresource _maxresourcestored _baseresourcespawnrate _baseresourcedistancefromturret _baseresourcetospawn _resourcevalue) (break `/Game/Blueprint/Turrets/TurretFeature/Leveling/DONTUSE_TurretStructs/S_F_TurretFarmStats` _returnvalue))
      (bind _output_get (set `self.MaxHealth` _maxhealth))
      (set `self.CurrentHealth` _output_get)
      (set `self.HealthRepairPercentage` _basehealthrepairpercentage)
      (set `self.ChargeTimePerResource` _chargetimeperresource)
      (set `self.CdTimePerResource` _cdtimeperresource)
      (set `self.MaxResourceStored` _maxresourcestored)
      (set `self.TimeBetweenResourceSpawn` _baseresourcespawnrate)
      (set `self.SpawnDistanceFromTurret` _baseresourcedistancefromturret)
      (set `self.ResourceToSpawn` _baseresourcetospawn)
      (set `self.ResourceValue` _resourcevalue)
      (`self.SetActorTickEnabled` true)
      (set `self.IsInitialized` true))))

(fn `UserConstructionScript`
  (`parent.UserConstructionScript`))

(fn `WhichInteraction`
  (returns (TypeInteraction :type "/Game/Blueprint/Enum/EInteractable Enum"))
  (return "NewEnumerator0"))