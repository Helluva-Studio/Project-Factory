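; Turret crowd-control AoE actor that acts as a gravity well, periodically pulling nearby enemies toward its location.
; Initialization stores the settings, calls SetAoe and starts a looping timer that sphere-traces for enemy pawns and sends each an AttractionMessage.
; GetGravityForceVector computes a horizontal pull that weakens with distance, capped so enemies stop at MinRange instead of overshooting.
; A debug PrintString of the force remains in that function.
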(event `/Game/Blueprint/Turrets/Interfaces/BPI_TurretCcAmmo.InitializeGravityAmmo`
  (params (CanHitPlayer :type Boolean) (CcType :type "/Game/Blueprint/Turrets/TurretFeature/Aoe/E_CcType Enum" :default "NewEnumerator5") (TypeOfAoe :type "/Game/Blueprint/Turrets/TurretFeature/Aoe/E_AoeType Enum" :default "NewEnumerator3") (`MaxDistance(Cone)/MaxRadius(Sphere)` :type "Float (double-precision)") (GravityForce :type "Float (double-precision)") (MinGravityForcePercentage :type "Float (double-precision)") (GravityTick :type "Float (double-precision)"))
  (set `self.CanHitPlayer` CanHitPlayer)
  (set `self.CcType` CcType)
  (set `self.TypeOfAoe` TypeOfAoe)
  (set `self.MaxDistance(Cone)/MaxRadius(Sphere)` `MaxDistance(Cone)/MaxRadius(Sphere)`)
  (set `self.GravityForce` GravityForce)
  (set `self.Min Gravity Force Percentage` MinGravityForcePercentage)
  (set `self.GravityTick` GravityTick)
  (`self.SetAoe`)
  (`KismetSystemLibrary.K2_SetTimerDelegate` (delegate `DoGravity`) (`self.GravityTick`) true))

(event `DoGravity`
  (bind _returnvalue (`self.K2_GetActorLocation`))
  (bind _outhits (`KismetSystemLibrary.SphereTraceMultiForObjects` _returnvalue _returnvalue (`self.MaxDistance(Cone)/MaxRadius(Sphere)`) (`|MakeArray` "ObjectTypeQuery3" :!type "EObjectTypeQuery Enum")))
  (for _array_element _outhits
    (bind (_bblockinghit _binitialoverlap _time _distance _location _impactpoint _normal _impactnormal _physmat _hitactor) (`GameplayStatics.BreakHitResult` _array_element))
    (if (`KismetSystemLibrary.DoesImplementInterface` _hitactor "/Game/Blueprint/Enemies/Interfaces/BPI_Enemy.BPI_Enemy_C")
      (bind _asbp_base_enemy (cast `/Game/Blueprint/Enemies/BP_BaseEnemy` _hitactor))
      (`KismetArrayLibrary.Array_AddUnique` (`self.AttractedEnemies`) _asbp_base_enemy)))
  (for _array_element_2 (`self.AttractedEnemies`)
    (`/Engine/EditorBlueprintResources/StandardMacros.IsValid` _array_element_2
      (:`Is Valid`
        (message `/Game/Blueprint/Enemies/Interfaces/BPI_Enemy.Attraction` _array_element_2 (`self.GravityTick`) (`self.K2_GetActorLocation` _array_element_2) (`self.GetGravityForceVector` _array_element_2)))))
  (`KismetArrayLibrary.Array_Clear` (`self.AttractedEnemies`)))

(fn `GetGravityForceVector`
  (params (Actor :type "Actor Object Reference"))
  (returns (Force :type "Vector Structure"))
  (locals (MinRange :type "Float (double-precision)" :default 100.0))
  (bind (_returnvalue_x _returnvalue_y) (`KismetMathLibrary.BreakVector` (`self.K2_GetActorLocation`)))
  (bind (_returnvalue_x_2 _returnvalue_y_2) (`KismetMathLibrary.BreakVector` (`self.K2_GetActorLocation` Actor)))
  (bind _minrange (`local.MinRange`))
  (bind _gravityforce (`self.GravityForce`))
  (bind (_returnvalue_x_3 _returnvalue_y_3) (`KismetMathLibrary.BreakVector` (- (`self.K2_GetActorLocation`) (`self.K2_GetActorLocation` Actor))))
  (bind _returnvalue (`KismetMathLibrary.Vector_Distance` (`KismetMathLibrary.MakeVector` _returnvalue_x _returnvalue_y) (`KismetMathLibrary.MakeVector` _returnvalue_x_2 _returnvalue_y_2)))
  (bind _returnvalue_2 (`KismetMathLibrary.Normal` (`KismetMathLibrary.MakeVector` _returnvalue_x_3 _returnvalue_y_3)))
  (bind _returnvalue_3 (`KismetMathLibrary.MapRangeClamped` _returnvalue (`local.MinRange`) (`self.MaxDistance(Cone)/MaxRadius(Sphere)`) _gravityforce (* _gravityforce (/ (`self.Min Gravity Force Percentage`) 100.0))))
  (`KismetSystemLibrary.PrintString` (`KismetStringLibrary.Conv_DoubleToString` _returnvalue_3))
  (if (< (- _returnvalue _returnvalue_3) _minrange)
    (return (* (- _returnvalue _minrange) _returnvalue_2))
    (else
      (return (* _returnvalue_3 _returnvalue_2)))))

(fn `UserConstructionScript`
  (`parent.UserConstructionScript`))