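; Base actor for turret area-of-effect damage, configured through InitializeDamageAmmo, which then calls an empty DoDamage event, likely for children to override.
; Enemies, and optionally the player, entering the AOE component take on-hit damage and start damage over time through BPC_DamageSystem, stopped on exit.
; Damage over time falls off with distance, computed once at overlap.
; Cone and chain settings are stored but, apart from maximum range, unused here.
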(event `self.AOE.OnComponentBeginOverlap`
  (params (OverlappedComponent :type "PrimitiveComponent Object Reference") (OtherActor :type "Actor Object Reference") (OtherComp :type "PrimitiveComponent Object Reference") (OtherBodyIndex :type Integer) (bFromSweep :type Boolean) (SweepResult :type "HitResult Structure (by ref)"))
  (bind _damageovertime (`self.DamageOverTime`))
  (if (`KismetSystemLibrary.DoesImplementInterface` OtherActor "/Game/Blueprint/Enemies/Interfaces/BPI_Enemy.BPI_Enemy_C")
    (message `/Game/Blueprint/Interfaces/BPI_Damageable.TakeDamageOverTime` (`self.GetComponentByClass` OtherActor "/Game/Blueprint/DamageSystem/BPC_DamageSystem.BPC_DamageSystem_C") (`self.TimeTick`) (`KismetMathLibrary.MapRangeClamped` (`KismetMathLibrary.Vector_Distance` (`self.K2_GetActorLocation` OtherActor) (`self.K2_GetActorLocation`)) (`KismetMathLibrary.SelectFloat` 60.0 0.0 (== (`self.TypeOfAoe`) 1)) (`self.MaxDistance(Cone)/MaxRadius(Sphere)`) _damageovertime (* _damageovertime (/ (- 100.0 (`self.DamageReduction`)) 100.0))) self (`self.DamageType`) :!label _label)
    (`GameplayStatics.ApplyDamage` OtherActor (`self.DamageOnHit`) null (`self.Instigator`))
    (elif (and (`self.CanHitPlayer`) (== OtherActor (`GameplayStatics.GetPlayerPawn` 0)))
      (goto _label))))

(event `self.AOE.OnComponentEndOverlap`
  (params (OverlappedComponent :type "PrimitiveComponent Object Reference") (OtherActor :type "Actor Object Reference") (OtherComp :type "PrimitiveComponent Object Reference") (OtherBodyIndex :type Integer))
  (if (`KismetSystemLibrary.DoesImplementInterface` OtherActor "/Game/Blueprint/Enemies/Interfaces/BPI_Enemy.BPI_Enemy_C")
    (message `/Game/Blueprint/Interfaces/BPI_Damageable.StopDamageOverTime` (`self.GetComponentByClass` OtherActor "/Game/Blueprint/DamageSystem/BPC_DamageSystem.BPC_DamageSystem_C") (`self.DamageType`) self :!label _label_2)
    (elif (and (`self.CanHitPlayer`) (== OtherActor (`GameplayStatics.GetPlayerPawn` 0)))
      (goto _label_2))))

(event `/Game/Blueprint/Turrets/Interfaces/BPI_TurretDamageAmmo.InitializeDamageAmmo`
  (params (CanHitPlayer :type Boolean) (DamageType :type "/Game/Blueprint/Interfaces/E_DamageType Enum" :default "NewEnumerator4") (TypeOfAoe :type "/Game/Blueprint/Turrets/TurretFeature/Aoe/E_AoeType Enum" :default "NewEnumerator3") (`MaxAngleOfEffect(Cone)` :type "Float (double-precision)") (`MaxDistance(Cone)/MaxRadius(Sphere)` :type "Float (double-precision)") (DamageTick :type "Float (double-precision)") (DamageOnHit :type "Float (double-precision)") (DamageOverTime :type "Float (double-precision)") (DamageReduction :type "Float (double-precision)") (NumberOfTarget :type Integer) (RangeReductionPerTarget :type "Float (double-precision)") (TimeBetweenChain :type "Float (double-precision)"))
  (set `self.CanHitPlayer` CanHitPlayer)
  (set `self.DamageType` DamageType)
  (set `self.TypeOfAoe` TypeOfAoe)
  (set `self.MaxAngleOfEffect(Cone)` `MaxAngleOfEffect(Cone)`)
  (set `self.MaxDistance(Cone)/MaxRadius(Sphere)` `MaxDistance(Cone)/MaxRadius(Sphere)`)
  (set `self.DamageOnHit` DamageOnHit)
  (set `self.TimeTick` DamageTick)
  (set `self.DamageOverTime` DamageOverTime)
  (set `self.DamageReduction` DamageReduction)
  (set `self.NumberOfTarget` NumberOfTarget)
  (set `self.RangeReductionPerTarget` RangeReductionPerTarget)
  (set `self.TimeBetweenStrike` TimeBetweenChain)
  (`self.DoDamage`))

(event `DoDamage`)

(fn `UserConstructionScript`
  (`parent.UserConstructionScript`))