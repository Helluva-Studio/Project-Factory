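; BP_CcStun is an area-of-effect crowd-control turret feature that stuns enemies.
; On DoEffect it calls the parent, then walks the enemies overlapping its AOE in reverse and sends EmpCCMessage with StunDuration to each BPI_Enemy implementer.
; BeginPlay and Tick only defer to the parent; the empty DoStun event and its looping-timer setup are unused leftovers.
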(event `self.ReceiveBeginPlay`
  (`parent.ReceiveBeginPlay`))

(event `self.ReceiveTick`
  (params (DeltaSeconds :type "Float (single-precision)"))
  (`parent.ReceiveTick` DeltaSeconds))

(event `DoStun`)

(fn `DoEffect`
  (`parent.DoEffect`)
  (bind (_arrayindex _arrayelement) (`/Engine/EditorBlueprintResources/StandardMacros.ReverseForEachLoop` (`PrimitiveComponent.GetOverlappingActors` (`self.AOE`) "/Game/Blueprint/Enemies/BP_BaseEnemy.BP_BaseEnemy_C"))
    (:`LoopBody`
      (if (`KismetSystemLibrary.DoesImplementInterface` _arrayelement "/Game/Blueprint/Enemies/Interfaces/BPI_Enemy.BPI_Enemy_C")
        (message `/Game/Blueprint/Enemies/Interfaces/BPI_Enemy.EmpCC` _arrayelement (`self.StunDuration`))))))

(fn `UserConstructionScript`
  (`parent.UserConstructionScript`))