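; Base turret area-of-effect actor that holds damage, damage-over-time, slow, stun and gravity settings alongside the shape of its zone.
; Initialize stores the settings passed in, then calls SetAoe to pick a sphere or cone mesh, or none.
; The mesh scales from radius or distance, with cone width derived from the tangent of its half-angle.
; The construction script repeats this sizing, and no damage or effect logic runs here.
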(event `self.ReceiveBeginPlay`
  (`parent.ReceiveBeginPlay`))

(event `self.ReceiveTick`
  (params (DeltaSeconds :type "Float (single-precision)"))
  (`parent.ReceiveTick` DeltaSeconds))

(event `Initialize`
  (params (CanHitPlayer :type Boolean) (DamageOnHit :type "Float (double-precision)") (DamageOverTime :type "Float (double-precision)") (DamageReduction :type "Float (double-precision)") (TypeOfAoe :type "/Game/Blueprint/Turrets/TurretFeature/Aoe/E_AoeType Enum" :default "NewEnumerator3") (TypeOfDamage :type "/Game/Blueprint/Interfaces/E_DamageType Enum" :default "NewEnumerator0") (`MaxDistance(Cone)/MaxRadius(Sphere)` :type "Float (double-precision)") (`MaxAngleOfEffect(Cone)` :type "Float (double-precision)") (TimeTick :type "Float (double-precision)") (TypeOfEffect :type "/Game/Blueprint/Turrets/TurretFeature/Aoe/E_CcType Enum" :default "NewEnumerator3") (SlowEffect :type "Float (double-precision)") (StunTime :type "Float (double-precision)") (GravityForce :type "Float (double-precision)"))
  (set `self.CanHitPlayer` CanHitPlayer)
  (set `self.DamageOnHit` DamageOnHit)
  (set `self.DamageOverTime` DamageOverTime)
  (set `self.DamageReduction` DamageReduction)
  (set `self.TypeOfAoe` TypeOfAoe)
  (set `self.TypeOfDamage` TypeOfDamage)
  (set `self.MaxDistance(Cone)/MaxRadius(Sphere)` `MaxDistance(Cone)/MaxRadius(Sphere)`)
  (set `self.MaxAngleOfEffect(Cone)` `MaxAngleOfEffect(Cone)`)
  (set `self.TimeTick` TimeTick)
  (set `self.TypeOfEffect` TypeOfEffect)
  (set `self.SlowEffect` SlowEffect)
  (set `self.StunDuration` StunTime)
  (set `self.GravityForce` GravityForce)
  (`self.SetAoe`))

(event `SetAoe`
  (bind _returnvalue (/ (`self.MaxDistance(Cone)/MaxRadius(Sphere)`) 100.0))
  (bind _returnvalue_2 (/ (`self.MaxAngleOfEffect(Cone)`) 2))
  (bind _returnvalue_3 (/ (* (* (`self.MaxDistance(Cone)/MaxRadius(Sphere)`) 2.0) (/ (`KismetMathLibrary.DegSin` _returnvalue_2) (`KismetMathLibrary.DegCos` _returnvalue_2))) 100.0))
  (switch `/Game/Blueprint/Turrets/TurretFeature/Aoe/E_AoeType` (`self.TypeOfAoe`)
    (:`NewEnumerator3`
      (`StaticMeshComponent.SetStaticMesh` (`self.AOE`) null))
    (:`NewEnumerator2`
      (`StaticMeshComponent.SetStaticMesh` (`self.AOE`) "/Game/Models/Turret/Meshes/AreaOfEffect/SM_AOE_Sphere.SM_AOE_Sphere")
      (`SceneComponent.SetRelativeScale3D` (`self.AOE`) (`KismetMathLibrary.MakeVector` _returnvalue _returnvalue _returnvalue)))
    (:`NewEnumerator1`
      (`StaticMeshComponent.SetStaticMesh` (`self.AOE`) "/Game/Models/Turret/Meshes/AreaOfEffect/SM_AOE_Cone.SM_AOE_Cone")
      (`SceneComponent.SetRelativeScale3D` (`self.AOE`) (`KismetMathLibrary.MakeVector` (/ (`self.MaxDistance(Cone)/MaxRadius(Sphere)`) 100.0) _returnvalue_3 _returnvalue_3)))))

(fn `UserConstructionScript`
  (bind _returnvalue (/ (`self.MaxDistance(Cone)/MaxRadius(Sphere)`) 100.0))
  (bind _returnvalue_2 (/ (`self.MaxAngleOfEffect(Cone)`) 2))
  (bind _returnvalue_3 (/ (* (* (`self.MaxDistance(Cone)/MaxRadius(Sphere)`) 2.0) (/ (`KismetMathLibrary.DegSin` _returnvalue_2) (`KismetMathLibrary.DegCos` _returnvalue_2))) 100.0))
  (`parent.UserConstructionScript`)
  (switch `/Game/Blueprint/Turrets/TurretFeature/Aoe/E_AoeType` (`self.TypeOfAoe`)
    (:`NewEnumerator3`
      (`StaticMeshComponent.SetStaticMesh` (`self.AOE`) null))
    (:`NewEnumerator2`
      (`StaticMeshComponent.SetStaticMesh` (`self.AOE`) "/Game/Models/Turret/Meshes/AreaOfEffect/SM_AOE_Sphere.SM_AOE_Sphere")
      (`SceneComponent.SetRelativeScale3D` (`self.AOE`) (`KismetMathLibrary.MakeVector` _returnvalue _returnvalue _returnvalue)))
    (:`NewEnumerator1`
      (`StaticMeshComponent.SetStaticMesh` (`self.AOE`) "/Game/Models/Turret/Meshes/AreaOfEffect/SM_AOE_Cone.SM_AOE_Cone")
      (`SceneComponent.SetRelativeScale3D` (`self.AOE`) (`KismetMathLibrary.MakeVector` (/ (`self.MaxDistance(Cone)/MaxRadius(Sphere)`) 100.0) _returnvalue_3 _returnvalue_3)))))