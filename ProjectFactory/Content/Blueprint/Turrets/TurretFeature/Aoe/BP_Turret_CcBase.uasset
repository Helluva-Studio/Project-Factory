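; Base Blueprint for turret crowd-control area effects, configured through InitializeCcAmmo.
; The initializer stores player-hit permission, CC type, AoE shape settings and the slow, stun and gravity parameters.
; For the Stun type only, it starts a looping timer at the stun tick interval that fires CcEffect.
; CcEffect calls DoEffect, which is empty here, and BeginPlay, overlap and Tick are unused.
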(event `/Game/Blueprint/Turrets/Interfaces/BPI_TurretCcAmmo.InitializeCcAmmo`
  (params (CanHitPlayer :type Boolean) (CcType :type "/Game/Blueprint/Turrets/TurretFeature/Aoe/E_CcType Enum" :default "NewEnumerator5") (TypeOfAoe :type "/Game/Blueprint/Turrets/TurretFeature/Aoe/E_AoeType Enum" :default "NewEnumerator3") (`MaxAngleOfEffect(Cone)` :type "Float (double-precision)") (`MaxDistance(Cone)/MaxRadius(Sphere)` :type "Float (double-precision)") (SlowEffect :type "Float (double-precision)") (StunDuration :type "Float (double-precision)") (StunTick :type "Float (double-precision)") (GravityForce :type "Float (double-precision)"))
  (set `self.CanHitPlayer` CanHitPlayer)
  (set `self.CcType` CcType)
  (set `self.TypeOfAoe` TypeOfAoe)
  (set `self.MaxDistance(Cone)/MaxRadius(Sphere)` `MaxAngleOfEffect(Cone)`)
  (set `self.MaxDistance(Cone)/MaxRadius(Sphere)` `MaxDistance(Cone)/MaxRadius(Sphere)`)
  (set `self.SlowEffect` SlowEffect)
  (set `self.StunDuration` StunDuration)
  (set `self.StunTick` StunTick)
  (set `self.GravityForce` GravityForce)
  (switch `/Game/Blueprint/Turrets/TurretFeature/Aoe/E_CcType` (`self.CcType`)
    (:`NewEnumerator1`
      (bind _returnvalue (`KismetSystemLibrary.K2_SetTimerDelegate` (delegate `CcEffect`) (`self.StunTick`) true))
      (set `self.EffectTimer` _returnvalue))))

(event `CcEffect`
  (`self.DoEffect`))

(fn `DoEffect`)

(fn `UserConstructionScript`
  (`parent.UserConstructionScript`))