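; Turret area-of-effect actor, named as a crowd-control effect, that shows a spherical or conical volume and destroys itself on its instigator turret's destroy-ammo event.
; The construction script disables collision and sizes the mesh from radius or distance, using the cone angle's tangent for width.
; SetAoe replays that sizing as a timeline-driven growth, enabling collision once finished.
; No effect is applied in this graph; its overlap event is disabled.
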(event `self.ReceiveBeginPlay`
  (`parent.ReceiveBeginPlay`)
  (bind _asbp_turret_base (cast `/Game/Blueprint/Turrets/BP_Turret_Base` (`self.Instigator`)))
  (add `/Game/Blueprint/Turrets/BP_Turret_Base.DestroyAmmo` _asbp_turret_base (delegate `DestroyAoe`)))

(event `DestroyAoe`
  (`self.K2_DestroyActor`))

(event `self.ReceiveTick`
  (params (DeltaSeconds :type "Float (single-precision)"))
  (`parent.ReceiveTick` DeltaSeconds))

(event `SetAoe`
  (bind _returnvalue (/ (`self.MaxAngleOfEffect(Cone)`) 2))
  (switch `/Game/Blueprint/Turrets/TurretFeature/Aoe/E_AoeType` (`self.TypeOfAoe`)
    (:`NewEnumerator3`
      (`StaticMeshComponent.SetStaticMesh` (`self.AOE`) null))
    (:`NewEnumerator2`
      (`StaticMeshComponent.SetStaticMesh` (`self.AOE`) "/Game/Models/Turret/Meshes/AreaOfEffect/SM_Sphere.SM_Sphere")
      (bind (_direction _scale) (`Timeline|Scaling`)
        (:`Update`
          (`SceneComponent.SetWorldScale3D` (`self.AOE`) (`KismetMathLibrary.Conv_DoubleToVector` (* _scale (/ (`self.MaxDistance(Cone)/MaxRadius(Sphere)`) 100.0)))))
        (:`Finished`
          (`self.SetActorEnableCollision` true))))
    (:`NewEnumerator1`
      (`StaticMeshComponent.SetStaticMesh` (`self.AOE`) "/Game/Models/Turret/Meshes/AreaOfEffect/SM_AOE_Cone.SM_AOE_Cone")
      (bind (_direction_2 _scale_2) (`Timeline|Timeline`)
        (:`Update`
          (bind _returnvalue_2 (* _scale_2 (/ (* (* (`self.MaxDistance(Cone)/MaxRadius(Sphere)`) 2.0) (/ (`KismetMathLibrary.DegSin` _returnvalue) (`KismetMathLibrary.DegCos` _returnvalue))) 100.0)))
          (`SceneComponent.SetWorldScale3D` (`self.AOE`) (`KismetMathLibrary.MakeVector` (* _scale_2 (/ (`self.MaxDistance(Cone)/MaxRadius(Sphere)`) 100.0)) _returnvalue_2 _returnvalue_2)))
        (:`Finished`
          (`self.SetActorEnableCollision` true))))))

(fn `UserConstructionScript`
  (bind _returnvalue (/ (`self.MaxDistance(Cone)/MaxRadius(Sphere)`) 100.0))
  (bind _returnvalue_2 (/ (`self.MaxAngleOfEffect(Cone)`) 2))
  (bind _returnvalue_3 (/ (* (* (`self.MaxDistance(Cone)/MaxRadius(Sphere)`) 2.0) (/ (`KismetMathLibrary.DegSin` _returnvalue_2) (`KismetMathLibrary.DegCos` _returnvalue_2))) 100.0))
  (`parent.UserConstructionScript`)
  (`self.SetActorEnableCollision` false)
  (switch `/Game/Blueprint/Turrets/TurretFeature/Aoe/E_AoeType` (`self.TypeOfAoe`)
    (:`NewEnumerator3`
      (`StaticMeshComponent.SetStaticMesh` (`self.AOE`) null))
    (:`NewEnumerator2`
      (`StaticMeshComponent.SetStaticMesh` (`self.AOE`) "/Game/Models/Turret/Meshes/AreaOfEffect/SM_Sphere.SM_Sphere")
      (`SceneComponent.SetRelativeScale3D` (`self.AOE`) (`KismetMathLibrary.MakeVector` _returnvalue _returnvalue _returnvalue)))
    (:`NewEnumerator1`
      (`StaticMeshComponent.SetStaticMesh` (`self.AOE`) "/Game/Models/Turret/Meshes/AreaOfEffect/SM_AOE_Cone.SM_AOE_Cone")
      (`SceneComponent.SetRelativeScale3D` (`self.AOE`) (`KismetMathLibrary.MakeVector` (/ (`self.MaxDistance(Cone)/MaxRadius(Sphere)`) 100.0) _returnvalue_3 _returnvalue_3)))))