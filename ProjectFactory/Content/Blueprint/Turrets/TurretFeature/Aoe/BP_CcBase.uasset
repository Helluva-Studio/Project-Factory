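; Base actor for a turret area-of-effect feature that holds damage settings and sizes the AOE mesh to match its shape.
; Initialize stores the hit, damage and shape parameters, then calls SetAoe to assign no mesh, a sphere or a cone.
; Sphere scale follows the radius, while cone width derives from distance and the tangent of half the angle.
; The Construction Script duplicates this sizing logic; no damage is applied here.
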(event `self.ReceiveBeginPlay`
  (`parent.ReceiveBeginPlay`))

(event `self.ReceiveTick`
  (params (DeltaSeconds :type "Float (single-precision)"))
  (`parent.ReceiveTick` DeltaSeconds))

(event `Initialize`
  (params (CanHitPlayer :type Boolean) (DamageOnHit :type "Float (double-precision)") (DamageOverTime :type "Float (double-precision)") (DamageReduction :type "Float (double-precision)") (TypeOfAoe :type "/Game/Blueprint/Turrets/TurretFeature/Aoe/AOEType Enum" :default "NewEnumerator3") (TypeOfDamage :type "/Game/Blueprint/Interfaces/E_DamageType Enum" :default "NewEnumerator0") (`MaxDistance(Cone)/MaxRadius(Sphere)` :type "Float (double-precision)") (`MaxAngleOfEffect(Cone)` :type "Float (double-precision)") (MaxTimeBetweenDamage :type "Float (double-precision)"))
  (set `self.CanHitPlayer` CanHitPlayer)
  (set `self.DamageOnHit` DamageOnHit)
  (set `self.DamageOverTime` DamageOverTime)
  (set `self.DamageReduction` DamageReduction)
  (set `self.TypeOfAoe` TypeOfAoe)
  (set `self.TypeOfDamage` TypeOfDamage)
  (set `self.MaxDistance(Cone)/MaxRadius(Sphere)` `MaxDistance(Cone)/MaxRadius(Sphere)`)
  (set `self.MaxAngleOfEffect(Cone)` `MaxAngleOfEffect(Cone)`)
  (set `self.MaxTimeBetweenDamage` MaxTimeBetweenDamage)
  (`self.SetAoe`))

(event `SetAoe`
  (bind _returnvalue (/ (`self.MaxDistance(Cone)/MaxRadius(Sphere)`) 100.0))
  (bind _returnvalue_2 (/ (`self.MaxAngleOfEffect(Cone)`) 2))
  (bind _returnvalue_3 (/ (* (* (`self.MaxDistance(Cone)/MaxRadius(Sphere)`) 2.0) (/ (`KismetMathLibrary.DegSin` _returnvalue_2) (`KismetMathLibrary.DegCos` _returnvalue_2))) 100.0))
  (switch `/Game/Blueprint/Turrets/TurretFeature/Aoe/AOEType` (`self.TypeOfAoe`)
    (:`NewEnumerator3`
      (`StaticMeshComponent.SetStaticMesh` (`self.AOE`) null))
    (:`NewEnumerator2`
      (`StaticMeshComponent.SetStaticMesh` (`self.AOE`) "/Game/Models/Turret/Meshes/AreaOfEffect/SM_AOE_Sphere.SM_AOE_Sphere")
      (`SceneComponent.SetRelativeScale3D` (`self.AOE`) (`KismetMathLibrary.MakeVector` _returnvalue _returnvalue _returnvalue)))
    (:`NewEnumerator1`
      (`StaticMeshComponent.SetStaticMesh` (`self.AOE`) "/Game/Models/Turret/Meshes/AreaOfEffect/SM_AOE_Cone.SM_AOE_Cone")
      (`SceneComponent.SetRelativeScale3D` (`self.AOE`) (`KismetMathLibrary.MakeVector` (/ (`self.MaxDistance(Cone)/MaxRadius(Sphere)`) 100.0) _returnvalue_3 _returnvalue_3)))))

(fn `UserConstructionScript`
  (bind _returnvalue (/ (`self.MaxDistance(Cone)/MaxRadius(Sphere)`) 100.0))
  (bind _returnvalue_2 (/ (`self.MaxAngleOfEffect(Cone)`) 2))
  (bind _returnvalue_3 (/ (* (* (`self.MaxDistance(Cone)/MaxRadius(Sphere)`) 2.0) (/ (`KismetMathLibrary.DegSin` _returnvalue_2) (`KismetMathLibrary.DegCos` _returnvalue_2))) 100.0))
  (`parent.UserConstructionScript`)
  (switch `/Game/Blueprint/Turrets/TurretFeature/Aoe/AOEType` (`self.TypeOfAoe`)
    (:`NewEnumerator3`
      (`StaticMeshComponent.SetStaticMesh` (`self.AOE`) null))
    (:`NewEnumerator2`
      (`StaticMeshComponent.SetStaticMesh` (`self.AOE`) "/Game/Models/Turret/Meshes/AreaOfEffect/SM_AOE_Sphere.SM_AOE_Sphere")
      (`SceneComponent.SetRelativeScale3D` (`self.AOE`) (`KismetMathLibrary.MakeVector` _returnvalue _returnvalue _returnvalue)))
    (:`NewEnumerator1`
      (`StaticMeshComponent.SetStaticMesh` (`self.AOE`) "/Game/Models/Turret/Meshes/AreaOfEffect/SM_AOE_Cone.SM_AOE_Cone")
      (`SceneComponent.SetRelativeScale3D` (`self.AOE`) (`KismetMathLibrary.MakeVector` (/ (`self.MaxDistance(Cone)/MaxRadius(Sphere)`) 100.0) _returnvalue_3 _returnvalue_3)))))