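; BP_CcSlow is a turret area-of-effect actor that slows enemies while they are inside its area.
; InitializeSlowAmmo stores the hit-player flag, CC type, AoE type, size and slow effect, then calls SetAoe.
; AOE overlap begin and end events send start and stop slow messages through BPI_Enemy, only to actors implementing that interface.
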(event `self.ReceiveBeginPlay`
  (`parent.ReceiveBeginPlay`))

(event `self.ReceiveTick`
  (params (DeltaSeconds :type "Float (single-precision)"))
  (`parent.ReceiveTick` DeltaSeconds))

(event `/Game/Blueprint/Turrets/Interfaces/BPI_TurretCcAmmo.InitializeSlowAmmo`
  (params (CanHitPlayer :type Boolean) (CcType :type "/Game/Blueprint/Turrets/TurretFeature/Aoe/E_CcType Enum" :default "NewEnumerator5") (TypeOfAoe :type "/Game/Blueprint/Turrets/TurretFeature/Aoe/E_AoeType Enum" :default "NewEnumerator3") (`MaxDistance(Cone)/MaxRadius(Sphere)` :type "Float (double-precision)") (SlowEffect :type "Float (double-precision)"))
  (set `self.CanHitPlayer` CanHitPlayer)
  (set `self.CcType` CcType)
  (set `self.TypeOfAoe` TypeOfAoe)
  (set `self.MaxDistance(Cone)/MaxRadius(Sphere)` `MaxDistance(Cone)/MaxRadius(Sphere)`)
  (set `self.Slow Effect` SlowEffect)
  (`self.SetAoe`))

(event `self.AOE.OnComponentBeginOverlap`
  (params (OverlappedComponent :type "PrimitiveComponent Object Reference") (OtherActor :type "Actor Object Reference") (OtherComp :type "PrimitiveComponent Object Reference") (OtherBodyIndex :type Integer) (bFromSweep :type Boolean) (SweepResult :type "HitResult Structure (by ref)"))
  (if (`KismetSystemLibrary.DoesImplementInterface` OtherActor "/Game/Blueprint/Enemies/Interfaces/BPI_Enemy.BPI_Enemy_C")
    (message `/Game/Blueprint/Enemies/Interfaces/BPI_Enemy.StartSlowCC` OtherActor (`self.Slow Effect`))))

(event `self.AOE.OnComponentEndOverlap`
  (params (OverlappedComponent :type "PrimitiveComponent Object Reference") (OtherActor :type "Actor Object Reference") (OtherComp :type "PrimitiveComponent Object Reference") (OtherBodyIndex :type Integer))
  (if (`KismetSystemLibrary.DoesImplementInterface` OtherActor "/Game/Blueprint/Enemies/Interfaces/BPI_Enemy.BPI_Enemy_C")
    (message `/Game/Blueprint/Enemies/Interfaces/BPI_Enemy.StopSlowCC` OtherActor)))

(fn `UserConstructionScript`
  (`parent.UserConstructionScript`))