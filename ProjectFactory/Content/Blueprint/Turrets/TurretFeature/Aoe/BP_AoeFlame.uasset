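; Flame area-of-effect actor for turrets that burns enemies, and optionally the player, inside its AOE component.
; InitializeFlameAmmo stores the damage and shape settings, then calls SetAoe.
; Overlap begin applies hit damage and starts damage over time through BPC_DamageSystem, scaled down by distance at entry.
; Overlap end stops that damage, ignoring enemy components tagged "punch"; audio fades in on BeginPlay.
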(event `self.ReceiveBeginPlay`
  (`parent.ReceiveBeginPlay`)
  (`AudioComponent.FadeIn` (`self.Audio`) 1.0 1.0 0.0 "Linear"))

(event `self.ReceiveTick`
  (params (DeltaSeconds :type "Float (single-precision)"))
  (`parent.ReceiveTick` DeltaSeconds))

(event `/Game/Blueprint/Turrets/Interfaces/BPI_TurretDamageAmmo.InitializeFlameAmmo`
  (params (CanHitPlayer :type Boolean) (DamageType :type "/Game/Blueprint/Interfaces/E_DamageType Enum" :default "NewEnumerator4") (TypeOfAoe :type "/Game/Blueprint/Turrets/TurretFeature/Aoe/E_AoeType Enum" :default "NewEnumerator3") (MaxAngleOfEffect :type "Float (double-precision)") (DamageTick :type "Float (double-precision)") (DamageOnHit :type "Float (double-precision)") (DotInsideAoe :type "Float (double-precision)") (DotOutsideAoe :type "Float (double-precision)") (DotDuration :type "Float (double-precision)") (DamageReductionByDistance :type "Float (double-precision)"))
  (set `self.CanHitPlayer` CanHitPlayer)
  (set `self.DamageType` DamageType)
  (set `self.TypeOfAoe` TypeOfAoe)
  (set `self.MaxAngleOfEffect(Cone)` MaxAngleOfEffect)
  (set `self.TimeTick` DamageTick)
  (set `self.DamageOnHit` DamageOnHit)
  (set `self.Dot Inside Aoe` DotInsideAoe)
  (set `self.Dot Outside Aoe` DotOutsideAoe)
  (set `self.Dot Duration` DotDuration)
  (set `self.Damage Reduction by Distance` DamageReductionByDistance)
  (`self.SetAoe`))

(event `self.AOE.OnComponentBeginOverlap`
  (params (OverlappedComponent :type "PrimitiveComponent Object Reference") (OtherActor :type "Actor Object Reference") (OtherComp :type "PrimitiveComponent Object Reference") (OtherBodyIndex :type Integer) (bFromSweep :type Boolean) (SweepResult :type "HitResult Structure (by ref)"))
  (bind _dot_inside_aoe (`self.Dot Inside Aoe`))
  (if (`KismetSystemLibrary.DoesImplementInterface` OtherActor "/Game/Blueprint/Enemies/Interfaces/BPI_Enemy.BPI_Enemy_C")
    (message `/Game/Blueprint/Interfaces/BPI_Damageable.TakeDamageOverTime` (`self.GetComponentByClass` OtherActor "/Game/Blueprint/DamageSystem/BPC_DamageSystem.BPC_DamageSystem_C") (`self.TimeTick`) (`KismetMathLibrary.MapRangeClamped` (`KismetMathLibrary.Vector_Distance` (`self.K2_GetActorLocation` OtherActor) (`self.K2_GetActorLocation`)) 60.0 (`self.MaxDistance(Cone)/MaxRadius(Sphere)`) _dot_inside_aoe (* _dot_inside_aoe (/ (- 100.0 (`self.Damage Reduction by Distance`)) 100.0))) self (`self.DamageType`) :!label _label)
    (`GameplayStatics.ApplyDamage` OtherActor (`self.DamageOnHit`) null (`self.Instigator`))
    (elif (and (`self.CanHitPlayer`) (== OtherActor (`GameplayStatics.GetPlayerPawn` 0)))
      (goto _label))))

(event `self.AOE.OnComponentEndOverlap`
  (params (OverlappedComponent :type "PrimitiveComponent Object Reference") (OtherActor :type "Actor Object Reference") (OtherComp :type "PrimitiveComponent Object Reference") (OtherBodyIndex :type Integer))
  (if (`KismetSystemLibrary.DoesImplementInterface` OtherActor "/Game/Blueprint/Enemies/Interfaces/BPI_Enemy.BPI_Enemy_C")
    (if (not (`ActorComponent.ComponentHasTag` OtherComp "punch"))
      (message `/Game/Blueprint/Interfaces/BPI_Damageable.StopDamageOverTime` (`self.GetComponentByClass` OtherActor "/Game/Blueprint/DamageSystem/BPC_DamageSystem.BPC_DamageSystem_C") (`self.DamageType`) self :!label _label_2))
    (elif (and (`self.CanHitPlayer`) (== OtherActor (`GameplayStatics.GetPlayerPawn` 0)))
      (goto _label_2))))

(fn `UserConstructionScript`
  (`parent.UserConstructionScript`))