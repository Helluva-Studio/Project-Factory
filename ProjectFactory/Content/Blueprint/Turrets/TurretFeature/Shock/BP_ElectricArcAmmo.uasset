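; Shock turret ammo actor that draws a chain of electric arcs jumping between nearby enemies.
; After a startup delay, it repeatedly sphere-traces from the last target, randomly picks an unvisited enemy and shrinks the range, caching positions in a map.
; Strike then spawns staggered Niagara beams between cached positions and later destroys them.
; An older self-spawning chain remains disconnected, including the only damage call.
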(event `self.ReceiveBeginPlay`
  (`KismetSystemLibrary.Delay` 3.0)
  (`self.PickNextTarget`))

(event `PickNextTarget`
  (bind _returnvalue (`self.K2_GetActorLocation` (`self.Target`)))
  (while (> (`self.NumberOfTarget`) 0)
    (bind _keys (`BlueprintMapLibrary.Map_Keys` (`self.ConnectedEnemy`)))
    (bind _outhits (`KismetSystemLibrary.SphereTraceMultiForObjects` _returnvalue _returnvalue (`self.Range`) (`|MakeArray` "ObjectTypeQuery3" :!type "EObjectTypeQuery Enum") false _keys))
    (for _array_element _outhits
      (bind (_bblockinghit _binitialoverlap _time _distance _location _impactpoint _normal _impactnormal _physmat _hitactor) (`GameplayStatics.BreakHitResult` _array_element))
      (if (`KismetSystemLibrary.DoesImplementInterface` _hitactor "/Game/Blueprint/Enemies/Interfaces/BPI_Enemy.BPI_Enemy_C")
        (`KismetArrayLibrary.Array_AddUnique` (`self.PreviusTargets`) _hitactor)))
    (if (<= (`KismetArrayLibrary.Array_Length` (`self.PreviusTargets`)) 0)
      (set `self.NumberOfTarget` 0)
      (else
        (bind _output_get (set `self.Target` (`|GetArrayItem` (`self.PreviusTargets`) (`KismetMathLibrary.RandomIntegerInRange` 0 (- (`KismetArrayLibrary.Array_Length` (`self.PreviusTargets`)) 1)))))
        (`BlueprintMapLibrary.Map_Add` (`self.ConnectedEnemy`) _output_get (`self.K2_GetActorLocation` _output_get))
        (`/Engine/EditorBlueprintResources/StandardMacros.DecrementInt` (`self.NumberOfTarget`)
          (:`  `
            (bind (_arrayindex _arrayelement) (`/Engine/EditorBlueprintResources/StandardMacros.ReverseForEachLoop` (`self.PreviusTargets`))
              (:`LoopBody`
                (`KismetArrayLibrary.Array_RemoveItem` (`self.PreviusTargets`) _arrayelement)
                (set `self.Range` (* (`self.Range`) (- 1.0 (/ (`self.RangeReduction`) 100.0)))))))))))
  (`self.Strike`))

(event `TakeAroundEnemies`
  (bind _returnvalue (`self.K2_GetActorLocation`))
  (`KismetArrayLibrary.Array_Add` (`self.PreviusArc`) self)
  (bind _outhits (`KismetSystemLibrary.SphereTraceMultiForObjects` :`Start` _returnvalue :`End` _returnvalue :`Radius` (`self.Range`) :`ObjectTypes` (`|MakeArray` "ObjectTypeQuery3" :!type "EObjectTypeQuery Enum") :`DrawDebugType` "Persistent"))
  (for _array_element _outhits
    (bind (_bblockinghit _binitialoverlap _time _distance _location _impactpoint _normal _impactnormal _physmat _hitactor) (`GameplayStatics.BreakHitResult` _array_element))
    (if (`KismetSystemLibrary.DoesImplementInterface` _hitactor "/Game/Blueprint/Enemies/Interfaces/BPI_Enemy.BPI_Enemy_C")
      (`KismetArrayLibrary.Array_AddUnique` (`self.AroundTarget`) _hitactor)))
  (if (<= (`KismetArrayLibrary.Array_Length` (`self.AroundTarget`)) 0)
    (`self.DestroyChainLight`)
    (else
      (`self.PickNextTarget`))))

(event `Strike`
  (bind _keys (`BlueprintMapLibrary.Map_Keys` (`self.ConnectedEnemy`)))
  (if (> (`KismetArrayLibrary.Array_Length` _keys) 0)
    (bind _keys_2 (`BlueprintMapLibrary.Map_Keys` (`self.ConnectedEnemy`)))
    (bind _index (`/Game/Blueprint/BP_MacroLibrary_Actor.For Loop With Delay` 0 (- (`KismetArrayLibrary.Array_Length` _keys_2) 2) 0.1)
      (:`Loop Body`
        (bind _values (`BlueprintMapLibrary.Map_Values` (`self.ConnectedEnemy`)))
        (bind _returnvalue (`NiagaraFunctionLibrary.SpawnSystemAtLocation` "/Game/Blueprint/Turrets/TurretFeature/Shock/NS_ElectricArc.NS_ElectricArc" (`|GetArrayItem` _values _index) (struct) (1.0 1.0 1.0) false))
        (set `self.LightningChain` _returnvalue)
        (bind _values_2 (`BlueprintMapLibrary.Map_Values` (`self.ConnectedEnemy`)))
        (`FXSystemComponent.SetVectorParameter` (`self.LightningChain`) "BeamEnd" (`|GetArrayItem` _values_2 (+ _index 1)))
        (`KismetArrayLibrary.Array_AddUnique` (`self.LightningChains`) (`self.LightningChain`)))
      (:`Completed`
        (`KismetSystemLibrary.Delay` 3.0)
        (bind (_arrayindex _arrayelement) (`/Engine/EditorBlueprintResources/StandardMacros.ReverseForEachLoop` (`self.LightningChains`))
          (:`LoopBody`
            (`/Engine/EditorBlueprintResources/StandardMacros.IsValid` _arrayelement
              (:`Is Valid`
                (`ActorComponent.K2_DestroyComponent` _arrayelement)))))))))

(event `StrikeNewLight`
  (`KismetSystemLibrary.Delay` (`self.TimeBetweenStrike`))
  (if (> (`self.NumberOfTarget`) 0)
    (bind _returnvalue (`|SpawnActorFromClass` :`Class` "BP_ElectricArcAmmo_C" :`SpawnTransform` (`KismetMathLibrary.MakeTransform` (`self.K2_GetActorLocation` (`self.EndTarget`))) :`CollisionHandlingOverride` "AdjustIfPossibleButAlwaysSpawn" :`TransformScaleMethod` "MultiplyWithRoot" :`ShockTurret` (`self.ShockTurret`) :`TimeBetweenStrike` (`self.TimeBetweenStrike`) :`NumberOfTarget` (`self.NumberOfTarget`) :`StartTarget` (`self.EndTarget`) :`ConnectedTarget2` (`self.ConnectedTarget2`) :`PreviusArc` (`self.PreviusArc`) :`Range` (* (`self.Range`) (- 1.0 (/ (`self.RangeReduction`) 100.0))) :`RangeReduction` (`self.RangeReduction`) :`Damage` (* (`self.Damage`) (- 1.0 (/ (`self.DamageReductionByBounce`) 100.0))) :`DamageReductionByBounce` (`self.DamageReductionByBounce`) :`LightningChain` null :`Instigator` null))
    (`self.K2_AttachToActor` _returnvalue self "None" "KeepWorld" "KeepWorld" "KeepWorld" true)
    (else
      (`self.DestroyChainLight`))))

(event `DestroyChainLight`
  (bind (_arrayindex _arrayelement) (`/Engine/EditorBlueprintResources/StandardMacros.ReverseForEachLoop` (`self.PreviusArc`))
    (:`LoopBody`
      (`self.K2_DestroyActor` _arrayelement))
    (:`Completed`
      (`self.K2_DestroyActor`))))

(event `self.ReceiveTick`
  (params (DeltaSeconds :type "Float (single-precision)"))
  (`/Engine/EditorBlueprintResources/StandardMacros.IsValid` self
    (:`Is Valid`
      (`|ExecutionSequence`
        (:`then_0`
          (`/Engine/EditorBlueprintResources/StandardMacros.IsValid` (`self.StartTarget`)
            (:`Is Valid`
              (`SceneComponent.K2_SetWorldLocation` (`self.Start`) (`self.K2_GetActorLocation` (`self.StartTarget`)) false false))))
        (:`then_1`
          (`/Engine/EditorBlueprintResources/StandardMacros.IsValid` (`self.EndTarget`)
            (:`Is Valid`
              (`SceneComponent.K2_SetWorldLocation` (`self.End`) (`self.K2_GetActorLocation` (`self.EndTarget`)) false false))))))))

(fn `UserConstructionScript`
  (`SceneComponent.SetWorldScale3D` (`self.RangeMesh`) (`KismetMathLibrary.Conv_DoubleToVector` (/ (`self.Range`) 100.0)))
  (bind _output_get (set `self.Target` self))
  (`BlueprintMapLibrary.Map_Add` (`self.ConnectedEnemy`) _output_get (`self.K2_GetActorLocation` self)))