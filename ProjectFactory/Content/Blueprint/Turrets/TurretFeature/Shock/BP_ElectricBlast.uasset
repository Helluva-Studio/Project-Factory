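; Electric blast actor spawned by a turret that charges an arc effect, then zaps nearby enemies with area damage.
; A timeline scales the spark over the AoE tick, then a sphere trace damages BPI_Enemy pawns and spawns an arc to each.
; Tick updates arc endpoints from an arc-to-target map to follow moving victims.
; All effects and the actor are destroyed after a despawn delay or when the turret's destroy-ammo event fires.
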(event `self.ReceiveBeginPlay`
  (bind _singlestrike (`self.SingleStrike`))
  (`self.SpawnSparkle`)
  (bind _asbp_turret_base (cast `/Game/Blueprint/Turrets/BP_Turret_Base` (`self.Instigator`)))
  (`/Engine/EditorBlueprintResources/StandardMacros.IsValid` _asbp_turret_base
    (:`Is Valid`
      (add `/Game/Blueprint/Turrets/BP_Turret_Base.DestroyAmmo` _asbp_turret_base (delegate `DestroyNiagara`)))
    (:`Is Not Valid`
      (`|ExecutionSequence` :!label _label
        (:`then_0`
          (`/Engine/EditorBlueprintResources/StandardMacros.IsValid` _singlestrike
            (:`Is Valid`
              (`ActorComponent.K2_DestroyComponent` _singlestrike))))
        (:`then_1`
          (bind _keys (`BlueprintMapLibrary.Map_Keys` (`self.LightningStrikes`)))
          (for _array_element _keys
            (`/Engine/EditorBlueprintResources/StandardMacros.IsValid` _array_element
              (:`Is Valid`
                (`ActorComponent.K2_DestroyComponent` _array_element))))
          (`self.K2_DestroyActor`))))))

(event `DestroyNiagara`
  (goto _label))

(event `SpawnSparkle`
  (bind _returnvalue (`self.K2_GetActorLocation`))
  (bind _singlestrike (`self.SingleStrike`))
  (bind _returnvalue_2 (`NiagaraFunctionLibrary.SpawnSystemAtLocation` "/Game/Blueprint/Turrets/TurretFeature/Shock/NS_ElectricArc.NS_ElectricArc" (`self.K2_GetActorLocation`) (struct) (0.0 0.0 0.0) false))
  (`PrimitiveComponent.SetHiddenInSceneCapture` _returnvalue_2 false)
  (bind _output_get (set `self.SingleStrike` _returnvalue_2))
  (`FXSystemComponent.SetVectorParameter` _output_get "BeamEnd" (`SceneComponent.K2_GetComponentLocation` _output_get))
  (`TimelineComponent.SetPlayRate` (`self.ScalingLight`) (`KismetMathLibrary.SafeDivide` 1.0 (`self.AoeTick`)))
  (bind (_direction _scaling) (`Timeline|ScalingLight`)
    (:`Update`
      (`/Engine/EditorBlueprintResources/StandardMacros.IsValid` _singlestrike
        (:`Is Valid`
          (bind (_returnvalue_x _returnvalue_y _returnvalue_z) (`KismetMathLibrary.BreakVector` (* _scaling 30.0)))
          (`SceneComponent.SetWorldScale3D` _singlestrike (`KismetMathLibrary.MakeVector` _returnvalue_x _returnvalue_y _returnvalue_z))
          (`KismetSystemLibrary.PrintString` (`KismetStringLibrary.Conv_DoubleToString` _returnvalue_z) true true (struct :`G` 0.66 :`B` 1.0 :`A` 1.0) 2.0 "asdas"))))
    (:`Finished`
      (bind _outhits (`KismetSystemLibrary.SphereTraceMultiForObjects` _returnvalue _returnvalue (`self.Radius`) (`|MakeArray` "ObjectTypeQuery3" :!type "EObjectTypeQuery Enum")))
      (for _array_element _outhits
        (bind (_bblockinghit _binitialoverlap _time _distance _location _impactpoint _normal _impactnormal _physmat _hitactor) (`GameplayStatics.BreakHitResult` _array_element))
        (if (`KismetSystemLibrary.DoesImplementInterface` _hitactor "/Game/Blueprint/Enemies/Interfaces/BPI_Enemy.BPI_Enemy_C")
          (`GameplayStatics.ApplyDamage` _hitactor (`self.AoeDamage`) null (`self.Instigator`))
          (`GameplayStatics.PlaySoundAtLocation` "/Game/Audio/SFX/Turrets/Shock/SC_Zap.SC_Zap" (`self.K2_GetActorLocation` _hitactor) (struct) 1.0 1.0 0.0 null null null null)
          (bind _returnvalue_3 (`NiagaraFunctionLibrary.SpawnSystemAtLocation` "/Game/Blueprint/Turrets/TurretFeature/Shock/NS_ElectricArc.NS_ElectricArc" (`self.K2_GetActorLocation`) (struct) (1.0 1.0 1.0) false))
          (`PrimitiveComponent.SetHiddenInSceneCapture` _returnvalue_3 true)
          (`FXSystemComponent.SetVectorParameter` _returnvalue_3 "BeamEnd" (`self.K2_GetActorLocation` _hitactor))
          (`BlueprintMapLibrary.Map_Add` (`self.LightningStrikes`) _returnvalue_3 _hitactor)))
      (`self.SetActorTickEnabled` true)
      (`KismetSystemLibrary.Delay` (`self.DespawnTimer`))
      (`self.DestroyNiagara`))))

(event `self.ReceiveTick`
  (params (DeltaSeconds :type "Float (single-precision)"))
  (bind _lightningstrikes (`self.LightningStrikes`))
  (bind _keys (`BlueprintMapLibrary.Map_Keys` _lightningstrikes))
  (bind _values (`BlueprintMapLibrary.Map_Values` _lightningstrikes))
  (for (_array_element _array_index) _keys
    (`/Engine/EditorBlueprintResources/StandardMacros.IsValid` _array_element
      (:`Is Valid`
        (`FXSystemComponent.SetVectorParameter` _array_element "BeamEnd" (`self.K2_GetActorLocation` (`|GetArrayItem` _values _array_index)))))))

(fn `UserConstructionScript`)