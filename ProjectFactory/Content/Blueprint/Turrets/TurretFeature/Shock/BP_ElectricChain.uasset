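; Chain-lightning actor for a turret that arcs from its own position through nearby enemies, damaging each one.
; On spawn it picks random BPI_Enemy targets via repeated sphere traces, shrinking the radius each hop and excluding those already chained.
; Niagara arcs and damage land with a delay between links, then Tick keeps beams attached to moving actors.
; Arcs despawn sequentially after a timer, or immediately through the turret's destroy-ammo event.
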(event `self.ReceiveBeginPlay`
  (`self.PickNextTarget`)
  (bind _asbp_turret_base (cast `/Game/Blueprint/Turrets/BP_Turret_Base` (`self.Instigator`)))
  (add `/Game/Blueprint/Turrets/BP_Turret_Base.DestroyAmmo` _asbp_turret_base (delegate `DestroyNiagara`)))

(event `DestroyNiagara`
  (bind _keys (`BlueprintMapLibrary.Map_Keys` (`self.LightningChains`)))
  (for _array_element _keys
    (`/Engine/EditorBlueprintResources/StandardMacros.IsValid` _array_element
      (:`Is Valid`
        (`ActorComponent.K2_DestroyComponent` _array_element))))
  (`self.K2_DestroyActor`))

(event `PickNextTarget`
  (bind _returnvalue (`self.K2_GetActorLocation` (`self.Target`)))
  ;[0 0 0] ChainLighting
  (while (> (`self.EnemiesReachable`) 0)
    (bind _keys (`BlueprintMapLibrary.Map_Keys` (`self.ConnectedEnemy`)))
    (bind _outhits (`KismetSystemLibrary.SphereTraceMultiForObjects` _returnvalue _returnvalue (`self.Radius`) (`|MakeArray` "ObjectTypeQuery3" :!type "EObjectTypeQuery Enum") false _keys))
    (for _array_element _outhits
      (bind (_bblockinghit _binitialoverlap _time _distance _location _impactpoint _normal _impactnormal _physmat _hitactor) (`GameplayStatics.BreakHitResult` _array_element))
      (if (`KismetSystemLibrary.DoesImplementInterface` _hitactor "/Game/Blueprint/Enemies/Interfaces/BPI_Enemy.BPI_Enemy_C")
        (`KismetArrayLibrary.Array_AddUnique` (`self.PreviusTargets`) _hitactor)))
    (if (<= (`KismetArrayLibrary.Array_Length` (`self.PreviusTargets`)) 0)
      (set `self.EnemiesReachable` 0)
      (else
        (bind _output_get (set `self.Target` (`|GetArrayItem` (`self.PreviusTargets`) (`KismetMathLibrary.RandomIntegerInRange` 0 (- (`KismetArrayLibrary.Array_Length` (`self.PreviusTargets`)) 1)))))
        (`BlueprintMapLibrary.Map_Add` (`self.ConnectedEnemy`) _output_get (`self.K2_GetActorLocation` _output_get))
        (`/Engine/EditorBlueprintResources/StandardMacros.DecrementInt` (`self.EnemiesReachable`)
          (:`  `
            (`KismetArrayLibrary.Array_Clear` (`self.PreviusTargets`))
            (set `self.Radius` (* (`self.Radius`) (- 1.0 (/ (`self.RadiusReduction`) 100.0)))))))))
  (bind _keys_2 (`BlueprintMapLibrary.Map_Keys` (`self.ConnectedEnemy`)))
  (if (> (`KismetArrayLibrary.Array_Length` _keys_2) 0)
    (`self.Strike`)
    (else
      (`self.K2_DestroyActor`))))

(event `Strike`
  ;[0 0 0] ChainLighting
  (bind _keys (`BlueprintMapLibrary.Map_Keys` (`self.ConnectedEnemy`)))
  (bind (_arrayelement _arrayindex) (`/Game/Blueprint/BP_MacroLibrary_Actor.ForEachLoopWithDelay` _keys (`self.TimeBetweenChain`))
    (:`LoopBody`
      (if (< _arrayindex (- (`KismetArrayLibrary.Array_Length` _keys) 1))
        (bind _returnvalue (`NiagaraFunctionLibrary.SpawnSystemAtLocation` "/Game/Blueprint/Turrets/TurretFeature/Shock/NS_ElectricArc.NS_ElectricArc" (`self.K2_GetActorLocation` _arrayelement) (struct) (1.0 1.0 1.0) false))
        (bind _values (`BlueprintMapLibrary.Map_Values` (`self.ConnectedEnemy`)))
        (bind _returnvalue_2 (+ _arrayindex 1))
        (bind _output (`|GetArrayItem` _values _returnvalue_2))
        (`FXSystemComponent.SetVectorParameter` _returnvalue "BeamEnd" _output)
        (bind _keys_2 (`BlueprintMapLibrary.Map_Keys` (`self.ConnectedEnemy`)))
        (`GameplayStatics.ApplyDamage` (`|GetArrayItem` _keys_2 _returnvalue_2) (`self.Damage`) null (`self.Instigator`))
        (`BlueprintMapLibrary.Map_Add` (`self.LightningChains`) _returnvalue _output)))
    (:`Completed`
      (`self.SetActorTickEnabled` true)
      (`KismetSystemLibrary.Delay` (`self.DespawnTimer`))
      (bind _keys_3 (`BlueprintMapLibrary.Map_Keys` (`self.LightningChains`)))
      (bind _arrayelement_2 (`/Game/Blueprint/BP_MacroLibrary_Actor.ForEachLoopWithDelay` _keys_3 (`self.TimeBetweenChain`))
        (:`LoopBody`
          (`ActorComponent.K2_DestroyComponent` _arrayelement_2))
        (:`Completed`
          (`self.K2_DestroyActor`))))))

(event `self.ReceiveTick`
  (params (DeltaSeconds :type "Float (single-precision)"))
  (bind _keys (`BlueprintMapLibrary.Map_Keys` (`self.LightningChains`)))
  (for (_array_element _array_index) _keys
    (`/Engine/EditorBlueprintResources/StandardMacros.IsValid` _array_element
      (:`Is Valid`
        (bind _keys_2 (`BlueprintMapLibrary.Map_Keys` (`self.ConnectedEnemy`)))
        (bind _output (`|GetArrayItem` _keys _array_index))
        (`SceneComponent.K2_SetWorldLocation` _output (`self.K2_GetActorLocation` (`|GetArrayItem` _keys_2 _array_index)) false false)
        (`FXSystemComponent.SetVectorParameter` _output "BeamEnd" (`self.K2_GetActorLocation` (`|GetArrayItem` _keys_2 (+ _array_index 1))))))))

(fn `UserConstructionScript`
  (bind _output_get (set `self.Target` self))
  (`BlueprintMapLibrary.Map_Add` (`self.ConnectedEnemy`) _output_get (`self.K2_GetActorLocation` self)))