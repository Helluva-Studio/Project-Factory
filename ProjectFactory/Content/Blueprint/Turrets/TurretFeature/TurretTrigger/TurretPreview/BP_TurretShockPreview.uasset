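; Placement preview for the shock turret, extending a parent turret preview.
; The construction script sets the Shock effect's BeamEnd to the Scene component's world location and shows extra lights according to the current level.
; SetPreview runs the parent logic, then tints both beam colors green when the turret can be built and red when it cannot.
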(event `self.ReceiveTick`
  (params (DeltaSeconds :type "Float (single-precision)")))

(fn `SetPreview`
  (params (CanBeBuild :type Boolean))
  (bind _shock (`self.Shock`))
  (bind _shock_2 (`self.Shock`))
  (`parent.SetPreview` CanBeBuild)
  (if CanBeBuild
    (`NiagaraComponent.SetVariableLinearColor` _shock "Beam1Color" (make `LinearColor` 0.0 1.0 0.0 1.0))
    (`NiagaraComponent.SetVariableLinearColor` _shock_2 "Beam2Color" (make `LinearColor` 0.0 1.0 0.0 1.0))
    (else
      (`NiagaraComponent.SetVariableLinearColor` _shock "Beam1Color" (make `LinearColor` 1.0 0.0 0.0 1.0))
      (`NiagaraComponent.SetVariableLinearColor` _shock_2 "Beam2Color" (make `LinearColor` 1.0 0.0 0.0 1.0)))))

(fn `UserConstructionScript`
  (`parent.UserConstructionScript`)
  (`FXSystemComponent.SetVectorParameter` (`self.Shock`) "BeamEnd" (`SceneComponent.K2_GetComponentLocation` (`self.Scene`)))
  (switch `int` (`self.CurrentLevel`)
    (:`1`
      (`SceneComponent.SetVisibility` (`self.Light2`) false false)
      (`SceneComponent.SetVisibility` (`self.Light3`) false false))
    (:`2`
      (`SceneComponent.SetVisibility` (`self.Light2`) true false)
      (`SceneComponent.SetVisibility` (`self.Light3`) false false))
    (:`3`
      (`SceneComponent.SetVisibility` (`self.Light2`) true false)
      (`SceneComponent.SetVisibility` (`self.Light3`) true false))))