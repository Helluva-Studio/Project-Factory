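; Preview actor for the bombard turret that shows the level-specific barrel and idly sweeps its neck to random headings.
; The construction script runs the parent's, then picks one of three barrel meshes from CurrentLevel.
; A looping Patrol timer chooses a new random yaw each interval.
; A timeline, rate-scaled by that same interval, interpolates the neck there along the shortest path.
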(event `self.ReceiveBeginPlay`
  (bind _time (`self.Time`))
  (`TimelineComponent.SetPlayRate` (`self.LerpTimeline`) (/ 1.0 _time))
  (`KismetSystemLibrary.K2_SetTimerDelegate` (delegate `Patrol`) _time true)
  (set `self.NeckInitialRotation` (`SceneComponent.RelativeRotation` (`self.Neck`)) :!label _label)
  (set `self.NeckNextRotation` (`KismetMathLibrary.MakeRotator` 0.0 0.0 (`KismetMathLibrary.RandomFloatInRange` 0.0 360.0)))
  (bind (_direction _lerpvalue) (`Timeline|LerpTimeLine` :!via `PlayFromStart`)
    (:`Update`
      (`SceneComponent.K2_SetRelativeRotation` (`self.Neck`) (`KismetMathLibrary.RLerp` (`self.NeckInitialRotation`) (`self.NeckNextRotation`) _lerpvalue true) false false))))

(event `Patrol`
  (goto _label))

(fn `UserConstructionScript`
  (`parent.UserConstructionScript`)
  (switch `int` (`self.CurrentLevel`)
    (:`1`
      (`StaticMeshComponent.SetStaticMesh` (`self.Barrel1`) "/Game/Models/Turret/Meshes/Bombard/SM_BO_Barrel1.SM_BO_Barrel1"))
    (:`2`
      (`StaticMeshComponent.SetStaticMesh` (`self.Barrel1`) "/Game/Models/Turret/Meshes/Bombard/SM_BO_Barrel2.SM_BO_Barrel2"))
    (:`3`
      (`StaticMeshComponent.SetStaticMesh` (`self.Barrel1`) "/Game/Models/Turret/Meshes/Bombard/SM_BO_Barrel3.SM_BO_Barrel3"))))