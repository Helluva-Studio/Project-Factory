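; BP_TurretSlowPreview is the preview actor for the slow turret, showing one to three ice meshes based on CurrentLevel.
; The construction script toggles the second and third ice meshes per level.
; On Initialize, it gets the ice meshes' dynamic materials and drives their Brightness from the LightUp timeline.
; A looping timer replays the timeline every Time seconds, with play rate scaled to 1/Time to match that interval.
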(event `self.Initialize`
  (`TimelineComponent.SetPlayRate` (`self.LightUp`) (/ 1.0 (`self.Time`)))
  (set `self.Ice1Mat` (cast `MaterialInstanceDynamic` (`PrimitiveComponent.GetMaterial` (`self.Ice1`) 1) :!pure true))
  (set `self.Ice2Mat` (cast `MaterialInstanceDynamic` (`PrimitiveComponent.GetMaterial` (`self.Ice2`) 1) :!pure true))
  (set `self.Ice3Mat` (cast `MaterialInstanceDynamic` (`PrimitiveComponent.GetMaterial` (`self.Ice3`) 1) :!pure true))
  (`MaterialInstanceDynamic.SetScalarParameterValue` (`self.Ice1Mat`) "Brightness" 0.0)
  (`MaterialInstanceDynamic.SetScalarParameterValue` (`self.Ice2Mat`) "Brightness" 0.0)
  (`MaterialInstanceDynamic.SetScalarParameterValue` (`self.Ice3Mat`) "Brightness" 0.0)
  (`KismetSystemLibrary.K2_SetTimerDelegate` (delegate `LightUpIce`) (`self.Time`) true)
  (bind (_direction _lightvalue) (`Timeline|LightUp` :!label _label)
    (:`Update`
      (`MaterialInstanceDynamic.SetScalarParameterValue` (`self.Ice1Mat`) "Brightness" (* _lightvalue 5.0))
      (`MaterialInstanceDynamic.SetScalarParameterValue` (`self.Ice2Mat`) "Brightness" (* _lightvalue 5.0))
      (`MaterialInstanceDynamic.SetScalarParameterValue` (`self.Ice3Mat`) "Brightness" (* _lightvalue 5.0)))))

(event `LightUpIce`
  (goto _label :!via `PlayFromStart`))

(fn `UserConstructionScript`
  (`parent.UserConstructionScript`)
  (switch `int` (`self.CurrentLevel`)
    (:`1`
      (`SceneComponent.SetVisibility` (`self.Ice2`) false false)
      (`SceneComponent.SetVisibility` (`self.Ice3`) false false))
    (:`2`
      (`SceneComponent.SetVisibility` (`self.Ice2`) true false)
      (`SceneComponent.SetVisibility` (`self.Ice3`) false false))
    (:`3`
      (`SceneComponent.SetVisibility` (`self.Ice2`) true false)
      (`SceneComponent.SetVisibility` (`self.Ice3`) true false))))