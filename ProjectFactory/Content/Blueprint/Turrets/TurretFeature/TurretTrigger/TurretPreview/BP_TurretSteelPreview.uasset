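; Steel turret preview actor that displays the turret's form for its current level, from 1 to 3.
; The construction script calls the parent's, then switches on CurrentLevel to set the Scene scale, HandlerLR height and Neck visibility.
; Only level 3 shows the Neck and raises the handler; levels 2 and 3 resolve to the same scale.
; Tick spins Storage by a fixed step each frame, independent of delta time.
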(event `self.ReceiveTick`
  (params (DeltaSeconds :type "Float (single-precision)"))
  (`SceneComponent.K2_AddRelativeRotation` (`self.Storage`) (struct :`Yaw` 1.0) false false))

(fn `UserConstructionScript`
  (bind _currentlevel (`self.CurrentLevel`))
  (bind _currentlevel_2 (`self.CurrentLevel`))
  (bind _returnvalue (`KismetMathLibrary.Conv_IntToDouble` (`self.CurrentLevel`)))
  (bind _returnvalue_2 (`KismetMathLibrary.Conv_IntToDouble` _currentlevel))
  (bind _returnvalue_3 (* _currentlevel_2 1.5))
  (bind _returnvalue_4 (* _returnvalue 2.0))
  (`parent.UserConstructionScript`)
  (switch `int` (`self.CurrentLevel`)
    (:`1`
      (`SceneComponent.SetRelativeScale3D` (`self.Scene`) (`KismetMathLibrary.MakeVector` _returnvalue_4 _returnvalue_4 _returnvalue))
      (`SceneComponent.K2_SetRelativeLocation` (`self.HandlerLR`) (0.0 0.0 -25.0) false false)
      (`SceneComponent.SetVisibility` (`self.Neck`) false false))
    (:`2`
      (`SceneComponent.SetRelativeScale3D` (`self.Scene`) (`KismetMathLibrary.MakeVector` _returnvalue_3 _returnvalue_3 (* _currentlevel_2 0.75)))
      (`SceneComponent.K2_SetRelativeLocation` (`self.HandlerLR`) (0.0 0.0 -25.0) false false)
      (`SceneComponent.SetVisibility` (`self.Neck`) false false))
    (:`3`
      (`SceneComponent.SetRelativeScale3D` (`self.Scene`) (`KismetMathLibrary.MakeVector` _returnvalue_2 _returnvalue_2 (* _currentlevel 0.5)))
      (`SceneComponent.K2_SetRelativeLocation` (`self.HandlerLR`) (0.0 0.0 7.5) false false)
      (`SceneComponent.SetVisibility` (`self.Neck`) true false))))