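; Minigun turret preview that idles with a randomized scanning motion and shows upgrade parts for its current level.
; Initialize starts a looping timer that picks new random Neck and Center rotations, blended from the current ones by a timeline rate-scaled to the timer interval.
; Tick spins the barrels by a fixed step each frame.
; UpdateGraphicByLevel toggles the meshes: neither at level 1, Ammo at 2, Ammo and Aim at 3.
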(event `self.Initialize`
  (bind _time (`self.Time`))
  (`TimelineComponent.SetPlayRate` (`self.LerpTimeline`) (/ 1.0 _time))
  (`KismetSystemLibrary.K2_SetTimerDelegate` (delegate `Patrol`) _time true)
  (set `self.NeckInitialRotation` (`SceneComponent.RelativeRotation` (`self.Neck`)) :!label _label)
  (set `self.NeckNextRotation` (`KismetMathLibrary.MakeRotator` 0.0 0.0 (`KismetMathLibrary.RandomFloatInRange` 0.0 360.0)))
  (set `self.CenterInitialRotation` (`SceneComponent.RelativeRotation` (`self.Center`)))
  (set `self.CenterNextRotation` (`KismetMathLibrary.MakeRotator` 180.0 (`KismetMathLibrary.RandomFloatInRange` 60.0 120.0) -90.0))
  (bind (_direction _lerpvalue) (`Timeline|LerpTimeline` :!via `PlayFromStart`)
    (:`Update`
      (`SceneComponent.K2_SetRelativeRotation` (`self.Neck`) (`KismetMathLibrary.RLerp` (`self.NeckInitialRotation`) (`self.NeckNextRotation`) _lerpvalue true) false false)
      (`SceneComponent.K2_SetRelativeRotation` (`self.Center`) (`KismetMathLibrary.RLerp` (`self.CenterInitialRotation`) (`self.CenterNextRotation`) _lerpvalue true) false false))))

(event `Patrol`
  (goto _label))

(event `self.ReceiveTick`
  (params (DeltaSeconds :type "Float (single-precision)"))
  (`SceneComponent.K2_AddLocalRotation` (`self.Barrels`) (struct :`Pitch` 1.0) false false))

(fn `UpdateGraphicByLevel`
  (switch `int` (`self.CurrentLevel`)
    (:`1`
      (`SceneComponent.SetVisibility` (`self.Ammo`) false true)
      (`SceneComponent.SetVisibility` (`self.Aim`) false true))
    (:`2`
      (`SceneComponent.SetVisibility` (`self.Aim`) false true)
      (`SceneComponent.SetVisibility` (`self.Ammo`) true true))
    (:`3`
      (`SceneComponent.SetVisibility` (`self.Ammo`) true true)
      (`SceneComponent.SetVisibility` (`self.Aim`) true true))))

(fn `UserConstructionScript`
  (`parent.UserConstructionScript`))