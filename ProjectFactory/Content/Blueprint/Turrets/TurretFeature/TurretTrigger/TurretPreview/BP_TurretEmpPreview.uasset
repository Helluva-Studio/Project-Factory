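; Placement preview Blueprint for the EMP turret, showing a ring model that reflects the turret's level.
; The construction script runs the parent's script, then switches on CurrentLevel to set ring visibility.
; Level 1 hides the medium and big rings, level 2 shows only the medium one, and level 3 shows both.
; The event graph holds no logic.
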(event `self.ReceiveTick`
  (params (DeltaSeconds :type "Float (single-precision)")))

(fn `UserConstructionScript`
  (`parent.UserConstructionScript`)
  (switch `int` (`self.CurrentLevel`)
    (:`1`
      (`SceneComponent.SetVisibility` (`self.MediumRing`) false false)
      (`SceneComponent.SetVisibility` (`self.BigRing`) false false))
    (:`2`
      (`SceneComponent.SetVisibility` (`self.MediumRing`) true false)
      (`SceneComponent.SetVisibility` (`self.BigRing`) false false))
    (:`3`
      (`SceneComponent.SetVisibility` (`self.MediumRing`) true false)
      (`SceneComponent.SetVisibility` (`self.BigRing`) true false))))