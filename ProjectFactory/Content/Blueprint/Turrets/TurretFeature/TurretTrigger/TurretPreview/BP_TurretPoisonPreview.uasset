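; Preview actor for the poison turret, showing the flower model that matches its current level.
; The construction script runs the parent script, then shows one of three neck component hierarchies for levels 1 to 3 and hides the other two.
; Every tick, a sine of time since creation bobs the flower parts up and down, some in opposite phase, while they slowly spin in opposing directions.
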(event `self.ReceiveTick`
  (params (DeltaSeconds :type "Float (single-precision)"))
  (bind _returnvalue (/ (`KismetMathLibrary.DegSin` (* (`self.GetGameTimeSinceCreation`) 200.0)) 20.0))
  (`SceneComponent.K2_AddWorldOffset` (`self.FlowerB`) (`KismetMathLibrary.MakeVector` 0.0 0.0 _returnvalue) false false)
  (`SceneComponent.K2_AddWorldOffset` (`self.FlowerA`) (`KismetMathLibrary.MakeVector` 0.0 0.0 _returnvalue) false false)
  (`SceneComponent.K2_AddWorldOffset` (`self.FlowerC`) (`KismetMathLibrary.MakeVector` 0.0 0.0 _returnvalue) false false)
  (`SceneComponent.K2_AddWorldOffset` (`self.FlowerA2`) (`KismetMathLibrary.MakeVector` 0.0 0.0 (* _returnvalue -1.0)) false false)
  (`SceneComponent.K2_AddWorldOffset` (`self.FlowerB2`) (`KismetMathLibrary.MakeVector` 0.0 0.0 (* _returnvalue -1.0)) false false)
  (`SceneComponent.K2_AddWorldOffset` (`self.FlowerA1`) (`KismetMathLibrary.MakeVector` 0.0 0.0 _returnvalue) false false)
  (`SceneComponent.K2_AddLocalRotation` (`self.FlowerA1`) (struct :`Yaw` 0.3) false false)
  (`SceneComponent.K2_AddLocalRotation` (`self.FlowerA2`) (struct :`Yaw` 0.3) false false)
  (`SceneComponent.K2_AddLocalRotation` (`self.FlowerA`) (struct :`Yaw` 0.3) false false)
  (`SceneComponent.K2_AddLocalRotation` (`self.FlowerC`) (struct :`Yaw` 0.3) false false)
  (`SceneComponent.K2_AddLocalRotation` (`self.FlowerB`) (struct :`Yaw` -0.3) false false)
  (`SceneComponent.K2_AddLocalRotation` (`self.FlowerB2`) (struct :`Yaw` -0.3) false false))

(fn `UserConstructionScript`
  (`parent.UserConstructionScript`)
  (switch `int` (`self.CurrentLevel`)
    (:`1`
      (`SceneComponent.SetVisibility` (`self.Neck`) false true)
      (`SceneComponent.SetVisibility` (`self.Neck2`) false true)
      (`SceneComponent.SetVisibility` (`self.Neck1`) true true))
    (:`2`
      (`SceneComponent.SetVisibility` (`self.Neck`) false true)
      (`SceneComponent.SetVisibility` (`self.Neck2`) true true)
      (`SceneComponent.SetVisibility` (`self.Neck1`) false true))
    (:`3`
      (`SceneComponent.SetVisibility` (`self.Neck`) true true)
      (`SceneComponent.SetVisibility` (`self.Neck2`) false true)
      (`SceneComponent.SetVisibility` (`self.Neck1`) false true))))