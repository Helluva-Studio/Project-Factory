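; Preview actor for the gravity turret that shows a pulsing black hole made of upper and lower components.
; The construction script runs the parent's setup, then sizes both components by CurrentLevel across three levels and stores that as the initial scale.
; From BeginPlay, a looping timer restarts a Scaling timeline, with play rate matched to the timer interval, that multiplies the initial scale to animate both.
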(event `self.ReceiveBeginPlay`
  (`KismetSystemLibrary.K2_SetTimerDelegate` (delegate `ScaleBlackHole`) 0.5 true)
  (`self.ScaleBlackHole`))

(event `ScaleBlackHole`
  (`TimelineComponent.SetPlayRate` (`self.Scaling`) (`KismetMathLibrary.SafeDivide` 1.0 0.5))
  (bind (_direction _scalebh) (`Timeline|Scaling` :!via `PlayFromStart`)
    (:`Update`
      (`SceneComponent.SetRelativeScale3D` (`self.UpperBH`) (* _scalebh (`self.InitialScale`)))
      (`SceneComponent.SetRelativeScale3D` (`self.LowerBH`) (* _scalebh (`self.InitialScale`))))))

(event `self.ReceiveTick`
  (params (DeltaSeconds :type "Float (single-precision)")))

(fn `UserConstructionScript`
  (`parent.UserConstructionScript`)
  (switch `int` (`self.CurrentLevel`)
    (:`1`
      (`SceneComponent.SetWorldScale3D` (`self.UpperBH`) (0.1 0.1 0.1))
      (`SceneComponent.SetWorldScale3D` (`self.LowerBH`) (0.1 0.1 0.1))
      (set `self.InitialScale` (`SceneComponent.RelativeScale3D` (`self.LowerBH`))))
    (:`2`
      (`SceneComponent.SetWorldScale3D` (`self.UpperBH`) (0.3 0.3 0.3))
      (`SceneComponent.SetWorldScale3D` (`self.LowerBH`) (0.3 0.3 0.3))
      (set `self.InitialScale` (`SceneComponent.RelativeScale3D` (`self.LowerBH`))))
    (:`3`
      (`SceneComponent.SetWorldScale3D` (`self.UpperBH`) (0.5 0.5 0.5))
      (`SceneComponent.SetWorldScale3D` (`self.LowerBH`) (0.5 0.5 0.5))
      (set `self.InitialScale` (`SceneComponent.RelativeScale3D` (`self.LowerBH`))))))