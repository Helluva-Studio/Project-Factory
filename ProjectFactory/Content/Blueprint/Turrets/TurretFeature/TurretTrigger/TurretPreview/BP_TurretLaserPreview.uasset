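; Laser turret preview that idly swings its neck to random angles and shows the gun mesh for its current level.
; Initialize scales the lerp timeline to the Time variable and starts a looping Patrol timer with that same interval.
; Each cycle picks a random single-axis target, and the timeline interpolates the neck toward it along the shortest path.
; UpdateGraphicByLevel swaps the gun static mesh among three level variants.
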(event `self.ReceiveTick`
  (params (DeltaSeconds :type "Float (single-precision)")))

(event `self.Initialize`
  (bind _time (`self.Time`))
  (`TimelineComponent.SetPlayRate` (`self.LerpTimeline`) (/ 1.0 _time))
  (`KismetSystemLibrary.K2_SetTimerDelegate` (delegate `Patrol`) _time true)
  (set `self.NeckInitialRotation` (`SceneComponent.RelativeRotation` (`self.Neck`)) :!label _label)
  (set `self.NeckNextRotation` (`KismetMathLibrary.MakeRotator` 0.0 0.0 (`KismetMathLibrary.RandomFloatInRange` 0.0 360.0)))
  (bind (_direction _lerpvalue) (`Timeline|LerpTimeline` :!via `PlayFromStart`)
    (:`Update`
      (`SceneComponent.K2_SetRelativeRotation` (`self.Neck`) (`KismetMathLibrary.RLerp` (`self.NeckInitialRotation`) (`self.NeckNextRotation`) _lerpvalue true) false false))))

(event `Patrol`
  (goto _label))

(fn `UpdateGraphicByLevel`
  (switch `int` (`self.CurrentLevel`)
    (:`1`
      (`StaticMeshComponent.SetStaticMesh` (`self.Gun`) "/Game/Models/Turret/Meshes/Laser/SM_L_Gun1.SM_L_Gun1"))
    (:`2`
      (`StaticMeshComponent.SetStaticMesh` (`self.Gun`) "/Game/Models/Turret/Meshes/Laser/SM_L_Gun2.SM_L_Gun2"))
    (:`3`
      (`StaticMeshComponent.SetStaticMesh` (`self.Gun`) "/Game/Models/Turret/Meshes/Laser/SM_L_Gun3.SM_L_Gun3"))))

(fn `UserConstructionScript`
  (`parent.UserConstructionScript`))