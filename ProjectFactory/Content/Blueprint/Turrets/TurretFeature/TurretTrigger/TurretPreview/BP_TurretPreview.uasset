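; Turret placement preview actor that shows whether a turret can be built by tinting its meshes.
; The construction script gathers all static mesh components and passes the CanBeBuild flag to SetPreview.
; SetPreview swaps every material slot on those meshes to the OK or NO preview material instance.
; The event graph has no active logic.
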(fn `SetPreview`
  (params (CanBeBuild :type Boolean))
  (if CanBeBuild
    (for _array_element (`self.ActorMeshes`)
      (for (_ _array_index) (`MeshComponent.GetMaterials` _array_element)
        (`PrimitiveComponent.SetMaterial` _array_element _array_index "/Game/Blueprint/Turrets/TurretFeature/TurretTrigger/MI_TurretPreviewOK.MI_TurretPreviewOK")))
    (else
      (for _array_element_2 (`self.ActorMeshes`)
        (for (_ _array_index_2) (`MeshComponent.GetMaterials` _array_element_2)
          (`PrimitiveComponent.SetMaterial` _array_element_2 _array_index_2 "/Game/Blueprint/Turrets/TurretFeature/TurretTrigger/MI_TurretPreviewNO.MI_TurretPreviewNO"))))))

(fn `UserConstructionScript`
  (set `self.ActorMeshes` (`self.K2_GetComponentsByClass` "/Script/Engine.StaticMeshComponent"))
  (`self.SetPreview` (`self.CanBeBuild`)))