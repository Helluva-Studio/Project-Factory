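; Slow turret Blueprint, a child turret that applies a crowd-control slow through an area-of-effect ammo.
; On initialization it reads the slow strength from its initialization row, then triggers the CC AoE spawn.
; After the parent spawn logic, it passes CC type, area shape and size, player-hit flag and slow effect to the CcAmmo.
; Turret level sets how many of its extra ice components are visible.
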(event `self.ReceiveTick`
  (params (DeltaSeconds :type "Float (single-precision)"))
  (`parent.ReceiveTick` DeltaSeconds))

(event `self.SpawnCcAoe`
  (`parent.SpawnCcAoe`)
  (`/Engine/EditorBlueprintResources/StandardMacros.IsValid` (`self.CcAmmo`)
    (:`Is Valid`
      (message `/Game/Blueprint/Turrets/Interfaces/BPI_TurretCcAmmo.InitializeCcAmmo` (`self.CcAmmo`) (`self.CanHitPlayer`) (`self.TypeOfCc`) (`self.TypeOfAoe`) (`self.MaxAngleOfEffect(Cone)`) (`self.MaxDistance(Cone)/MaxRadius(Sphere)`) (`self.SlowEffect`) 0.0 0.0 0.0))))

(fn `InitializeTurret`
  (`parent.InitializeTurret`)
  (set `self.SlowEffect` (`.SlowEffectCc_140_2F2F630B4C476F688F1F7FB7EEDA8012` (break `/Game/Blueprint/Turrets/TurretFeature/Leveling/S_TurretChangebleValue` (`self.InitializationRow`))))
  (`self.SpawnCcAoe`))

(fn `UpdateGraphicByLevel`
  (params (Level :type Integer))
  (`/Engine/EditorBlueprintResources/StandardMacros.IsValid` self
    (:`Is Valid`
      (switch `int` Level
        (:`1`
          (`SceneComponent.SetVisibility` (`self.Ice2`) false false)
          (`SceneComponent.SetVisibility` (`self.Ice3`) false false))
        (:`2`
          (`SceneComponent.SetVisibility` (`self.Ice2`) true false)
          (`SceneComponent.SetVisibility` (`self.Ice3`) false false))
        (:`3`
          (`SceneComponent.SetVisibility` (`self.Ice2`) true false)
          (`SceneComponent.SetVisibility` (`self.Ice3`) true false))))))

(fn `UserConstructionScript`
  (`parent.UserConstructionScript`))