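; Shock turret that spawns a chain-lightning AoE ammo actor (DamageAmmo) to deal electric damage, configured per level from DT_H_Shock.
; Interacting, free outside cooldown, toggles single-target mode: a timeline plays or reverses to scale the radius and move the beam end vertically, then re-initializes the ammo.
; Cooldown destroys the ammo and hides or fades its effects and sound; level also controls which lights show.
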(event `self.ReceiveBeginPlay`
  (`parent.ReceiveBeginPlay`)
  (`SceneComponent.SetVisibility` (`self.Shock`) false false)
  (`SceneComponent.SetVisibility` (`self.Terrain`) false false))

(event `self.ReceiveTick`
  (params (DeltaSeconds :type "Float (single-precision)"))
  (`parent.ReceiveTick` DeltaSeconds))

(event `self.SpawnAmmo`
  (`parent.SpawnAmmo`)
  (`/Engine/EditorBlueprintResources/StandardMacros.IsValid` (`self.DamageAmmo`)
    (:`Is Valid`
      (`SceneComponent.SetVisibility` (`self.Shock`) true false)
      (`SceneComponent.SetVisibility` (`self.Terrain`) true false)
      (message `/Game/Blueprint/Turrets/Interfaces/BPI_TurretDamageAmmo.InitializeShockAmmo` (`self.DamageAmmo`) (`self.CanHitPlayer`) (`self.D_TypeOfDamage`) (`self.D_TypeOfAoe`) (`self.MaxDistance(Cone)/MaxRadius(Sphere)`) (`self.RadiusReductionPercentageOnPropagation`) (`self.DamageTick`) (`self.MaxDamageOnHit`) (`self.DamageReductionPercentageOnPropagation`) (`self.AoeTick`) (`self.AoeDamage`) (`self.ReachableEnemies`) (`self.NumberOfInitialChain`) (`self.ModeSingleTarget`))
      (set `self.CanChangeMode` true)
      (`AudioComponent.FadeIn` (`self.SW_Electricity`) 1.0 1.0 0.0 "Linear"))))

(event `self.Focus`
  (params (IsFocused :type Boolean))
  (for _array_element (`self.MeshesToOutline`)
    (`PrimitiveComponent.SetRenderCustomDepth` _array_element IsFocused)))

(event `/Game/Blueprint/Turrets/Interfaces/BI_Interactable.Interact`
  (bind _damageammo (`self.DamageAmmo`))
  (bind _damageammo_2 (`self.DamageAmmo`))
  (bind _shock (`self.Shock`))
  (bind _d_basedistance_cone__baseradius_sphere_ (`self.D_BaseDistance(Cone)/BaseRadius(Sphere)`))
  (bind (_returnvalue_x _returnvalue_y _returnvalue_z) (`KismetMathLibrary.BreakVector` (`SceneComponent.K2_GetComponentLocation` _shock)))
  (set `self.CanChangeMode` false)
  (bind _isa (`/Engine/EditorBlueprintResources/StandardMacros.FlipFlop`)
    (:`A`
      _)
    (:`B`
      _))
  (set `self.ModeSingleTarget` _isa)
  (`/Engine/EditorBlueprintResources/StandardMacros.IsValid` _damageammo
    (:`Is Valid`
      (bind _asbp_aoe_shock (cast `/Game/Blueprint/Turrets/TurretFeature/Aoe/BP_AoeShock` _damageammo))
      (`/Game/Blueprint/Turrets/TurretFeature/Aoe/BP_AoeShock.DestroyNiagara` _asbp_aoe_shock)
      (if (`self.ModeSingleTarget`)
        (bind (_direction _value) (`Timeline|Timeline_0` :!via `PlayFromStart` :!label _label)
          (:`Update`
            (`|ExecutionSequence`
              (:`then_0`
                (set `self.MaxDistance(Cone)/MaxRadius(Sphere)` (`KismetMathLibrary.Lerp` _d_basedistance_cone__baseradius_sphere_ (* _d_basedistance_cone__baseradius_sphere_ (- 2.0 (`self.ChangeModeModifier`))) _value))
                (`/Engine/EditorBlueprintResources/StandardMacros.IsValid` _damageammo_2
                  (:`Is Valid`
                    (`SceneComponent.SetWorldScale3D` (`Actor.RootComponent` _damageammo_2) (`KismetMathLibrary.Conv_DoubleToVector` (/ (`self.MaxDistance(Cone)/MaxRadius(Sphere)`) 100.0))))))
              (:`then_1`
                (`FXSystemComponent.SetVectorParameter` _shock "BeamEnd" (`KismetMathLibrary.MakeVector` _returnvalue_x _returnvalue_y (`KismetMathLibrary.Lerp` _returnvalue_z (+ _returnvalue_z 150.0) _value))))))
          (:`Finished`
            (`/Engine/EditorBlueprintResources/StandardMacros.IsValid` (`self.DamageAmmo`)
              (:`Is Valid`
                (message `/Game/Blueprint/Turrets/Interfaces/BPI_TurretDamageAmmo.InitializeShockAmmo` (`self.DamageAmmo`) (`self.CanHitPlayer`) (`self.D_TypeOfDamage`) (`self.D_TypeOfAoe`) (`self.MaxDistance(Cone)/MaxRadius(Sphere)`) (`self.RadiusReductionPercentageOnPropagation`) (`self.DamageTick`) (`self.MaxDamageOnHit`) (`self.DamageReductionPercentageOnPropagation`) (`self.AoeTick`) (`self.AoeDamage`) (`self.ReachableEnemies`) (`self.NumberOfInitialChain`) false)
                (`/Game/Blueprint/Turrets/TurretFeature/Aoe/BP_Turret_DamageBase.ChangeMode` (`self.DamageAmmo`) (`self.ModeSingleTarget`))
                (set `self.CanChangeMode` true)))))
        (else
          (goto _label :!via `ReverseFromEnd`))))))

(fn `CanInteract`
  (returns (CanInteract :type Boolean))
  (return (and (`self.CanChangeMode`) (not (`self.IsInCooldown`)))))

(fn `GetCost`
  (returns (GetCost :type "Float (double-precision)"))
  (return 0.0))

(fn `GetInteractImage`
  (returns (Image :type "Texture Object Reference"))
  (return "/Game/2DImage/Rotate.Rotate"))

(fn `GetInteractMessage`
  (returns (InteractMessage :type Text) (Image :type "Texture Object Reference"))
  (return "" "/Game/2DImage/Rotate.Rotate"))

(fn `InitializeTurret`
  (bind _returnvalue (`|GetDataTableRow` "/Game/Blueprint/Turrets/TurretFeature/Leveling/TurretSpecificDataTable/DT_H_Shock.DT_H_Shock" (`KismetStringLibrary.Conv_StringToName` (`KismetStringLibrary.Conv_IntToString` (`self.CurrentLevel`))))
    (:`then`
      (bind (_maxhealth _maxactivitytime _maxcdtime _baseaoetype _baseradius _radiuspercentagemodifier _baseradiusreductionpercentageperpropagation _damagetype _basetickbetweenstrike _damageonhit _basedamagereductionpercentageperpropagation _basechangemodemodifierpercentage _aoetick _aoedamage _reachableenemies _numberofinitialchain) (break `/Game/Blueprint/Turrets/TurretFeature/Leveling/TurretStructs/S_H_Shock` _returnvalue))
      (bind _output_get (set `self.MaxHealth` _maxhealth))
      (set `self.CurrentHealth` _output_get)
      (set `self.MaxActivityTime(NoFarm)` _maxactivitytime)
      (set `self.MaxCdTime` _maxcdtime)
      (set `self.D_TypeOfAoe` _baseaoetype)
      (bind _output_get_2 (set `self.MaxDistance(Cone)/MaxRadius(Sphere)` (+ _baseradius (* _baseradius (/ _radiuspercentagemodifier 100.0)))))
      (set `self.D_BaseDistance(Cone)/BaseRadius(Sphere)` _output_get_2)
      (set `self.RadiusReductionPercentageOnPropagation` _baseradiusreductionpercentageperpropagation)
      (set `self.D_TypeOfDamage` _damagetype)
      (set `self.DamageTick` _basetickbetweenstrike)
      (set `self.MaxDamageOnHit` _damageonhit)
      (set `self.DamageReductionPercentageOnPropagation` _basedamagereductionpercentageperpropagation)
      (set `self.ChangeModeModifier` (+ 1.0 (/ _basechangemodemodifierpercentage 100.0)))
      (set `self.AoeTick` _aoetick)
      (set `self.AoeDamage` _aoedamage)
      (set `self.ReachableEnemies` _reachableenemies)
      (set `self.NumberOfInitialChain` _numberofinitialchain)
      (`FXSystemComponent.SetFloatParameter` (`self.Terrain`) "Radius" (`self.MaxDistance(Cone)/MaxRadius(Sphere)`)))))

(fn `OnCDEnded`
  (`parent.OnCDEnded`)
  (`SceneComponent.SetVisibility` (`self.Shock`) true false)
  (`SceneComponent.SetVisibility` (`self.Shock`) true false))

(fn `OnCDStarted`
  (bind _damageammo (`self.DamageAmmo`))
  (`parent.OnCDStarted`)
  (`SceneComponent.SetVisibility` (`self.Shock`) false false)
  (`SceneComponent.SetVisibility` (`self.Terrain`) false false)
  (`AudioComponent.FadeOut` (`self.SW_Electricity`) 1.0 0.0 "Linear")
  (`/Engine/EditorBlueprintResources/StandardMacros.IsValid` _damageammo
    (:`Is Valid`
      (bind _asbp_aoe_shock (cast `/Game/Blueprint/Turrets/TurretFeature/Aoe/BP_AoeShock` _damageammo))
      (`/Game/Blueprint/Turrets/TurretFeature/Aoe/BP_AoeShock.DestroyNiagara` _asbp_aoe_shock)
      (`self.K2_DestroyActor` _damageammo))))

(fn `UpdateGraphicByLevel`
  (params (Level :type Integer))
  (`/Engine/EditorBlueprintResources/StandardMacros.IsValid` self
    (:`Is Valid`
      (switch `int` Level
        (:`1`
          (`SceneComponent.SetVisibility` (`self.Light2`) false false)
          (`SceneComponent.SetVisibility` (`self.Light3`) false false))
        (:`2`
          (`SceneComponent.SetVisibility` (`self.Light2`) true false)
          (`SceneComponent.SetVisibility` (`self.Light3`) false false))
        (:`3`
          (`SceneComponent.SetVisibility` (`self.Light2`) true false)
          (`SceneComponent.SetVisibility` (`self.Light3`) true false))))))

(fn `UserConstructionScript`
  (`parent.UserConstructionScript`)
  (`FXSystemComponent.SetVectorParameter` (`self.Shock`) "BeamEnd" (`SceneComponent.K2_GetComponentLocation` (`self.Shock`))))

(fn `WhichInteraction`
  (returns (TypeInteraction :type "/Game/Blueprint/Enum/EInteractable Enum"))
  (return "NewEnumerator0"))