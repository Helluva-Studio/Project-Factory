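; Flamethrower turret that fires on a repeating timer, alternating between a rest delay and a timed flame, with no targeting.
; Each cycle spawns a BP_Flame at the Arrow, passes it Damage, then destroys it after FlameTime.
; Interacting costs nothing and rotates the turret in 45-degree steps, carrying any active flame along.
; Tick turns the visible widget toward the camera, but its overlap-driven visibility toggles are disconnected.
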(event `self.ReceiveBeginPlay`
  (`parent.ReceiveBeginPlay`)
  (`self.Rest`))

(event `self.ReceiveTick`
  (params (DeltaSeconds :type "Float (single-precision)"))
  (`parent.ReceiveTick` DeltaSeconds)
  (bind _widget_0 (`self.Widget_0`)
    (:`then`
      (if (`SceneComponent.IsVisible` _widget_0)
        (`SceneComponent.K2_SetWorldRotation` (`self.Widget_0`) (`KismetMathLibrary.FindLookAtRotation` (`SceneComponent.K2_GetComponentLocation` _widget_0) (`SceneComponent.K2_GetComponentLocation` (`PlayerCameraManager.TransformComponent` (`GameplayStatics.GetPlayerCameraManager` 0)))) false false)))
    (:`else`)))

(event `Flame`
  (bind (_returnvalue_location _returnvalue_rotation) (`KismetMathLibrary.BreakTransform` (`SceneComponent.K2_GetComponentToWorld` (`self.Arrow`))))
  (bind _returnvalue (`|SpawnActorFromClass` "/Game/Blueprint/Turrets/Ammunation/BP_Flame.BP_Flame_C" (`KismetMathLibrary.MakeTransform` _returnvalue_location _returnvalue_rotation) "AdjustIfPossibleButAlwaysSpawn" "MultiplyWithRoot" null null))
  (`/Game/Blueprint/Turrets/Ammunation/BP_Flame.Initialize` _returnvalue (`self.Damage`) 0.0 0.0)
  (bind _output_get (set `self.FlameShooted` _returnvalue))
  (`KismetSystemLibrary.Delay` (`self.FlameTime`))
  (`self.K2_DestroyActor` _output_get)
  (`self.Rest`))

(event `Rest`
  (`KismetSystemLibrary.Delay` (`self.RestTime`))
  (`self.Flame`))

(event `/Game/Blueprint/Turrets/Interfaces/BI_Interactable.Interact`
  (`self.K2_SetActorRotation` (`KismetMathLibrary.ComposeRotators` (`self.K2_GetActorRotation`) (struct :`Yaw` 45.0)))
  (bind _flameshooted (`self.FlameShooted`)
    (:`then`
      (`self.K2_SetActorTransform` _flameshooted (`KismetMathLibrary.MakeTransform` (`SceneComponent.K2_GetComponentLocation` (`self.Arrow`)) (`KismetMathLibrary.ComposeRotators` (`self.K2_GetActorRotation` (`self.FlameShooted`)) (struct :`Yaw` 45.0))) false false))
    (:`else`)))

(event `self.ReceiveDestroyed`
  (bind _flameshooted (`self.FlameShooted`)
    (:`then`
      (`self.K2_DestroyActor` _flameshooted))
    (:`else`)))

(event `self.Box.OnComponentBeginOverlap`
  (params (OverlappedComponent :type "PrimitiveComponent Object Reference") (OtherActor :type "Actor Object Reference") (OtherComp :type "PrimitiveComponent Object Reference") (OtherBodyIndex :type Integer) (bFromSweep :type Boolean) (SweepResult :type "HitResult Structure (by ref)")))

(event `self.Box.OnComponentEndOverlap`
  (params (OverlappedComponent :type "PrimitiveComponent Object Reference") (OtherActor :type "Actor Object Reference") (OtherComp :type "PrimitiveComponent Object Reference") (OtherBodyIndex :type Integer)))

(fn `CanInteract`
  (returns (CanInteract :type Boolean))
  (return true))

(fn `GetCost`
  (returns (GetCost :type "Float (double-precision)"))
  (return 0.0))

(fn `UserConstructionScript`
  (`parent.UserConstructionScript`))

(fn `WhichInteraction`
  (returns (TypeInteraction :type "/Game/Blueprint/Enum/EInteractable Enum"))
  (return "NewEnumerator0"))