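; Crowd-control turret that keeps an area-effect actor active while it is not in cooldown.
; Tick uses paired DoOnce gates that reset each other, destroying the effect when cooldown starts and respawning it when cooldown ends.
; SpawnCC picks a class by CC type, attaches it at Center and initializes it as a BP_Turret_Effect with area, slow, stun and gravity settings.
; Death destroys a valid CcActorAmmo before running parent death logic.
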(event `self.ReceiveTick`
  (params (DeltaSeconds :type "Float (single-precision)"))
  (if (`self.IsInCooldown`)
    (`/Engine/EditorBlueprintResources/StandardMacros.DoOnce` false :!label _label
      (:`Completed`
        (`self.K2_DestroyActor` (`self.CcActor`))
        (goto _label_2 :!via `Reset`)))
    (else
      (`/Engine/EditorBlueprintResources/StandardMacros.DoOnce` false :!label _label_2
        (:`Completed`
          (`self.SpawnCC`)
          (goto _label :!via `Reset`))))))

(event `SpawnCC`
  (bind _keys (`BlueprintMapLibrary.Map_Keys` (`self.CcActors`)))
  (bind _values (`BlueprintMapLibrary.Map_Values` (`self.CcActors`)))
  (bind _returnvalue (`|SpawnActorFromClass` (`|GetArrayItem` _values (`KismetArrayLibrary.Array_Find` _keys (`self.TypeOfCC`))) (`KismetMathLibrary.MakeTransform` (`SceneComponent.K2_GetComponentLocation` (`self.Center`))) "AlwaysSpawn" "MultiplyWithRoot" null null))
  (bind _output_get (set `self.CcActor` _returnvalue))
  (`self.K2_AttachToComponent` _output_get (`self.Center`) "None" "KeepWorld" "KeepRelative" "KeepWorld" true)
  (bind _asbp_turret_effect (cast `/Game/Blueprint/Turrets/TurretFeature/Aoe/BP_Turret_Effect` _returnvalue))
  (`/Game/Blueprint/Turrets/TurretFeature/Aoe/BP_Turret_Effect.Initialize` _asbp_turret_effect (`self.Can Hit Player`) 0.0 0.0 0.0 (`self.TypeOfAoe`) "NewEnumerator0" (`self.Max Distance(Cone)/ Max Radius(Sphere)`) (`self.Max Angle Of Effect(Cone)`) (`self.Time Tick`) (`self.Slow Effect`) (`self.Stun Time`) (`self.Gravity Force`)))

(fn `Death`
  (bind _ccactorammo (`self.CcActorAmmo`))
  (`/Engine/EditorBlueprintResources/StandardMacros.IsValid` _ccactorammo
    (:`Is Valid`
      (`self.K2_DestroyActor` _ccactorammo)
      (`parent.Death`))))

(fn `UserConstructionScript`
  (`parent.UserConstructionScript`))