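; Save data object that captures a snapshot of a run: world, player and placed-object state.
; Initialize copies seed, room progression, day, clock and frenzy values from the GameInstance and GameMode, and stats, resources, shop items and turret selection from BP_Roberto.
; GameMode getters supply doors, junk, turrets, triggers, rechargers, levers, farmers and blueprints, flattened into struct or key arrays via AddUnique.
; Only the passed-in turret blueprint list is cleared before refilling.
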(fn `Initialize`
  (params (Player :type "Actor Object Reference") (GameMode :type "GameModeBase Object Reference") (GameInstance :type "GameInstance Object Reference") (BlueprintList :type "Array of /Game/Blueprint/Turrets/TurretGetter/BP_TurretBlueprint Object Reference (by ref)"))
  (`self.SetWorld` GameMode GameInstance)
  (`self.SetPlayer` Player)
  (`self.SaveBlueprints` BlueprintList))

(fn `SaveBlueprints`
  (params (BlueprintList :type "Array of /Game/Blueprint/Turrets/TurretGetter/BP_TurretBlueprint Object Reference"))
  (`KismetArrayLibrary.Array_Clear` (`self.TurretBlueprintStruct`))
  (for _array_element BlueprintList
    (`KismetArrayLibrary.Array_Add` (`self.TurretBlueprintStruct`) (make `/Game/2DImage/Levers/S_TurrretBlueprintStruct` (`Actor.GetTransform` _array_element) (`/Game/Blueprint/Turrets/TurretGetter/BP_TurretBlueprint.Type` _array_element) (`/Game/Blueprint/Turrets/TurretGetter/BP_TurretBlueprint.Turret` _array_element))))
  (`KismetSystemLibrary.PrintString` null (`KismetStringLibrary.Conv_IntToString` (`KismetArrayLibrary.Array_Length` (`self.TurretBlueprintStruct`)))))

(fn `SetBlueprint`
  (params (self2 :type "/Game/GameMode/BP_NewGameMode Object Reference"))
  (bind _turretblueprint (`/Game/GameMode/BP_NewGameMode.GetAllBlueprints` self2))
  (for _array_element _turretblueprint
    (`KismetArrayLibrary.Array_AddUnique` (`self.BlueprintInGame`) (`/Game/Blueprint/Turrets/TurretGetter/BP_TurretBlueprint.Type` _array_element))))

(fn `SetDoors`
  (params (self2 :type "/Game/GameMode/BP_NewGameMode Object Reference"))
  (bind _outdoors (`/Game/GameMode/BP_NewGameMode.GetAllDoors` self2))
  (if (`KismetArrayLibrary.Array_IsNotEmpty` _outdoors)
    (for _array_element _outdoors
      (if (`/Game/Blueprint/Envirorment/Doors/BP_WFC_Door.Purchased` _array_element)
        (`KismetArrayLibrary.Array_AddUnique` (`self.Doors `) (`/Game/Blueprint/Envirorment/Doors/BP_WFC_Door.Index` _array_element))))))

(fn `SetEnergyRecharger`
  (params (self2 :type "/Game/GameMode/BP_NewGameMode Object Reference"))
  (bind _energyrecharger (`/Game/GameMode/BP_NewGameMode.GetAllEnergyRecharger` self2))
  (for _array_element _energyrecharger
    (`KismetArrayLibrary.Array_AddUnique` (`self.EnergyRechargers`) (make `/Game/Blueprint/Save/S_EnergyRechargersForSave` (`/Game/Blueprint/EnergyRecharger/BP_EnergyRecharger.Location` _array_element) (`/Game/Blueprint/EnergyRecharger/BP_EnergyRecharger.EnergyStorage` _array_element) (`/Game/Blueprint/EnergyRecharger/BP_EnergyRecharger.IsInCooldown` _array_element) (`/Game/Blueprint/EnergyRecharger/BP_EnergyRecharger.Reactivation Percentage Normalized` _array_element)))))

(fn `SetFarmer`
  (params (Gamemodee :type "/Game/GameMode/BP_NewGameMode Object Reference"))
  (bind _outactors (`/Game/GameMode/BP_NewGameMode.GetAllFarmer` Gamemodee))
  (for _array_element _outactors
    (`KismetArrayLibrary.Array_AddUnique` (`self.Farmer`) (make `/Game/Blueprint/Save/S_FarmerForSave` (`/Game/Blueprint/Turrets/BP_Turret_Base.LocationForSave` _array_element) (`/Game/Blueprint/Turrets/BP_F_Farming.ResourceStored` _array_element) (`/Game/Blueprint/Turrets/BP_F_Farming.IsSpawningResource` _array_element) (`/Game/Blueprint/Turrets/BP_Turret_Base.CdTime` _array_element)))))

(fn `SetJunk`
  (params (self2 :type "/Game/GameMode/BP_NewGameMode Object Reference"))
  (bind _junks (`/Game/GameMode/BP_NewGameMode.GetAllJunks` self2))
  (for _array_element _junks
    (`KismetArrayLibrary.Array_AddUnique` (`self.JunksInGame`) (make `/Game/Blueprint/Save/S_JunkForSave` (`/Game/Blueprint/Junks/BP_Junk.Position` _array_element) (`/Game/Blueprint/Junks/BP_Junk.Health` _array_element)))))

(fn `SetJunkSpawner`
  (params (self2 :type "/Game/GameMode/BP_NewGameMode Object Reference"))
  (bind _junkspawner (`/Game/GameMode/BP_NewGameMode.GetAllJunkSpawner` self2))
  (for _array_element _junkspawner
    (`KismetArrayLibrary.Array_AddUnique` (`self.JunksSpawnerInGame`) (make `/Game/Blueprint/Save/S_JunkSpawnerForSave` (`/Game/Blueprint/Junks/BP_JunkSpawner.Location` _array_element) (`/Game/Blueprint/Junks/BP_JunkSpawner.HasSpawnJunk` _array_element)))))

(fn `SetLevel`
  (params (Gamemodee :type "/Game/GameMode/BP_NewGameMode Object Reference"))
  (bind _turretblueprint (`/Game/GameMode/BP_NewGameMode.Get Lever` Gamemodee))
  (for _array_element _turretblueprint
    (`KismetArrayLibrary.Array_AddUnique` (`self.Lever`) (make `/Game/Blueprint/Save/S_LeverForSave` (`/Game/Blueprint/Envirorment/BP_Lever.Index` _array_element) (`/Game/Blueprint/Envirorment/BP_Lever.LeverPulled` _array_element)))))

(fn `SetPlayer`
  (params (Actor :type "Actor Object Reference"))
  (bind _asbp_roberto (cast `/Game/Blueprint/Robot/Blueprints/BP_Roberto` Actor))
  (set `self.PlayerPos` (`Actor.GetTransform` _asbp_roberto))
  (set `self.Health` (`/Game/Blueprint/Robot/Blueprints/BP_Roberto.Health` _asbp_roberto))
  (set `self.MaxHealth` (`/Game/Blueprint/Robot/Blueprints/BP_Roberto.MaxHealth` _asbp_roberto))
  (set `self.Energy` (`/Game/Blueprint/Robot/Blueprints/BP_Roberto.Energy` _asbp_roberto))
  (set `self.MaxEnergy` (`/Game/Blueprint/Robot/Blueprints/BP_Roberto.MaxEnergy` _asbp_roberto))
  (set `self.Gear` (`/Game/Blueprint/Robot/Blueprints/BP_Roberto.Gear` _asbp_roberto))
  (set `self.Steel` (`/Game/Blueprint/Robot/Blueprints/BP_Roberto.Steel` _asbp_roberto))
  (set `self.Circuit` (`/Game/Blueprint/Robot/Blueprints/BP_Roberto.Circuit` _asbp_roberto))
  (set `self.Essence` (`/Game/Blueprint/Robot/Blueprints/BP_Roberto.Essence` _asbp_roberto))
  (set `self.JunkDamage` (`/Game/Blueprint/Robot/Blueprints/BP_Roberto.Base Damage` _asbp_roberto))
  (set `self.powerUpItems` (`/Game/Blueprint/Robot/Blueprints/BPC_Shop.PowerUpItems` (`/Game/Blueprint/Robot/Blueprints/BP_Roberto.BPC_Shop` _asbp_roberto)))
  (bind _bpc_turretselectionsystem (`/Game/Blueprint/Robot/Blueprints/BP_Roberto.BPC_TurretSelectionSystem` _asbp_roberto))
  (set `self.TurretLevel` (`/Game/Blueprint/Robot/Blueprints/BPC_TurretSelectionSystem.TurretLevel` _bpc_turretselectionsystem))
  (set `self.SelectedTurret` (`.TurretType` (defaults `Object` (`/Game/Blueprint/Robot/Blueprints/BPC_TurretSelectionSystem.TurretSelected` _bpc_turretselectionsystem)))))

(fn `SetTurret`
  (params (self2 :type "/Game/GameMode/BP_NewGameMode Object Reference"))
  (bind _turrets (`/Game/GameMode/BP_NewGameMode.GetAllTurrets` self2))
  (for _array_element _turrets
    (`KismetArrayLibrary.Array_AddUnique` (`self.TurretsInGame`) (make `/Game/Blueprint/Save/S_TurretForSave` (`/Game/Blueprint/Turrets/BP_Turret_Base.LocationForSave` _array_element) (`/Game/Blueprint/Turrets/BP_Turret_Base.CurrentHealth` _array_element) (`/Game/Blueprint/Turrets/BP_Turret_Base.IsInFunction(NoFarm)` _array_element) (`/Game/Blueprint/Turrets/BP_Turret_Base.IsInCooldown` _array_element) (`/Game/Blueprint/Turrets/BP_Turret_Base.CDEndedCondition` _array_element) (`/Game/Blueprint/Turrets/BP_Turret_Base.CDStartCondition` _array_element) (`/Game/Blueprint/Turrets/BP_Turret_Base.CurrentLevel` _array_element) (`/Game/Blueprint/Turrets/BP_Turret_Base.TurretType` _array_element) (`/Game/Blueprint/Turrets/BP_Turret_Base.CdTime` _array_element) (`/Game/Blueprint/Turrets/BP_Turret_Base.RotationForSave` _array_element)))))

(fn `SetTurretTrigger`
  (params (self2 :type "/Game/GameMode/BP_NewGameMode Object Reference"))
  (bind _turrettrigger (`/Game/GameMode/BP_NewGameMode.GetAllTurretsTrigger` self2))
  (for _array_element _turrettrigger
    (`KismetArrayLibrary.Array_AddUnique` (`self.TurretTriggers`) (make `/Game/Blueprint/Save/S_TurretTriggersForSave` (`/Game/Blueprint/Turrets/BP_TurretTrigger.Location` _array_element) (`/Game/Blueprint/Turrets/BP_TurretTrigger.CanBuild` _array_element) (`/Game/Blueprint/Turrets/BP_TurretTrigger.IsInCooldown` _array_element) (`/Game/Blueprint/Turrets/BP_TurretTrigger.ValueToReactivate` _array_element) (`/Game/Blueprint/Turrets/BP_TurretTrigger.HasSpawn` _array_element)))))

(fn `SetWorld`
  (params (GameMode :type "GameModeBase Object Reference") (GameInstance :type "GameInstance Object Reference"))
  (bind _asbp_new_game_mode (cast `/Game/GameMode/BP_NewGameMode` GameMode))
  (`|ExecutionSequence`
    (:`then_0`
      (bind _asbp_new_game_instance (cast `/Game/Blueprint/BP_NewGameInstance` GameInstance))
      (set `self.Seed` (`/Game/Blueprint/BP_NewGameInstance.Seed` _asbp_new_game_instance)))
    (:`then_1`
      (set `self.ActiveRoom` (`/Game/Blueprint/Envirorment/Rooms/BP_WFC_BaseRoom.RoomProgressionIndex` (`/Game/GameMode/BP_NewGameMode.ActiveRoom` _asbp_new_game_mode)))
      (for _array_element (`/Game/GameMode/BP_NewGameMode.ActiveRooms` _asbp_new_game_mode)
        (`KismetArrayLibrary.Array_AddUnique` (`self.ActiveRooms`) (`/Game/Blueprint/Envirorment/Rooms/BP_WFC_BaseRoom.RoomProgressionIndex` _array_element)))
      (set `self.DoorCost` (`/Game/GameMode/BP_NewGameMode.DoorCost` _asbp_new_game_mode))
      (set `self.CurrentDay` (`/Game/GameMode/BP_NewGameMode.CurrrentDay` _asbp_new_game_mode))
      (set `self.FrenzyCumulativeProbability` (`/Game/GameMode/BP_NewGameMode.CumulativeProbability` _asbp_new_game_mode))
      (bind _returnvalue (`/Game/GameMode/BP_NewGameMode.GetRemainingFrenzyTimer` _asbp_new_game_mode))
      (set `self.NextFrenzyCheck` _returnvalue)
      (set `self.TotalTime` (`/Game/GameMode/BP_NewGameMode.Total Time` _asbp_new_game_mode))
      (set `self.Seconds` (`/Game/GameMode/BP_NewGameMode.Seconds` _asbp_new_game_mode))
      (set `self.D_Minutes` (`/Game/GameMode/BP_NewGameMode.Day_Minutes` _asbp_new_game_mode))
      (set `self.Minutes` (`/Game/GameMode/BP_NewGameMode.Minutes` _asbp_new_game_mode)))
    (:`then_2`
      (`self.SetDoors` _asbp_new_game_mode)
      (`self.SetBlueprint` _asbp_new_game_mode)
      (`self.SetJunk` _asbp_new_game_mode)
      (`self.SetJunkSpawner` _asbp_new_game_mode)
      (`self.SetTurret` _asbp_new_game_mode)
      (`self.SetTurretTrigger` _asbp_new_game_mode)
      (`self.SetEnergyRecharger` _asbp_new_game_mode)
      (`self.SetLevel` _asbp_new_game_mode)
      (`self.SetFarmer` _asbp_new_game_mode))))