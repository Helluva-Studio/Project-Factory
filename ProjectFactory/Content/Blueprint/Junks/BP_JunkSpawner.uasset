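; BP_JunkSpawner is a placed spawn point that creates and respawns a BP_Junk of a chosen type.
; The construction script previews the mesh from the Junks data table row mapped to that type, and BeginPlay clears it before spawning.
; SpawnJunk attaches the new actor and initializes it with row data and a pointer to the spawner.
; StartRespawnTimer schedules another spawn after a randomized delay set in minutes.
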(event `self.ReceiveBeginPlay`
  (`StaticMeshComponent.SetStaticMesh` (`self.StaticMesh`) null)
  (`self.SpawnJunk`))

(event `StartRespawnTimer`
  (`KismetSystemLibrary.K2_SetTimerDelegate` (delegate `RespawnJunk`) (* (`self.TimeToRespawn`) 60.0) false 0.0 (* (`self.RandomnessTimeToRespawn`) 60.0)))

(event `RespawnJunk`
  (`self.SpawnJunk`))

(fn `SpawnJunk`
  (set `self.HasSpawnJunk` true)
  (bind _returnvalue (`|GetDataTableRow` "/Game/Blueprint/Junks/Junks.Junks" (`BlueprintMapLibrary.Map_Find` (`self.MapType`) (`self.TypeOfJunk`)))
    (:`then`
      (bind _returnvalue_2 (`|SpawnActorFromClass` "/Game/Blueprint/Junks/BP_Junk.BP_Junk_C" (`KismetMathLibrary.MakeTransform` (`self.K2_GetActorLocation`) (`self.K2_GetActorRotation`) (`self.GetActorScale3D`)) "AdjustIfPossibleButAlwaysSpawn" "MultiplyWithRoot" null null))
      (`self.K2_AttachToActor` _returnvalue_2 self "None" "KeepWorld" "KeepWorld" "KeepWorld" true)
      (`/Game/Blueprint/Junks/BP_Junk.Initalize` _returnvalue_2 (`.Mesh_14_FD634E4F4E932F60C025418E90B6C0C2` (break `/Game/Blueprint/Junks/S_Junk` _returnvalue)) (break `/Game/Blueprint/Junks/S_Junk` _returnvalue) (`.Drop_15_E82C233F4F6EC3B56822B1B7DDE1567E` (break `/Game/Blueprint/Junks/S_Junk` _returnvalue)) (`.DropValue_11_E1FDF07B4652B5EBFAB3A0B82FBDF70D` (break `/Game/Blueprint/Junks/S_Junk` _returnvalue)) (`.MaxHealth_18_F81ED421453B4D56C78FA1B59BBFD82A` (break `/Game/Blueprint/Junks/S_Junk` _returnvalue)) self (`.SFX_21_98B9857149E76A5CBC9D3BB1C30D98C1` (break `/Game/Blueprint/Junks/S_Junk` _returnvalue))))))

(fn `UserConstructionScript`
  (bind _returnvalue (`|GetDataTableRow` "/Game/Blueprint/Junks/Junks.Junks" (`BlueprintMapLibrary.Map_Find` (`self.MapType`) (`self.TypeOfJunk`)))
    (:`then`
      (`StaticMeshComponent.SetStaticMesh` (`self.StaticMesh`) (`.Mesh_14_FD634E4F4E932F60C025418E90B6C0C2` (break `/Game/Blueprint/Junks/S_Junk` _returnvalue)))
      (set `self.Location` (`self.K2_GetActorLocation`)))))