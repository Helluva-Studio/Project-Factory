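; BP_Junk is a damageable junk object that drops a resource pickup when destroyed.
; Initalize configures mesh, health, drop, sound and spawn point, resizing the trace area for Steel Tier 1.
; Hits have a half-second cooldown and trigger a timeline scale pulse plus an AI noise event; focus toggles custom depth.
; Destruction spawns the drop relative to the player's height and clears the spawn point's junk flag.
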(event `self.ReceiveBeginPlay`
  ;[1 1 1] Begin Play
  (set `self.OriginalScale` (`SceneComponent.RelativeScale3D` (`self.StaticMesh`))))

(event `/Game/Blueprint/Junks/BPI_Junk.GetDamage`
  (params (Damage :type "Float (double-precision)"))
  ;[1 0.2448 0.2448] Handle Damage
  (if (`self.CanBeHit`)
    (`GameplayStatics.PlaySoundAtLocation` (`self.SFX`) (`self.K2_GetActorLocation`) (struct) 1.0 1.0 0.0 null null null null)
    (if (< Damage (`self.Health`))
      (set `self.CanBeHit` false)
      (set `self.Health` (- (`self.Health`) Damage))
      (`self.HitReact`)
      (`KismetSystemLibrary.Delay` 0.5)
      (set `self.CanBeHit` true)
      (else
        (set `self.Health` 0.0)
        (`GameplayStatics.PlaySoundAtLocation` "/Game/Audio/SFX/Environment/Junk/SC_JunkDestroyedSFX_Cue.SC_JunkDestroyedSFX_Cue" (`self.K2_GetActorLocation`) (struct) 1.0 1.0 0.0 null null null null)
        (`self.Destroy`)))))

(event `/Game/Blueprint/InteractionArea/BPI_Focusable.ToggleFocus`
  (params (Focus :type Boolean))
  ;[1 1 1] Focus
  (`PrimitiveComponent.SetRenderCustomDepth` (`self.StaticMesh`) Focus))

(event `HitReact`
  ;[1 0.8803 0.2678] Hit React Animation
  (`/Engine/EditorBlueprintResources/StandardMacros.DoOnce` false :!label _label
    (:`Completed`
      (`AISense_Hearing.ReportNoiseEvent` (`self.K2_GetActorLocation`) 1.0 self 1500.0)
      (bind (_direction _hiteffect) (`Timeline|HitReactTimeline` :!via `PlayFromStart`)
        (:`Update`
          (`SceneComponent.SetRelativeScale3D` (`self.StaticMesh`) (* _hiteffect (`self.OriginalScale`))))
        (:`Finished`
          (goto _label :!via `Reset`))))))

(fn `Destroy`
  (bind (_returnvalue_x _returnvalue_y) (`KismetMathLibrary.BreakVector` (`self.K2_GetActorLocation`)))
  (bind (_returnvalue_x_2 _returnvalue_y_2 _returnvalue_z) (`KismetMathLibrary.BreakVector` (`self.K2_GetActorLocation` (`GameplayStatics.GetPlayerPawn` 0))))
  (`|SpawnActorFromClass` (`self.JunkToSpawn`) (`KismetMathLibrary.MakeTransform` (`KismetMathLibrary.MakeVector` _returnvalue_x _returnvalue_y (+ _returnvalue_z 40.0)) (`KismetMathLibrary.MakeRotator` 0.0)) "AlwaysSpawn" "MultiplyWithRoot" null (`self.ValueDrop`) null)
  (`self.K2_DestroyActor`)
  (set `/Game/Blueprint/Junks/BP_JunkSpawner.HasSpawnJunk` false (`self.SpawnPointer`)))

(fn `Initalize`
  (params (NewMesh :type "StaticMesh Object Reference") (JunkType :type "/Game/Blueprint/Junks/E_JunkType Enum" :default "NewEnumerator0") (JunkToSpawn :type "/Game/Blueprint/Resources/BP_Resource Class Reference") (ValueDrop :type "Float (double-precision)") (MaxHealth :type "Float (double-precision)") (SpawnPointer :type "/Game/Blueprint/Junks/BP_JunkSpawner Object Reference") (SFX :type "SoundCue Object Reference"))
  (bind (_returnvalue_x _returnvalue_y) (`KismetMathLibrary.BreakVector` (`SceneComponent.K2_GetComponentLocation` (`self.TraceArea`))))
  (`|ExecutionSequence`
    (:`then_0`
      (`StaticMeshComponent.SetStaticMesh` (`self.StaticMesh`) NewMesh))
    (:`then_1`
      (bind _output_get (set `self.JunkType` JunkType))
      (switch `/Game/Blueprint/Junks/E_JunkType` _output_get
        (:`NewEnumerator3`
          (`SceneComponent.SetWorldScale3D` (`self.TraceArea`) (7.0 1.0 6.0))
          (`SceneComponent.K2_SetWorldLocation` (`self.TraceArea`) (`KismetMathLibrary.MakeVector` _returnvalue_x _returnvalue_y 180.0) false false)
          (`SceneComponent.K2_SetWorldLocation` (`self.TraceArea`) (`KismetMathLibrary.MakeVector` _returnvalue_x _returnvalue_y 180.0) false false))))
    (:`then_2`
      (set `self.JunkToSpawn` JunkToSpawn))
    (:`then_3`
      (set `self.ValueDrop` ValueDrop))
    (:`then_4`
      (bind _output_get_2 (set `self.MaxHealth` MaxHealth))
      (set `self.Health` _output_get_2))
    (:`then_5`
      (set `self.SpawnPointer` SpawnPointer)
      (set `self.SFX` SFX))))

(fn `UserConstructionScript`)