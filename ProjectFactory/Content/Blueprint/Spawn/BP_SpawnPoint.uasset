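; BP_SpawnPoint is a spawn point actor that spawns enemies at its own transform from a queue of enemy classes.
; AddEnemyToQueue appends a class and immediately calls SpawnEnemy, which spawns the front entry with collision handling set to always spawn.
; SpawnEnemy initializes the spawned enemy with the given level, removes that entry and returns whether the queue had an entry to process.
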(event `self.ReceiveBeginPlay`)

(event `self.ReceiveTick`
  (params (DeltaSeconds :type "Float (single-precision)")))

(fn `AddEnemyToQueue`
  (params (EnemyClass :type "/Game/Blueprint/Enemies/BP_BaseEnemy Class Reference (by ref)") (Level :type Integer))
  (`KismetArrayLibrary.Array_Add` (`self.EnemyQueue`) EnemyClass)
  (`self.SpawnEnemy` Level))

(fn `SpawnEnemy`
  (params (Level :type Integer))
  (returns (Success :type Boolean))
  (if (`KismetArrayLibrary.Array_IsValidIndex` (`self.EnemyQueue`))
    (bind _returnvalue (`|SpawnActorFromClass` (`|GetArrayItem` (`self.EnemyQueue`)) (`self.GetTransform`) "AlwaysSpawn" "MultiplyWithRoot" null null))
    (`/Engine/EditorBlueprintResources/StandardMacros.IsValid` _returnvalue
      (:`Is Valid`
        (`/Game/Blueprint/Enemies/BP_BaseEnemy.Initialize` _returnvalue Level))
      (:`Is Not Valid`
        _))
    (`KismetArrayLibrary.Array_Remove` (`self.EnemyQueue`))
    (return true)
    (else
      (return false))))

(fn `UserConstructionScript`)