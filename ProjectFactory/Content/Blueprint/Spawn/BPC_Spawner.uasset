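; BPC_Spawner is a one-shot component that respawns an enemy after a delay, away from the player.
; On BeginPlay it gathers the active room and nearby active rooms, waits, picks one at random, then chooses that room's spawn point farthest from the player.
; It queues the enemy class there, unregisters from BP_NewGameMode's active spawners and destroys itself.
; An older random respawn path is disconnected, and SelectRoom is empty.
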(event `self.ReceiveBeginPlay`
  ;[1 1 1] RESPAWN IN THE MOST FAR SPAWN POINT
  (`KismetArrayLibrary.Array_Add` (`self.SuitableRooms`) (`self.ActiveRoom`))
  (for _array_element (`self.ActiveRooms`)
    (if (<= (`Actor.GetHorizontalDistanceTo` (`self.ActiveRoom`) _array_element) 7000.0)
      (`KismetArrayLibrary.Array_Add` (`self.SuitableRooms`) _array_element)))
  (`KismetSystemLibrary.Delay` (`self.SpawnTime`))
  (bind _output_get (set `self.RoomChosen` (`KismetArrayLibrary.Array_Random` (`self.SuitableRooms`))))
  (bind _spawnpoints (`/Game/Blueprint/Envirorment/Rooms/BP_WFC_BaseRoom.SpawnPoints` _output_get))
  (set `self.ActiveSpawnPoint` (`KismetArrayLibrary.Array_Random` _spawnpoints))
  (for _array_element_2 _spawnpoints
    (bind _returnvalue (`KismetMathLibrary.Vector_Distance` (`Actor.K2_GetActorLocation` _array_element_2) (`Actor.K2_GetActorLocation` (`GameplayStatics.GetPlayerPawn` 0))))
    (if (> _returnvalue (`self.MaxDistance`))
      (set `self.MaxDistance` _returnvalue)
      (set `self.ActiveSpawnPoint` _array_element_2)))
  (`/Game/Blueprint/Spawn/BP_SpawnPoint.AddEnemyToQueue` (`self.ActiveSpawnPoint`) (`self.EnemyClass`))
  (`KismetArrayLibrary.Array_RemoveItem` (`/Game/GameMode/BP_NewGameMode.ActiveSpawners` (cast `/Game/GameMode/BP_NewGameMode` (`GameplayStatics.GetGameMode`) :!pure true)) self)
  (`KismetSystemLibrary.PrintString` (`KismetStringLibrary.Concat_StrStr` "SPAWNING IN: " (`KismetSystemLibrary.GetDisplayName` (`self.RoomChosen`))))
  (`self.K2_DestroyComponent`))

(event `SelectRoom`)