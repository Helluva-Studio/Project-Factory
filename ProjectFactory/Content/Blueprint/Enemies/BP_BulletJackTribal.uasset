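; BP_BulletJackTribal is an enemy homing projectile that damages the player on overlap, or turrets on hit with a separate damage value.
; Init receives both damage values, speed, lifespan and the homing component, storing that component's owner as Target.
; Tick switches homing off once, within close range of Target, so the bullet stops tracking on final approach.
; It destroys itself on player overlap or any hit; rotation nodes are left unconnected.
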(event `self.Sphere.OnComponentBeginOverlap`
  (params (OverlappedComponent :type "PrimitiveComponent Object Reference") (OtherActor :type "Actor Object Reference") (OtherComp :type "PrimitiveComponent Object Reference") (OtherBodyIndex :type Integer) (bFromSweep :type Boolean) (SweepResult :type "HitResult Structure (by ref)"))
  (if (== OtherActor (`GameplayStatics.GetPlayerPawn` 0))
    (`GameplayStatics.ApplyDamage` OtherActor (`self.Damage`))
    (set `ProjectileMovementComponent.bIsHomingProjectile` false (`self.ProjectileMovement`))
    (`self.K2_DestroyActor`)))

(event `self.Sphere.OnComponentHit`
  (params (HitComponent :type "PrimitiveComponent Object Reference") (OtherActor :type "Actor Object Reference") (OtherComp :type "PrimitiveComponent Object Reference") (NormalImpulse :type "Vector Structure") (Hit :type "HitResult Structure (by ref)"))
  (if (`KismetSystemLibrary.DoesImplementInterface` OtherActor "/Game/Blueprint/Turrets/Interfaces/BPI_Turret.BPI_Turret_C")
    (`GameplayStatics.ApplyDamage` OtherActor (`self.DamageVsTurrets`))
    (`self.K2_DestroyActor`)
    (else
      (`self.K2_DestroyActor`))))

(event `self.ReceiveTick`
  (params (DeltaSeconds :type "Float (single-precision)"))
  (if (<= (`KismetMathLibrary.Vector_Distance` (`self.K2_GetActorLocation`) (`self.K2_GetActorLocation` (`self.Target`))) 150.0)
    (`/Engine/EditorBlueprintResources/StandardMacros.DoOnce` false
      (:`Completed`
        (set `ProjectileMovementComponent.bIsHomingProjectile` false (`self.ProjectileMovement`))))))

(fn `Init`
  (params (Damage :type "Float (double-precision)") (Speed :type "Float (double-precision)") (Target :type "SceneComponent Object Reference") (BulletLifeSpan :type "Float (double-precision)") (DamageVsTurrets :type "Float (double-precision)"))
  (bind _projectilemovement (`self.ProjectileMovement`))
  (set `self.Damage` Damage)
  (set `ProjectileMovementComponent.HomingTargetComponent` Target _projectilemovement)
  (set `ProjectileMovementComponent.InitialSpeed` Speed _projectilemovement)
  (set `ProjectileMovementComponent.MaxSpeed` Speed _projectilemovement)
  (bind _output_get (set `self.LifeSpan` BulletLifeSpan))
  (`self.SetLifeSpan` _output_get)
  (set `self.DamageVsTurrets` DamageVsTurrets)
  (set `self.Target` (`ActorComponent.GetOwner` Target)))

(fn `UserConstructionScript`)