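; Dragon flame hazard actor that burns the player and turrets that enter its Flame component.
; On overlap begin it applies instant damage and messages the target to start timed damage over time, with separate amounts for player and turrets; overlap end sends a stop message.
; Init supplies the damage amounts and lifespan.
; An older timer-based damage loop remains disconnected.
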(event `self.ReceiveBeginPlay`)

(event `CheckForDamage`)

(event `self.Flame.OnComponentBeginOverlap`
  (params (OverlappedComponent :type "PrimitiveComponent Object Reference") (OtherActor :type "Actor Object Reference") (OtherComp :type "PrimitiveComponent Object Reference") (OtherBodyIndex :type Integer) (bFromSweep :type Boolean) (SweepResult :type "HitResult Structure (by ref)"))
  (if (== OtherActor (`GameplayStatics.GetPlayerPawn` 0))
    (`GameplayStatics.ApplyDamage` OtherActor (`self.Damage to Player`))
    (message `/Game/Blueprint/Interfaces/BPI_Damageble.TakeDamageOverTime` OtherActor 2.0 (`self.Damage to Player Over Time`) false null "NewEnumerator0")
    (elif (`KismetSystemLibrary.DoesImplementInterface` OtherActor "/Game/Blueprint/Turrets/Interfaces/BPI_Turret.BPI_Turret_C")
      (message `/Game/Blueprint/Interfaces/BPI_Damageble.TakeDamageOverTime` OtherActor 2.0 (`self.Damage to Turrets Over Time`) false null "NewEnumerator0")
      (`GameplayStatics.ApplyDamage` OtherActor (`self.Damage to Turrets`)))))

(event `self.Flame.OnComponentEndOverlap`
  (params (OverlappedComponent :type "PrimitiveComponent Object Reference") (OtherActor :type "Actor Object Reference") (OtherComp :type "PrimitiveComponent Object Reference") (OtherBodyIndex :type Integer))
  (if (or (== OtherActor (`GameplayStatics.GetPlayerPawn` 0)) (`KismetSystemLibrary.DoesImplementInterface` OtherActor "/Game/Blueprint/Turrets/Interfaces/BPI_Turret.BPI_Turret_C"))
    (message `/Game/Blueprint/Interfaces/BPI_Damageble.StopDamageOverTime` OtherActor "NewEnumerator0" null)))

(fn `Init`
  (params (LDamageToPlayer :type "Float (double-precision)") (LDamageToTurrets :type "Float (double-precision)") (LDamageToPlayerOverTime :type "Float (double-precision)") (LDamageToTurretsOverTime :type "Float (double-precision)") (LifeSpan :type "Float (double-precision)"))
  (`|ExecutionSequence`
    (:`then_0`
      (set `self.Damage to Player` (`local.LDamageToPlayer`)))
    (:`then_1`
      (set `self.Damage to Turrets` (`local.LDamageToTurrets`)))
    (:`then_2`
      (set `self.Damage to Player Over Time` (`local.LDamageToPlayerOverTime`)))
    (:`then_3`
      (set `self.Damage to Turrets Over Time` (`local.LDamageToTurretsOverTime`)))
    (:`then_4`
      (`self.SetLifeSpan` LifeSpan))))

(fn `UserConstructionScript`)