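; BP_EnemyFlame is an enemy flame that deals periodic damage to the player pawn and turrets inside its cone.
; Cone overlap events maintain the list of targets, admitting only the player pawn or actors implementing BPI_Turret.
; A looping timer started on BeginPlay applies Damage to every listed actor.
; Initialize stores Damage, Length and Width, though these graphs never use Length or Width.
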(event `self.ReceiveBeginPlay`
  (`KismetSystemLibrary.K2_SetTimerDelegate` (delegate `FlameDamage`) (`self.TimeToDealDamage`) true))

(event `FlameDamage`
  (for _array_element (`self.ActorsToDamage`)
    (`GameplayStatics.ApplyDamage` _array_element (`self.Damage`))))

(event `self.Cone.OnComponentBeginOverlap`
  (params (OverlappedComponent :type "PrimitiveComponent Object Reference") (OtherActor :type "Actor Object Reference") (OtherComp :type "PrimitiveComponent Object Reference") (OtherBodyIndex :type Integer) (bFromSweep :type Boolean) (SweepResult :type "HitResult Structure (by ref)"))
  (if (or (`KismetSystemLibrary.DoesImplementInterface` OtherActor "/Game/Blueprint/Turrets/Interfaces/BPI_Turret.BPI_Turret_C") (== OtherActor (`GameplayStatics.GetPlayerPawn` 0)))
    (`KismetArrayLibrary.Array_Add` (`self.ActorsToDamage`))))

(event `self.Cone.OnComponentEndOverlap`
  (params (OverlappedComponent :type "PrimitiveComponent Object Reference") (OtherActor :type "Actor Object Reference") (OtherComp :type "PrimitiveComponent Object Reference") (OtherBodyIndex :type Integer))
  (bind _returnvalue (`KismetArrayLibrary.Array_Find` (`self.ActorsToDamage`) OtherActor))
  (if (>= _returnvalue 0)
    (`KismetArrayLibrary.Array_Remove` (`self.ActorsToDamage`) _returnvalue)))

(fn `Initialize`
  (params (Damage :type "Float (double-precision)") (Length :type "Float (double-precision)") (Width :type "Float (double-precision)"))
  (set `self.Damage` Damage)
  (set `self.Length` Length)
  (set `self.Width` Width))

(fn `UserConstructionScript`)