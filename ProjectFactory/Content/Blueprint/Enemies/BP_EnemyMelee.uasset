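; BP_EnemyMelee is a melee enemy Blueprint that damages the player at close range.
; DoDamage checks whether its Mesh overlaps a BP_Roberto actor, then applies AttackDamage to player pawn 0 rather than the overlapped actor.
; It returns whether the hit landed and prints a debug message on success.
; The event graph only forwards BeginPlay, overlap and Tick to the parent class.
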(event `self.ReceiveBeginPlay`
  (`parent.ReceiveBeginPlay`))

(event `self.ReceiveActorBeginOverlap`
  (params (OtherActor :type "Actor Object Reference"))
  (`parent.ReceiveActorBeginOverlap` OtherActor))

(event `self.ReceiveTick`
  (params (DeltaSeconds :type "Float (single-precision)"))
  (`parent.ReceiveTick` DeltaSeconds))

(fn `DoDamage`
  (returns (Success :type Boolean))
  (if (`KismetArrayLibrary.Array_IsValidIndex` (`PrimitiveComponent.GetOverlappingActors` (`self.Mesh`) "/Game/Blueprint/Robot/Blueprints/BP_Roberto.BP_Roberto_C"))
    (`GameplayStatics.ApplyDamage` (`GameplayStatics.GetPlayerPawn` 0) (`self.AttackDamage`))
    (`KismetSystemLibrary.PrintString` "ATTACKED PLAYER" true true (struct :`R` 1.0 :`B` 0.926622 :`A` 1.0))
    (return true)
    (else
      (return false))))

(fn `UserConstructionScript`)