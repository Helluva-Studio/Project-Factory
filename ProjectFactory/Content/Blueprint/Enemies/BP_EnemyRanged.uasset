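; BP_EnemyRanged is a ranged enemy that attacks the player by firing projectiles.
; Its Attack event calls Shoot, which rotates ShootingPoint toward the player pawn and spawns a BP_BulletJack there.
; The bullet is initialized with the enemy's damage, speed and lifespan values, plus the player's root component as target.
; DoDamage only prints a debug message and returns true.
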(event `/Game/Blueprint/Enemies/Interfaces/BPI_Enemy.Attack`
  (`self.Shoot`))

(fn `DoDamage`
  (returns (Success :type Boolean))
  (`KismetSystemLibrary.PrintString` "RANGED ATTACK" true true (struct :`R` 0.108311 :`G` 1.0 :`B` 0.0636 :`A` 1.0))
  (return true))

(fn `Shoot`
  (bind _returnvalue (`GameplayStatics.GetPlayerPawn` 0))
  (`SceneComponent.K2_SetWorldRotation` (`self.ShootingPoint`) (`KismetMathLibrary.FindLookAtRotation` (`SceneComponent.K2_GetComponentLocation` (`self.ShootingPoint`)) (`self.K2_GetActorLocation` _returnvalue)) false false)
  (`KismetSystemLibrary.PrintString` "SHOOTING")
  (bind _returnvalue_2 (`|SpawnActorFromClass` "/Game/Blueprint/Enemies/BP_BulletJack.BP_BulletJack_C" (`SceneComponent.K2_GetComponentToWorld` (`self.ShootingPoint`)) "AlwaysSpawn" "MultiplyWithRoot" null null))
  (`/Game/Blueprint/Enemies/BP_BulletJack.Init` _returnvalue_2 (`self.AttackDamage`) (`self.BulletSpeed`) (`Actor.RootComponent` _returnvalue) (`self.BulletLifeSpan`)))

(fn `UserConstructionScript`
  (`parent.UserConstructionScript`))