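; BP_TribalRanged is a tribal enemy that extends a parent class with a punch hitbox and a shooting point.
; Construction attaches both to hand sockets on the mesh, though no firing logic appears here.
; Attack enables punch collision, which damages the player or BPI_Turret actors by separate amounts, then switches off on that hit.
; AnyDamage defers to the parent; its turret check is empty and the hit-react montage is disconnected.
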(event `self.ReceiveBeginPlay`
  (`parent.ReceiveBeginPlay`)
  (`PrimitiveComponent.SetCollisionEnabled` (`self.Punch`) "NoCollision"))

(event `/Game/Blueprint/Enemies/Interfaces/BPI_Enemy.Attack`
  (`PrimitiveComponent.SetCollisionEnabled` (`self.Punch`) "QueryOnly"))

(event `self.Punch.OnComponentBeginOverlap`
  (params (OverlappedComponent :type "PrimitiveComponent Object Reference") (OtherActor :type "Actor Object Reference") (OtherComp :type "PrimitiveComponent Object Reference") (OtherBodyIndex :type Integer) (bFromSweep :type Boolean) (SweepResult :type "HitResult Structure (by ref)"))
  (if (== OtherActor (`GameplayStatics.GetPlayerPawn` 0))
    (`GameplayStatics.ApplyDamage` OtherActor (`self.AttackDamage`))
    (`PrimitiveComponent.SetCollisionEnabled` (`self.Punch`) "NoCollision")
    (elif (`KismetSystemLibrary.DoesImplementInterface` OtherActor "/Game/Blueprint/Turrets/Interfaces/BPI_Turret.BPI_Turret_C")
      (`GameplayStatics.ApplyDamage` OtherActor (`self.AttackDamageVsTurrets`))
      (`PrimitiveComponent.SetCollisionEnabled` (`self.Punch`) "NoCollision"))))

(event `self.ReceiveAnyDamage`
  (params (Damage :type "Float (single-precision)") (DamageType :type "DamageType Object Reference") (InstigatedBy :type "Controller Object Reference") (DamageCauser :type "Actor Object Reference"))
  (`parent.ReceiveAnyDamage` Damage DamageType InstigatedBy DamageCauser)
  (if (`KismetSystemLibrary.DoesImplementInterface` DamageCauser "/Game/Blueprint/Turrets/Interfaces/BPI_Turret.BPI_Turret_C")
    _))

(fn `DoDamage`
  (returns (Success :type Boolean))
  (bind _success (`parent.DoDamage`))
  (return _success))

(fn `GetSkeletalMesh`
  (returns (Mesh :type "SkeletalMeshComponent Object Reference"))
  (return (`self.Mesh`)))

(fn `UserConstructionScript`
  (`parent.UserConstructionScript`)
  (`SceneComponent.K2_AttachToComponent` (`self.Punch`) (`self.Mesh`) "Middle1_R" "KeepRelative" "KeepRelative" "KeepRelative" true)
  (`SceneComponent.K2_AttachToComponent` (`self.ShootingPoint`) (`self.Mesh`) "Middle3_L_end" "KeepRelative" "KeepRelative" "KeepWorld" true))