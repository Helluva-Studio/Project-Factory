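; BP_BaseEnemy is a base enemy Character that tracks health and, on death, notifies BP_NewGameMode, spawns an essence drop and destroys itself.
; EMP stuns it through blackboard keys, and the behavior tree drives its walk speed.
; Hits and damage report touch events to AI perception.
; Damage from BPI_Robot actors also interrupts montages, launches it along the player's view, flags PlayerSeen and briefly blocks further robot damage.
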(event `self.ReceiveBeginPlay`
  (set `self.CurrentHealth` (`self.Health`)))

(event `Death`
  (bind _returnvalue_location (`KismetMathLibrary.BreakTransform` (`self.GetTransform`)))
  (bind _asbp_new_game_mode (cast `/Game/GameMode/BP_NewGameMode` (`GameplayStatics.GetGameMode`))
    (:`then`
      (`/Game/GameMode/BP_NewGameMode.EnemyKilled` _asbp_new_game_mode))
    (:`CastFailed`
      _))
  (bind _returnvalue (`|SpawnActorFromClass` "/Game/Blueprint/Essence/BP_Essence.BP_Essence_C" (`KismetMathLibrary.MakeTransform` _returnvalue_location) "Undefined" "MultiplyWithRoot" null null))
  (`/Game/Blueprint/Essence/BP_Essence.Initialize` _returnvalue (`self.EssenceDrop`))
  (`self.K2_DestroyActor`))

(event `self.EMP`
  (params (Duration :type "Float (double-precision)"))
  (bind _returnvalue (`AIBlueprintHelperLibrary.GetBlackboard` (`AIBlueprintHelperLibrary.GetAIController` self)))
  ;[1 1 1] EMP
  (`BlackboardComponent.SetValueAsFloat` _returnvalue (`self.EMPDuration`) Duration)
  (`BlackboardComponent.SetValueAsBool` _returnvalue (`self.IsStunned`) true))

(event `self.Attack`
  ;[1 1 1] Attack
  (set `self.IsAttacking` true))

(event `self.UpdateSpeed`
  (params (Speed :type "Float (double-precision)"))
  ;[1 1 1] Update speed from Behavior Tree
  (set `CharacterMovementComponent.MaxWalkSpeed` Speed (`self.CharacterMovement`)))

(event `self.ReceiveHit`
  (params (MyComp :type "PrimitiveComponent Object Reference") (Other :type "Actor Object Reference") (OtherComp :type "PrimitiveComponent Object Reference") (bSelfMoved :type Boolean) (HitLocation :type "Vector Structure") (HitNormal :type "Vector Structure") (NormalImpulse :type "Vector Structure") (Hit :type "HitResult Structure (by ref)"))
  ;[1 1 1] Touch response
  (`AISense_Touch.ReportTouchEvent` self Other HitLocation))

(event `self.ReceiveAnyDamage`
  (params (Damage :type "Float (single-precision)") (DamageType :type "DamageType Object Reference") (InstigatedBy :type "Controller Object Reference") (DamageCauser :type "Actor Object Reference"))
  (bind _returnvalue (`KismetSystemLibrary.DoesImplementInterface` DamageCauser "/Game/Blueprint/Robot/Interfaces/BPI_Robot.BPI_Robot_C"))
  (if (not (and _returnvalue (`self.IsAttackedByPlayer`)))
    (`self.TakeDamage` Damage)
    (`/Engine/EditorBlueprintResources/StandardMacros.IsValid` DamageCauser
      (:`Is Valid`
        (`AISense_Touch.ReportTouchEvent` self DamageCauser (`self.K2_GetActorLocation` DamageCauser))
        (if _returnvalue
          (`self.StopAnimMontage` (`self.GetCurrentMontage`))
          (set `self.IsAttackedByPlayer` true)
          (`self.LaunchCharacter` (* (`KismetMathLibrary.GetForwardVector` (`self.GetControlRotation` (`GameplayStatics.GetPlayerPawn` 0))) 1000.0) true)
          (`/Engine/EditorBlueprintResources/StandardMacros.IsValid` self
            (:`Is Valid`
              (`AISense_Touch.ReportTouchEvent` self DamageCauser (`self.K2_GetActorLocation` DamageCauser))
              (`BlackboardComponent.SetValueAsBool` (`AIController.Blackboard` (`AIBlueprintHelperLibrary.GetAIController` self)) (`self.PlayerSeen`) true)
              (`KismetSystemLibrary.Delay` 0.5)
              (set `self.IsAttackedByPlayer` false))))))))

(fn `DoDamage`
  (returns (Success :type Boolean))
  (return true))

(fn `GetSkeletalMesh`
  (returns (Mesh :type "SkeletalMeshComponent Object Reference"))
  (return null))

(fn `TakeDamage`
  (params (Damage :type "Float (double-precision)"))
  (if (< Damage (`self.CurrentHealth`))
    (set `self.CurrentHealth` (- (`self.CurrentHealth`) Damage))
    (else
      (`self.Death`))))

(fn `UpdateMaxSpeed`
  (params (`Max Walk Speed` :type "Float (single-precision)"))
  (set `CharacterMovementComponent.MaxWalkSpeed` `Max Walk Speed` (`self.CharacterMovement`)))

(fn `UserConstructionScript`)