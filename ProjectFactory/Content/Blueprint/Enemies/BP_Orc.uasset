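; BP_Orc is an enemy orc that deals melee damage with a bat attached to a hand socket on its mesh.
; Attack turns on the bat's query collision, and StopAttacking or the first valid hit turns it off, so each swing damages one target at most.
; Overlaps apply separate damage amounts to the player pawn and to actors implementing BPI_Turret.
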(event `self.ReceiveBeginPlay`
  (`parent.ReceiveBeginPlay`)
  (`PrimitiveComponent.SetCollisionEnabled` (`self.Bat`) "NoCollision"))

(event `/Game/Blueprint/Enemies/Interfaces/BPI_Enemy.Attack`
  (`PrimitiveComponent.SetCollisionEnabled` (`self.Bat`) "QueryOnly"))

(event `self.Bat.OnComponentBeginOverlap`
  (params (OverlappedComponent :type "PrimitiveComponent Object Reference") (OtherActor :type "Actor Object Reference") (OtherComp :type "PrimitiveComponent Object Reference") (OtherBodyIndex :type Integer) (bFromSweep :type Boolean) (SweepResult :type "HitResult Structure (by ref)"))
  (if (== OtherActor (`GameplayStatics.GetPlayerPawn` 0))
    (`GameplayStatics.ApplyDamage` OtherActor (`self.AttackDamage`))
    (`PrimitiveComponent.SetCollisionEnabled` (`self.Bat`) "NoCollision")
    (elif (`KismetSystemLibrary.DoesImplementInterface` OtherActor "/Game/Blueprint/Turrets/Interfaces/BPI_Turret.BPI_Turret_C")
      (`GameplayStatics.ApplyDamage` OtherActor (`self.AttackDamageVsTurrets`))
      (`PrimitiveComponent.SetCollisionEnabled` (`self.Bat`) "NoCollision"))))

(event `/Game/Blueprint/Enemies/Interfaces/BPI_Enemy.StopAttacking`
  (`PrimitiveComponent.SetCollisionEnabled` (`self.Bat`) "NoCollision"))

(fn `GetSkeletalMesh`
  (returns (Mesh :type "SkeletalMeshComponent Object Reference"))
  (return (`self.Mesh`)))

(fn `UserConstructionScript`
  (`parent.UserConstructionScript`)
  (`SceneComponent.K2_AttachToComponent` (`self.Bat`) (`self.Mesh`) "Middle1_L" "KeepRelative" "KeepRelative" "KeepWorld" true))