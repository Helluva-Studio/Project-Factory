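; BP_Dragon is a dragon enemy that attacks a target with a flame breath.
; Shoot aims the head-socketed ShootingPoint at the target, spawns a BP_DragonFlame initialized with player and turret damage, including over-time values, then attaches it to the head.
; StopShooting and Death destroy that flame, with Death also calling the parent.
; AnyDamage's turret-interface check leads nowhere, and the hit-react montage is unwired.
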(event `self.ReceiveAnyDamage`
  (params (Damage :type "Float (single-precision)") (DamageType :type "DamageType Object Reference") (InstigatedBy :type "Controller Object Reference") (DamageCauser :type "Actor Object Reference"))
  (`parent.ReceiveAnyDamage` Damage DamageType InstigatedBy DamageCauser)
  (if (`KismetSystemLibrary.DoesImplementInterface` DamageCauser "/Game/Blueprint/Turrets/Interfaces/BPI_Turret.BPI_Turret_C")
    _))

(event `/Game/Blueprint/Enemies/Interfaces/BPI_RangedEnemy.StopShooting`
  (`/Engine/EditorBlueprintResources/StandardMacros.IsValid` (`self.Flame`)
    (:`Is Valid`
      (`self.K2_DestroyActor` (`self.Flame`)))))

(event `self.Death`
  (bind _flame (`self.Flame`))
  (`/Engine/EditorBlueprintResources/StandardMacros.IsValid` _flame
    (:`Is Valid`
      (`self.K2_DestroyActor` _flame))
    (:`Is Not Valid`
      _))
  (`parent.Death`))

(fn `GetSkeletalMesh`
  (returns (Mesh :type "SkeletalMeshComponent Object Reference"))
  (return (`self.Mesh`)))

(fn `Shoot`
  (params (TargetActor :type "Actor Object Reference") (LifeSpan :type "Float (double-precision)"))
  (bind (_returnvalue_location _returnvalue_rotation) (`KismetMathLibrary.BreakTransform` (`SceneComponent.K2_GetComponentToWorld` (`self.ShootingPoint`))))
  (`/Engine/EditorBlueprintResources/StandardMacros.IsValid` TargetActor
    (:`Is Valid`
      (`SceneComponent.K2_SetWorldRotation` (`self.ShootingPoint`) (`KismetMathLibrary.FindLookAtRotation` (`SceneComponent.K2_GetComponentLocation` (`self.ShootingPoint`)) (`self.K2_GetActorLocation` (`local.TargetActor`))) false false)
      (bind _returnvalue (`|SpawnActorFromClass` "/Game/Blueprint/Enemies/BP_DragonFlame.BP_DragonFlame_C" (`KismetMathLibrary.MakeTransform` _returnvalue_location _returnvalue_rotation) "AlwaysSpawn" "MultiplyWithRoot" null null))
      (`/Engine/EditorBlueprintResources/StandardMacros.IsValid` _returnvalue
        (:`Is Valid`
          (`/Game/Blueprint/Enemies/BP_DragonFlame.Init` _returnvalue (`self.AttackDamage`) (`self.AttackDamageVsTurrets`) (`self.DamageToPlayerOverTime`) (`self.DamageToTurretOverTime`) LifeSpan (`self.DamageTick`))
          (bind _output_get (set `self.Flame` _returnvalue))
          (`SceneComponent.K2_AttachToComponent` (`Actor.RootComponent` _output_get) (`self.Mesh`) "Head_end" "KeepWorld" "KeepWorld" "KeepWorld" true))))))

(fn `UserConstructionScript`
  (`parent.UserConstructionScript`)
  (`SceneComponent.K2_AttachToComponent` (`self.ShootingPoint`) (`self.Mesh`) "Head_end" "KeepRelative" "KeepRelative" "KeepWorld" true))