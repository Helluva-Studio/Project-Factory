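; Flying melee enemy that spawns raised above its placed position and attacks by dashing at the player.
; Attack disables gravity, lets the capsule pass through pawns and world, then a timeline lerps it to the player's captured position.
; A FlipFlop on timeline completion reverses the dash to the start point, then restores blocking collision and gravity.
; Capsule overlap with the player's capsule applies attack damage and prints a debug message.
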(event `self.ReceiveBeginPlay`
  (`parent.ReceiveBeginPlay`)
  (`self.K2_SetActorLocation` (+ (`self.K2_GetActorLocation`) (0.0 0.0 180.0))))

(event `/Game/Blueprint/Enemies/Interfaces/BPI_Enemy.Attack`
  (bind _capsulecomponent (`self.CapsuleComponent`))
  (bind _charactermovement (`self.CharacterMovement`))
  (bind _capsulecomponent_2 (`self.CapsuleComponent`))
  ;[1 1 1] Flying Melee Attack
  (set `self.StartPos` (`self.K2_GetActorLocation`))
  (set `self.TargetPos` (`self.K2_GetActorLocation` (`GameplayStatics.GetPlayerPawn` 0)))
  (`PrimitiveComponent.SetCollisionResponseToChannel` _capsulecomponent "ECC_GameTraceChannel1" "ECR_Overlap")
  (`PrimitiveComponent.SetCollisionResponseToChannel` _capsulecomponent "ECC_Pawn" "ECR_Overlap")
  (`PrimitiveComponent.SetCollisionResponseToChannel` _capsulecomponent "ECC_WorldStatic" "ECR_Ignore")
  (`PrimitiveComponent.SetCollisionResponseToChannel` _capsulecomponent "ECC_WorldDynamic" "ECR_Ignore")
  (set `CharacterMovementComponent.GravityScale` 0.0 _charactermovement)
  (set `MovementComponent.Velocity` (0.0 0.0 0.0) _charactermovement)
  (bind (_direction _track) (`Timeline|DashAttack` :!label _label)
    (:`Update`
      (`self.K2_SetActorLocation` (`KismetMathLibrary.VLerp` (`self.StartPos`) (`self.TargetPos`) _track)))
    (:`Finished`
      (`/Engine/EditorBlueprintResources/StandardMacros.FlipFlop`
        (:`A`
          (goto _label :!via `ReverseFromEnd`))
        (:`B`
          (`PrimitiveComponent.SetCollisionResponseToChannel` _capsulecomponent_2 "ECC_GameTraceChannel1" "ECR_Block")
          (`PrimitiveComponent.SetCollisionResponseToChannel` _capsulecomponent_2 "ECC_Pawn" "ECR_Block")
          (`PrimitiveComponent.SetCollisionResponseToChannel` _capsulecomponent_2 "ECC_WorldStatic" "ECR_Block")
          (`PrimitiveComponent.SetCollisionResponseToChannel` _capsulecomponent_2 "ECC_WorldDynamic" "ECR_Block")
          (set `CharacterMovementComponent.GravityScale` 1.0 (`self.CharacterMovement`)))))))

(event `self.CapsuleComponent.OnComponentBeginOverlap`
  (params (OverlappedComponent :type "PrimitiveComponent Object Reference") (OtherActor :type "Actor Object Reference") (OtherComp :type "PrimitiveComponent Object Reference") (OtherBodyIndex :type Integer) (bFromSweep :type Boolean) (SweepResult :type "HitResult Structure (by ref)"))
  (bind _returnvalue (`GameplayStatics.GetPlayerPawn` 0))
  (if (and (== OtherActor _returnvalue) (== OtherComp (`self.GetComponentByClass` _returnvalue "/Script/Engine.CapsuleComponent")))
    (`GameplayStatics.ApplyDamage` _returnvalue (`self.AttackDamage`))
    (`KismetSystemLibrary.PrintString` "ATTACKED PLAYER" true true (struct :`R` 1.0 :`G` 0.023497 :`B` 0.203665 :`A` 1.0))))

(fn `UserConstructionScript`
  (`parent.UserConstructionScript`))