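; Enemy character Blueprint that tracks health, movement speed and attack state, with stub DoDamage and GetSkeletalMesh functions.
; Damage arrives through an interface event and reduces health; lethal damage calls Death, which reports the kill to BP_MLGameMode and destroys the actor.
; EMP hits write stun state and duration to the AI controller's Blackboard, while Attack only sets a flag.
; Walk speed is set at construction and can be changed at runtime.
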(event `self.ReceiveBeginPlay`
  (set `self.CurrentHealth` (`self.Health`)))

(event `Death`
  (bind _asbp_mlgame_mode (cast `/Game/GameMode/BP_MLGameMode` (`GameplayStatics.GetGameMode`)))
  (`/Game/GameMode/BP_MLGameMode.EnemyKill` _asbp_mlgame_mode)
  (`self.K2_DestroyActor`))

(event `self.CapsuleComponent.OnComponentHit`
  (params (HitComponent :type "PrimitiveComponent Object Reference") (OtherActor :type "Actor Object Reference") (OtherComp :type "PrimitiveComponent Object Reference") (NormalImpulse :type "Vector Structure") (Hit :type "HitResult Structure (by ref)")))

(event `/Game/Blueprint/Enemies/Interfaces/BPI_Enemy.EMP`
  (params (Duration :type "Float (double-precision)"))
  (bind _returnvalue (`AIBlueprintHelperLibrary.GetBlackboard` (`AIBlueprintHelperLibrary.GetAIController` self)))
  ;[1 1 1] EMP
  (`BlackboardComponent.SetValueAsFloat` _returnvalue (`self.EMPDuration`) Duration)
  (`BlackboardComponent.SetValueAsBool` _returnvalue (`self.IsStunned`) true))

(event `/Game/Blueprint/Enemies/Interfaces/BPI_Enemy.Attack`
  ;[1 1 1] Attack
  (set `self.IsAttacking` true))

(event `/Game/Blueprint/Enemies/Interfaces/BPI_Enemy.UpdateSpeed`
  (params (Speed :type "Float (double-precision)"))
  (set `CharacterMovementComponent.MaxWalkSpeed` Speed (`self.CharacterMovement`)))

(event `/Game/Blueprint/Interfaces/BPI_TakeDamage.TakeDamageByInterface`
  (params (Damage :type "Float (double-precision)"))
  (`self.TakeDamage` Damage))

(fn `DoDamage`
  (returns (Success :type Boolean))
  (return true))

(fn `GetSkeletalMesh`
  (returns (Mesh :type "SkeletalMeshComponent Object Reference"))
  (return null))

(fn `TakeDamage`
  (params (Damage :type "Float (double-precision)"))
  (if (< Damage (`self.CurrentHealth`))
    (set `self.CurrentHealth` (- (`self.CurrentHealth`) Damage))
    (else
      (`self.Death`))))

(fn `UpdateMaxSpeed`
  (params (`Max Walk Speed` :type "Float (single-precision)"))
  (set `CharacterMovementComponent.MaxWalkSpeed` `Max Walk Speed` (`self.CharacterMovement`)))

(fn `UserConstructionScript`
  (set `CharacterMovementComponent.MaxWalkSpeed` (`self.Max Walk Speed`) (`self.CharacterMovement`)))