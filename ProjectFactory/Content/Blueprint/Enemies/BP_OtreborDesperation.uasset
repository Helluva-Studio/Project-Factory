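; BP_OtreborDesperation is the expanding sphere of Otrebor's desperation move, which plays its sound on spawn.
; The Explosion event scales the mesh on a timeline toward DesperationSphereRadius, then calls CallDesperationDestruction and destroys the actor.
; Overlaps damage the player behind a short timer-reset cooldown, damage turrets identified by BPI_Turret, and destroy other actors whose overlapping component is a Projectile.
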(event `self.ReceiveBeginPlay`
  (`GameplayStatics.PlaySoundAtLocation` "/Game/Audio/SFX/Otrebor/SC_Otrebor_DesperationMove.SC_Otrebor_DesperationMove" (`self.K2_GetActorLocation`) (struct) 1.0 1.0 0.0 null null null null))

(event `Explosion`
  (bind (_direction _scale) (`Timeline|Scaling`)
    (:`Update`
      (`SceneComponent.SetWorldScale3D` (`self.StaticMesh`) (`KismetMathLibrary.Conv_DoubleToVector` (* _scale (/ (`self.DesperationSphereRadius`) 100.0)))))
    (:`Finished`
      (`self.DesperationDestruction`)
      (`self.K2_DestroyActor`))))

(event `self.StaticMesh.OnComponentBeginOverlap`
  (params (OverlappedComponent :type "PrimitiveComponent Object Reference") (OtherActor :type "Actor Object Reference") (OtherComp :type "PrimitiveComponent Object Reference") (OtherBodyIndex :type Integer) (bFromSweep :type Boolean) (SweepResult :type "HitResult Structure (by ref)"))
  (if (== OtherActor (`GameplayStatics.GetPlayerPawn` 0))
    (if (`self.CanDamagePlayer`)
      (`GameplayStatics.ApplyDamage` OtherActor (`self.DesperationDamageToPlayer`) null self)
      (set `self.CanDamagePlayer` false)
      (`KismetSystemLibrary.K2_SetTimerDelegate` (delegate `ResetDamagePlayer`) 0.2))
    (elif (`KismetSystemLibrary.DoesImplementInterface` OtherActor "/Game/Blueprint/Turrets/Interfaces/BPI_Turret.BPI_Turret_C")
      (`GameplayStatics.ApplyDamage` OtherActor (`self.DesperationDamageToTurrets`) null self)
      (else
        (switch `ECollisionChannel` (`PrimitiveComponent.GetCollisionObjectType` OtherComp)
          (:`ECC_GameTraceChannel3`
            (`self.K2_DestroyActor` OtherActor)))))))

(event `ResetDamagePlayer`
  (set `self.CanDamagePlayer` true))

(fn `UserConstructionScript`)