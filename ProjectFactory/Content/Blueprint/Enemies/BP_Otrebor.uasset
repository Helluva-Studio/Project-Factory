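; Otrebor boss enemy that builds turrets on BP_BossTurretTrigger spots and fights the player and turrets with a wrench.
; Stats load from DT_Otrebor; a StateTree drives behavior, receiving PlayerFound on random player hits and DesperationMove when accumulated damage crosses a threshold.
; Turret choice depends on player distance and the previous pick.
; Attacks use timer-looped capsule traces or a launch toward the player; death stops logic and opens the bossfight door.
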(event `self.ReceiveBeginPlay`)

(event `Start`
  ;[0.07146 0.2755 1] Populate the available turret triggers array
  (`self.Initialize` 1)
  (`parent.ReceiveBeginPlay`)
  (bind _outactors (`GameplayStatics.GetAllActorsOfClass` "/Game/Blueprint/Turrets/BP_BossTurretTrigger.BP_BossTurretTrigger_C"))
  (set `self.AvailableTurretTriggers` _outactors)
  (`SceneComponent.K2_AttachToComponent` (`self.Wrench`) (`self.Mesh`) "Palm2_R" "KeepRelative" "KeepRelative" "KeepWorld" true)
  (`KismetSystemLibrary.Delay` 5.0)
  (`BrainComponent.StartLogic` (`self.StateTree`)))

(event `BuildTurret`
  ;[1 1 1] Build Turret
  (set `self.CanBuildTurret` false)
  (bind _turretchosen (`self.ChooseTurret`))
  (`/Game/Blueprint/Turrets/BP_TurretTrigger.InteractPurchaseWithTurret` (`self.TargetTurretTrigger`) _turretchosen 3)
  (`/Engine/EditorBlueprintResources/StandardMacros.IncrementInt` (`self.TurretOwned`)
    (:`  `
      (`KismetSystemLibrary.Delay` (`self.TurretBuildCooldown`))
      (set `self.CanBuildTurret` true))))

(event `/Game/Blueprint/Enemies/Interfaces/BPI_Otrebor.AddTurretTrigger`
  (params (TurretTrigger :type "/Game/Blueprint/Turrets/BP_TurretTrigger Object Reference"))
  ;[1 1 1] Build Turret
  (`KismetArrayLibrary.Array_AddUnique` (`self.AvailableTurretTriggers`) TurretTrigger))

(event `/Game/Blueprint/Enemies/Interfaces/BPI_Otrebor.RemoveTurretTrigger`
  (params (TurretTrigger :type "/Game/Blueprint/Turrets/BP_TurretTrigger Object Reference"))
  ;[1 1 1] Build Turret
  (`KismetArrayLibrary.Array_RemoveItem` (`self.AvailableTurretTriggers`) TurretTrigger))

(event `ResetDesperation`
  (set `self.TotalDamage` 0.0))

(event `StartAttack`
  ;[1 0.1979 0.1979] Attack
  (bind _returnvalue (`KismetSystemLibrary.K2_SetTimerDelegate` (delegate `PerformAttack`) 0.01 true))
  (set `self.AttackTimer` _returnvalue))

(event `StopAttack`
  ;[1 0.1979 0.1979] Attack
  (`KismetSystemLibrary.K2_ClearAndInvalidateTimerHandle` (`self.AttackTimer`))
  (`KismetArrayLibrary.Array_Clear` (`self.Actors to Ignore`)))

(event `PerformAttack`
  (bind _wrench (`self.Wrench`))
  (bind _returnvalue (`SceneComponent.K2_GetComponentLocation` _wrench))
  (bind (_min _max) (`StaticMeshComponent.GetLocalBounds` _wrench))
  ;[1 0.1979 0.1979] Attack
  (bind _outhit (`KismetSystemLibrary.CapsuleTraceSingleForObjects` (- _returnvalue _min) (+ _returnvalue _max) 30.0 40.0 (`self.Object Types`) false (`self.Actors to Ignore`)))
  (bind (_bblockinghit _binitialoverlap _time _distance _location _impactpoint _normal _impactnormal _physmat _hitactor) (`GameplayStatics.BreakHitResult` _outhit))
  (if (== _hitactor (`GameplayStatics.GetPlayerPawn` 0))
    (`GameplayStatics.ApplyDamage` _hitactor (`self.AttackDamage`) null self)
    (`KismetArrayLibrary.Array_AddUnique` (`self.Actors to Ignore`) _hitactor)
    (elif (`KismetSystemLibrary.DoesImplementInterface` _hitactor "/Game/Blueprint/Turrets/Interfaces/BPI_Turret.BPI_Turret_C")
      (`GameplayStatics.ApplyDamage` _hitactor (`self.AttackDamageVsTurrets`) null self)
      (`KismetArrayLibrary.Array_AddUnique` (`self.Actors to Ignore`) _hitactor))))

(event `/Game/Blueprint/Enemies/Interfaces/BPI_Enemy.Initialize`
  (params (Level :type Integer))
  ;[0.07146 0.2755 1] Initialization
  (bind _returnvalue (`|GetDataTableRow` "/Game/Blueprint/Enemies/Data/DT_Otrebor.DT_Otrebor" "1")
    (:`then`
      (`|ExecutionSequence`
        (:`then_0`
          (bind (__health __attackdamage_player __attackdamage_turrets __speed __essencedrop __knockbackable __noise _maxturretsownable _turretbuildingcd _maxdistancefromrobertotobuildturret _maxchasingtime _maxdistancetostartchasingplayer _timebeforedesperationmove _maxbearabledamagebeforedesperation _desperationsphereradius _desperationdamagetoturrets _desperationdamagetoplayer _probabilitytobedistractedonhit) (break `/Game/Blueprint/Enemies/Data/S_Otrebor` _returnvalue))
          (bind _output_get (set `self.Health` __health))
          (set `self.CurrentHealth` _output_get)
          (set `CharacterMovementComponent.MaxWalkSpeed` __speed (`self.CharacterMovement`))
          (set `self.EssenceDrop` __essencedrop)
          (set `self.CanBeKnockedback` __knockbackable))
        (:`then_1`
          (set `self.AttackDamage` __attackdamage_player)
          (set `self.AttackDamageVsTurrets` __attackdamage_turrets))
        (:`then_2`
          (set `self.MonsterNoise` __noise))
        (:`then_3`
          (set `self.MaxTurretsOwnable` _maxturretsownable)
          (set `self.TurretBuildCooldown` _turretbuildingcd)
          (set `self.MaxDistanceFromRobertoToBuildTurret` _maxdistancefromrobertotobuildturret))
        (:`then_4`
          (set `self.MaxChaseTime` _maxchasingtime)
          (set `self.MaxDistanceToChasePlayer` _maxdistancetostartchasingplayer))
        (:`then_5`
          (set `self.TimeBeforeDesperationMove` _timebeforedesperationmove)
          (set `self.DesperationMaxBearableDamage` _maxbearabledamagebeforedesperation))
        (:`then_6`
          (set `self.DesperationSphereRadius` _desperationsphereradius)
          (set `self.DesperationDamageToTurrets` _desperationdamagetoturrets)
          (set `self.DesperationDamageToPlayer` _desperationdamagetoplayer)
          (set `self.ProbabilityToBeDistractedOnHit` (`KismetMathLibrary.FClamp` _probabilitytobedistractedonhit)))))))

(event `JumpAttack`
  (bind _returnvalue (`self.K2_GetActorLocation`))
  (bind _returnvalue_2 (`self.K2_GetActorLocation` (`GameplayStatics.GetPlayerPawn` 0)))
  (bind _returnvalue_3 (`KismetMathLibrary.FindLookAtRotation` _returnvalue _returnvalue_2))
  (bind (_returnvalue_x _returnvalue_y) (`KismetMathLibrary.BreakVector` (* (`KismetMathLibrary.GetForwardVector` _returnvalue_3) (+ (`KismetMathLibrary.Vector_Distance` _returnvalue _returnvalue_2) 100.0))))
  (bind (_returnvalue_x_2 _returnvalue_y_2 _returnvalue_z) (`KismetMathLibrary.BreakVector` (* (`KismetMathLibrary.GetUpVector` _returnvalue_3) 200.0)))
  (`self.LaunchCharacter` (`KismetMathLibrary.MakeVector` _returnvalue_x _returnvalue_y _returnvalue_z)))

(event `/Game/Blueprint/Enemies/Interfaces/BPI_Enemy.Death`
  (`BrainComponent.StopLogic` (`self.StateTree`) "")
  (`MovementComponent.StopMovementImmediately` (`self.CharacterMovement`))
  (`PrimitiveComponent.SetCollisionEnabled` (`self.CapsuleComponent`) "NoCollision")
  (`PrimitiveComponent.SetCollisionEnabled` (`self.Mesh`) "NoCollision")
  (`SkeletalMeshComponent.PlayAnimation` (`self.Mesh`) "/Game/Models/Robot/Animations/Robot/MM_Robot_Death.MM_Robot_Death" false)
  (`KismetSystemLibrary.Delay` 1.5)
  (bind _returnvalue (`GameplayStatics.GetActorOfClass` "/Game/Blueprint/Envirorment/Doors/BP_BossfightDoor.BP_BossfightDoor_C"))
  (`/Game/Blueprint/Tutorial/BP_DoorTutorial.OpenDoor` _returnvalue))

(fn `ChooseTurret`
  (returns (TurretChosen :type "/Game/Blueprint/Turrets/BP_Turret_Base Class Reference"))
  (locals (LastTurretBuilt :type "/Game/Blueprint/Turrets/BP_Turret_Base Class Reference"))
  (if (>= (`KismetMathLibrary.Vector_Distance` (`self.K2_GetActorLocation`) (`self.K2_GetActorLocation` (`GameplayStatics.GetPlayerPawn` 0))) (`self.MaxDistanceFromRobertoToBuildTurret`))
    (return "/Game/Blueprint/Turrets/OtreborTurrets/BP_O_Laser.BP_O_Laser_C")
    (elif (>= (`self.LastTurretPosition`) 0)
      (switch `int` (`self.LastTurretPosition`)
        (:`0`
          (set `self.LastTurretPosition` -1)
          (return "/Game/Blueprint/Turrets/OtreborTurrets/BP_O_Slow.BP_O_Slow_C"))
        (:`1`
          (set `self.LastTurretPosition` -1)
          (return "/Game/Blueprint/Turrets/OtreborTurrets/BP_O_Laser.BP_O_Laser_C"))
        (:`2`
          (bind _output_get (set `self.LastTurretPosition` (`.OutIndex` (`KismetArrayLibrary.Array_Random` (`self.OtreborTurrets`)))))
          (return (`|GetArrayItem` (`self.OtreborTurrets`) _output_get))))
      (else
        (bind _output_get_2 (set `self.LastTurretPosition` (`.OutIndex` (`KismetArrayLibrary.Array_Random` (`self.OtreborTurrets`)))))
        (return (`|GetArrayItem` (`self.OtreborTurrets`) _output_get_2))))))

(fn `GetTurretTriggers`)

(fn `Stun`
  (if (`self.IsStunned`)
    (`BrainComponent.StopLogic` (`self.StateTree`) "")
    (else
      (`BrainComponent.RestartLogic` (`self.StateTree`)))))

(fn `Take Damage`
  (params (Damage :type "Float (double-precision)") (Actor :type "Actor Object Reference"))
  (locals (DesperationTimer :type "TimerHandle Structure"))
  (`parent.Take Damage` Damage Actor)
  (`|ExecutionSequence`
    (:`then_0`
      (if (not (`KismetSystemLibrary.K2_IsValidTimerHandle` (`local.DesperationTimer`)))
        (bind _returnvalue (`KismetSystemLibrary.K2_SetTimerDelegate` (`|CreateDelegate` :!event `ResetDesperation`) (`self.TimeBeforeDesperationMove`)))
        (set `local.DesperationTimer` _returnvalue))
      (set `self.TotalDamage` (+ (`self.TotalDamage`) (`local.Damage`)))
      (if (>= (`self.TotalDamage`) (`self.DesperationMaxBearableDamage`))
        (set `self.TotalDamage` 0.0)
        (`StateTreeComponent.SendStateTreeEvent` (`self.StateTree`) (make `StateTreeEvent` (struct :`TagName` "DesperationMove")))))
    (:`then_1`
      (if (and (== Actor (`GameplayStatics.GetPlayerPawn` 0)) (> (`self.CurrentHealth`) 0.0) (`KismetMathLibrary.RandomBoolWithWeight` (`self.ProbabilityToBeDistractedOnHit`)))
        (`StateTreeComponent.SendStateTreeEvent` (`self.StateTree`) (make `StateTreeEvent` (struct :`TagName` "PlayerFound")))))))

(fn `UserConstructionScript`
  (`parent.UserConstructionScript`))