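; Recharge station that transfers its stored energy to an overlapping BPI_Robot actor, then cools down once empty.
; A re-armed timer ticks faster with each transfer, raising the SFX pitch, dimming the light and reporting noise at the station.
; On depletion, a timeline scaled by TimeToReactivate drives the cooldown, then refills storage and resumes if the player still overlaps.
; World and minimap radial widgets show charge in blue and cooldown in red.
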(event `self.ReceiveBeginPlay`
  (bind (_as_normal_widget _as_minimap_widget) (`self.GetWidget`))
  (`|ExecutionSequence`
    (:`then_0`
      (`SceneComponent.K2_SetWorldRotation` (`self.MinimapIcon`) (struct :`Yaw` 90.0) false false))
    (:`then_1`
      (`RadialSlider.SetSliderProgressColor` (`/Game/Blueprint/Turrets/TurretFeature/TurretTrigger/WB_ReactivationTime.RadialSlider` _as_normal_widget) (struct :`G` 0.5 :`B` 1.0 :`A` 1.0))
      (`RadialSlider.SetSliderProgressColor` (`/Game/Blueprint/Turrets/TurretFeature/TurretTrigger/WB_ReactivationTime.RadialSlider` _as_minimap_widget) (struct :`G` 0.5 :`B` 1.0 :`A` 1.0))
      (set `/Game/Blueprint/Turrets/TurretFeature/TurretTrigger/WB_ReactivationTime.CurrentValue` 1.0 _as_normal_widget)
      (set `/Game/Blueprint/Turrets/TurretFeature/TurretTrigger/WB_ReactivationTime.CurrentValue` 1.0 _as_minimap_widget))
    (:`then_2`
      (bind _output_get (set `self.EnergyStorage` (`self.MaxEnergyStorage`)))
      (`LightComponent.SetIntensity` (`self.PointLight`) (* (/ _output_get (`self.MaxEnergyStorage`)) (`self.LightIntensityMultiplier`)))
      (set `self.IsInCooldown` false))))

(event `self.PlayerTrigger.OnComponentBeginOverlap`
  (params (OverlappedComponent :type "PrimitiveComponent Object Reference") (OtherActor :type "Actor Object Reference") (OtherComp :type "PrimitiveComponent Object Reference") (OtherBodyIndex :type Integer) (bFromSweep :type Boolean) (SweepResult :type "HitResult Structure (by ref)"))
  (if (`KismetSystemLibrary.DoesImplementInterface` OtherActor "/Game/Blueprint/Robot/Interfaces/BPI_Robot.BPI_Robot_C")
    (set `self.RobotToRecharge` OtherActor)
    (if (not (`self.IsInCooldown`))
      (set `self.RechargeTick` (`self.OriginalRechargeTick`))
      (set `self.Pitch Multiplier` 1.0)
      (`self.StartRecharging`))))

(event `StartRecharging`
  (bind _returnvalue (`KismetSystemLibrary.K2_SetTimerDelegate` (delegate `RechargeRobot`) (`self.RechargeTick`)))
  (set `self.RechargeTimer` _returnvalue)
  (`RadialSlider.SetSliderProgressColor` (`/Game/Blueprint/Turrets/TurretFeature/TurretTrigger/WB_ReactivationTime.RadialSlider` (`self.GetWidget`)) (struct :`G` 0.5 :`B` 1.0 :`A` 1.0))
  (`RadialSlider.SetSliderProgressColor` (`/Game/Blueprint/Turrets/TurretFeature/TurretTrigger/WB_ReactivationTime.RadialSlider` (`.As Minimap Widget` (`self.GetWidget`))) (struct :`G` 0.5 :`B` 1.0 :`A` 1.0)))

(event `RechargeRobot`
  (bind (_as_normal_widget _as_minimap_widget) (`self.GetWidget`))
  (bind _rechargesfx (`self.RechargeSFX`))
  (bind _returnvalue (/ (`self.EnergyStorage`) (`self.MaxEnergyStorage`)))
  (`/Engine/EditorBlueprintResources/StandardMacros.IsValid` (`self.RobotToRecharge`)
    (:`Is Valid`
      (if (> (`self.EnergyStorage`) 0.0)
        (bind _output_get (set `self.EnergyStorage` (- (`self.EnergyStorage`) (`self.EnergyXTime`))))
        (`LightComponent.SetIntensity` (`self.PointLight`) (* (/ _output_get (`self.MaxEnergyStorage`)) (`self.LightIntensityMultiplier`)))
        (message `/Game/Blueprint/Robot/Interfaces/BPI_Robot.RechargeEnergy` (`self.RobotToRecharge`) (`self.EnergyXTime`))
        (set `self.RechargeTick` (`KismetMathLibrary.FClamp` (- (`self.RechargeTick`) (`self.RechargeTickDecrement`)) (`self.MinimumRechargeTick`)))
        (bind _output_get_2 (set `self.Pitch Multiplier` (+ (`self.Pitch Multiplier`) 0.05)))
        (set `AudioComponent.PitchMultiplier` _output_get_2 _rechargesfx)
        (`AudioComponent.Play` _rechargesfx 0.0)
        (set `/Game/Blueprint/Turrets/TurretFeature/TurretTrigger/WB_ReactivationTime.CurrentValue` _returnvalue _as_normal_widget)
        (set `/Game/Blueprint/Turrets/TurretFeature/TurretTrigger/WB_ReactivationTime.CurrentValue` _returnvalue _as_minimap_widget)
        (`AISense_Hearing.ReportNoiseEvent` (`self.K2_GetActorLocation`) 1.0 self 10000.0)
        (`self.StartRecharging`)
        (else
          (`KismetSystemLibrary.K2_ClearAndInvalidateTimerHandle` (`self.RechargeTimer`))
          (set `self.IsInCooldown` true)
          (bind _output_get_3 (set `self.EnergyStorage` 0.0))
          (`LightComponent.SetIntensity` (`self.PointLight`) _output_get_3)
          (message `/Game/Blueprint/Robot/Interfaces/BPI_Robot.StopRechargeEnergy` (`self.RobotToRecharge`))
          (`RadialSlider.SetSliderProgressColor` (`/Game/Blueprint/Turrets/TurretFeature/TurretTrigger/WB_ReactivationTime.RadialSlider` (`self.GetWidget`)) (struct :`R` 1.0 :`A` 1.0))
          (`RadialSlider.SetSliderProgressColor` (`/Game/Blueprint/Turrets/TurretFeature/TurretTrigger/WB_ReactivationTime.RadialSlider` (`.As Minimap Widget` (`self.GetWidget`))) (struct :`R` 1.0 :`A` 1.0))
          (`self.ReactivateRechargePoint`)
          (`AudioComponent.FadeOut` (`self.RechargeSFX`) 0.5 0.0 "Linear"))))))

(event `self.PlayerTrigger.OnComponentEndOverlap`
  (params (OverlappedComponent :type "PrimitiveComponent Object Reference") (OtherActor :type "Actor Object Reference") (OtherComp :type "PrimitiveComponent Object Reference") (OtherBodyIndex :type Integer))
  (if (`KismetSystemLibrary.DoesImplementInterface` OtherActor "/Game/Blueprint/Robot/Interfaces/BPI_Robot.BPI_Robot_C")
    (`KismetSystemLibrary.K2_ClearAndInvalidateTimerHandle` (`self.RechargeTimer`))
    (message `/Game/Blueprint/Robot/Interfaces/BPI_Robot.StopRechargeEnergy` (`self.RobotToRecharge`))
    (set `self.RobotToRecharge` null)
    (`AudioComponent.FadeOut` (`self.RechargeSFX`) 0.5 0.0 "Linear")
    (if (and (<= (`self.EnergyStorage`) 0.0) (not (`self.IsInCooldown`)))
      (set `self.IsInCooldown` true)
      (`self.ReactivateRechargePoint`))))

(event `ReactivateRechargePoint`
  (bind (_as_normal_widget _as_minimap_widget) (`self.GetWidget`))
  (bind (_as_normal_widget_2 _as_minimap_widget_2) (`self.GetWidget`))
  (bind (_as_normal_widget_3 _as_minimap_widget_3) (`self.GetWidget`))
  (bind _returnvalue (`GameplayStatics.GetPlayerPawn` 0))
  (set `self.RobotToRecharge` null)
  (`TimelineComponent.SetPlayRate` (`self.ReactivationTimeline`) (/ 1.0 (`self.TimeToReactivate`)))
  (set `/Game/Blueprint/Turrets/TurretFeature/TurretTrigger/WB_ReactivationTime.CurrentValue` 0.0 _as_normal_widget_3)
  (set `/Game/Blueprint/Turrets/TurretFeature/TurretTrigger/WB_ReactivationTime.CurrentValue` 0.0 _as_minimap_widget_3)
  (bind (_direction _reactivationpercentagenormalized) (`Timeline|ReactivationTimeline` :!via `ReverseFromEnd`)
    (:`Update`
      (set `/Game/Blueprint/Turrets/TurretFeature/TurretTrigger/WB_ReactivationTime.CurrentValue` _reactivationpercentagenormalized _as_normal_widget_2)
      (`RadialSlider.SetSliderProgressColor` (`/Game/Blueprint/Turrets/TurretFeature/TurretTrigger/WB_ReactivationTime.RadialSlider` _as_normal_widget_2) (struct :`R` 1.0 :`A` 1.0))
      (`RadialSlider.SetSliderProgressColor` (`/Game/Blueprint/Turrets/TurretFeature/TurretTrigger/WB_ReactivationTime.RadialSlider` _as_minimap_widget_2) (struct :`R` 1.0 :`A` 1.0))
      (set `/Game/Blueprint/Turrets/TurretFeature/TurretTrigger/WB_ReactivationTime.CurrentValue` _reactivationpercentagenormalized _as_minimap_widget_2))
    (:`Finished`
      (bind _output_get (set `self.EnergyStorage` (`self.MaxEnergyStorage`)))
      (`LightComponent.SetIntensity` (`self.PointLight`) (* (/ _output_get (`self.MaxEnergyStorage`)) (`self.LightIntensityMultiplier`)))
      (`RadialSlider.SetSliderProgressColor` (`/Game/Blueprint/Turrets/TurretFeature/TurretTrigger/WB_ReactivationTime.RadialSlider` _as_normal_widget) (struct :`G` 0.5 :`B` 1.0 :`A` 1.0))
      (`RadialSlider.SetSliderProgressColor` (`/Game/Blueprint/Turrets/TurretFeature/TurretTrigger/WB_ReactivationTime.RadialSlider` _as_minimap_widget) (struct :`G` 0.5 :`B` 1.0 :`A` 1.0))
      (set `/Game/Blueprint/Turrets/TurretFeature/TurretTrigger/WB_ReactivationTime.CurrentValue` 1.0 _as_normal_widget)
      (set `/Game/Blueprint/Turrets/TurretFeature/TurretTrigger/WB_ReactivationTime.CurrentValue` 1.0 _as_minimap_widget)
      (`PrimitiveComponent.SetMaterial` (`self.Base`) 0 "/Game/LevelPrototyping/Materials/MI_Solid_Blue.MI_Solid_Blue")
      (if (`self.IsOverlappingActor` _returnvalue)
        (set `self.RobotToRecharge` _returnvalue)
        (set `self.RechargeTick` (`self.OriginalRechargeTick`))
        (set `self.Pitch Multiplier` 1.0)
        (`self.StartRecharging`)
        (else
          (set `self.IsInCooldown` false))))))

(fn `GetWidget`
  (returns (`As Normal Widget` :type "/Game/Blueprint/Turrets/TurretFeature/TurretTrigger/WB_ReactivationTime Object Reference") (`As Minimap Widget` :type "/Game/Blueprint/Turrets/TurretFeature/TurretTrigger/WB_ReactivationTime Object Reference"))
  (bind _aswb_reactivation_time (cast `/Game/Blueprint/Turrets/TurretFeature/TurretTrigger/WB_ReactivationTime` (`WidgetComponent.GetWidget` (`self.ReactivationWidget`))))
  (bind _aswb_reactivation_time_2 (cast `/Game/Blueprint/Turrets/TurretFeature/TurretTrigger/WB_ReactivationTime` (`WidgetComponent.GetWidget` (`self.MinimapReactivationWidget`))))
  (return _aswb_reactivation_time _aswb_reactivation_time_2))

(fn `UserConstructionScript`)