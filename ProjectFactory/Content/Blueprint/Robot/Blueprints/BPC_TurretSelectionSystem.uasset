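; Robot component that tracks known turrets, their levels and the currently selected turret.
; The IA_SelectTurret input steps through the known turrets with wrap-around at both ends and broadcasts OnTurretSelectedChange.
; AddTurret registers a turret by key at level one and auto-selects the first one added.
; LevelUpTurret increments the stored level for a given turret type.
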(event `EnhancedInput|/Game/Blueprint/Robot/Input/Actions/IA_SelectTurret`
  (params (ActionValue :type "Float (double-precision)") (ElapsedSeconds :type "Float (double-precision)") (TriggeredSeconds :type "Float (double-precision)") (InputAction :type "InputAction Object Reference" :default "/Game/Blueprint/Robot/Input/Actions/IA_SelectTurret.IA_SelectTurret"))
  (bind _returnvalue (- (`KismetArrayLibrary.Array_Find` (`self.TurretKnownValues`) (`self.TurretSelected`)) ActionValue))
  ;[1 1 1] Selection turret
  (:`Triggered`
    (bind _values (`BlueprintMapLibrary.Map_Values` (`self.TurretKnown`)))
    (set `self.TurretKnownValues` _values)
    (if (< _returnvalue 0.0)
      (set `self.TurretSelected` (`|GetArrayItem` (`self.TurretKnownValues`) (- (`KismetArrayLibrary.Array_Length` (`self.TurretKnownValues`)) 1)))
      (`self.OnTurretSelectedChange`)
      (elif (> _returnvalue (- (`KismetArrayLibrary.Array_Length` (`self.TurretKnownValues`)) 1))
        (set `self.TurretSelected` (`|GetArrayItem` (`self.TurretKnownValues`)))
        (`self.OnTurretSelectedChange`)
        (else
          (set `self.TurretSelected` (`|GetArrayItem` (`self.TurretKnownValues`) (`KismetMathLibrary.FTrunc` _returnvalue)))
          (`self.OnTurretSelectedChange`))))))

(fn `AddTurret`
  (params (`New Turret` :type "/Game/Blueprint/Turrets/BP_Turret_Base Class Reference") (Key :type "/Game/Blueprint/Turrets/TurretGetter/E_TurretType Enum (by ref)"))
  (`BlueprintMapLibrary.Map_Add` (`self.TurretKnown`) Key `New Turret`)
  (`BlueprintMapLibrary.Map_Add` (`self.TurretLevel`) Key 1)
  (if (<= (`BlueprintMapLibrary.Map_Length` (`self.TurretKnown`)) 1)
    (set `self.TurretSelected` `New Turret`)))

(fn `LevelUpTurret`
  (params (TurreteType :type "/Game/Blueprint/Turrets/TurretGetter/E_TurretType Enum" :default "NewEnumerator0"))
  (bind _turretlevel (`self.TurretLevel`))
  (`BlueprintMapLibrary.Map_Add` _turretlevel TurreteType (+ (`BlueprintMapLibrary.Map_Find` _turretlevel TurreteType) 1)))