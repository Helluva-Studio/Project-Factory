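; Interaction trace component that finds the focusable actor the player camera is looking at and toggles its focus message.
; Each tick it box-traces on Visibility from the camera along its forward vector out to InteractRange, which is set through Initialize.
; When the hit actor changes, it clears the previous HitActor's message and shows it on the new one if that implements BPI_Focusable.
; Older BP_InteractionArea focus logic remains in TraceInteractionArea but never runs.
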(event `self.ReceiveTick`
  (params (DeltaSeconds :type "Float (single-precision)"))
  (`self.Trace`))

(fn `Initialize`
  (params (InteractRange :type "Float (double-precision)"))
  (set `self.InteractRange` InteractRange))

(fn `Trace`
  (bind _returnvalue (`GameplayStatics.GetPlayerCameraManager` 0))
  (bind _returnvalue_2 (`PlayerCameraManager.GetCameraLocation` _returnvalue))
  (bind (_outhit _returnvalue_3) (`KismetSystemLibrary.BoxTraceSingle` _returnvalue_2 (+ _returnvalue_2 (* (`KismetMathLibrary.GetForwardVector` (`PlayerCameraManager.GetCameraRotation` _returnvalue)) (`self.InteractRange`))) (10.0 10.0 10.0) (struct) "TraceTypeQuery1"))
  (if _returnvalue_3
    (bind (_bblockinghit _binitialoverlap _time _distance _location _impactpoint _normal _impactnormal _physmat _hitactor) (`GameplayStatics.BreakHitResult` _outhit))
    (if (not (== (`self.Hit Actor`) _hitactor))
      (`|ExecutionSequence`
        (:`then_0`
          (`self.TraceInteractionArea` false))
        (:`then_1`
          (if (`KismetSystemLibrary.DoesImplementInterface` _hitactor "/Game/Blueprint/InteractionArea/BPI_Focusable.BPI_Focusable_C")
            (set `self.Hit Actor` _hitactor)
            (`self.TraceInteractionArea` true)
            (else
              (`self.TraceInteractionArea` false))))))
    (else
      (`self.TraceInteractionArea` false))))

(fn `TraceInteractionArea`
  (params (Trace :type Boolean))
  (bind _hit_actor (`self.Hit Actor`))
  (if Trace
    (message `/Game/Blueprint/InteractionArea/BPI_Focusable.ToggleFocus` (`self.Hit Actor`) true)
    (else
      (`/Engine/EditorBlueprintResources/StandardMacros.IsValid` _hit_actor
        (:`Is Valid`
          (message `/Game/Blueprint/InteractionArea/BPI_Focusable.ToggleFocus` _hit_actor false)
          (set `self.Hit Actor` null))))))