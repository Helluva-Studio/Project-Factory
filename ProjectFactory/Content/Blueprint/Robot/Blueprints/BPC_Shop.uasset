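; Shop component for the player robot that sells power-ups and turret upgrades.
; It loads items from the PowerUps DataTable, and IA_Shop toggles a WB_Shop widget that pauses the game and hides the HUD.
; On close, it saves the widget's item list and restores play.
; Purchases raise BP_Roberto's max health or energy or level up turrets through its turret selection component, while AddTurret makes turret entries visible.
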(event `self.ReceiveBeginPlay`
  (for _index (range 1 (+ (`self.NumberOfPowerUps`) 1))
    (bind _returnvalue (`|GetDataTableRow` "/Game/Blueprint/PowerUps/PowerUps.PowerUps" (`KismetStringLibrary.Conv_StringToName` (`KismetStringLibrary.Conv_IntToString` _index)))
      (:`then`
        (`KismetArrayLibrary.Array_Add` (`self.PowerUpItems`) _returnvalue)))))

(event `EnhancedInput|/Game/Blueprint/Robot/Input/Actions/IA_Shop`
  (params (ActionValue :type Boolean) (ElapsedSeconds :type "Float (double-precision)") (TriggeredSeconds :type "Float (double-precision)") (InputAction :type "InputAction Object Reference" :default "/Game/Blueprint/Robot/Input/Actions/IA_Shop.IA_Shop"))
  (bind _returnvalue (`GameplayStatics.GetPlayerController` 0))
  (bind _returnvalue_2 (`GameplayStatics.GetPlayerController` 0))
  (:`Started`
    (if (not (`GameplayStatics.IsGamePaused`))
      (bind _returnvalue_3 (`|CreateWidget` "/Game/HUD/PowerUpHUD/WB_Shop.WB_Shop_C" _returnvalue))
      (`/Game/HUD/PowerUpHUD/WB_Shop.Initialize` _returnvalue_3 (`self.PowerUpItems`))
      (set `PlayerController.bShowMouseCursor` true _returnvalue)
      (set `self.ShopPanel` _returnvalue_3)
      (`WidgetBlueprintLibrary.SetInputMode_GameAndUIEx` _returnvalue null "LockAlways")
      (`UserWidget.AddToViewport` _returnvalue_3 0)
      (`GameplayStatics.SetGamePaused` true)
      (bind _foundwidgets (`WidgetBlueprintLibrary.GetAllWidgetsOfClass` "/Game/HUD/PlayerHUD/WB_PlayerHUD.WB_PlayerHUD_C"))
      (for _array_element _foundwidgets
        (if (`Widget.IsVisible` _array_element)
          (`Widget.SetVisibility` _array_element "Hidden")))
      (else
        (bind _shoppanel (`self.ShopPanel` :!label _label)
          (:`then`
            (`self.UpdateOnClose` (`/Game/HUD/PowerUpHUD/WB_Shop.PowerUpList` _shoppanel))
            (`Widget.RemoveFromParent` _shoppanel)
            (`GameplayStatics.SetGamePaused` false)
            (`WidgetBlueprintLibrary.SetInputMode_GameOnly` _returnvalue_2)
            (set `PlayerController.bShowMouseCursor` false _returnvalue_2)
            (bind _foundwidgets_2 (`WidgetBlueprintLibrary.GetAllWidgetsOfClass` "/Game/HUD/PlayerHUD/WB_PlayerHUD.WB_PlayerHUD_C"))
            (for _array_element_2 _foundwidgets_2
              (if (not (`Widget.IsVisible` _array_element_2))
                (`Widget.SetVisibility` _array_element_2 "Visible")
                (set `self.ShopPanel` null))))
          (:`else`))))))

(event `CloseShop`
  (goto _label))

(fn `AddTurret`
  (params (`E Turret` :type "/Game/Blueprint/Turrets/TurretGetter/E_TurretType Enum" :default "NewEnumerator0"))
  (switch `/Game/Blueprint/Turrets/TurretGetter/E_TurretType` `E Turret`
    (:`NewEnumerator0`
      (`self.SetTurretVisible` 2))
    (:`NewEnumerator2`
      (`self.SetTurretVisible` 3))
    (:`NewEnumerator3`
      (`self.SetTurretVisible` 4))
    (:`NewEnumerator4`
      (`self.SetTurretVisible` 5))
    (:`NewEnumerator5`
      (`self.SetTurretVisible` 6))
    (:`NewEnumerator6`
      (`self.SetTurretVisible` 7))
    (:`NewEnumerator7`
      (`self.SetTurretVisible` 8))
    (:`NewEnumerator8`
      (`self.SetTurretVisible` 9))
    (:`NewEnumerator9`
      (`self.SetTurretVisible` 10))
    (:`NewEnumerator1`
      (`self.SetTurretVisible` 11))
    (:`NewEnumerator10`
      (`self.SetTurretVisible` 12))
    (:`NewEnumerator11`
      (`self.SetTurretVisible` 13))))

(fn `OnItemBought`
  (params (PowerUpType :type "/Game/Blueprint/PowerUps/PowerUpEnum Enum" :default "NewEnumerator0"))
  (locals (TurretType :type "/Game/Blueprint/Turrets/TurretGetter/E_TurretType Enum" :default "NewEnumerator0"))
  (switch `/Game/Blueprint/PowerUps/PowerUpEnum` PowerUpType
    (:`NewEnumerator0`
      (bind _asbp_roberto (cast `/Game/Blueprint/Robot/Blueprints/BP_Roberto` (`GameplayStatics.GetPlayerPawn` 0)))
      (set `/Game/Blueprint/Robot/Blueprints/BP_Roberto.MaxHealth` (+ (`/Game/Blueprint/Robot/Blueprints/BP_Roberto.MaxHealth` _asbp_roberto) (/ (`/Game/Blueprint/Robot/Blueprints/BP_Roberto.StartingHealth` _asbp_roberto) 4.0)) _asbp_roberto)
      (bind _foundwidgets (`WidgetBlueprintLibrary.GetAllWidgetsOfClass` "/Game/HUD/PlayerHUD/WB_PlayerHUD.WB_PlayerHUD_C"))
      (message `/Game/HUD/PlayerHUD/BPI_PlayerHUD.UpdateHealthBar` (`|GetArrayItem` _foundwidgets)))
    (:`NewEnumerator1`
      (bind _asbp_roberto_2 (cast `/Game/Blueprint/Robot/Blueprints/BP_Roberto` (`GameplayStatics.GetPlayerPawn` 0)))
      (set `/Game/Blueprint/Robot/Blueprints/BP_Roberto.MaxEnergy` (+ (`/Game/Blueprint/Robot/Blueprints/BP_Roberto.MaxEnergy` _asbp_roberto_2) (/ (`/Game/Blueprint/Robot/Blueprints/BP_Roberto.StartingEnergy` _asbp_roberto_2) 4.0)) _asbp_roberto_2)
      (bind _foundwidgets_2 (`WidgetBlueprintLibrary.GetAllWidgetsOfClass` "/Game/HUD/PlayerHUD/WB_PlayerHUD.WB_PlayerHUD_C"))
      (message `/Game/HUD/PlayerHUD/BPI_PlayerHUD.UpdateEnergyBar` (`|GetArrayItem` _foundwidgets_2)))
    (:`NewEnumerator5`
      (set `local.TurretType` "NewEnumerator0")
      (bind _asbp_roberto_3 (cast `/Game/Blueprint/Robot/Blueprints/BP_Roberto` (`self.GetOwner`) :!label _label))
      (`/Game/Blueprint/Robot/Blueprints/BPC_TurretSelectionSystem.LevelUpTurret` (`/Game/Blueprint/Robot/Blueprints/BP_Roberto.BPC_TurretSelectionSystem` _asbp_roberto_3) (`local.TurretType`)))
    (:`NewEnumerator6`
      (set `local.TurretType` "NewEnumerator2")
      (goto _label))
    (:`NewEnumerator7`
      (set `local.TurretType` "NewEnumerator3")
      (goto _label))
    (:`NewEnumerator8`
      (set `local.TurretType` "NewEnumerator4")
      (goto _label))
    (:`NewEnumerator9`
      (set `local.TurretType` "NewEnumerator5")
      (goto _label))
    (:`NewEnumerator10`
      (set `local.TurretType` "NewEnumerator6")
      (goto _label))
    (:`NewEnumerator11`
      (set `local.TurretType` "NewEnumerator7")
      (goto _label))
    (:`NewEnumerator12`
      (set `local.TurretType` "NewEnumerator8")
      (goto _label))
    (:`NewEnumerator13`
      (set `local.TurretType` "NewEnumerator9")
      (goto _label))
    (:`NewEnumerator14`
      (set `local.TurretType` "NewEnumerator1")
      (goto _label))
    (:`NewEnumerator15`
      (set `local.TurretType` "NewEnumerator10")
      (goto _label))
    (:`NewEnumerator16`
      (set `local.TurretType` "NewEnumerator11")
      (goto _label))))

(fn `SetTurretVisible`
  (params (IndexPowerUp :type Integer))
  (bind (_type _maxavailability _availability _name _description _image _basecost _percentageonavailabilityoncost _cost _isvisible _isdisable) (break `/Game/Blueprint/PowerUps/S_PowerUpItems` (`|GetArrayItem` (`self.PowerUpItems`) IndexPowerUp)))
  (`KismetArrayLibrary.Array_Set` (`self.PowerUpItems`) IndexPowerUp (make `/Game/Blueprint/PowerUps/S_PowerUpItems` _type _maxavailability _availability _name _description _image _basecost _percentageonavailabilityoncost _cost true _isdisable)))

(fn `UpdateOnClose`
  (params (PowerUpItems :type "Array of /Game/Blueprint/PowerUps/S_PowerUpItems Structure"))
  (set `self.PowerUpItems` PowerUpItems)
  (bind _foundwidgets (`WidgetBlueprintLibrary.GetAllWidgetsOfClass` "/Game/HUD/PowerUpHUD/WB_ShopItem.WB_ShopItem_C"))
  (for _array_element _foundwidgets
    (`Widget.RemoveFromParent` _array_element))
  (bind _foundwidgets_2 (`WidgetBlueprintLibrary.GetAllWidgetsOfClass` "/Game/HUD/PowerUpHUD/WB_ShopItemDescription.WB_ShopItemDescription_C"))
  (for _array_element_2 _foundwidgets_2
    (`Widget.RemoveFromParent` _array_element_2)))