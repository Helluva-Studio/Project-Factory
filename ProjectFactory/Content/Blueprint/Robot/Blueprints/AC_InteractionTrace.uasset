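; Actor component that line-traces from the player camera each tick to find BI_Interactable actors and send them focus messages.
; The trace uses the Visibility channel over an InteractRange set through Initialize.
; As written, a constant false in the hit check stops HitActor from ever being set or focused.
; The miss branch messages and clears any stored actor, and FocusElement is an empty stub.
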(event `self.ReceiveTick`
  (params (DeltaSeconds :type "Float (single-precision)"))
  (`self.Trace`))

(fn `FocusElement`)

(fn `Initialize`
  (params (InteractRange :type "Float (double-precision)"))
  (set `self.InteractRange` InteractRange))

(fn `Trace`
  (bind _returnvalue (`GameplayStatics.GetPlayerCameraManager` 0))
  (bind _returnvalue_2 (`PlayerCameraManager.GetCameraLocation` _returnvalue))
  (bind (_outhit _returnvalue_3) (`KismetSystemLibrary.LineTraceSingle` _returnvalue_2 (+ _returnvalue_2 (* (`KismetMathLibrary.GetForwardVector` (`PlayerCameraManager.GetCameraRotation` _returnvalue)) (`self.InteractRange`))) "TraceTypeQuery1"))
  (if _returnvalue_3
    (bind (_bblockinghit _binitialoverlap _time _distance _location _impactpoint _normal _impactnormal _physmat _hitactor) (`GameplayStatics.BreakHitResult` _outhit))
    (if (and false (`KismetSystemLibrary.DoesImplementInterface` _hitactor "/Game/Blueprint/Turrets/Interfaces/BI_Interactable.BI_Interactable_C"))
      (bind _output_get (set `self.Hit Actor` _hitactor))
      (message `/Game/Blueprint/Turrets/Interfaces/BI_Interactable.Focus` _output_get true))
    (else
      (bind _hit_actor (`self.Hit Actor`)
        (:`then`
          (message `/Game/Blueprint/Turrets/Interfaces/BI_Interactable.Focus` _hit_actor (!= (`self.Hit Actor`) _hitactor))
          (set `self.Hit Actor` null))
        (:`else`)))))