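; Collectible resource pickup that spins and bobs, passing its type and value to any overlapping BPI_Robot actor before destroying itself.
; On spawn it traces downward for the ground, then a timeline scales it up from zero, pops it upward and lerps it onto the hit point while modulating material brightness.
; Collision stays off until landing finishes, then a despawn delay starts that destroys uncollected pickups.
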(event `self.ReceiveTick`
  (params (DeltaSeconds :type "Float (single-precision)"))
  (`SceneComponent.K2_AddWorldRotation` (`self.ResourceMesh`) (struct :`Yaw` 1.0) false false)
  (`SceneComponent.K2_SetRelativeLocation` (`self.ResourceMesh`) (`KismetMathLibrary.MakeVector` 0.0 0.0 (* (`KismetMathLibrary.DegSin` (* (`self.GetGameTimeSinceCreation`) 350.0)) 2.0)) false false))

(event `self.ReceiveBeginPlay`
  (bind (_spawnposition_x _spawnposition_y _spawnposition_z) (`KismetMathLibrary.BreakVector` (`self.SpawnPosition`)))
  (bind (_spawnposition_x_2 _spawnposition_y_2 _spawnposition_z_2) (`KismetMathLibrary.BreakVector` (`self.SpawnPosition`)))
  (bind _returnvalue (`PrimitiveComponent.CreateDynamicMaterialInstance` (`self.ResourceMesh`) 0 null "None"))
  (bind _output_get (set `self.MeshColor` _returnvalue))
  (bind _returnvalue_2 (`MaterialInstanceDynamic.K2_GetScalarParameterValue` _output_get "Brightness"))
  (set `self.StartingBrightness` _returnvalue_2)
  (`self.SetActorEnableCollision` false)
  (set `self.SpawnPosition` (`self.K2_GetActorLocation`))
  (set `self.Sphere Radius` (`SphereComponent.SphereRadius` (`self.Sphere`)))
  (`self.SetActorScale3D` (0.0 0.0 0.0))
  (bind _outhit (`KismetSystemLibrary.LineTraceSingleForObjects` (`self.K2_GetActorLocation`) (+ (`self.K2_GetActorLocation`) (* (`KismetMathLibrary.Vector_Down`) 500.0)) (`|MakeArray` "ObjectTypeQuery1" "ObjectTypeQuery2" :!type "EObjectTypeQuery Enum") false (`self.SpawnersToIgnore`)))
  (`TimelineComponent.SetPlayRate` (`self.ScalingAndLanding`) (`KismetMathLibrary.SafeDivide` 1.0 (`self.LandingSpeed`)))
  (bind (_bblockinghit _binitialoverlap _time _distance _location _impactpoint _normal _impactnormal _physmat _hitactor) (`GameplayStatics.BreakHitResult` _outhit))
  (`KismetSystemLibrary.PrintString` (`KismetSystemLibrary.GetDisplayName` _hitactor))
  (bind (_direction _newscale _brightnessvalue _jumpz _positionlerp) (`Timeline|ScalingAndLanding`)
    (:`Update`
      (`|ExecutionSequence`
        (:`then_0`
          (`MaterialInstanceDynamic.SetScalarParameterValue` (`self.MeshColor`) "Brightness" (+ (`self.StartingBrightness`) (* _brightnessvalue (`self.BrightnessModifier`)))))
        (:`then_1`
          (`self.SetActorScale3D` _newscale))
        (:`then_2`
          (if (< _positionlerp 1.0)
            (`self.K2_SetActorLocation` (`KismetMathLibrary.MakeVector` _spawnposition_x _spawnposition_y (+ _spawnposition_z (* _jumpz (`self.Sphere Radius`)))))
            (else
              (`self.K2_SetActorLocation` (`KismetMathLibrary.MakeVector` _spawnposition_x_2 _spawnposition_y_2 (`KismetMathLibrary.Lerp` _spawnposition_z_2 (+ (+ (`self.Sphere Radius`) 20.0) (.z _impactpoint)) (- _positionlerp 1.0)))))))))
    (:`Finished`
      (`self.SetActorEnableCollision` true)
      (`self.Despawn`))))

(event `self.Sphere.OnComponentBeginOverlap`
  (params (OverlappedComponent :type "PrimitiveComponent Object Reference") (OtherActor :type "Actor Object Reference") (OtherComp :type "PrimitiveComponent Object Reference") (OtherBodyIndex :type Integer) (bFromSweep :type Boolean) (SweepResult :type "HitResult Structure (by ref)"))
  (if (`KismetSystemLibrary.DoesImplementInterface` OtherActor "/Game/Blueprint/Robot/Interfaces/BPI_Robot.BPI_Robot_C")
    (message `/Game/Blueprint/Robot/Interfaces/BPI_Robot.GetResource` OtherActor (`self.Type`) (`self.ResourceValue`))
    (`self.K2_DestroyActor`)))

(event `Despawn`
  (`KismetSystemLibrary.Delay` (`self.DespawnTime`))
  (`self.K2_DestroyActor`))

(fn `UserConstructionScript`)