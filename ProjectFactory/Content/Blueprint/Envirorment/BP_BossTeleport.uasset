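; Boss teleporter that unlocks after enough levers are pulled and sends the player to the L_Bossfight level.
; Each Interact call records the count in the game instance and lights a compass direction on the dynamic material.
; At the game mode's threshold, two chained timelines scale up the portal, then enable its collision.
; Player overlap starts a timer, cleared on exit, that shows a loading screen, saves and opens the level.
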(event `self.ReceiveBeginPlay`
  (bind _teleport (`self.Teleport`))
  (set `self.LeversToPull` (`/Game/GameMode/BP_NewGameMode.LeversToPullToActivateTeleport` (`/Game/Blueprint/BP_MacroLibrary_Actor.GetNewGameMode`)))
  (bind _returnvalue (`PrimitiveComponent.CreateDynamicMaterialInstance` _teleport 3 null "None"))
  (bind _output_get (set `self.Material` _returnvalue))
  (`PrimitiveComponent.SetMaterial` _teleport 3 _output_get)
  (`self.K2_SetActorRotation` (`KismetMathLibrary.MakeRotator` 0.0)))

(event `Interact`
  (params (Index :type Integer))
  (`/Engine/EditorBlueprintResources/StandardMacros.IncrementInt` (`self.LeverPulled`)
    (:`  `
      (bind _asbp_new_game_instance (cast `/Game/Blueprint/BP_NewGameInstance` (`GameplayStatics.GetGameInstance`)))
      (set `/Game/Blueprint/BP_NewGameInstance.LeversPulled` (`self.LeverPulled`) _asbp_new_game_instance)
      (switch `int` Index
        (:`0`
          (`MaterialInstanceDynamic.SetScalarParameterValue` (`self.Material`) "Nord" 1.0))
        (:`1`
          (`MaterialInstanceDynamic.SetScalarParameterValue` (`self.Material`) "Sud" 1.0))
        (:`2`
          (`MaterialInstanceDynamic.SetScalarParameterValue` (`self.Material`) "Est" 1.0))
        (:`3`
          (`MaterialInstanceDynamic.SetScalarParameterValue` (`self.Material`) "Ovest" 1.0)))
      (if (>= (`self.LeverPulled`) (`self.LeversToPull`))
        (`self.ActivateTeleport`)))))

(event `self.Collision.OnComponentEndOverlap`
  (params (OverlappedComponent :type "PrimitiveComponent Object Reference") (OtherActor :type "Actor Object Reference") (OtherComp :type "PrimitiveComponent Object Reference") (OtherBodyIndex :type Integer))
  (if (== OtherActor (`GameplayStatics.GetPlayerPawn` 0))
    (`KismetSystemLibrary.K2_ClearAndInvalidateTimerHandle` (`self.TeleportTimer`))))

(event `ActivateTeleport`
  (bind _tp (`self.TP`))
  (bind (_returnvalue_x _returnvalue_y) (`KismetMathLibrary.BreakVector` (`SceneComponent.K2_GetComponentScale` _tp)))
  (bind (_returnvalue_x_2 _returnvalue_y_2 _returnvalue_z) (`KismetMathLibrary.BreakVector` (`SceneComponent.K2_GetComponentScale` (`self.TP`))))
  (set `self.Active` true)
  (`/Engine/EditorBlueprintResources/StandardMacros.DoOnce` false
    (:`Completed`
      (bind (_direction _newtrack_0) (`Timeline|ScaleHeight`)
        (:`Update`
          (`SceneComponent.SetWorldScale3D` _tp (`KismetMathLibrary.MakeVector` _returnvalue_x _returnvalue_y (* _newtrack_0 2.0))))
        (:`Finished`
          (bind (_direction_2 _newtrack_0_2) (`Timeline|ScaleSize`)
            (:`Update`
              (bind _returnvalue (`KismetMathLibrary.Lerp` _returnvalue_x_2 2.0 _newtrack_0_2))
              (`SceneComponent.SetWorldScale3D` (`self.TP`) (`KismetMathLibrary.MakeVector` _returnvalue _returnvalue _returnvalue_z)))
            (:`Finished`
              (`PrimitiveComponent.SetCollisionEnabled` (`self.Collision`) "QueryOnly"))))))))

(event `self.Collision.OnComponentBeginOverlap`
  (params (OverlappedComponent :type "PrimitiveComponent Object Reference") (OtherActor :type "Actor Object Reference") (OtherComp :type "PrimitiveComponent Object Reference") (OtherBodyIndex :type Integer) (bFromSweep :type Boolean) (SweepResult :type "HitResult Structure (by ref)"))
  (if (== OtherActor (`GameplayStatics.GetPlayerPawn` 0))
    (bind _returnvalue (`KismetSystemLibrary.K2_SetTimerDelegate` (delegate `TeleportPlayer`) (`self.TimeToTeleport`)))
    (set `self.TeleportTimer` _returnvalue)))

(event `TeleportPlayer`
  (bind _returnvalue (`|CreateWidget` "/Game/HUD/WB_LoadingScreen.WB_LoadingScreen_C"))
  (`UserWidget.AddToViewport` _returnvalue 0)
  (bind _asbp_new_game_instance (cast `/Game/Blueprint/BP_NewGameInstance` (`GameplayStatics.GetGameInstance`)))
  (`/Game/Blueprint/BP_NewGameInstance.Save` _asbp_new_game_instance)
  (`self.onTeleport`)
  (`GameplayStatics.OpenLevelBySoftObjectPtr` "/Game/Levels/L_Bossfight.L_Bossfight"))

(fn `GetLeverStatus`
  (params (LerpValue :type "Float (double-precision)"))
  (returns (LeverStatus :type "Float (double-precision)"))
  (return 0.0))

(fn `UserConstructionScript`)