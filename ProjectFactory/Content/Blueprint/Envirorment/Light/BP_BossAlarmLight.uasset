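; Rotating alarm light for the boss encounter, with two purple spotlights that switch on at BeginPlay.
; BeginPlay randomizes the spin speed, direction and starting yaw, so placed instances rotate out of sync.
; It also binds to the boss game mode's lights-off dispatcher.
; The TurnOff event zeroes both spotlights' intensity and deactivates the rotating movement.
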(event `self.ReceiveBeginPlay`
  (set `RotatingMovementComponent.RotationRate` (`KismetMathLibrary.MakeRotator` 0.0 0.0 (* (`KismetMathLibrary.RandomFloatInRange` 250.0 290.0) (`KismetMathLibrary.SelectFloat` 1.0 -1.0 (`KismetMathLibrary.RandomBool`)))) (`self.RotatingMovement`))
  (`SceneComponent.K2_SetRelativeRotation` (`self.Cylinder1`) (`KismetMathLibrary.MakeRotator` 0.0 0.0 (`KismetMathLibrary.RandomFloatInRange` 0.0 360.0)) false false)
  (`self.SetActorTickEnabled` true)
  (set `self.On` true)
  (`LightComponent.SetIntensity` (`self.SpotLight1`) 5000.0)
  (`LightComponent.SetIntensity` (`self.SpotLight`) 5000.0)
  (`LightComponent.SetLightColor` (`self.SpotLight`) (struct :`R` 0.34902 :`B` 0.341176 :`A` 1.0) true)
  (`LightComponent.SetLightColor` (`self.SpotLight1`) (struct :`R` 0.34902 :`B` 0.341176 :`A` 1.0) true)
  (bind _asbp_boss_gamemode (cast `/Game/GameMode/BP_BossGamemode` (`GameplayStatics.GetGameMode`)))
  (add `/Game/GameMode/BP_BossGamemode.onTurnOffLighs` _asbp_boss_gamemode (`|CreateDelegate` :!event `TurnOff`)))

(event `TurnOff`
  (set `self.On` false)
  (`LightComponent.SetIntensity` (`self.SpotLight1`) 0.0)
  (`LightComponent.SetIntensity` (`self.SpotLight`) 0.0)
  (`ActorComponent.Deactivate` (`self.RotatingMovement`)))

(fn `UserConstructionScript`)