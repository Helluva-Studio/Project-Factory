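; BP_AlarmLight is a rotating alarm light prop that switches on and off with the game mode's frenzy environment event.
; BeginPlay randomizes spin speed, direction and starting cylinder yaw, then binds SetAlarmLight to BP_NewGameMode's OnFrenzyEnvironment.
; Each event call flip-flops rotation and both spotlights.
; While on, Tick pulses intensity and bulb brightness with a time-based sine, lazily creating the bulb's dynamic material once.
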(event `self.ReceiveBeginPlay`
  (set `RotatingMovementComponent.RotationRate` (`KismetMathLibrary.MakeRotator` 0.0 0.0 (* (`KismetMathLibrary.RandomFloatInRange` 250.0 290.0) (`KismetMathLibrary.SelectFloat` 1.0 -1.0 (`KismetMathLibrary.RandomBool`)))) (`self.RotatingMovement`))
  (`SceneComponent.K2_SetRelativeRotation` (`self.Cylinder1`) (`KismetMathLibrary.MakeRotator` 0.0 0.0 (`KismetMathLibrary.RandomFloatInRange` 0.0 360.0)) false false)
  (`self.SetActorTickEnabled` true)
  (bind _asbp_new_game_mode (cast `/Game/GameMode/BP_NewGameMode` (`GameplayStatics.GetGameMode`)))
  (add `/Game/GameMode/BP_NewGameMode.OnFrenzyEnvironment` _asbp_new_game_mode (delegate `SetAlarmLight`)))

(event `SetAlarmLight`
  (bind _bulbmaterial (`self.BulbMaterial`))
  (bind _isa (`/Engine/EditorBlueprintResources/StandardMacros.FlipFlop`)
    (:`A`
      (set `self.On` _isa)
      (`ActorComponent.Activate` (`self.RotatingMovement`) false)
      (`LightComponent.SetIntensity` (`self.SpotLight`) 5000.0)
      (`LightComponent.SetIntensity` (`self.SpotLight1`) 5000.0))
    (:`B`
      (set `self.On` _isa)
      (`ActorComponent.Deactivate` (`self.RotatingMovement`))
      (`LightComponent.SetIntensity` (`self.SpotLight`) 0.0)
      (`LightComponent.SetIntensity` (`self.SpotLight1`) 0.0)
      (`/Engine/EditorBlueprintResources/StandardMacros.IsValid` _bulbmaterial
        (:`Is Valid`
          (`MaterialInstanceDynamic.SetScalarParameterValue` _bulbmaterial "Brightness" 0.0))))))

(event `self.ReceiveTick`
  (params (DeltaSeconds :type "Float (single-precision)"))
  (bind _returnvalue (/ (+ (`KismetMathLibrary.DegSin` (* (`GameplayStatics.GetTimeSeconds`) 300.0)) 1.0) 2.0))
  (if (`self.On`)
    (`LightComponent.SetIntensity` (`self.SpotLight`) (* (+ _returnvalue 0.05) 5000.0))
    (`LightComponent.SetIntensity` (`self.SpotLight1`) (* (+ _returnvalue 0.05) 5000.0))
    (`/Engine/EditorBlueprintResources/StandardMacros.IsValid` (`self.BulbMaterial`)
      (:`Is Valid`
        (`MaterialInstanceDynamic.SetScalarParameterValue` (`self.BulbMaterial`) "Brightness" (`KismetMathLibrary.FClamp` (* _returnvalue 5.0) 0.0 5.0)))
      (:`Is Not Valid`
        (`self.Set Material`)))))

(event `Set Material`
  (`/Engine/EditorBlueprintResources/StandardMacros.DoOnce` false :!label _label
    (:`Completed`
      (`/Engine/EditorBlueprintResources/StandardMacros.IsValid` (`self.Bulbnew2`)
        (:`Is Valid`
          (bind _returnvalue (`PrimitiveComponent.CreateDynamicMaterialInstance` (`self.Bulbnew2`) 0 null "None"))
          (bind _output_get (set `self.BulbMaterial` _returnvalue))
          (`PrimitiveComponent.SetMaterial` (`self.Bulbnew1`) 0 _output_get)
          (`PrimitiveComponent.SetMaterial` (`self.Bulbnew1`) 0 _output_get))
        (:`Is Not Valid`
          (goto _label :!via `Reset`))))))

(fn `UserConstructionScript`)