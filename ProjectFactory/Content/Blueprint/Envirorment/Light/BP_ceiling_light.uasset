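; Ceiling light actor with a spotlight and mesh that can flicker and reacts to the game mode's Frenzy environment event.
; If flickering is enabled, a self-restarting loop waits randomly, then toggles spotlight intensity and a dynamic material's Brightness in short random bursts.
; TurnRed, bound to that event, alternates between reverse-playing the Frenzy timeline to drive clamped intensity and setting fixed intensity; it changes no color.
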(event `self.ReceiveBeginPlay`
  (`LocalLightComponent.SetAttenuationRadius` (`self.SpotLight`) (`self.AttenuationRadius`))
  (`LightComponent.SetIntensity` (`self.SpotLight`) (`self.MaxIntensity`))
  (`|ExecutionSequence`
    (:`then_0`
      (if (`self.CanFlickering`)
        (bind _returnvalue (`PrimitiveComponent.CreateDynamicMaterialInstance` (`self.LightMesh`) 1 null "None"))
        (`PrimitiveComponent.SetMaterial` (`self.LightMesh`) 1 _returnvalue)
        (`self.FlickeringEffect`)))
    (:`then_1`
      (bind _asbp_new_game_mode (cast `/Game/GameMode/BP_NewGameMode` (`GameplayStatics.GetGameMode`)))
      (add `/Game/GameMode/BP_NewGameMode.OnFrenzyEnvironment` _asbp_new_game_mode (delegate `TurnRed`)))))

(event `TurnRed`
  (`/Engine/EditorBlueprintResources/StandardMacros.FlipFlop`
    (:`A`
      (bind (_direction _lights) (`Timeline|Frenzy` :!via `Reverse`)
        (:`Update`
          (`LightComponent.SetIntensity` (`self.SpotLight`) (`KismetMathLibrary.FClamp` _lights 1500.0 5000.0)))))
    (:`B`
      (`LightComponent.SetIntensity` (`self.SpotLight`) 5000.0))))

(event `FlickeringEffect`
  (bind _spotlight (`self.SpotLight`))
  (`KismetSystemLibrary.Delay` (`KismetMathLibrary.RandomFloatInRange` (`self.MinFlickeringDelay`) (`self.MaxFlickeringDelay`)))
  (`/Game/Blueprint/BP_MacroLibrary_Actor.ForLoopWithDelay` 0 (`KismetMathLibrary.RandomIntegerInRange` 0 5) (`KismetMathLibrary.RandomFloatInRange` (`self.MinFlickeringTime`) (`self.MaxFlickeringTime`))
    (:`Loop Body`
      (`/Engine/EditorBlueprintResources/StandardMacros.IsValid` self
        (:`Is Valid`
          (`/Engine/EditorBlueprintResources/StandardMacros.FlipFlop`
            (:`A`
              (`LightComponent.SetIntensity` _spotlight (`self.MinIntensity`))
              (bind _asmaterial_instance_dynamic (cast `MaterialInstanceDynamic` (`PrimitiveComponent.GetMaterial` (`self.LightMesh`) 1)))
              (`MaterialInstanceDynamic.SetScalarParameterValue` _asmaterial_instance_dynamic "Brightness" 0.0))
            (:`B`
              (`LightComponent.SetIntensity` _spotlight (`self.MaxIntensity`))
              (bind _asmaterial_instance_dynamic_2 (cast `MaterialInstanceDynamic` (`PrimitiveComponent.GetMaterial` (`self.LightMesh`) 1)))
              (`MaterialInstanceDynamic.SetScalarParameterValue` _asmaterial_instance_dynamic_2 "Brightness" 1.0))))))
    (:`Completed`
      (`LightComponent.SetIntensity` (`self.SpotLight`) (`self.MaxIntensity`))
      (bind _asmaterial_instance_dynamic_3 (cast `MaterialInstanceDynamic` (`PrimitiveComponent.GetMaterial` (`self.LightMesh`) 1)))
      (`MaterialInstanceDynamic.SetScalarParameterValue` _asmaterial_instance_dynamic_3 "Brightness" 1.0)
      (`self.FlickeringEffect`))))

(fn `UserConstructionScript`)