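; One-shot interactable lever that signals BP_BossTeleport with its Index and quick-starts the game mode's Frenzy if not already active.
; Pulling plays a sound and a timeline that rotates the handle, dims its dynamic-material glow and switches the minimap icon, a scene-capture-only mesh, to off.
; Focus highlights it through custom depth until pulled.
; ReactivateLever replays the pulled state with sound, without triggering teleport or Frenzy.
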(event `self.ReceiveBeginPlay`
  (bind _minimapicon (`self.MinimapIcon`))
  (bind _leverhandle (`self.LeverHandle`))
  (bind _returnvalue (`PrimitiveComponent.CreateDynamicMaterialInstance` _leverhandle 1 null "None"))
  (`PrimitiveComponent.SetMaterial` _leverhandle 1 _returnvalue)
  (`/Engine/EditorBlueprintResources/StandardMacros.IsValid` _minimapicon
    (:`Is Valid`
      (`SceneComponent.K2_SetWorldRotation` _minimapicon (`KismetMathLibrary.MakeRotator` 0.0 0.0 90.0) false false))
    (:`Is Not Valid`
      (bind _returnvalue_2 (`AddComponent|NODE_AddStaticMeshComponent-0` :`RelativeTransform` (`KismetMathLibrary.MakeTransform` (450.0 0.0 150.0) (struct) (5.0 5.0 5.0))))
      (`SceneComponent.K2_SetWorldRotation` _returnvalue_2 (struct :`Yaw` 90.0) false false)
      (`StaticMeshComponent.SetStaticMesh` _returnvalue_2 "/Engine/BasicShapes/Plane.Plane")
      (`PrimitiveComponent.SetMaterial` _returnvalue_2 0 "/Game/Blueprint/Minimap/MI_LeverOn.MI_LeverOn")
      (set `self.MinimapIcon` _returnvalue_2)
      (`PrimitiveComponent.SetVisibleInSceneCaptureOnly` (`self.MinimapIcon`) true))))

(event `/Game/Blueprint/InteractionArea/BPI_Focusable.ToggleFocus`
  (params (Focus :type Boolean))
  (bind _returnvalue (and Focus (not (`self.LeverPulled`))))
  (`PrimitiveComponent.SetRenderCustomDepth` (`self.Lever`) _returnvalue)
  (`PrimitiveComponent.SetRenderCustomDepth` (`self.LeverHandle`) _returnvalue))

(event `/Game/Blueprint/Turrets/Interfaces/BI_Interactable.Interact`
  (bind _newgamemode (`/Game/Blueprint/BP_MacroLibrary_Actor.GetNewGameMode`))
  (if (not (`self.LeverPulled`))
    (`self.PullLever`)
    (bind _returnvalue (`GameplayStatics.GetActorOfClass` "/Game/Blueprint/Envirorment/Teleport/BP_BossTeleport.BP_BossTeleport_C"))
    (`/Game/Blueprint/Envirorment/Teleport/BP_BossTeleport.Interact` _returnvalue (`self.Index`))
    (`GameplayStatics.PlaySoundAtLocation` "/Game/Audio/SFX/Environment/SC_Lever.SC_Lever" (`self.K2_GetActorLocation`) (struct) 1.0 1.0 0.0 null null null null)
    (if (not (`/Game/GameMode/BP_NewGameMode.Frenzy` _newgamemode))
      (`/Game/GameMode/BP_NewGameMode.QuickStartFrenzy` _newgamemode))))

(event `PullLever`
  (set `self.LeverPulled` true)
  (bind (_direction _newtrack_0) (`Timeline|LeverMovement`)
    (:`Update`
      (`SceneComponent.K2_SetRelativeRotation` (`self.LeverHandle`) (`KismetMathLibrary.MakeRotator` 0.0 (* _newtrack_0 120.0)) false false)
      (`MaterialInstanceDynamic.SetScalarParameterValue` (cast `MaterialInstanceDynamic` (`PrimitiveComponent.GetMaterial` (`self.LeverHandle`) 1) :!pure true) "Brigthness" (* (- 1.0 _newtrack_0) 3.0))
      (`PrimitiveComponent.SetMaterial` (`self.MinimapIcon`) 0 "/Game/Blueprint/Minimap/MI_LeverOff.MI_LeverOff"))))

(event `ReactivateLever`
  (set `self.LeverPulled` true)
  (`GameplayStatics.PlaySoundAtLocation` "/Game/Audio/SFX/Environment/SC_Lever.SC_Lever" (`self.K2_GetActorLocation`) (struct) 1.0 1.0 0.0 null null null null)
  (bind (_direction _newtrack_0) (`Timeline|Timeline`)
    (:`Update`
      (`SceneComponent.K2_SetRelativeRotation` (`self.LeverHandle`) (`KismetMathLibrary.MakeRotator` 0.0 (* _newtrack_0 120.0)) false false)
      (`MaterialInstanceDynamic.SetScalarParameterValue` (cast `MaterialInstanceDynamic` (`PrimitiveComponent.GetMaterial` (`self.LeverHandle`) 1) :!pure true) "Brigthness" (* (- 1.0 _newtrack_0) 3.0))
      (`PrimitiveComponent.SetMaterial` (`self.MinimapIcon`) 0 "/Game/Blueprint/Minimap/MI_LeverOff.MI_LeverOff"))))

(fn `CanInteract`
  (returns (CanInteract :type Boolean))
  (return (not (`self.LeverPulled`))))

(fn `GetCost`
  (returns (GetCost :type "Float (double-precision)"))
  (return 0.0))

(fn `GetInteractImage`
  (returns (Image :type "Texture Object Reference"))
  (return "/Game/2DImage/Levers/Lever_INTERACTION.Lever_INTERACTION"))

(fn `GetInteractMessage`
  (returns (InteractMessage :type Text) (Image :type "Texture Object Reference"))
  (return "" null))

(fn `UserConstructionScript`
  (set `self.Location` (`self.K2_GetActorLocation`)))

(fn `WhichInteraction`
  (returns (TypeInteraction :type "/Game/Blueprint/Enum/EInteractable Enum"))
  (return "NewEnumerator0"))