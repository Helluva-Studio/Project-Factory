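; Boss teleporter that unlocks once the lever count set by the game mode is pulled, then sends the player to L_Boss_Cinematic.
; Each lever interaction updates the HUD and game instance and lights a compass segment through a dynamic material.
; Activation plays a HUD cinematic, scales up the portal with chained timelines, then enables collision.
; Player overlap runs a cancellable timer with effects, then saves and loads the level behind a loading screen.
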(event `self.ReceiveBeginPlay`
  (bind (_newgamemode _success) (`/Game/Blueprint/BP_MacroLibrary_Actor.GetNewGameMode`))
  (if _success
    (set `self.LeversToPull` (`/Game/GameMode/BP_NewGameMode.LeversToPullToActivateTeleport` _newgamemode))
    (`self.K2_SetActorRotation` (`KismetMathLibrary.MakeRotator` 0.0))))

(event `Interact`
  (params (Index :type Integer))
  (`/Engine/EditorBlueprintResources/StandardMacros.IsValid` (`self.PlayerHUD`)
    (:`Is Valid`
      _)
    (:`Is Not Valid`
      (bind _foundwidgets (`WidgetBlueprintLibrary.GetAllWidgetsOfClass` "/Game/HUD/PlayerHUD/WB_PlayerHUD.WB_PlayerHUD_C"))
      (set `self.PlayerHUD` (`|GetArrayItem` _foundwidgets))))
  (`self.UpdateTeleport` Index)
  (`GameplayStatics.PlaySoundAtLocation` "/Game/Audio/SFX/Environment/Teleport/SC_TeleportSingle.SC_TeleportSingle" (`self.K2_GetActorLocation`) (struct) 1.0 1.0 0.0 null null null null)
  (`/Game/HUD/PlayerHUD/WB_PlayerHUD.TurretUnlockedEvent` (`self.PlayerHUD`) "LEVER PULLED"))

(event `self.ReceiveTick`
  (params (DeltaSeconds :type "Float (single-precision)"))
  (if (`self.Active`)
    (`SceneComponent.K2_AddRelativeRotation` (`self.MinimapIcon`) (struct :`Yaw` 1.0) false false)))

(event `ActivateTeleport`
  (bind _tp (`self.TP`))
  (bind (_returnvalue_x _returnvalue_y _returnvalue_z) (`KismetMathLibrary.BreakVector` (`SceneComponent.K2_GetComponentScale` (`self.Ring`))))
  (bind (_returnvalue_x_2 _returnvalue_y_2 _returnvalue_z_2) (`KismetMathLibrary.BreakVector` (`SceneComponent.K2_GetComponentScale` (`self.TP`))))
  (bind (_returnvalue_x_3 _returnvalue_y_3) (`KismetMathLibrary.BreakVector` (`SceneComponent.K2_GetComponentScale` _tp)))
  (set `self.Active` true)
  (`SceneComponent.SetHiddenInGame` (`self.TP`) false false)
  (`SceneComponent.SetHiddenInGame` (`self.MinimapIcon`) false false)
  (`PrimitiveComponent.SetHiddenInSceneCapture` (`self.Teleport`) true)
  (`/Engine/EditorBlueprintResources/StandardMacros.DoOnce` false
    (:`Completed`
      (bind _foundwidgets (`WidgetBlueprintLibrary.GetAllWidgetsOfClass` "/Game/HUD/PlayerHUD/WB_PlayerHUD.WB_PlayerHUD_C"))
      (`/Game/HUD/PlayerHUD/WB_PlayerHUD.PlayCinematic` (`|GetArrayItem` _foundwidgets))
      (bind (_direction _newtrack_0) (`Timeline|ScaleHeight`)
        (:`Update`
          (`SceneComponent.SetWorldScale3D` _tp (`KismetMathLibrary.MakeVector` _returnvalue_x_3 _returnvalue_y_3 (* _newtrack_0 2.0))))
        (:`Finished`
          (`SceneComponent.SetHiddenInGame` (`self.Ring`) false false)
          (bind (_direction_2 _newtrack_0_2) (`Timeline|ScaleSize`)
            (:`Update`
              (bind _returnvalue (`KismetMathLibrary.Lerp` _returnvalue_x_2 1.925 _newtrack_0_2))
              (`SceneComponent.SetWorldScale3D` (`self.TP`) (`KismetMathLibrary.MakeVector` _returnvalue _returnvalue _returnvalue_z_2))
              (bind _returnvalue_2 (`KismetMathLibrary.Lerp` _returnvalue_x 0.32 _newtrack_0_2))
              (`SceneComponent.SetWorldScale3D` (`self.Ring`) (`KismetMathLibrary.MakeVector` _returnvalue_2 _returnvalue_2 _returnvalue_z)))
            (:`Finished`
              (`PrimitiveComponent.SetCollisionEnabled` (`self.Collision`) "QueryOnly"))))))))

(event `self.Collision.OnComponentEndOverlap`
  (params (OverlappedComponent :type "PrimitiveComponent Object Reference") (OtherActor :type "Actor Object Reference") (OtherComp :type "PrimitiveComponent Object Reference") (OtherBodyIndex :type Integer))
  (if (== OtherActor (`GameplayStatics.GetPlayerPawn` 0))
    (`KismetSystemLibrary.K2_ClearAndInvalidateTimerHandle` (`self.TeleportTimer`))
    (`ActorComponent.SetActive` (`self.Niagara`) false false)
    (`AudioComponent.FadeOut` (`self.Audio`) 0.3 0.0 "Linear")))

(event `self.Collision.OnComponentBeginOverlap`
  (params (OverlappedComponent :type "PrimitiveComponent Object Reference") (OtherActor :type "Actor Object Reference") (OtherComp :type "PrimitiveComponent Object Reference") (OtherBodyIndex :type Integer) (bFromSweep :type Boolean) (SweepResult :type "HitResult Structure (by ref)"))
  (if (== OtherActor (`GameplayStatics.GetPlayerPawn` 0))
    (bind _returnvalue (`KismetSystemLibrary.K2_SetTimerDelegate` (delegate `TeleportPlayer`) (`self.TimeToTeleport`)))
    (set `self.TeleportTimer` _returnvalue)
    (`ActorComponent.SetActive` (`self.Niagara`) true false)
    (`AudioComponent.FadeIn` (`self.Audio`) 1.0 1.0 0.0 "Linear")))

(event `TeleportPlayer`
  (bind _returnvalue (`|CreateWidget` "/Game/HUD/WB_LoadingScreen.WB_LoadingScreen_C"))
  (`UserWidget.AddToViewport` _returnvalue 0)
  (bind _returnvalue_2 (`/Game/HUD/WB_LoadingScreen.FadeInAnim` _returnvalue))
  (bind _asbp_new_game_instance (cast `/Game/Blueprint/BP_NewGameInstance` (`GameplayStatics.GetGameInstance`)))
  (`/Game/Blueprint/BP_NewGameInstance.Save` _asbp_new_game_instance)
  (`KismetSystemLibrary.Delay` _returnvalue_2)
  (`self.onTeleport`)
  (`GameplayStatics.OpenLevelBySoftObjectPtr` "/Game/Levels/Ro_Levels/L_Boss_Cinematic.L_Boss_Cinematic"))

(event `Cheat`
  (bind _outactors (`GameplayStatics.GetAllActorsOfClass` "/Game/Blueprint/Envirorment/BP_Lever.BP_Lever_C"))
  (for (_array_element _array_index) _outactors
    (`/Engine/EditorBlueprintResources/StandardMacros.IsValid` _array_element
      (:`Is Valid`
        (`self.K2_SetActorLocation` _array_element (`KismetMathLibrary.MakeVector` 150.0 (`KismetMathLibrary.Conv_IntToDouble` (* _array_index 150)) 200.0) false false)
        (bind _leverindex (`/Game/Blueprint/Envirorment/BP_Lever.LeverIndex` _array_element))
        (`TextRenderComponent.K2_SetText` _leverindex (`KismetTextLibrary.Conv_IntToText` (`/Game/Blueprint/Envirorment/BP_Lever.Index` _array_element)))
        (`SceneComponent.SetHiddenInGame` _leverindex false false))))
  (bind _outactors_2 (`GameplayStatics.GetAllActorsOfClass` "/Game/Blueprint/Envirorment/BP_SavePC.BP_SavePC_C"))
  (for (_array_element_2 _array_index_2) _outactors_2
    (`self.K2_SetActorLocation` _array_element_2 (`KismetMathLibrary.MakeVector` 0.0 (`KismetMathLibrary.Conv_IntToDouble` (* _array_index_2 -150))) false false)))

(fn `GetLeverStatus`
  (params (LerpValue :type "Float (double-precision)"))
  (returns (LeverStatus :type "Float (double-precision)"))
  (return 0.0))

(fn `UpdateTeleport`
  (params (InputPin :type Integer))
  (`/Engine/EditorBlueprintResources/StandardMacros.IncrementInt` (`self.LeverPulled`)
    (:`  `
      (bind _asbp_new_game_instance (cast `/Game/Blueprint/BP_NewGameInstance` (`GameplayStatics.GetGameInstance`)))
      (set `/Game/Blueprint/BP_NewGameInstance.LeversPulled` (`self.LeverPulled`) _asbp_new_game_instance)
      (bind _foundwidgets (`WidgetBlueprintLibrary.GetAllWidgetsOfClass` "/Game/HUD/PlayerHUD/WB_PlayerHUD.WB_PlayerHUD_C"))
      (`/Game/HUD/PlayerHUD/WB_PlayerHUD.UpdateLeversImage` (`|GetArrayItem` _foundwidgets) (`self.LeverPulled`))
      (`self.UpdateTeleportZone` InputPin))))

(fn `UpdateTeleportZone`
  (params (Selection :type Integer))
  (switch `int` Selection
    (:`0`
      (`MaterialInstanceDynamic.SetScalarParameterValue` (`self.Material`) "Nord" 1.0))
    (:`1`
      (`MaterialInstanceDynamic.SetScalarParameterValue` (`self.Material`) "Sud" 1.0))
    (:`2`
      (`MaterialInstanceDynamic.SetScalarParameterValue` (`self.Material`) "Est" 1.0))
    (:`3`
      (`MaterialInstanceDynamic.SetScalarParameterValue` (`self.Material`) "Ovest" 1.0)))
  (if (>= (`self.LeverPulled`) (`self.LeversToPull`))
    (`self.ActivateTeleport`)))

(fn `UserConstructionScript`
  (bind _teleport (`self.Teleport`))
  (bind _returnvalue (`PrimitiveComponent.CreateDynamicMaterialInstance` _teleport 3 null "None"))
  (bind _output_get (set `self.Material` _returnvalue))
  (`PrimitiveComponent.SetMaterial` _teleport 3 _output_get))