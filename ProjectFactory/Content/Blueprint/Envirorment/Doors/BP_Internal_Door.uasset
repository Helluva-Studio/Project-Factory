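; BP_Internal_Door is a sliding double door for interiors that opens when something overlaps its trigger volume.
; A timeline plays on overlap and offsets the left and right panels in opposite directions along X, scaled by the opening amount from a start position.
; When the overlap ends, the timeline reverses to close the door unless the StayOpened flag is set.
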(event `self.OpeningTrigger.OnComponentBeginOverlap`
  (params (OverlappedComponent :type "PrimitiveComponent Object Reference") (OtherActor :type "Actor Object Reference") (OtherComp :type "PrimitiveComponent Object Reference") (OtherBodyIndex :type Integer) (bFromSweep :type Boolean) (SweepResult :type "HitResult Structure (by ref)"))
  (bind _doorstartposition (`self.DoorStartPosition`))
  (bind (_direction _dooraperturenormalize) (`Timeline|Timeline` :`NewTime` 0.75 :!label _label)
    (:`Update`
      (bind _returnvalue (* _dooraperturenormalize (`self.DoorOpeningAmount`)))
      (`SceneComponent.K2_SetRelativeLocation` (`self.DoorRight`) (`KismetMathLibrary.MakeVector` (+ _doorstartposition _returnvalue) -5.25) false false)
      (`SceneComponent.K2_SetRelativeLocation` (`self.DoorLeft`) (`KismetMathLibrary.MakeVector` (- (* _doorstartposition -1.0) _returnvalue) -5.25) false false))))

(event `self.OpeningTrigger.OnComponentEndOverlap`
  (params (OverlappedComponent :type "PrimitiveComponent Object Reference") (OtherActor :type "Actor Object Reference") (OtherComp :type "PrimitiveComponent Object Reference") (OtherBodyIndex :type Integer))
  (if (not (`self.StayOpened`))
    (goto _label :!via `Reverse`)))

(fn `UserConstructionScript`)