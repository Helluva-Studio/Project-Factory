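; Purchasable sliding double door between BP_WFC_BaseRoom rooms, exposing a cost, prompt and icon for interaction and a custom-depth highlight on focus until bought.
; On purchase, it marks overlapping unvisited rooms as visited, registers them with BP_NewGameMode, then plays a sound and a timeline that slides both panels apart for good.
; Payment is not handled here, and the overlap-based trigger and closing logic is disconnected.
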(event `self.OpeningTrigger.OnComponentBeginOverlap`
  (params (OverlappedComponent :type "PrimitiveComponent Object Reference") (OtherActor :type "Actor Object Reference") (OtherComp :type "PrimitiveComponent Object Reference") (OtherBodyIndex :type Integer) (bFromSweep :type Boolean) (SweepResult :type "HitResult Structure (by ref)")))

(event `/Game/Blueprint/Turrets/Interfaces/BI_Interactable.InteractPurchase`
  (bind _doorstartposition (`self.DoorStartPosition`))
  (if (not (`self.Purchased`))
    (set `self.StayOpened` true)
    (bind _asbp_new_game_mode (cast `/Game/GameMode/BP_NewGameMode` (`GameplayStatics.GetGameMode`)))
    (for _array_element (`self.GetOverlappingActors` "/Game/Blueprint/Envirorment/Rooms/BP_WFC_BaseRoom.BP_WFC_BaseRoom_C")
      (bind _asbp_wfc_base_room (cast `/Game/Blueprint/Envirorment/Rooms/BP_WFC_BaseRoom` _array_element))
      (if (not (`/Game/Blueprint/Envirorment/Rooms/BP_WFC_BaseRoom.Is Visited` _asbp_wfc_base_room))
        (set `/Game/Blueprint/Envirorment/Rooms/BP_WFC_BaseRoom.Is Visited` true _asbp_wfc_base_room)
        (`/Game/GameMode/BP_NewGameMode.AddRoom` _asbp_new_game_mode _asbp_wfc_base_room)
        (set `self.GoingToRoom` _asbp_wfc_base_room)
        (set `self.Purchased` true)
        (`GameplayStatics.PlaySoundAtLocation` "/Game/Audio/SFX/Environment/SC_DoorOpening_Cue.SC_DoorOpening_Cue" (`self.K2_GetActorLocation`) (struct) 1.0 1.0 0.0 null null null null)
        (bind (_direction _dooraperturenormalize) (`Timeline|Timeline_0` :`NewTime` 0.75 :!via `PlayFromStart`)
          (:`Update`
            (bind _returnvalue (* _dooraperturenormalize (`self.DoorOpeningAmount`)))
            (`SceneComponent.K2_SetRelativeLocation` (`self.DoorRight`) (`KismetMathLibrary.MakeVector` (+ _doorstartposition _returnvalue) -5.25) false false)
            (`SceneComponent.K2_SetRelativeLocation` (`self.DoorLeft`) (`KismetMathLibrary.MakeVector` (- (* _doorstartposition -1.0) _returnvalue) -5.25) false false)
            (`PrimitiveComponent.SetRenderCustomDepth` (`self.DoorRight`) false)
            (`PrimitiveComponent.SetRenderCustomDepth` (`self.DoorLeft`) false)))
        (else
          (set `self.ComingFromRoom` _asbp_wfc_base_room))))))

(event `self.Focus`
  (params (IsFocused :type Boolean)))

(event `/Game/Blueprint/InteractionArea/BPI_Focusable.ToggleFocus`
  (params (Focus :type Boolean))
  (if (not (`self.Purchased`))
    (`PrimitiveComponent.SetRenderCustomDepth` (`self.DoorLeft`) Focus)
    (`PrimitiveComponent.SetRenderCustomDepth` (`self.DoorRight`) Focus)))

(fn `CanInteract`
  (returns (CanInteract :type Boolean))
  (return (not (`self.Purchased`))))

(fn `GetCost`
  (returns (GetCost :type "Float (double-precision)"))
  (return (`self.DoorCost`)))

(fn `GetInteractImage`
  (returns (Image :type "Texture Object Reference"))
  (return "/Game/2DImage/porta.porta"))

(fn `GetInteractMessage`
  (returns (InteractMessage :type Text) (Image :type "Texture Object Reference"))
  (return (`KismetTextLibrary.Conv_StringToText` (`KismetTextLibrary.Conv_TextToString` (`KismetTextLibrary.Conv_DoubleToText` (`/Game/GameMode/BP_NewGameMode.DoorCost` (`/Game/Blueprint/BP_MacroLibrary_Actor.GetNewGameMode`)) "HalfToEven" false false 3))) "/Game/2DImage/essenza.essenza"))

(fn `UserConstructionScript`)

(fn `WhichInteraction`
  (returns (TypeInteraction :type "/Game/Blueprint/Enum/EInteractable Enum"))
  (return "NewEnumerator1"))