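; Boss fight door that cannot be interacted with and instead starts a scripted sequence ending in the victory screen when the player collides with it.
; Collision shows a boss animation widget, disables pawn input and auto-walks the player to a hardcoded X/Y position.
; Completion callbacks chain the widgets: the animation's end pauses the game and opens a UI-focused lore dialogue, whose end adds the victory screen.
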(event `self.ReceiveBeginPlay`)

(event `/Game/Blueprint/InteractionArea/BPI_Focusable.ToggleFocus`
  (params (Focus :type Boolean)))

(event `self.CollisionWithPlayer`
  (bind _returnvalue (`GameplayStatics.GetPlayerController` 0))
  (bind (_returnvalue_x _returnvalue_y _returnvalue_z) (`KismetMathLibrary.BreakVector` (`self.K2_GetActorLocation` (`GameplayStatics.GetPlayerPawn` 0))))
  (bind _returnvalue_2 (`|CreateWidget` "/Game/HUD/EndBossfight/WB_BossAnimation.WB_BossAnimation_C"))
  (add `/Game/HUD/EndBossfight/WB_BossAnimation.onEffectCompleted` _returnvalue_2 (delegate `EffectComplete`))
  (`UserWidget.AddToViewport` _returnvalue_2 0)
  (`self.DisableInput` (`GameplayStatics.GetPlayerPawn` 0) _returnvalue)
  (`AIBlueprintHelperLibrary.SimpleMoveToLocation` _returnvalue (`KismetMathLibrary.MakeVector` 6750.0 0.0 _returnvalue_z)))

(event `EffectComplete`
  (`GameplayStatics.SetGamePaused` true)
  (bind _returnvalue (`|CreateWidget` "/Game/HUD/Tutorial/WB_LoreTutorial.WB_LoreTutorial_C" null "NewEnumerator1" null))
  (add `/Game/HUD/Tutorial/WB_LoreTutorial.onCutsceneFinished` _returnvalue (delegate `CutsceneFinished`))
  (`UserWidget.AddToViewport` _returnvalue 0)
  (`WidgetBlueprintLibrary.SetInputMode_UIOnlyEx` (`GameplayStatics.GetPlayerController` 0) _returnvalue)
  (`Widget.SetFocus` _returnvalue)
  (`Widget.SetKeyboardFocus` _returnvalue))

(event `CutsceneFinished`
  (bind _returnvalue (`|CreateWidget` "/Game/HUD/WB_VictoryScreen.WB_VictoryScreen_C"))
  (`UserWidget.AddToViewport` _returnvalue 0))

(fn `CanInteract`
  (returns (CanInteract :type Boolean))
  (return false))

(fn `UserConstructionScript`
  (`parent.UserConstructionScript`))