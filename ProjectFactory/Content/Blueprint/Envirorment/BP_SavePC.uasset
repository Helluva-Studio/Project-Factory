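; BP_SavePC is an interactable computer that serves as a free, always available save point with a "Save Game" prompt.
; On interaction it creates a BP_SaveData object, initializes it from the player pawn, game mode and game instance, then writes it to a fixed slot.
; Focus toggles custom depth rendering on its mesh.
; Unconnected leftover nodes would animate a material's brightness through a PoweringUp timeline, but never run.
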(event `self.ReceiveBeginPlay`)

(event `/Game/Blueprint/Turrets/Interfaces/BI_Interactable.Interact`
  (bind _returnvalue (`GameplayStatics.CreateSaveGameObject` "/Game/Blueprint/Save/BP_SaveData.BP_SaveData_C"))
  (`/Game/Blueprint/Save/BP_SaveData.Initialize` _returnvalue (`GameplayStatics.GetPlayerPawn` 0) (`GameplayStatics.GetGameMode`) (`GameplayStatics.GetGameInstance`))
  (`GameplayStatics.SaveGameToSlot` _returnvalue "Saveslot"))

(event `/Game/Blueprint/InteractionArea/BPI_Focusable.ToggleFocus`
  (params (Focus :type Boolean))
  (`PrimitiveComponent.SetRenderCustomDepth` (`self.StaticMesh`) Focus))

(fn `CanInteract`
  (returns (CanInteract :type Boolean))
  (return true))

(fn `GetCost`
  (returns (GetCost :type "Float (double-precision)"))
  (return 0.0))

(fn `GetInteractImage`
  (returns (Image :type "Texture Object Reference"))
  (return null))

(fn `GetInteractMessage`
  (returns (InteractMessage :type Text) (Image :type "Texture Object Reference"))
  (return "Save Game" null))

(fn `UserConstructionScript`)

(fn `WhichInteraction`
  (returns (TypeInteraction :type "/Game/Blueprint/Enum/EInteractable Enum"))
  (return "NewEnumerator0"))