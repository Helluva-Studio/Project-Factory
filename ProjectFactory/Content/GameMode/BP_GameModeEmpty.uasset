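; Game mode that runs game startup, the day clock and enemy waves across active rooms.
; Initialization randomly assigns turret types to placed blueprints via seeded stream, spawns Roberto, swaps loading screen for HUD and builds a weighted enemy pool.
; Rooms' spawn points queue pooled enemies, with delayed respawns batching kills.
; A looping timer rolls accumulating probability to trigger frenzy: lights, delayed siren, dispatcher, then cooldown.
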(event `Initialize`
  (bind _returnvalue (`GameplayStatics.GetPlayerController` 0))
  (`self.InitializeTurretBlueprint`)
  (`|SpawnActorFromClass` "/Game/Blueprint/Robot/Blueprints/BP_Roberto.BP_Roberto_C" (`KismetMathLibrary.MakeTransform` (0.0 0.0 100.0)) "AlwaysSpawn" "MultiplyWithRoot" null null)
  (`KismetSystemLibrary.Delay` 1.0)
  (bind _foundwidgets (`WidgetBlueprintLibrary.GetAllWidgetsOfClass` "/Game/HUD/WB_LoadingScreen.WB_LoadingScreen_C"))
  (for _array_element _foundwidgets
    (`Widget.RemoveFromParent` _array_element)
    (bind _returnvalue_2 (`|CreateWidget` "/Game/HUD/PlayerHUD/WB_PlayerHUD.WB_PlayerHUD_C" _returnvalue))
    (`UserWidget.AddToViewport` _returnvalue_2 0)
    (`WidgetBlueprintLibrary.SetInputMode_GameOnly` _returnvalue)
    (set `PlayerController.bShowMouseCursor` false _returnvalue)
    (set `self.IsGameLoaded` true)
    (`self.BuildPool`)
    (`self.NewDay`)
    (`self.StartDay`)
    (set `self.CumulativeProbability` (`self.InitialProbability`))
    (`KismetSystemLibrary.K2_SetTimerDelegate` (delegate `FrenzyProb`) (* (`self.FrenzyCheck`) 60.0) true)))

(event `FrenzyProb`
  (`self.HandleFrenzyProbability` (`self.ProbabilityIncrement`)))

(event `self.ReceiveTick`
  (params (DeltaSeconds :type "Float (single-precision)"))
  ;[1 1 1] Handle Clock and Day Time
  (if (`self.IsGameLoaded`)
    (`self.Clock` DeltaSeconds)
    (`KismetSystemLibrary.PrintString` (`KismetStringLibrary.Concat_StrStr` (`KismetStringLibrary.Conv_IntToString` (`self.Hours`)) ":" (`KismetStringLibrary.Conv_IntToString` (`self.Minutes`)) ":" (`KismetStringLibrary.Conv_IntToString` (`self.Seconds`))) true true (struct :`R` 0.199721 :`G` 1.0 :`B` 0.028119 :`A` 1.0) 0.0)
    (`KismetSystemLibrary.PrintString` (`KismetStringLibrary.Conv_IntToString` (`self.Day_Minutes`)) true true (struct :`G` 0.66 :`B` 1.0 :`A` 1.0) 0.0)
    (`self.HandleDay`)))

(event `EnemyKilled`
  (params (WasInFrenzy :type Boolean))
  ;[1 1 1] Keep wave intact
  (if (not (`self.Frenzy`))
    (set `self.SpawnTime` (`self.PatrolSpawnTime`))
    (if (> (`self.EnemySurplus`) 0)
      (`/Engine/EditorBlueprintResources/StandardMacros.DecrementInt` (`self.EnemySurplus`))
      (else
        (if (not (not WasInFrenzy)) :!label _label
          (`/Engine/EditorBlueprintResources/StandardMacros.DecrementInt` (`self.EnemiesInFrenzy`)
            (:`  `
              (if (== (`self.EnemiesInFrenzy`) 0)
                (`self.FrenzyLights`)))))
        (if (> (`self.EnemiesDead`) 0)
          (`/Engine/EditorBlueprintResources/StandardMacros.IncrementInt` (`self.EnemiesDead`))
          (else
            (`KismetSystemLibrary.K2_SetTimerDelegate` (delegate `MantainWave`) (`self.SpawnTime`))
            (`/Engine/EditorBlueprintResources/StandardMacros.IncrementInt` (`self.EnemiesDead`))))))
    (else
      (set `self.SpawnTime` (`self.FrenzySpawnTime`))
      (goto _label))))

(event `MantainWave`
  (bind _activeroom (`self.ActiveRoom`))
  ;[1 1 1] Keep wave intact
  (for _ (range 1 (+ (`self.EnemiesDead`) 1))
    (`/Engine/EditorBlueprintResources/StandardMacros.IsValid` _activeroom
      (:`Is Valid`
        (`self.RespawnEnemies` (`/Game/Blueprint/Envirorment/Rooms/BP_WFC_BaseRoom.SpawnPoints` _activeroom)))
      (:`Is Not Valid`
        (`self.RespawnEnemies` (`/Game/Blueprint/Envirorment/Rooms/BP_WFC_BaseRoom.SpawnPoints` (`KismetArrayLibrary.Array_Random` (`self.ActiveRooms`)))))))
  (set `self.EnemiesDead` 0))

(event `PrepareFrenzy`
  (set `self.Frenzy` true)
  (`self.FrenzyLights`)
  (`KismetSystemLibrary.Delay` 30.0)
  (`GameplayStatics.PlaySound2D` "/Game/Audio/SFX/Environment/SW_AlarmSiren.SW_AlarmSiren" 0.5 1.0 0.0 null null false)
  (`KismetSystemLibrary.Delay` 30.0)
  (`self.StartFrenzy`)
  (`KismetSystemLibrary.Delay` (* (`self.FrenzyCooldown`) 60.0))
  (set `self.Frenzy` false))

(fn `AddRoom`
  (params (NewRoom :type "/Game/Blueprint/Envirorment/Rooms/BP_WFC_BaseRoom Object Reference"))
  (`KismetArrayLibrary.Array_Add` (`self.ActiveRooms`) NewRoom)
  (`self.PopulateRoom` NewRoom (`self.EnemiesPerRoom`)))

(fn `BuildPool`
  (bind _enemyweighted (`self.EnemyWeighted`))
  (`KismetArrayLibrary.Array_Clear` (`self.AllEnemies`))
  (bind _keys (`BlueprintMapLibrary.Map_Keys` _enemyweighted))
  (for _array_element _keys
    (for _ (range 1 (+ (`BlueprintMapLibrary.Map_Find` _enemyweighted _array_element) 1))
      (`KismetArrayLibrary.Array_Add` (`self.AllEnemies`) _array_element)))
  (return))

(fn `Clock`
  (params (DeltaSeconds :type "Float (double-precision)"))
  (bind _output_get (set `self.Total Time` (+ (* DeltaSeconds 1.0) (`self.Total Time`))))
  (if (>= _output_get 60.0)
    (set `self.Total Time` (- (`self.Total Time`) 60.0))
    (`/Engine/EditorBlueprintResources/StandardMacros.IncrementInt` (`self.Day_Minutes`)
      (:`  `
        (bind _output_get_2 (set `self.Minutes` (+ (`self.Minutes`) 1)))
        (if (>= _output_get_2 60)
          (set `self.Minutes` (- (`self.Minutes`) 60))
          (set `self.Hours` (+ (`self.Hours`) 1)))))
    (else
      (set `self.Seconds` (`KismetMathLibrary.FTrunc` (`self.Total Time`))))))

(fn `GetEnemyFromPool`
  (returns (SelectedEnemy :type "/Game/Blueprint/Enemies/BP_BaseEnemy Class Reference"))
  (return (`KismetArrayLibrary.Array_Random` (`self.AllEnemies`))))

(fn `HandleDay`
  (if (== (`self.Day_Minutes`) (`self.DayDurationMinutes`))
    (`self.NewDay`)
    (`KismetSystemLibrary.PrintString` "NEW DAY" true true (struct :`G` 0.142314 :`B` 0.286458 :`A` 1.0))))

(fn `HandleFrenzyProbability`
  (params (ProbabilityIncrement :type "Float (double-precision)"))
  (if (not (`self.Frenzy`))
    (if (< (`KismetMathLibrary.RandomIntegerFromStream` (`/Game/Blueprint/BP_NewGameInstance.Seed` (cast `/Game/Blueprint/BP_NewGameInstance` (`GameplayStatics.GetGameInstance`) :!pure true)) 100) (`self.CumulativeProbability`))
      (`self.PrepareFrenzy`)
      (set `self.CumulativeProbability` (`KismetMathLibrary.FClamp` (+ (* (- 1.0 (/ (`self.StartProbabilityPerDayPercentage`) 100.0)) (`KismetMathLibrary.Conv_IntToDouble` (`self.CurrrentDay`))) (`self.InitialProbability`)) 0.0 (`self.MaxStartFrenzyProbability`)))
      (else
        (set `self.CumulativeProbability` (`KismetMathLibrary.FClamp` (+ ProbabilityIncrement (`self.CumulativeProbability`)) 0.0 100.0))))))

(fn `InitializeTurretBlueprint`
  (locals (TurretTypeMap :type "Map of /Game/Blueprint/Turrets/TurretGetter/E_TurretType Enum to /Game/Blueprint/Turrets/BP_Turret_Base Class Reference") (NumberOfTurrets :type Integer :default 12) (TurretBlueprints :type "Array of /Game/Blueprint/Turrets/TurretGetter/BP_TurretBlueprint Object Reference") (ItemToDelete :type "/Game/Blueprint/Turrets/TurretGetter/BP_TurretBlueprint Object Reference"))
  (bind _itemtodelete (`local.ItemToDelete`))
  (for _index (range 1 (+ (`local.NumberOfTurrets`) 1))
    (bind _returnvalue (`|GetDataTableRow` "/Game/Blueprint/Turrets/TurretGetter/Turrets.Turrets" (`KismetStringLibrary.Conv_StringToName` (`KismetStringLibrary.Conv_IntToString` _index)))
      (:`then`
        (`BlueprintMapLibrary.Map_Add` (`local.TurretTypeMap`) (break `/Game/Blueprint/Turrets/TurretGetter/S_Turrets` _returnvalue) (`.Turret_8_A6EC76C84679FDD6ABD9D4842CDC8B0A` (break `/Game/Blueprint/Turrets/TurretGetter/S_Turrets` _returnvalue))))))
  (bind _outactors (`GameplayStatics.GetAllActorsOfClass` "/Game/Blueprint/Turrets/TurretGetter/BP_TurretBlueprint.BP_TurretBlueprint_C"))
  (set `local.TurretBlueprints` _outactors)
  (bind _keys (`BlueprintMapLibrary.Map_Keys` (`local.TurretTypeMap`)))
  (bind _values (`BlueprintMapLibrary.Map_Values` (`local.TurretTypeMap`)))
  (for _index_2 (range (`KismetArrayLibrary.Array_Length` _keys))
    (set `local.ItemToDelete` (`|GetArrayItem` (`local.TurretBlueprints`) (`KismetMathLibrary.RandomIntegerFromStream` (`/Game/Blueprint/BP_NewGameInstance.Seed` (cast `/Game/Blueprint/BP_NewGameInstance` (`GameplayStatics.GetGameInstance`) :!pure true)) (`KismetArrayLibrary.Array_Length` (`local.TurretBlueprints`)))))
    (`|SpawnActorFromClass` "/Game/Blueprint/Turrets/TurretGetter/BP_TurretBlueprint.BP_TurretBlueprint_C" (`SceneComponent.K2_GetComponentToWorld` (`Actor.RootComponent` (`local.ItemToDelete`))) "Undefined" "MultiplyWithRoot" null (`|GetArrayItem` _keys _index_2) (`|GetArrayItem` _values _index_2) null)
    (`KismetArrayLibrary.Array_RemoveItem` (`local.TurretBlueprints`) _itemtodelete)
    (`self.K2_DestroyActor` _itemtodelete))
  (bind (_arrayindex _arrayelement) (`/Engine/EditorBlueprintResources/StandardMacros.ReverseForEachLoop` (`local.TurretBlueprints`))
    (:`LoopBody`
      (`self.K2_DestroyActor` _arrayelement))))

(fn `NewDay`
  (`self.Set Day`))

(fn `PopulatePool`
  (returns (Success :type Boolean))
  (locals (CurrentEnemy :type "/Game/Blueprint/Enemies/BP_BaseEnemy Class Reference"))
  (if (`KismetArrayLibrary.Array_IsValidIndex` (`self.AllEnemies`))
    (bind _output_get (set `local.CurrentEnemy` (`KismetArrayLibrary.Array_Random` (`self.AllEnemies`))))
    (`KismetArrayLibrary.Array_Add` (`self.PossibleEnemies`) _output_get)
    (`KismetArrayLibrary.Array_RemoveItem` (`self.AllEnemies`) (`local.CurrentEnemy`))
    (return true)
    (else
      (return false))))

(fn `PopulateRoom`
  (params (Room :type "/Game/Blueprint/Envirorment/Rooms/BP_WFC_BaseRoom Object Reference") (NumberOfEnemies :type Integer))
  (for _ (range NumberOfEnemies)
    (bind _selectedenemy (`self.GetEnemyFromPool`))
    (`/Game/Blueprint/Spawn/BP_SpawnPoint.AddEnemyToQueue` (`KismetArrayLibrary.Array_Random` (`/Game/Blueprint/Envirorment/Rooms/BP_WFC_BaseRoom.SpawnPoints` Room)) _selectedenemy)))

(fn `RespawnEnemies`
  (params (SpawnPoints :type "Array of /Game/Blueprint/Spawn/BP_SpawnPoint Object Reference"))
  (locals (MaxDistance :type "Float (double-precision)"))
  (bind _selectedenemy (`self.GetEnemyFromPool`))
  (`/Game/Blueprint/Spawn/BP_SpawnPoint.AddEnemyToQueue` (`KismetArrayLibrary.Array_Random` SpawnPoints) _selectedenemy))

(fn `Set Day`
  (`/Engine/EditorBlueprintResources/StandardMacros.IncrementInt` (`self.CurrrentDay`)
    (:`  `
      (set `self.Day_Minutes` 0))))

(fn `Set First Room`
  (params (FirstRoom :type "/Game/Blueprint/Envirorment/Rooms/BP_WFC_BaseRoom Object Reference"))
  (`KismetArrayLibrary.Array_Add` (`self.ActiveRooms`) FirstRoom)
  (set `self.ActiveRoom` FirstRoom))

(fn `SetEnemies`
  (set `self.EnemiesToSpawn` (- (* (`KismetArrayLibrary.Array_Length` (`self.ActiveRooms`)) (`self.EnemiesPerRoom`)) (`self.EnemiesAlreadyPresent`))))

(fn `StartDay`
  (locals (PoolSize :type Integer))
  (for _array_element (`self.ActiveRooms`)
    (`self.PopulateRoom` _array_element (`self.EnemiesPerRoom`))))

(fn `StartFrenzy`
  (`self.FrenzyDispatcher`))

(fn `UserConstructionScript`)