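; Game mode for a wave survival game with purchasable rooms that either restores player, rooms and doors from a save or spawns a fresh player and seeded turret blueprints.
; A tick clock advances days, each rebuilding a weighted enemy pool gated by day difficulty.
; Rooms fill from that pool, and kills trigger spawner-based respawns in the active room.
; A periodic seeded roll with accumulating probability starts timed Frenzy events that switch music and environment.
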(event `Initialize`
  ;[0.06667 0.1294 1] Initialize the map
  (bind _asbp_new_game_instance (cast `/Game/Blueprint/BP_NewGameInstance` (`GameplayStatics.GetGameInstance`)))
  (if (`/Game/Blueprint/BP_NewGameInstance.IsContinue?` _asbp_new_game_instance)
    (bind _saveslot (`/Game/Blueprint/BP_NewGameInstance.SaveSlot` _asbp_new_game_instance))
    (`self.Initialize Player` _saveslot)
    (`self.InitializeWorld` _saveslot)
    (`KismetSystemLibrary.Delay` 2.0)
    (`self.EndLoading`)
    (else
      (`self.InitializeTurretBlueprint`)
      (bind _returnvalue (`|SpawnActorFromClass` "/Game/Blueprint/Robot/Blueprints/BP_Roberto.BP_Roberto_C" (`KismetMathLibrary.MakeTransform` (0.0 0.0 100.0)) "AlwaysSpawn" "MultiplyWithRoot" null null))
      (add `/Game/Blueprint/Robot/Blueprints/BP_Roberto.onDeath` _returnvalue (`|CreateDelegate` :!event `WriteToGameInstance`))
      (`KismetSystemLibrary.Delay` 2.0)
      (`self.EndLoading`))))

(event `EndLoading`
  ;[0.06667 0.1294 1] Loading ended
  (`self.OnLoadingEnded`)
  (set `self.IsGameLoaded` true)
  (`self.CreatePlayerHUD`)
  (`self.InitializeOST`)
  (`self.NewDay`)
  (`self.PopulateRoom` (`self.ActiveRoom`) (`self.EnemiesPerRoom`))
  (set `self.CumulativeProbability` (`self.InitialProbability`))
  (`KismetSystemLibrary.K2_SetTimerDelegate` (delegate `FrenzyProb`) (* (`self.FrenzyCheck`) 60.0) true)
  (`KismetSystemLibrary.K2_SetTimerDelegate` (delegate `PlayDistantNoises`) (`KismetMathLibrary.RandomFloatInRange` 30.0 50.0) true))

(event `WriteToGameInstance`
  ;[0.06667 0.1294 1] Loading ended
  (bind _asbp_new_game_instance (cast `/Game/Blueprint/BP_NewGameInstance` (`GameplayStatics.GetGameInstance`)))
  (`/Game/Blueprint/BP_NewGameInstance.SaveForDeathScreen` _asbp_new_game_instance (`self.LeversToPullToActivateTeleport`) 0 0 (`self.CurrrentDay`) (`self.Day_Minutes`) (`self.Seconds`)))

(event `FrenzyProb`
  ;[0.06667 0.1294 1] Loading ended
  (`self.HandleFrenzyProbability` (`self.ProbabilityIncrement`)))

(event `PlayDistantNoises`
  (bind (_returnvalue_x _returnvalue_y _returnvalue_z) (`KismetMathLibrary.BreakVector` (`self.K2_GetActorLocation` (`GameplayStatics.GetPlayerPawn` 0))))
  ;[0.06667 0.1294 1] Loading ended
  (`GameplayStatics.PlaySoundAtLocation` "/Game/Audio/SFX/Environment/FactoryNoises/SC_DistantNoises.SC_DistantNoises" (`KismetMathLibrary.MakeVector` (+ _returnvalue_x 3750.0) _returnvalue_y _returnvalue_z) (struct) 1.0 1.0 0.0 null null null null))

(event `self.ReceiveTick`
  (params (DeltaSeconds :type "Float (single-precision)"))
  ;[0.4053 1 0.2555] Handle Clock and Day Time
  (if (`self.IsGameLoaded`)
    (`self.Clock` DeltaSeconds)
    (`KismetSystemLibrary.PrintString` (`KismetStringLibrary.Concat_StrStr` (`KismetStringLibrary.Conv_IntToString` (`self.Hours`)) ":" (`KismetStringLibrary.Conv_IntToString` (`self.Minutes`)) ":" (`KismetStringLibrary.Conv_IntToString` (`self.Seconds`))) true true (struct :`R` 0.199721 :`G` 1.0 :`B` 0.028119 :`A` 1.0) 0.0 "TIME")
    (`self.HandleDay`)))

(event `EnemyKilled`
  (params (WasInFrenzy :type Boolean))
  ;[1 0.6804 0.202] Respawn Enemies
  (if (not (not WasInFrenzy))
    (bind _result (`/Engine/EditorBlueprintResources/StandardMacros.DecrementInt` (`self.EnemiesInFrenzy`))
      (:`  `
        (if (not (> _result 0))
          (`self.TurnOffFrenzy`)))))
  (`/Engine/EditorBlueprintResources/StandardMacros.IncrementInt` (`self.EnemiesDead`)
    (:`  `
      (`self.RespawnEnemiesInActiveRoom`))))

(event `MantainWave`
  (bind _activeroom (`self.ActiveRoom`))
  ;[1 1 1] RIP (FINALLY DEPRECATED)
  (for _ (range 1 (+ (`self.EnemiesDead`) 1))
    (`/Engine/EditorBlueprintResources/StandardMacros.IsValid` _activeroom
      (:`Is Valid`
        (`self.RespawnEnemies` (`/Game/Blueprint/Envirorment/Rooms/BP_WFC_BaseRoom.SpawnPoints` _activeroom)))
      (:`Is Not Valid`
        (`self.RespawnEnemies` (`/Game/Blueprint/Envirorment/Rooms/BP_WFC_BaseRoom.SpawnPoints` (`KismetArrayLibrary.Array_Random` (`self.ActiveRooms`)))))))
  (set `self.EnemiesDead` 0))

(event `TurnOffFrenzy`
  (bind _audiocomponent (`AmbientSound.AudioComponent` (`self.MusicPlayer`)))
  ;[1 0.1771 0.1771] Stop Frenzy
  (`self.OnFrenzyEnvironment`)
  (`AudioComponent.FadeOut` _audiocomponent 2.0 0.0 "Linear")
  (`KismetSystemLibrary.Delay` 2.0)
  (`AudioComponent.SetSound` _audiocomponent "/Game/Audio/SFX/Environment/SC_AmbientSFX_Cue.SC_AmbientSFX_Cue")
  (`AudioComponent.FadeIn` _audiocomponent 1.0 1.0 0.0 "Linear")
  (set `self.Frenzy` false))

(event `PrepareFrenzy`
  (bind _audiocomponent (`AmbientSound.AudioComponent` (`self.MusicPlayer`)))
  ;[1 0.1771 0.1771] Prepare Frenzy
  (set `self.Frenzy` true)
  (`self.OnFrenzyEnvironment`)
  (`KismetSystemLibrary.Delay` 30.0)
  (`GameplayStatics.PlaySound2D` "/Game/Audio/SFX/Environment/SC_AlarmSiren.SC_AlarmSiren" 0.5 1.0 0.0 null null false)
  (`KismetSystemLibrary.Delay` 29.0)
  (`AudioComponent.FadeOut` (`AmbientSound.AudioComponent` (`self.MusicPlayer`)) 1.0 0.0 "Linear")
  (`KismetSystemLibrary.Delay` 1.0)
  (`AudioComponent.SetSound` _audiocomponent "/Game/Audio/Music/SC_FrenzyOST.SC_FrenzyOST")
  (`AudioComponent.FadeIn` _audiocomponent 1.0 1.0 0.0 "Linear")
  (`self.StartFrenzy`)
  (`KismetSystemLibrary.Delay` (* (`self.FrenzyCooldown`) 60.0))
  (set `self.Frenzy` false))

(fn `AddRoom`
  (params (NewRoom :type "/Game/Blueprint/Envirorment/Rooms/BP_WFC_BaseRoom Object Reference"))
  (`KismetArrayLibrary.Array_Add` (`self.ActiveRooms`) NewRoom)
  (`self.PopulateRoom` NewRoom (`self.EnemiesPerRoom`))
  (set `self.DoorCost` (`KismetMathLibrary.Conv_IntToDouble` (`KismetMathLibrary.FCeil` (* (`self.DoorCost`) (`self.DoorCostMultiplier`))))))

(fn `BuildPool`
  (bind _enemyweighted (`self.EnemyWeighted`))
  (`KismetArrayLibrary.Array_Clear` (`self.AllEnemies`))
  (bind _keys (`BlueprintMapLibrary.Map_Keys` _enemyweighted))
  (for _array_element _keys
    (bind (_value _returnvalue) (`BlueprintMapLibrary.Map_Find` (`self.EnemiesDifficulty`) _array_element))
    (if _returnvalue
      (if (<= _value (`self.CurrrentDay`))
        (for _ (range 1 (+ (`BlueprintMapLibrary.Map_Find` _enemyweighted _array_element) 1))
          (`KismetArrayLibrary.Array_Add` (`self.AllEnemies`) _array_element)))))
  (return))

(fn `Clock`
  (params (DeltaSeconds :type "Float (double-precision)"))
  (bind _output_get (set `self.Total Time` (+ (* DeltaSeconds 1.0) (`self.Total Time`))))
  (if (>= _output_get 60.0)
    (set `self.Total Time` (- (`self.Total Time`) 60.0))
    (`/Engine/EditorBlueprintResources/StandardMacros.IncrementInt` (`self.Day_Minutes`)
      (:`  `
        (bind _output_get_2 (set `self.Minutes` (+ (`self.Minutes`) 1)))
        (if (>= _output_get_2 60)
          (set `self.Minutes` (- (`self.Minutes`) 60))
          (set `self.Hours` (+ (`self.Hours`) 1)))))
    (else
      (set `self.Seconds` (`KismetMathLibrary.FTrunc` (`self.Total Time`))))))

(fn `CreatePlayerHUD`
  (bind _returnvalue (`GameplayStatics.GetPlayerController` 0))
  (bind _returnvalue_2 (`|CreateWidget` "/Game/HUD/PlayerHUD/WB_PlayerHUD.WB_PlayerHUD_C" _returnvalue))
  (`UserWidget.AddToViewport` _returnvalue_2 0)
  (`WidgetBlueprintLibrary.SetInputMode_GameOnly` _returnvalue)
  (set `PlayerController.bShowMouseCursor` false _returnvalue))

(fn `GetAllDoors`
  (returns (OutDoors :type "Array of /Game/Blueprint/Envirorment/Doors/BP_WFC_Door Object Reference"))
  (bind _outactors (`GameplayStatics.GetAllActorsOfClass` "/Game/Blueprint/Envirorment/Doors/BP_WFC_Door.BP_WFC_Door_C"))
  (return _outactors))

(fn `GetAllEnergyRecharger`
  (returns (EnergyRecharger :type "Array of /Game/Blueprint/EnergyRecharger/BP_EnergyRecharger Object Reference"))
  (bind _outactors (`GameplayStatics.GetAllActorsOfClass` "/Game/Blueprint/EnergyRecharger/BP_EnergyRecharger.BP_EnergyRecharger_C"))
  (return _outactors))

(fn `GetAllJunks`
  (returns (Junks :type "Array of /Game/Blueprint/Junks/BP_Junk Object Reference"))
  (bind _outactors (`GameplayStatics.GetAllActorsOfClass` "/Game/Blueprint/Junks/BP_Junk.BP_Junk_C"))
  (return _outactors))

(fn `GetAllJunkSpawner`
  (returns (JunkSpawner :type "Array of /Game/Blueprint/Junks/BP_JunkSpawner Object Reference"))
  (bind _outactors (`GameplayStatics.GetAllActorsOfClass` "/Game/Blueprint/Junks/BP_JunkSpawner.BP_JunkSpawner_C"))
  (return _outactors))

(fn `GetAllTurrets`
  (returns (Turrets :type "Array of /Game/Blueprint/Turrets/BP_Turret_Base Object Reference"))
  (bind _outactors (`GameplayStatics.GetAllActorsOfClass` "/Game/Blueprint/Turrets/BP_Turret_Base.BP_Turret_Base_C"))
  (return _outactors))

(fn `GetAllTurretsTrigger`
  (returns (TurretTrigger :type "Array of /Game/Blueprint/Turrets/BP_TurretTrigger Object Reference"))
  (bind _outactors (`GameplayStatics.GetAllActorsOfClass` "/Game/Blueprint/Turrets/BP_TurretTrigger.BP_TurretTrigger_C"))
  (return _outactors))

(fn `GetEnemyFromPool`
  (returns (SelectedEnemy :type "/Game/Blueprint/Enemies/BP_BaseEnemy Class Reference"))
  (return (`KismetArrayLibrary.Array_Random` (`self.AllEnemies`))))

(fn `HandleDay`
  (if (== (`self.Day_Minutes`) (`self.DayDurationMinutes`))
    (`GameplayStatics.PlaySound2D` "/Game/Audio/SFX/Environment/SC_SurvivalDaySFX_Cue.SC_SurvivalDaySFX_Cue" 1.0 1.0 0.0 null null)
    (`self.NewDay`)))

(fn `HandleFrenzyProbability`
  (params (ProbabilityIncrement :type "Float (double-precision)"))
  (if (not (`self.Frenzy`))
    (if (< (`KismetMathLibrary.RandomIntegerFromStream` (`/Game/Blueprint/BP_NewGameInstance.Seed` (cast `/Game/Blueprint/BP_NewGameInstance` (`GameplayStatics.GetGameInstance`) :!pure true)) 100) (`self.CumulativeProbability`))
      (if (!= (`KismetArrayLibrary.Array_Length` (`self.ActiveSpawners`)) (* (`KismetArrayLibrary.Array_Length` (`self.ActiveRooms`)) (`self.EnemiesPerRoom`)))
        (`self.PrepareFrenzy`)
        (set `self.CumulativeProbability` (`KismetMathLibrary.FClamp` (+ (* (/ (`self.StartProbabilityPerDayPercentage`) 100.0) (`KismetMathLibrary.Conv_IntToDouble` (`self.CurrrentDay`))) (`self.InitialProbability`)) 0.0 (`self.MaxStartFrenzyProbability`)))
        (else
          (set `self.CumulativeProbability` (`KismetMathLibrary.FClamp` (+ ProbabilityIncrement (`self.CumulativeProbability`)) 0.0 100.0) :!label _label)))
      (else
        (goto _label)))))

(fn `Initialize Player`
  (params (SaveData :type "/Game/Blueprint/Save/BP_SaveData Object Reference"))
  (bind (_playerpos_location _playerpos_rotation _playerpos_scale) (`KismetMathLibrary.BreakTransform` (`/Game/Blueprint/Save/BP_SaveData.PlayerPos` SaveData)))
  (bind _returnvalue (`|SpawnActorFromClass` "/Game/Blueprint/Robot/Blueprints/BP_Roberto.BP_Roberto_C" (`KismetMathLibrary.MakeTransform` _playerpos_location _playerpos_rotation _playerpos_scale) "AlwaysSpawn" "MultiplyWithRoot" null null))
  (`/Game/Blueprint/Robot/Blueprints/BP_Roberto.InitializeFromSave` _returnvalue (`/Game/Blueprint/Save/BP_SaveData.Health` SaveData) (`/Game/Blueprint/Save/BP_SaveData.MaxHealth` SaveData) (`/Game/Blueprint/Save/BP_SaveData.Energy` SaveData) (`/Game/Blueprint/Save/BP_SaveData.MaxEnergy` SaveData) (`/Game/Blueprint/Save/BP_SaveData.Gear` SaveData) (`/Game/Blueprint/Save/BP_SaveData.Steel` SaveData) (`/Game/Blueprint/Save/BP_SaveData.Circuit` SaveData) (`/Game/Blueprint/Save/BP_SaveData.Essence` SaveData) (`/Game/Blueprint/Save/BP_SaveData.JunkDamage` SaveData) (`/Game/Blueprint/Save/BP_SaveData.powerUpItems` SaveData) (`/Game/Blueprint/Save/BP_SaveData.TurretLevel` SaveData))
  (add `/Game/Blueprint/Robot/Blueprints/BP_Roberto.onDeath` _returnvalue (`|CreateDelegate` :!event `WriteToGameInstance`)))

(fn `InitializeOST`
  (bind _audiocomponent (`AmbientSound.AudioComponent` (`self.MusicPlayer`)))
  (bind _returnvalue (`GameplayStatics.GetActorOfClass` "/Script/Engine.AmbientSound"))
  (set `self.MusicPlayer` _returnvalue)
  (`AudioComponent.SetSound` _audiocomponent "/Game/Audio/SFX/Environment/SC_AmbientSFX_Cue.SC_AmbientSFX_Cue")
  (`AudioComponent.FadeIn` _audiocomponent 1.0 1.0 0.0 "Linear"))

(fn `InitializeTurretBlueprint`
  (locals (TurretTypeMap :type "Map of /Game/Blueprint/Turrets/TurretGetter/E_TurretType Enum to /Game/Blueprint/Turrets/BP_Turret_Base Class Reference") (NumberOfTurrets :type Integer :default 12) (TurretBlueprints :type "Array of /Game/Blueprint/Turrets/TurretGetter/BP_TurretBlueprint Object Reference") (ItemToDelete :type "/Game/Blueprint/Turrets/TurretGetter/BP_TurretBlueprint Object Reference"))
  (bind _itemtodelete (`local.ItemToDelete`))
  (for _index (range 1 (+ (`local.NumberOfTurrets`) 1))
    (bind _returnvalue (`|GetDataTableRow` "/Game/Blueprint/Turrets/TurretGetter/Turrets.Turrets" (`KismetStringLibrary.Conv_StringToName` (`KismetStringLibrary.Conv_IntToString` _index)))
      (:`then`
        (`BlueprintMapLibrary.Map_Add` (`local.TurretTypeMap`) (break `/Game/Blueprint/Turrets/TurretGetter/S_Turrets` _returnvalue) (`.Turret_8_A6EC76C84679FDD6ABD9D4842CDC8B0A` (break `/Game/Blueprint/Turrets/TurretGetter/S_Turrets` _returnvalue))))))
  (`BlueprintMapLibrary.Map_Remove` (`local.TurretTypeMap`) "NewEnumerator0")
  (bind _outactors (`GameplayStatics.GetAllActorsOfClass` "/Game/Blueprint/Turrets/TurretGetter/BP_TurretBlueprint.BP_TurretBlueprint_C"))
  (set `local.TurretBlueprints` _outactors)
  (bind _keys (`BlueprintMapLibrary.Map_Keys` (`local.TurretTypeMap`)))
  (bind _values (`BlueprintMapLibrary.Map_Values` (`local.TurretTypeMap`)))
  (for _index_2 (range (`KismetArrayLibrary.Array_Length` _keys))
    (if (> (`KismetArrayLibrary.Array_Length` (`local.TurretBlueprints`)) 0)
      (set `local.ItemToDelete` (`|GetArrayItem` (`local.TurretBlueprints`) (`KismetMathLibrary.RandomIntegerFromStream` (`/Game/Blueprint/BP_NewGameInstance.Seed` (cast `/Game/Blueprint/BP_NewGameInstance` (`GameplayStatics.GetGameInstance`) :!pure true)) (`KismetArrayLibrary.Array_Length` (`local.TurretBlueprints`)))))
      (`|SpawnActorFromClass` "/Game/Blueprint/Turrets/TurretGetter/BP_TurretBlueprint.BP_TurretBlueprint_C" (`SceneComponent.K2_GetComponentToWorld` (`Actor.RootComponent` (`local.ItemToDelete`))) "Undefined" "MultiplyWithRoot" null (`|GetArrayItem` _keys _index_2) (`|GetArrayItem` _values _index_2) null)
      (`KismetArrayLibrary.Array_RemoveItem` (`local.TurretBlueprints`) _itemtodelete)
      (`self.K2_DestroyActor` _itemtodelete)))
  (bind (_arrayindex _arrayelement) (`/Engine/EditorBlueprintResources/StandardMacros.ReverseForEachLoop` (`local.TurretBlueprints`))
    (:`LoopBody`
      (`self.K2_DestroyActor` _arrayelement))))

(fn `InitializeWorld`
  (params (SaveData :type "/Game/Blueprint/Save/BP_SaveData Object Reference"))
  (bind _outactors (`GameplayStatics.GetAllActorsOfClass` "/Game/Blueprint/Envirorment/Rooms/BP_WFC_BaseRoom.BP_WFC_BaseRoom_C"))
  (`|ExecutionSequence`
    (:`then_0`
      (for _array_element _outactors
        (if (== (`/Game/Blueprint/Save/BP_SaveData.ActiveRoom` SaveData) (`/Game/Blueprint/Envirorment/Rooms/BP_WFC_BaseRoom.Index` _array_element))
          (bind _output_get (set `self.ActiveRoom` _array_element))
          (`self.SetActorHiddenInGame` _output_get false)
          (break))))
    (:`then_1`
      (for _array_element_2 _outactors
        (for _array_element_3 (`/Game/Blueprint/Save/BP_SaveData.ActiveRooms` SaveData)
          (if (== _array_element_3 (`/Game/Blueprint/Envirorment/Rooms/BP_WFC_BaseRoom.Index` _array_element_2))
            (`KismetArrayLibrary.Array_AddUnique` (`self.ActiveRooms`) _array_element_2)
            (`self.SetActorHiddenInGame` _array_element_2 false)))))
    (:`then_2`
      (bind _outactors_2 (`GameplayStatics.GetAllActorsOfClass` "/Game/Blueprint/Envirorment/Doors/BP_WFC_Door.BP_WFC_Door_C"))
      (for _array_element_4 _outactors_2
        (for _array_element_5 (`/Game/Blueprint/Save/BP_SaveData.Doors ` SaveData)
          (if (== _array_element_5 (`/Game/Blueprint/Envirorment/Doors/BP_WFC_Door.Index` _array_element_4))
            (set `/Game/Blueprint/Envirorment/Doors/BP_WFC_Door.StayOpened` true _array_element_4)
            (set `/Game/Blueprint/Envirorment/Doors/BP_WFC_Door.Purchased` true _array_element_4)
            (`/Game/Blueprint/Envirorment/Doors/BP_WFC_Door.OpenDoor` _array_element_4)))))
    (:`then_3`
      (set `self.DoorCost` (`/Game/Blueprint/Save/BP_SaveData.DoorCost` SaveData))
      (set `self.CurrrentDay` (- (`/Game/Blueprint/Save/BP_SaveData.CurrentDay` SaveData) 1))
      (set `self.CumulativeProbability` (`/Game/Blueprint/Save/BP_SaveData.FrenzyCumulativeProbability` SaveData)))))

(fn `NewDay`
  (`/Engine/EditorBlueprintResources/StandardMacros.IncrementInt` (`self.CurrrentDay`)
    (:`  `
      (set `self.Day_Minutes` 0)
      (`self.BuildPool`))))

(fn `PopulatePool`
  (returns (Success :type Boolean))
  (locals (CurrentEnemy :type "/Game/Blueprint/Enemies/BP_BaseEnemy Class Reference"))
  (if (`KismetArrayLibrary.Array_IsValidIndex` (`self.AllEnemies`))
    (bind _output_get (set `local.CurrentEnemy` (`KismetArrayLibrary.Array_Random` (`self.AllEnemies`))))
    (`KismetArrayLibrary.Array_Add` (`self.PossibleEnemies`) _output_get)
    (`KismetArrayLibrary.Array_RemoveItem` (`self.AllEnemies`) (`local.CurrentEnemy`))
    (return true)
    (else
      (return false))))

(fn `PopulateRoom`
  (params (Room :type "/Game/Blueprint/Envirorment/Rooms/BP_WFC_BaseRoom Object Reference") (NumberOfEnemies :type Integer))
  (for _ (range NumberOfEnemies)
    (bind _selectedenemy (`self.GetEnemyFromPool`))
    (`/Game/Blueprint/Spawn/BP_SpawnPoint.AddEnemyToQueue` (`KismetArrayLibrary.Array_Random` (`/Game/Blueprint/Envirorment/Rooms/BP_WFC_BaseRoom.SpawnPoints` Room)) _selectedenemy)))

(fn `QuickStartFrenzy`
  (bind _audiocomponent (`AmbientSound.AudioComponent` (`self.MusicPlayer`)))
  (if (!= (`KismetArrayLibrary.Array_Length` (`self.ActiveSpawners`)) (* (`KismetArrayLibrary.Array_Length` (`self.ActiveRooms`)) (`self.EnemiesPerRoom`)))
    (set `self.Frenzy` true)
    (`self.OnFrenzyEnvironment`)
    (`AudioComponent.FadeOut` (`AmbientSound.AudioComponent` (`self.MusicPlayer`)) 1.0 0.0 "Linear")
    (`AudioComponent.SetSound` _audiocomponent "/Game/Audio/Music/SC_FrenzyOST.SC_FrenzyOST")
    (`AudioComponent.FadeIn` _audiocomponent 1.0 1.0 0.0 "Linear")
    (`self.OnFrenzyEnemies`)))

(fn `RespawnEnemies`
  (params (SpawnPoints :type "Array of /Game/Blueprint/Spawn/BP_SpawnPoint Object Reference"))
  (locals (MaxDistance :type "Float (double-precision)"))
  (bind _selectedenemy (`self.GetEnemyFromPool`))
  (`|AddComponentByClass` "/Game/Blueprint/Spawn/BPC_Spawner.BPC_Spawner_C" (`self.PatrolSpawnTime`) SpawnPoints _selectedenemy))

(fn `RespawnEnemiesInActiveRoom`
  (bind _selectedenemy (`self.GetEnemyFromPool`))
  (bind _returnvalue (`|AddComponentByClass` "/Game/Blueprint/Spawn/BPC_Spawner.BPC_Spawner_C" (`self.SpawnTime`) (`/Game/Blueprint/Envirorment/Rooms/BP_WFC_BaseRoom.SpawnPoints` (`self.ActiveRoom`)) _selectedenemy))
  (`KismetArrayLibrary.Array_Add` (`self.ActiveSpawners`) _returnvalue))

(fn `Set Day`
  (`/Engine/EditorBlueprintResources/StandardMacros.IncrementInt` (`self.CurrrentDay`)
    (:`  `
      (set `self.Day_Minutes` 0))))

(fn `Set First Room`
  (params (FirstRoom :type "/Game/Blueprint/Envirorment/Rooms/BP_WFC_BaseRoom Object Reference"))
  (`KismetArrayLibrary.Array_Add` (`self.ActiveRooms`) FirstRoom)
  (set `self.ActiveRoom` FirstRoom))

(fn `SetEnemies`
  (set `self.EnemiesToSpawn` (- (* (`KismetArrayLibrary.Array_Length` (`self.ActiveRooms`)) (`self.EnemiesPerRoom`)) (`self.EnemiesAlreadyPresent`))))

(fn `StartDay`
  (locals (PoolSize :type Integer))
  (for _array_element (`self.ActiveRooms`)
    (`self.PopulateRoom` _array_element (`self.EnemiesPerRoom`))))

(fn `StartFrenzy`
  (if (!= (`KismetArrayLibrary.Array_Length` (`self.ActiveSpawners`)) (* (`KismetArrayLibrary.Array_Length` (`self.ActiveRooms`)) (`self.EnemiesPerRoom`)))
    (`self.OnFrenzyEnemies`)
    (else
      (`self.TurnOffFrenzy`))))

(fn `UserConstructionScript`)