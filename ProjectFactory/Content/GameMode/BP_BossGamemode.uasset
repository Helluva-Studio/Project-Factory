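; Boss-fight game mode that spawns BP_Roberto and the boss BP_Otrebor, then sets up the HUD, game-only input and ambient audio.
; Initialize restores the player's stats, resources, power-ups and turrets from BP_NewGameInstance, along with saved clock values.
; Once loading ends, Tick accumulates play time into seconds, minutes and hours.
; The player's death event writes Minutes and seconds back to the game instance.
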(event `Initialize`
  (bind _returnvalue (`GameplayStatics.GetPlayerController` 0))
  (bind _audiocomponent (`AmbientSound.AudioComponent` (`self.MusicPlayer`)))
  (bind _asbp_new_game_instance (cast `/Game/Blueprint/BP_NewGameInstance` (`GameplayStatics.GetGameInstance`)))
  (`self.InitPlayer` _asbp_new_game_instance)
  (`self.InitClock` _asbp_new_game_instance)
  (bind _returnvalue_2 (`|SpawnActorFromClass` "/Game/Blueprint/Enemies/BP_Otrebor.BP_Otrebor_C" (`KismetMathLibrary.MakeTransform` (2325.0 0.0 150.0) (struct :`Yaw` 180.0)) "AlwaysSpawn" "MultiplyWithRoot" null null))
  (`/Game/Blueprint/Enemies/BP_Otrebor.Start` _returnvalue_2)
  (`self.onLoadingEnded`)
  (set `self.IsGameLoaded` true)
  (bind _returnvalue_3 (`|CreateWidget` "/Game/HUD/PlayerHUD/WB_PlayerHUD.WB_PlayerHUD_C" _returnvalue))
  (`UserWidget.AddToViewport` _returnvalue_3 0)
  (`WidgetBlueprintLibrary.SetInputMode_GameOnly` _returnvalue)
  (set `PlayerController.bShowMouseCursor` false _returnvalue)
  (bind _returnvalue_4 (`GameplayStatics.GetActorOfClass` "/Script/Engine.AmbientSound"))
  (set `self.MusicPlayer` _returnvalue_4)
  (`AudioComponent.SetSound` _audiocomponent "/Game/Audio/SFX/Environment/SC_AmbientSFX_Cue.SC_AmbientSFX_Cue")
  (`AudioComponent.FadeIn` _audiocomponent 1.0 1.0 0.0 "Linear")
  (bind _asbp_roberto (cast `/Game/Blueprint/Robot/Blueprints/BP_Roberto` (`GameplayStatics.GetPlayerPawn` 0)))
  (add `/Game/Blueprint/Robot/Blueprints/BP_Roberto.onDeath` _asbp_roberto (delegate `WriteToGameInstance`)))

(event `WriteToGameInstance`
  (bind _asbp_new_game_instance (cast `/Game/Blueprint/BP_NewGameInstance` (`GameplayStatics.GetGameInstance`)))
  (set `/Game/Blueprint/BP_NewGameInstance.Minutes` (`self.Minutes`) _asbp_new_game_instance)
  (set `/Game/Blueprint/BP_NewGameInstance.Seconds` (`self.SaveSeconds`) _asbp_new_game_instance))

(event `self.ReceiveTick`
  (params (DeltaSeconds :type "Float (single-precision)"))
  (if (`self.IsGameLoaded`)
    (bind _output_get (set `self.Total Time` (+ (* DeltaSeconds 1.0) (`self.Total Time`))))
    (if (>= _output_get 60.0)
      (set `self.Total Time` (- (`self.Total Time`) 60.0))
      (`/Engine/EditorBlueprintResources/StandardMacros.IncrementInt` (`self.Day_Minutes`)
        (:`  `
          (bind _output_get_2 (set `self.Minutes` (+ (`self.Minutes`) 1)))
          (if (>= _output_get_2 60)
            (set `self.Minutes` (- (`self.Minutes`) 60))
            (set `self.Hours` (+ (`self.Hours`) 1)))))
      (else
        (set `self.SaveSeconds` (`KismetMathLibrary.FTrunc` (`self.Total Time`)))))))

(fn `InitClock`
  (params (GameInstance :type "/Game/Blueprint/BP_NewGameInstance Object Reference"))
  (set `self.SaveSeconds` (`/Game/Blueprint/BP_NewGameInstance.Seconds` GameInstance))
  (set `self.SaveCurrentDay` (`/Game/Blueprint/BP_NewGameInstance.Current Day` GameInstance))
  (set `self.Day_Minutes` (`/Game/Blueprint/BP_NewGameInstance.Minutes` GameInstance)))

(fn `InitPlayer`
  (params (GameInstance :type "/Game/Blueprint/BP_NewGameInstance Object Reference"))
  (bind (_transform _powerup _turretslevels _health _maxhealth _energy _maxenergy _gear _steel _circuit _essence _junkdamage _selectedturret) (break `/Game/DataStructures/S_PlayerData` (`/Game/Blueprint/BP_NewGameInstance.S Player Data` GameInstance)))
  (bind _returnvalue (`|SpawnActorFromClass` "/Game/Blueprint/Robot/Blueprints/BP_Roberto.BP_Roberto_C" (`KismetMathLibrary.MakeTransform` (-2625.0 0.0 150.0)) "AlwaysSpawn" "MultiplyWithRoot" null null))
  (`/Game/Blueprint/Robot/Blueprints/BP_Roberto.InitializeFromSave` _returnvalue _health _maxhealth _energy _maxenergy _gear _steel _circuit _essence _junkdamage _powerup _turretslevels _selectedturret))

(fn `UserConstructionScript`)