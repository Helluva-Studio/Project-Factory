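; Game mode that runs numbered enemy waves, starting the first on BeginPlay.
; Each wave loads an enemy-to-count map from the WawePoolData table row named by wave number, then draws random types, decrementing counts, and queues them on random BP_SpawnPoint actors.
; EnemyKill counts kills against the pool total and calls EnterTransition when reached.
; EnterTransition is empty and its delayed NewWawe timer is disconnected, so waves do not advance automatically.
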(event `self.ReceiveBeginPlay`
  (`self.GetSpawners`)
  (`self.NewWawe`))

(event `self.ReceiveTick`
  (params (DeltaSeconds :type "Float (single-precision)")))

(fn `BuildEnemyPool`
  (bind _returnvalue (`|GetDataTableRow` "/Game/DataStructures/WawePoolData.WawePoolData" (`KismetStringLibrary.Conv_StringToName` (`KismetStringLibrary.Conv_IntToString` (`self.WaweNumber`))))
    (:`then`
      (set `self.EnemyPool` (`.EnemyPools_6_72892FEE4D1510A571E390B0E3689759` (break `/Game/DataStructures/S_EnemyWawe` _returnvalue)))
      (set `self.EnemyRemaining` (`self.GetPoolSize`)))))

(fn `EndWawe`)

(fn `EnemyKill`
  (`/Engine/EditorBlueprintResources/StandardMacros.IncrementInt` (`self.EnemyKilled`)
    (:`  `
      (`KismetSystemLibrary.PrintString` (`KismetStringLibrary.Conv_IntToString` (`self.EnemyKilled`)))
      (if (>= (`self.EnemyKilled`) (`self.EnemyRemaining`))
        (`self.EnterTransition`)))))

(fn `EnterTransition`)

(fn `GetEnemyFromPool`
  (returns (Enemy :type "/Game/Blueprint/Enemies/BP_BaseEnemy Class Reference"))
  (locals (CurrentEnemy :type "/Game/Blueprint/Enemies/BP_BaseEnemy Class Reference"))
  (bind _keys (`BlueprintMapLibrary.Map_Keys` (`self.EnemyPool`)))
  (bind _output_get (set `local.CurrentEnemy` (`KismetArrayLibrary.Array_Random` _keys)))
  (bind _returnvalue (- (`BlueprintMapLibrary.Map_Find` (`self.EnemyPool`) _output_get) 1))
  (if (> _returnvalue 0)
    (`BlueprintMapLibrary.Map_Add` (`self.EnemyPool`) (`local.CurrentEnemy`) _returnvalue)
    (return (`local.CurrentEnemy`))
    (else
      (`BlueprintMapLibrary.Map_Remove` (`self.EnemyPool`) (`local.CurrentEnemy`))
      (return (`local.CurrentEnemy`)))))

(fn `GetPoolSize`
  (returns (Sum :type Integer))
  (locals (LocalSum :type Integer))
  (bind _values (`BlueprintMapLibrary.Map_Values` (`self.EnemyPool`)))
  (for _array_element _values
    (set `local.LocalSum` (+ _array_element (`local.LocalSum`))))
  (return (`local.LocalSum`)))

(fn `GetSpawners`
  (bind _outactors (`GameplayStatics.GetAllActorsOfClass` "/Game/Blueprint/Spawn/BP_SpawnPoint.BP_SpawnPoint_C"))
  (set `self.SpawnPoints` _outactors))

(fn `NewWawe`
  (`/Engine/EditorBlueprintResources/StandardMacros.IncrementInt` (`self.WaweNumber`)
    (:`  `
      (`KismetSystemLibrary.PrintString` (`KismetStringLibrary.Concat_StrStr` "STARTING WAWE N. " (`KismetStringLibrary.Conv_IntToString` (`self.WaweNumber`))))
      (set `self.EnemyKilled` 0)
      (`self.BuildEnemyPool`)
      (`self.StartWawe`))))

(fn `StartWawe`
  (bind _result (`/Engine/EditorBlueprintResources/StandardMacros.DecrementInt` (`self.GetPoolSize`))
    (:`  `
      (bind _output_get (set `self.PoolSize` _result))
      (for _ (range (+ _output_get 1))
        (bind _enemy (`self.GetEnemyFromPool`))
        (`/Game/Blueprint/Spawn/BP_SpawnPoint.AddEnemyToQueue` (`KismetArrayLibrary.Array_Random` (`self.SpawnPoints`)) _enemy)))))

(fn `UserConstructionScript`
  (`parent.UserConstructionScript`))